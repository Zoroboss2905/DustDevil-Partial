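; BP_MovingSandstorm is a sandstorm actor that trails the first player's pawn, keeping within a distance band.
; Each Tick it moves toward the pawn when too far away and backs off when too close, otherwise holding still.
; Distance and direction use only X and Z, leaving out Y.
; Steps are StormSpeed per frame, unscaled by delta time, applied without sweep.
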(event EventBeginPlay)

(event Collision|EventActorBeginOverlap
  (params (OtherActor :type Actor%20Object%20Reference)))

(event EventTick
  (params (DeltaSeconds :type Float%20%28single-precision%29))
  (bind _returnvalue (Game|Player|GetPlayerPawn 0))
  (bind _returnvalue_2 (Transformation|GetActorLocation))
  (bind _returnvalue_3 (Transformation|GetActorLocation))
  (bind _stormspeed (Variables|Default|GetStormSpeed))
  (bind _returnvalue_4 (Transformation|GetActorLocation _returnvalue))
  (bind _returnvalue_5 (Math|Vector|Distance(Vector) (Math|Vector|MakeVector (.x _returnvalue_4) 0.0 (.z _returnvalue_4)) (Math|Vector|MakeVector (.x _returnvalue_3) 0.0 (.z _returnvalue_3))))
  (bind _returnvalue_6 (Math|Vector|GetUnitDirection(Vector) (Math|Vector|MakeVector (.x _returnvalue_4) 0.0 (.z _returnvalue_4)) (Math|Vector|MakeVector (.x _returnvalue_3) 0.0 (.z _returnvalue_3))))
  (bind _returnvalue_7 (* _returnvalue_6 _stormspeed))
  (Utilities|IsValid _returnvalue
    (:Is%20Valid
      (if (> _returnvalue_5 2e+04)
        (Transformation|SetActorLocation (- _returnvalue_2 _returnvalue_7) false false)
        (elif (< _returnvalue_5 7.5e+03)
          (Transformation|SetActorLocation (+ _returnvalue_2 _returnvalue_7) false false))))))

(fn ConstructionScript)