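; A scalable large bug skeleton destruction prop that plays a skeleton sound when a vehicle first overlaps it.
; The construction script applies the NewScale3D value to the GCBugSkeletonL component, and BeginPlay gives the actor a random yaw.
; A DoOnce limits the sound to one play, with a concurrency setting applied.
; A fuller random scale and tilt function exists but is never called.
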(event EventBeginPlay
  (CallFunction|RandomYaw))

(event Collision|EventActorBeginOverlap
  (params (OtherActor :type Actor%20Object%20Reference))
  (Utilities|Casting|CastToVehicle OtherActor)
  (Utilities|FlowControl|DoOnce false
    (:Completed
      (Audio|PlaySoundatLocation "/Game/DustDevil/Audio/Feedback/Impacts/A_Skeleton_Cue.A_Skeleton_Cue" "0, 0, 0" "0, 0, 0" 1.0 1.0 0.0 0 "/Game/DustDevil/Player/Audio/SC_GlassImpact.SC_GlassImpact" 0 0))))

(fn ConstructionScript
  (Transformation|SetRelativeScale3D (Variables|Default|GetGC_BugSkeleton_L) (Math|Conversions|ToVector(Float) (Variables|Default|GetNew%20Scale%203D))))

(fn RandomiseTransform
  (bind _returnvalue (Math|Random|RandomFloatinRange 0.5 1.0))
  (Transformation|SetActorScale3D (Math|Vector|MakeVector _returnvalue _returnvalue _returnvalue))
  (Transformation|SetActorRotation (Math|Rotator|MakeRotator (Math|Random|RandomFloatinRange -15.0 15.0) (Math|Random|RandomFloatinRange -15.0 15.0) (Math|Random|RandomFloatinRange -1.8e+02 1.8e+02))))

(fn RandomYaw
  (Transformation|SetActorRotation (Math|Rotator|MakeRotator 0.0 0.0 (Math|Random|RandomFloatinRange -1.8e+02 1.8e+02))))