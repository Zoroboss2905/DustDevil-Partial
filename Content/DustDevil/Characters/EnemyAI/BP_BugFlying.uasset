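; Flying bug enemy Blueprint that handles the bug's visual fade and invisibility effects.
; SetDynamicMaterial puts dynamic dither materials on body and wings, which one timeline drives forward to fade in and in reverse to fade out.
; InvisibleBug swaps both slots to a shared invisibility material, whose refraction FadeInvisible animates on a second timeline.
; Damage, GetEnemy, Rammed and Squish are stubs with no logic.
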(event Custom|FadeInvisible
  (bind _newtrack_0 (Timeline|Timeline_0 PlayFromStart)
    (:Update
      (Rendering|Material|SetScalarParameterValue (Variables|Default|GetInvisibility) "Refraction" _newtrack_0 :!class /Script/Engine.MaterialInstanceDynamic))))

(event Custom|SetDynamicMaterial
  (Utilities|FlowControl|Sequence
    (:then_0
      (bind _returnvalue (Rendering|Material|CreateDynamicMaterialInstance "/Game/DustDevil/Art/Materials/Enemies/M_Enemy2.M_Enemy2" "None" "None" :!class /Script/Engine.KismetMaterialLibrary))
      (bind _output_get (Variables|Default|SetDitherMat _returnvalue))
      (Rendering|Material|SetMaterial (Variables|Character|GetMesh) 0 _output_get)
      (Rendering|Material|SetScalarParameterValue (Variables|Default|GetDitherMat) "Percent" 0.0 :!class /Script/Engine.MaterialInstanceDynamic))
    (:then_1
      (bind _returnvalue_2 (Rendering|Material|CreateDynamicMaterialInstance "/Game/DustDevil/Art/Materials/Enemies/M_Enemy2Wings.M_Enemy2Wings" "None" "None" :!class /Script/Engine.KismetMaterialLibrary))
      (bind _output_get_2 (Variables|Default|SetDitherMat2 _returnvalue_2))
      (Rendering|Material|SetMaterial (Variables|Character|GetMesh) 1 _output_get_2)
      (Rendering|Material|SetScalarParameterValue (Variables|Default|GetDitherMat2) "Percent2" 1.0 :!class /Script/Engine.MaterialInstanceDynamic))))

(event Custom|PlayBugFadeIn
  (bind _newtrack_0 (Timeline|Timeline PlayFromStart)
    (:Update
      (Rendering|Material|SetScalarParameterValue (Variables|Default|GetDitherMat) "Percent" _newtrack_0 :!class /Script/Engine.MaterialInstanceDynamic)
      (Rendering|Material|SetScalarParameterValue (Variables|Default|GetDitherMat2) "Percent2" _newtrack_0 :!class /Script/Engine.MaterialInstanceDynamic))))

(event Custom|PlayBugFadeOut
  (bind _newtrack_0 (Timeline|Timeline ReverseFromEnd)
    (:Update
      (Rendering|Material|SetScalarParameterValue (Variables|Default|GetDitherMat) "Percent" _newtrack_0 :!class /Script/Engine.MaterialInstanceDynamic)
      (Rendering|Material|SetScalarParameterValue (Variables|Default|GetDitherMat2) "Percent2" _newtrack_0 :!class /Script/Engine.MaterialInstanceDynamic))))

(event Custom|InvisibleBug
  (bind _returnvalue (Rendering|Material|CreateDynamicMaterialInstance "/Game/DustDevil/Art/Materials/M_Invisibility.M_Invisibility" "None" "None" :!class /Script/Engine.KismetMaterialLibrary))
  (Variables|Default|SetInvisibility _returnvalue)
  (Rendering|Material|SetMaterial (Variables|Character|GetMesh) 0 _returnvalue)
  (Rendering|Material|SetMaterial (Variables|Character|GetMesh) 1 _returnvalue))

(event EventBeginPlay
  (|CallParentFunction))

(event Collision|EventActorBeginOverlap
  (params (OtherActor :type Actor%20Object%20Reference)))

(event EventTick
  (params (DeltaSeconds :type Float%20%28single-precision%29))
  (|CallParentFunction DeltaSeconds) ; This node is disabled and will not be called.\nDrag off pins to build functionality.
)

(event EventDamage
  (params (Damage :type Float%20%28double-precision%29) (NewParam2 :type Boolean) (NewParam3 :type Gameplay%20Effect%20Class%20Reference)))

(fn ConstructionScript
  (|CallParentFunction))

(fn GetEnemy
  (return 0))

(fn Rammed
  (return 0))

(fn Squish
  (return 0))