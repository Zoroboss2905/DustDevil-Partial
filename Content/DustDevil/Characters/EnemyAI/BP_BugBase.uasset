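; Base character for bug enemies, using the Gameplay Ability System for stats, health and melee damage.
; BeginPlay applies set-by-caller stats and starts async listeners for health changes, driving hit flashes, reticle feedback and death, and for knocked-tag removal, restoring physics.
; Attacks check a melee sphere against the player's damageable capsule on a cooldown.
; Death rolls loot drops, notifies the player, MotherBrain and tutorial manager, then expires the actor.
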(event Custom|EnemyHitFlash
  (Rendering|Material|SetMaterial (Variables|Character|GetMesh) 0 (Utilities|Array|Get(acopy) (Variables|Default|GetFlashMaterial) (Variables|Default|GetFlashValue)))
  (Utilities|FlowControl|Delay 0.2)
  (Rendering|Material|SetMaterial (Variables|Character|GetMesh) 0 (Utilities|Array|Get(acopy) (Variables|Default|GetMaterial) (Variables|Default|GetMaterialValue))))

(event Custom|Die
  (bind _returnvalue (Transformation|GetActorTransform))
  (bind _returnvalue_2 (Transformation|GetActorTransform))
  (bind _returnvalue_3 (Transformation|GetActorTransform))
  (bind _returnvalue_4 (Ability|GetAbilitySystemComponent 0))
  (bind _returnvalue_5 (Game|Player|GetPlayerPawn 0))
  (bind _motherbrain (Variables|References|GetMotherBrain))
  (bind _tutorialmanagertwo (Variables|Default|GetTutorialManagerTwo))
  (bind _returnvalue_6 (Ability|GetAbilitySystemComponent _returnvalue_5))
  (bind _returnvalue_7 (Class|AbilitySystemComponent|GetGameplayAttributeValue _returnvalue_6 "(AttributeName=\"TankPermaBonus\",Attribute=/Script/DustDevil.VehicleAttributeSet:TankPermaBonus,AttributeOwner=\"/Script/CoreUObject.Class'/Script/DustDevil.VehicleAttributeSet'\")"))
  (Utilities|FlowControl|Sequence
    (:then_0
      (Ability|SendGameplayEventtoActor (Game|Player|GetPlayerPawn 0) "(TagName=\"Event.Enemy.Death\")" (Utilities|Struct|MakeGameplayEventData "(TagName=\"\")" self))
      (CallFunction|StopListening) ; Turn off All Asynchronous tasks 1 tick before deleting the actor
      (Collision|SetActorEnableCollision false)
      (Utilities|FlowControl|DelayUntilNextTick)
      (if (Math|Random|RandomBoolwithWeight (* (.ReturnValue (Class|AbilitySystemComponent|GetGameplayAttributeValue _returnvalue_4 "(AttributeName=\"NuclearMatter\",Attribute=/Script/DustDevil.BaseAttributeSet:NuclearMatter,AttributeOwner=\"/Script/CoreUObject.Class'/Script/DustDevil.BaseAttributeSet'\")")) _returnvalue_7))
        (Game|SpawnActorfromClass "/Game/DustDevil/ItemDrops/BP_NuclearMats.BP_NuclearMats_C" (Math|Transform|MakeTransform (+ (.location _returnvalue_2) "0.000000,0.000000,100.000000") (.rotation _returnvalue_2) "1.000000,1.000000,1.000000") "Undefined" "MultiplyWithRoot" 0 1 0))
      (if (Math|Random|RandomBoolwithWeight (* (Variables|Default|GetChitinDropChance) _returnvalue_7))
        (Game|SpawnActorfromClass "/Game/DustDevil/ItemDrops/BP_MutatedChitin.BP_MutatedChitin_C" (Math|Transform|MakeTransform (.location _returnvalue) (.rotation _returnvalue) "1.000000,1.000000,1.000000") "Undefined" "MultiplyWithRoot" 0 1 0))
      (if (Variables|/Game/DustDevil/Player/BP_Vehicle.BP_Vehicle_C|GetInStagedGameplay (Variables|References|GetPlayer))
        _
        (else
          (Game|SpawnActorfromClass "/Game/DustDevil/ItemDrops/BP_Biomass.BP_Biomass_C" (Math|Transform|MakeTransform (.location _returnvalue_3) (.rotation _returnvalue_3) "1.000000,1.000000,1.000000") "AlwaysSpawn" "MultiplyWithRoot" 0 (Math|Float|Truncate (* (.ReturnValue (Class|AbilitySystemComponent|GetGameplayAttributeValue _returnvalue_4 "(AttributeName=\"BioMatter\",Attribute=/Script/DustDevil.BaseAttributeSet:BioMatter,AttributeOwner=\"/Script/CoreUObject.Class'/Script/DustDevil.BaseAttributeSet'\")")) (.ReturnValue (Class|AbilitySystemComponent|GetGameplayAttributeValue _returnvalue_6 "(AttributeName=\"TankBioBonus\",Attribute=/Script/DustDevil.VehicleAttributeSet:TankBioBonus,AttributeOwner=\"/Script/CoreUObject.Class'/Script/DustDevil.VehicleAttributeSet'\")")))) 0)))
      (if (and (Utilities|IsValid _motherbrain) (Variables|Default|GetbInGroup))
        (Default|EnemyDeath _motherbrain self))
      (Components|Activation|Deactivate (Variables|/Script/AIModule.AIController|GetBrainComponent (AI|GetAIController self)))
      (Actor|SetLifeSpan 1.0)
      (Utilities|IsValid _tutorialmanagertwo
        (:Is%20Valid
          (Default|RemoveArray _tutorialmanagertwo)
          (Default|RemoveArrayRAD _tutorialmanagertwo)
          (Default|RemoveArrayTwo _tutorialmanagertwo))))
    (:then_1
      (bind _returnvalue_8 (Actor|GetActorOfClass "/Game/DustDevil/Characters/EnemyAI/BP_BugFlying.BP_BugFlying_C"))
      (Utilities|IsValid _returnvalue_8
        (:Is%20Valid
          (Default|PlayBugFadeOut _returnvalue_8))
        (:Is%20Not%20Valid
          (Niagara|SpawnSystemAttached "/Game/DustDevil/Effects/Explosions/NS_EnemyExplosion1.NS_EnemyExplosion1" (Variables|Character|GetMesh) "None" "0, 0, 0" "0, 0, 0" "KeepWorldPosition" false))))))

(event Custom|EnemyBurned
  (bind _returnvalue (Niagara|SpawnSystemAttached "/Game/DustDevil/Effects/EnemiesDOTEffects/NS_Burn.NS_Burn" (Variables|Character|GetMesh) "None" "0.000000,0.000000,100.000000" "0, 0, 0" "KeepRelativeOffset" false))
  (Audio|PlaySoundatLocation "/Game/DustDevil/Audio/Feedback/A_FlameBursts_Cue.A_FlameBursts_Cue" (Transformation|GetActorLocation) "0, 0, 0" 1.0 1.0 0.0 0 0 0 0))

(event Custom|ListenForEvents
  (bind _capsulecomponent (Variables|Collision|GetCapsuleComponent))
  (bind _enemyabilitysystem (Variables|Default|GetEnemyAbilitySystem))
  (Utilities|FlowControl|Sequence
    (:then_0
      (bind (_asynctaskproxy _attribute _newvalue _oldvalue) (Ability|Tasks|WaitForAttributeChanged 0 "(AttributeName=\"CurrentHealth\",Attribute=/Script/DustDevil.BaseAttributeSet:CurrentHealth,AttributeOwner=\"/Script/CoreUObject.Class'/Script/DustDevil.BaseAttributeSet'\")")
        (:then
          (Variables|Async|SetHealthChangeListener _asynctaskproxy))
        (:Changed
          ;[1 1 1] Damage has been taken
          (if (and (< _newvalue _oldvalue) (not (Class|ActorComponent|IsBeingDestroyed _enemyabilitysystem)))
            (CallFunction|EnemyDamaged _newvalue _oldvalue (.ReturnValue (Class|AbilitySystemComponent|GetGameplayAttributeValue _enemyabilitysystem "(AttributeName=\"MaxHealth\",Attribute=/Script/DustDevil.BaseAttributeSet:MaxHealth,AttributeOwner=\"/Script/CoreUObject.Class'/Script/DustDevil.BaseAttributeSet'\")")) false)
            (CallFunction|DamageFeedback (.ReturnValue (Class|AbilitySystemComponent|GetGameplayAttributeValue (Variables|Default|GetEnemyAbilitySystem) "(AttributeName=\"CurrentHealth\",Attribute=/Script/DustDevil.BaseAttributeSet:CurrentHealth,AttributeOwner=\"/Script/CoreUObject.Class'/Script/DustDevil.BaseAttributeSet'\")")))
            (Development|PrintString (Utilities|String|Append "ENEMY HEALTH: " (Utilities|String|ToString(Float) _newvalue)) true true "(R=1.000000,G=0.000000,B=0.006006,A=1.000000)")))))
    (:then_1
      (bind _asynctaskproxy_2 (Ability|Tasks|WaitGameplayTagRemoveFromActor 0 "(TagName=\"Event.Enemy.Knocked\")")
        (:then
          (Variables|Async|SetKnockedTagListener _asynctaskproxy_2))
        (:Removed
          (Collision|SetCollisionEnabled _capsulecomponent "QueryAndPhysics")
          (Physics|SetSimulatePhysics _capsulecomponent false)
          (Class|PrimitiveComponent|SetAllPhysicsLinearVelocity _capsulecomponent "0, 0, 0" false)
          (Transformation|SetActorRotation (Math|Rotator|MakeRotator 0.0 0.0 (Math|Random|RandomFloatinRange 0.0 359.0)) true))))))

(event Custom|StopListening
  (AsyncAction|Cancel (Variables|Async|GetHealthChangeListener))
  (AsyncAction|Cancel (Variables|Async|GetKnockedTagListener)))

(event Custom|FlyingBurn
  (bind _returnvalue (Niagara|SpawnSystemAttached "/Game/DustDevil/Effects/EnemiesDOTEffects/NS_Burn.NS_Burn" (Variables|Character|GetMesh) "None" "0, 0, 0" "0, 0, 0" "KeepRelativeOffset" false))
  (Audio|PlaySoundatLocation "/Game/DustDevil/Audio/Feedback/A_FlameBursts_Cue.A_FlameBursts_Cue" (Transformation|GetActorLocation) "0, 0, 0" 1.0 1.0 0.0 0 0 0 0))

(event Custom|EnemySquadEliminated
  (bind _flash1 (Variables|Default|GetFlash1))
  ;[1 1 1] EnemyFlash
  (Variables|Default|SetFlashEnded false)
  (Variables|/Game/DustDevil/UI/Feedback/WBP_Flash1.WBP_Flash1_C|SetFlashColour _flash1 (Variables|Default|GetFinalColour2))
  (UserInterface|Viewport|AddtoViewport _flash1 1)
  (Default|FlashEffect _flash1)
  (Utilities|FlowControl|Delay 0.5)
  (Widget|RemovefromParent _flash1)
  (Variables|Default|SetFlashEnded true))

(event Custom|EnemyDeath
  (bind _flasheffect (Variables|Default|GetFlashEffect))
  ;[1 1 1] EnemyFlash
  (if true
    (Variables|/Game/DustDevil/UI/Feedback/WBP_Flash.WBP_Flash_C|SetFlashColour _flasheffect (Variables|Default|GetFlashColour))
    (UserInterface|Viewport|AddtoViewport _flasheffect 0)
    (Default|FlashEffect _flasheffect)
    (Utilities|FlowControl|Delay 0.3)
    (Widget|RemovefromParent _flasheffect)))

(event Custom|FeedbackUI
  (bind _returnvalue (UserInterface|CreateWidget "/Game/DustDevil/UI/Feedback/WBP_Flash.WBP_Flash_C"))
  (Variables|Default|SetFlashEffect _returnvalue)
  (bind _returnvalue_2 (UserInterface|CreateWidget "/Game/DustDevil/UI/Feedback/WBP_Flash1.WBP_Flash1_C"))
  (Variables|Default|SetFlash1 _returnvalue_2))

(event Custom|FlyingBleed
  (bind _returnvalue (Niagara|SpawnSystemAttached "/Game/DustDevil/Effects/EnemiesDOTEffects/NS_Bleed.NS_Bleed" (Variables|Character|GetMesh) "None" "75.000000,100.000000,100.000000" "0, 0, 0" "KeepRelativeOffset" false))
  (Audio|PlaySound2D "/Game/DustDevil/Audio/Feedback/ks-motion-metal-hit-351564.ks-motion-metal-hit-351564" 2.0 2.0 0.0 0 0 false))

(event Custom|PlayBleed
  (bind _returnvalue (Niagara|SpawnSystemAttached "/Game/DustDevil/Effects/EnemiesDOTEffects/NS_Bleed.NS_Bleed" (Variables|Character|GetMesh) "None" "75.000000,100.000000,100.000000" "0, 0, 0" "KeepRelativeOffset" false))
  (Audio|PlaySound2D "/Game/DustDevil/Audio/Feedback/ks-motion-metal-hit-351564.ks-motion-metal-hit-351564" 2.0 2.0 0.0 0 0 false))

(event Custom|FlyingStun
  (bind _returnvalue (Niagara|SpawnSystemAttached "/Game/DustDevil/Effects/EnemiesDOTEffects/NS_Stun.NS_Stun" (Variables|Character|GetMesh) "None" "0.000000,0.000000,100.000000" "0, 0, 0" "KeepRelativeOffset" false))
  (Audio|PlaySound2D "/Game/DustDevil/Audio/Feedback/sci-fi-sfx-8-350836.sci-fi-sfx-8-350836" 1.0 1.0 0.0 0 0 false))

(event Custom|EnemyStunned
  (bind _returnvalue (Niagara|SpawnSystemAttached "/Game/DustDevil/Effects/EnemiesDOTEffects/NS_Stun.NS_Stun" (Variables|Character|GetMesh) "None" "0.000000,0.000000,100.000000" "0, 0, 0" "KeepRelativeOffset" false))
  (Audio|PlaySound2D "/Game/DustDevil/Audio/Feedback/sci-fi-sfx-8-350836.sci-fi-sfx-8-350836" 1.0 1.0 0.0 0 0 false))

(event EventBeginPlay
  (bind _maxhealth (Variables|Default|GetMaxHealth))
  (Utilities|FlowControl|Sequence
    (:then_0
      (bind _returnvalue (Actor|GetActorOfClass "/Game/DustDevil/Characters/EnemyAI/BP_MotherBrain.BP_MotherBrain_C"))
      (Variables|References|SetMotherBrain _returnvalue))
    (:then_1
      (CallFunction|SetDefaultStats _maxhealth _maxhealth 0.0 (Variables|Attack|GetAttackDamage) (Math|Conversions|ToFloat(Integer) (Variables|Default|GetBiomatterDropped)) (Variables|Default|GetNuclearMatDropChance) (Variables|Default|GetEnemySpeed))
      (CallFunction|ListenforEvents))
    (:then_2
      (WorldPartition|GetDataLayerManager))
    (:then_3
      (CallFunction|FeedbackUI))
    (:then_4
      (bind _player (Class|BPIPlayerTrigger|GetPlayerCharacter(Message) (Game|Player|GetPlayerPawn 0)))
      (Variables|References|SetPlayer _player))
    (:then_5
      (bind _player_2 (Variables|References|GetPlayer)
        (:then
          (Default|CreateMinimapMarkers _player_2))
        (:else)))
    (:then_6
      (bind _returnvalue_2 (Actor|GetActorOfClass "/Game/DustDevil/Tutorials/BP_TutorialManagerTwo.BP_TutorialManagerTwo_C"))
      (Utilities|IsValid _returnvalue_2
        (:Is%20Valid
          (Variables|Default|SetTutorialManagerTwo _returnvalue_2))))))

(event EventDamage
  (params (Damage :type Float%20%28double-precision%29) (NewParam2 :type Boolean) (NewParam3 :type Gameplay%20Effect%20Class%20Reference)))

(event EventEndPlay
  (params (EndPlayReason :type EEndPlayReason%20Enum :default "Destroyed"))
  (CallFunction|StopListening))

(event EventTick
  (params (DeltaSeconds :type Float%20%28single-precision%29))
  (CallFunction|TimerCounting DeltaSeconds)
  (Utilities|FlowControl|DoOnce false :!label _label
    (:Completed
      (Utilities|IsValid (Variables|References|GetMotherBrain)
        (:Is%20Not%20Valid
          (bind _returnvalue (Actor|GetActorOfClass "/Game/DustDevil/Characters/EnemyAI/BP_MotherBrain.BP_MotherBrain_C"))
          (Variables|References|SetMotherBrain _returnvalue)
          (goto _label Reset))))))

(fn ConstructionScript
  (Variables|Default|SetHealth (Variables|Default|GetMaxHealth))
  (Variables|Attack|SetAttackCooldown (Variables|Attack|GetMaxAttackCooldown))
  (Components|Sphere|SetSphereRadius (Variables|Default|GetMeleeRange) (Variables|Attack|GetAttackMeleeRange) true))

(fn TimerCounting
  (params (DeltaTime :type Float%20%28double-precision%29))
  (LocalVariables|SetDT DeltaTime)
  (Utilities|FlowControl|Sequence
    (:then_0
      (if (not (<= (Variables|Attack|GetAttackCooldown) 0.0))
        (Variables|Attack|SetAttackCooldown (- (Variables|Attack|GetAttackCooldown) (LocalVariables|GetDT)))))))

(fn ProjectileDamage
  (params (IncomingDamage :type Float%20%28double-precision%29) (DamageSource :type Actor%20Object%20Reference) (Player :type BP%20Vehicle%20Object%20Reference))
  (bind _output_get (Variables|Default|SetHealth (- (Variables|Default|GetHealth) IncomingDamage)))
  (Variables|References|SetPlayer Player)
  (bind _damagesource (LocalVariables|GetDamageSource)
    (:then
      (Actor|DestroyActor _damagesource))
    (:else
      _))
  (CallFunction|EnemyHitFlash)
  (Audio|PlaySound2D "/Game/DustDevil/Audio/Feedback/BugImpact/A_EnemyDamage_Cue.A_EnemyDamage_Cue" 1.0 1.0 0.0 0 0 false)
  (if (not (<= _output_get 0.0))
    (switch int (Variables|Default|GetMaterialValue)
      (:0
        (if (not (>= _output_get 25.0))
          (Variables|Default|SetFlashValue 1 :!label _label)))
      (:1
        (if (not (>= _output_get 5e+01))
          (goto _label)))
      (:2
        (if (not (>= _output_get 75.0))
          (goto _label))))))

(fn AttackPlayer
  (bind _returnvalue (Game|Player|GetPlayerPawn 0))
  (bind _returnvalue_2 (Transformation|GetActorLocation))
  (bind _returnvalue_3 (Actor|GetComponentsbyTag _returnvalue "/Script/Engine.CapsuleComponent" "Damageable"))
  (bind _output (Utilities|Array|Get(acopy) _returnvalue_3))
  (bind _returnvalue_4 (Transformation|GetWorldLocation _output))
  (Variables|Attack|SetAttackCooldown (Variables|Attack|GetMaxAttackCooldown))
  (Utilities|FlowControl|Sequence
    (:then_0
      (Development|PrintString "Bug Tried to Attack Player!" true true "(R=0.000000,G=1.000000,B=0.694906,A=1.000000)"))
    (:then_1
      (Variables|Default|SetAttackAnim true)
      (Utilities|Time|SetTimerbyFunctionName 0 "FinishAttackAnim" (Variables|Attack|GetMaxAttackCooldown))
      (Transformation|SetActorRotation (Math|Rotator|FindLookatRotation (Math|Vector|MakeVector (.x _returnvalue_2) (.y _returnvalue_2) 0.0) (Math|Vector|MakeVector (.x _returnvalue_4) (.y _returnvalue_4) 0.0)))
      (if (Class|PrimitiveComponent|IsOverlappingComponent (Variables|Default|GetMeleeRange) _output)
        (Utilities|FlowControl|Sequence
          (:then_0
            (Development|PrintString "Bug Attacked Player!"))
          (:then_1
            (GameplayEffects|ApplyGameplayEffectToTarget :self (Variables|Default|GetEnemyAbilitySystem) :GameplayEffectClass "/Game/DustDevil/Core/GAS/Effects/GE_Damage.GE_Damage_C" :Target (Ability|GetAbilitySystemComponent (Variables|References|GetPlayer)))))
        (else
          (Utilities|FlowControl|Sequence
            (:then_0
              (Development|PrintString "Bug Missed!"))))))))

(fn ChangeColourBasedonDamage
  (params (Health :type Float%20%28double-precision%29) (HealthMed :type Float%20%28double-precision%29) (HealthLow :type Float%20%28double-precision%29))
  (if (<= Health 0.0)
    (CallFunction|Die)
    (elif (>= Health HealthMed)
      (if (> (Variables|Default|GetHealth) (Variables|Default|GetMaxHealth))
        (Variables|Default|SetHealth (Variables|Default|GetMaxHealth)))
      (elif (>= Health HealthLow)
        (Rendering|Material|SetMaterial (Variables|Character|GetMesh) 1 "/Game/DustDevil/MaterialLibrary/Materials/M_OutlineEnemy.M_OutlineEnemy")
        (else
          (Rendering|Material|SetMaterial (Variables|Character|GetMesh) 1 "/Game/DustDevil/MaterialLibrary/Materials/M_OutlineLowHealthEnemy.M_OutlineLowHealthEnemy"))))))

(fn SetDefaultStats
  (params (MaxHealth :type Float%20%28double-precision%29) (StartingHealth :type Float%20%28double-precision%29) (Armour :type Float%20%28double-precision%29) (Damage :type Float%20%28double-precision%29) (BioMatter :type Float%20%28double-precision%29) (NuclearMatter :type Float%20%28double-precision%29) (Speed :type Float%20%28double-precision%29))
  (bind _enemyabilitysystem (Variables|Default|GetEnemyAbilitySystem))
  (bind _charactermovement (Variables|Character|GetCharacterMovement))
  (Class|AbilitySystemComponent|InitStats (Variables|Default|GetEnemyAbilitySystem) "/Script/DustDevil.BaseAttributeSet")
  (LocalVariables|SetSpec (GameplayEffects|MakeOutgoingSpec _enemyabilitysystem "/Game/DustDevil/Core/GAS/Effects/GE_DefaultEnemyValues.GE_DefaultEnemyValues_C" 1.0 (GameplayEffects|MakeEffectContext _enemyabilitysystem)))
  (Utilities|FlowControl|Sequence
    (:then_0
      (bind _returnvalue (Ability|GameplayEffect|AssignTagSetbyCallerMagnitude (LocalVariables|GetSpec) "(TagName=\"Stats.Base.MaxHealth\")" MaxHealth))
      (bind _returnvalue_2 (Ability|GameplayEffect|AssignTagSetbyCallerMagnitude _returnvalue "(TagName=\"Stats.Base.CurrentHealth\")" StartingHealth))
      (bind _returnvalue_3 (Ability|GameplayEffect|AssignTagSetbyCallerMagnitude _returnvalue_2 "(TagName=\"Stats.Base.Armour\")" Armour))
      (bind _returnvalue_4 (Ability|GameplayEffect|AssignTagSetbyCallerMagnitude _returnvalue_3 "(TagName=\"Stats.Base.Damage\")" Damage))
      (bind _returnvalue_5 (Ability|GameplayEffect|AssignTagSetbyCallerMagnitude _returnvalue_4 "(TagName=\"Stats.Base.BioMatter\")" BioMatter))
      (bind _returnvalue_6 (Ability|GameplayEffect|AssignTagSetbyCallerMagnitude _returnvalue_5 "(TagName=\"Stats.Base.NuclearMatter\")" NuclearMatter))
      (bind _returnvalue_7 (Ability|GameplayEffect|AssignTagSetbyCallerMagnitude _returnvalue_6 "(TagName=\"Stats.Base.ChitinChance\")" (Variables|Default|GetChitinDropChance)))
      (LocalVariables|SetSpec _returnvalue_7))
    (:then_1
      (GameplayEffects|ApplyGameplayEffectSpecToSelf (Variables|Default|GetEnemyAbilitySystem) (LocalVariables|GetSpec))
      (Variables|/Script/Engine.CharacterMovementComponent|SetMaxFlySpeed _charactermovement Speed)
      (Variables|/Script/Engine.CharacterMovementComponent|SetMaxWalkSpeed _charactermovement Speed))))

(fn EnemyDamaged
  (params (NewHealth :type Float%20%28double-precision%29) (OldHealth :type Float%20%28double-precision%29) (MaxHealth :type Float%20%28double-precision%29) (bWasCrit :type Boolean))
  (CallFunction|EnemyHitFlash)
  (if (<= NewHealth (* MaxHealth 0.0))
    (CallFunction|Die)
    ;[1 1 1] Modify Cursor on Vehicle
    (Default|BugKilled (Variables|/Game/DustDevil/Player/BP_Vehicle.BP_Vehicle_C|GetReticleCursor (Variables|References|GetPlayer)))
    (else
      (switch int (Variables|Default|GetMaterialValue)
        (:0
          (if (>= NewHealth (* MaxHealth 0.25))
            _
            (else
              (Variables|Default|SetFlashValue 1 :!label _label))))
        (:1
          (if (>= NewHealth (* MaxHealth 0.5))
            _
            (else
              (goto _label))))
        (:2
          (if (>= NewHealth (* MaxHealth 0.75))
            _
            (else
              (goto _label)))))
      ;[1 1 1] Update Cursor
      (Default|BugShot (Variables|/Game/DustDevil/Player/BP_Vehicle.BP_Vehicle_C|GetReticleCursor (Variables|References|GetPlayer))))))

(fn DamageFeedback
  (params (InputPin :type Float%20%28double-precision%29))
  (CallFunction|EnemyHitFlash)
  (Audio|PlaySound2D "/Game/DustDevil/Audio/Feedback/BugImpact/A_EnemyDamage_Cue.A_EnemyDamage_Cue" 1.0 1.0 0.0 0 0 false)
  (if (<= InputPin 0.0)
    (CallFunction|EnemyDeath)
    (else
      (switch int (Variables|Default|GetMaterialValue)
        (:0
          (if (not (>= InputPin 2e+01))
            (Variables|Default|SetFlashValue 1 :!label _label)))
        (:1
          (if (not (>= InputPin 5e+01))
            (goto _label)))
        (:2
          (if (not (>= InputPin 75.0))
            (goto _label)))))))

(fn EnemyFeedback
  (return (== (.ReturnValue (Class|AbilitySystemComponent|GetGameplayAttributeValue (Variables|Default|GetEnemyAbilitySystem) "(AttributeName=\"MaxHealth\",Attribute=/Script/DustDevil.BaseAttributeSet:MaxHealth,AttributeOwner=\"/Script/CoreUObject.Class'/Script/DustDevil.BaseAttributeSet'\")")) 0.0)))

(fn FinishAttackAnim
  (Variables|Default|SetAttackAnim false))

(fn RemovefromMinimap
  (bind _outactors (Actor|GetAttachedActors true false))
  (if (not (Utilities|Array|IsEmpty _outactors))
    (bind _filteredarray (Utilities|Array|FilterArray _outactors "/Game/DustDevil/UI/HUD/Minimap/SceneCapture/BP_MinimapIcons.BP_MinimapIcons_C"))
    (if (not (Utilities|Array|IsEmpty _filteredarray))
      (bind _output_get (LocalVariables|SetLocal_MapMarker (Utilities|Array|Get(acopy) _filteredarray)))
      (Utilities|IsValid _output_get
        (:Is%20Valid
          (Default|DestroySprite (LocalVariables|GetLocal_MapMarker)))
        (:Is%20Not%20Valid
          (Development|PrintString "Map marker not valid!"))))))

(fn GetEnemy
  (return self))

(fn Rammed
  (return self))

(fn Squish
  ;[1 1 1] Intended for running over bug, not implemented yet
  (CallFunction|Die)
  (return (Variables|Default|GetBiomatterDropped)))