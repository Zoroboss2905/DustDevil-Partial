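; BP_MotherBrain is the enemy AI coordinator that sorts BP_BugBase bugs into proximity-based attack groups.
; Looping timers assign ungrouped bugs, resync group indices, publish the player's location to the blackboard and move chasing groups' positions to it.
; EnemyDeath prunes members and dissolves empty groups, notifying one bug found by class lookup.
; It also controls combat music pause and fade, though the music creation and debug drawing nodes are unwired.
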(event Custom|ReGroupAll
  (Development|PrintString "Assigning Bugs to groups" true true "(R=1.000000,G=0.059039,B=0.000000,A=1.000000)" 2.0 "")
  (bind _outactors (Actor|GetAllActorsOfClass "/Game/DustDevil/Characters/EnemyAI/BP_BugBase.BP_BugBase_C"))
  (for _array_element _outactors
    (if (not (Variables|/Game/DustDevil/Characters/EnemyAI/BP_BugBase.BP_BugBase_C|GetbInGroup _array_element))
      (CallFunction|AddBugtoAttackGroup _array_element)
      (Development|PrintString "Added bug to Group" true true "(R=1.000000,G=0.059039,B=0.000000,A=1.000000)" 2.0 "")))
  (Development|PrintString "Completed Group Assignment" true true "(R=1.000000,G=0.059039,B=0.000000,A=1.000000)" 2.0 "")
  (CallFunction|UpdateGroupAllocation))

(event Custom|EnemyDeath
  (params (EnemyRef :type BP%20Bug%20Base%20Object%20Reference))
  (bind _owningattackgroupindex (Variables|/Game/DustDevil/Characters/EnemyAI/BP_BugBase.BP_BugBase_C|GetOwningAttackGroupIndex EnemyRef))
  (bind _attackgroups (Variables|Default|GetAttackGroups))
  (bind _output (Utilities|Array|Get(acopy) _attackgroups _owningattackgroupindex))
  (Utilities|Array|RemoveItem (Variables|Default|GetAllEnemies) EnemyRef)
  (if (!= _owningattackgroupindex -1)
    (Utilities|Array|RemoveItem (.members _output) EnemyRef)
    (if (== (Utilities|Array|Length (.members _output)) 0)
      (CallFunction|DissolveAttackGroup _owningattackgroupindex)
      (CallFunction|UpdateGroupAllocation)
      (Utilities|FlowControl|Delay 0.1))))

(event EventBeginPlay
  (Utilities|FlowControl|Sequence
    (:then_1
      (Development|PrintString "Preparing Bugs for assignment" true true "(R=1.000000,G=0.059039,B=0.000000,A=1.000000)")
      (Utilities|FlowControl|Sequence
        (:then_0
          (Utilities|Time|SetTimerbyEvent (delegate Custom|ReGroupAll) 2.0 true true)
          (Development|PrintString "Assigning Bugs to groups" true true "(R=1.000000,G=0.059039,B=0.000000,A=1.000000)" 2.0 "")
          (bind _outactors (Actor|GetAllActorsOfClass "/Game/DustDevil/Characters/EnemyAI/BP_BugBase.BP_BugBase_C"))
          (for _array_element _outactors
            (if (not (Variables|/Game/DustDevil/Characters/EnemyAI/BP_BugBase.BP_BugBase_C|GetbInGroup _array_element))
              (CallFunction|AddBugtoAttackGroup _array_element)
              (Development|PrintString "Added bug to Group" true true "(R=1.000000,G=0.059039,B=0.000000,A=1.000000)" 2.0 "")))
          (Development|PrintString "Completed Group Assignment" true true "(R=1.000000,G=0.059039,B=0.000000,A=1.000000)" 2.0 "")
          (CallFunction|UpdateGroupAllocation))
        (:then_1
          (Utilities|Time|SetTimerbyFunctionName 0 "UpdateGroupAllocation" 1.0 true false 2.0)
          (Utilities|Time|SetTimerbyFunctionName 0 "UpdateData" 0.05 true false 2.0)
          (Utilities|Time|SetTimerbyFunctionName 0 "UpdateGroupData" 0.5 true false 2.0)
          (Utilities|Time|SetTimerbyFunctionName 0 "EndAudio" 0.5 true false 2.0))))))

(event EventTick
  (params (DeltaSeconds :type Float%20%28single-precision%29)))

(fn ConstructionScript)

(fn AddBugtoAttackGroup
  (params (NewBug :type BP%20Bug%20Base%20Object%20Reference))
  (Utilities|Array|Add (Variables|Default|GetAllEnemies) NewBug)
  (LocalVariables|SetNewBugPos (Transformation|GetActorLocation NewBug))
  (for (_array_element _array_index) (Variables|Default|GetAttackGroups)
    (if (and (< (Math|Vector|Distance(Vector) (.grouppos _array_element) (LocalVariables|GetNewBugPos)) (Variables|Default|GetAttackGroupSearchRadius)) (<= (Utilities|Array|Length (.members _array_element)) (Variables|Default|GetGroupMaxCount)))
      (LocalVariables|SetBestDist (Math|Vector|Distance(Vector) (.grouppos _array_element) (LocalVariables|GetNewBugPos)))
      (LocalVariables|SetBestGroupIndex _array_index)))
  (if (== (LocalVariables|GetBestGroupIndex) -1)
    (bind _newgroupindex (CallFunction|MakeNewAttackGroup NewBug))
    (Variables|/Game/DustDevil/Characters/EnemyAI/BP_BugBase.BP_BugBase_C|SetOwningAttackGroupIndex NewBug _newgroupindex)
    (else
      (bind _returnvalue (Utilities|Array|Add (.members (Utilities|Array|Get(acopy) (Variables|Default|GetAttackGroups) (LocalVariables|GetBestGroupIndex))) NewBug))
      (Variables|/Game/DustDevil/Characters/EnemyAI/BP_BugBase.BP_BugBase_C|SetOwningAttackGroupIndex NewBug _returnvalue)))
  (Variables|/Game/DustDevil/Characters/EnemyAI/BP_BugBase.BP_BugBase_C|SetbInGroup NewBug true))

(fn MakeNewAttackGroup
  (params (Progenitor :type Actor%20Object%20Reference))
  (bind _returnvalue (Utilities|Array|Add (Variables|Default|GetAttackGroups) (Utilities|Struct|MakeS_AttackGroup (Utilities|Array|MakeArray Progenitor) (Transformation|GetActorLocation Progenitor) false false)))
  (return _returnvalue))

(fn DissolveAttackGroup
  (params (Index :type Integer))
  (Utilities|Array|RemoveIndex (Variables|Default|GetAttackGroups) Index)
  (bind _returnvalue (Actor|GetActorOfClass "/Game/DustDevil/Characters/EnemyAI/BP_BugBase.BP_BugBase_C"))
  (Utilities|IsValid _returnvalue
    (:Is%20Valid
      (Default|EnemySquadEliminated _returnvalue)
      (bind _musicplay (Variables|Default|GetMusicPlay)
        (:then
          (Class|AudioComponent|SetPaused _musicplay true)
          (Audio|PlaySound2D "/Game/DustDevil/Audio/Feedback/A_CombatEnd.A_CombatEnd" 1.0 1.0 0.0 0 0 false))
        (:else)))))

(fn UpdateGroupAllocation
  (for (_array_element _array_index) (Variables|Default|GetAttackGroups)
    (for _array_element_2 (.members _array_element)
      (Utilities|IsValid _array_element_2
        (:Is%20Valid
          (bind _asbp_bug_base (Utilities|Casting|CastToBP_BugBase _array_element_2))
          (Variables|/Game/DustDevil/Characters/EnemyAI/BP_BugBase.BP_BugBase_C|SetOwningAttackGroupIndex _asbp_bug_base _array_index))))))

(fn UpdateData
  (bind _output_get (Variables|Default|SetLastKnownPlayerLocation (Transformation|GetActorLocation (Game|Player|GetPlayerPawn 0))))
  (AI|Components|Blackboard|SetValueasVector (AI|GetBlackboard 0) (Utilities|Name|MakeLiteralName "LastKnownPlayerLocation") _output_get))

(fn UpdateGroupData
  (for (_array_element _array_index) (Variables|Default|GetAttackGroups)
    (bind _output_get (LocalVariables|SetTempGroupData _array_element))
    (Utilities|FlowControl|Sequence
      (:then_0
        (if (.bmoving _output_get)
          _))
      (:then_1
        (if (.bchasingplayer _output_get)
          (LocalVariables|SetTempGroupData (Utilities|Struct|MakeS_AttackGroup (.members (LocalVariables|GetTempGroupData)) (Variables|Default|GetLastKnownPlayerLocation) (.bmoving (LocalVariables|GetTempGroupData)) (.bchasingplayer (LocalVariables|GetTempGroupData))))
          (bind _musicplay (Variables|Default|GetMusicPlay)
            (:then
              (Class|AudioComponent|SetPaused _musicplay false))
            (:else))))
      (:then_2
        (Utilities|Array|SetArrayElem (Variables|Default|GetAttackGroups) _array_index (LocalVariables|GetTempGroupData))))))

(fn EndAudio
  (bind _returnvalue (Actor|GetActorOfClass "/Game/DustDevil/Player/BP_Vehicle.BP_Vehicle_C"))
  (Utilities|IsValid _returnvalue
    (:Is%20Valid
      (if (not (Variables|/Game/DustDevil/Player/BP_Vehicle.BP_Vehicle_C|GetbCanMove _returnvalue))
        (bind _musicplay (Variables|Default|GetMusicPlay)
          (:then
            (Audio|Components|Audio|FadeOut _musicplay 0.1 0.0 "Linear" :!class /Script/Engine.AudioComponent))
          (:else))))))

(fn CheckifEnemyCapReached
  (return (< (Utilities|Array|Length (Variables|Default|GetAllEnemies)) 100)))