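; Flesh Tearer enemy class that attacks and deals damage through the Gameplay Ability System.
; Attack start self-applies the shared basic enemy cooldown effect, passing AttackCooldown as a set-by-caller magnitude on the attacking cooldown tag.
; A successful attack applies GE_Damage to the target, and death destroys the actor after a short delay.
; It reports its damageable types, while health-change, damage and failed-attack events are empty.
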(event EventBeginPlay)

(event EventOnHealthChanged
  (params (OldValue :type Float%20%28single-precision%29) (NewValue :type Float%20%28single-precision%29)))

(event EventOnDeath
  (Utilities|FlowControl|Delay 2.0)
  (Actor|DestroyActor))

(event EventDamage
  (params (Damage :type Float%20%28double-precision%29) (NewParam2 :type Boolean) (NewParam3 :type Gameplay%20Effect%20Class%20Reference)))

(event EventOnAttackStart
  (params (TargetActor :type Actor%20Object%20Reference))
  (bind _returnvalue (Ability|GetAbilitySystemComponent 0))
  (bind _returnvalue_2 (Ability|GameplayEffect|AssignTagSetbyCallerMagnitude (GameplayEffects|MakeOutgoingSpec _returnvalue "/Game/DustDevil/Core/GAS/Effects/GE_BasicEnemyCD.GE_BasicEnemyCD_C" 1.0 (GameplayEffects|MakeEffectContext _returnvalue)) "(TagName=\"State.Enemy.Attacking.Cooldown\")" (Variables|Default|GetAttackCooldown)))
  (GameplayEffects|ApplyGameplayEffectSpecToSelf (Ability|GetAbilitySystemComponent 0) _returnvalue_2))

(event EventOnAttackFailed
  (params (TargetActor :type Actor%20Object%20Reference)))

(event EventOnAttackSuccess
  (params (TargetActor :type Actor%20Object%20Reference) (HitComponent :type Shape%20Component%20Object%20Reference))
  (GameplayEffects|ApplyGameplayEffectToTarget :self (Ability|GetAbilitySystemComponent 0) :GameplayEffectClass "/Game/DustDevil/Core/GAS/Effects/GE_Damage.GE_Damage_C" :Target (Ability|GetAbilitySystemComponent TargetActor)))

(fn ConstructionScript)

(fn GetDamageableType
  (return (Variables|Default|GetTypes)))

(fn GetEnemy
  (return 0))