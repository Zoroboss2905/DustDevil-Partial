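; Burrowing boss enemy that starts damage-immune, launches globs, deals telegraphed AOE damage and, once alerted, starts boss music and health bar.
; Gameplay tag listeners drive the burrow/emerge cycle, toggling collision and the Blackboard-positioned telegraph, damaging overlapping players and teleporting them clear.
; A looping timer slowly yaws it toward its target unless burrowed or dead.
; Accumulated damage triggers a material flash; death ends the fight and sprays player-stat-scaled loot before destruction.
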(event Custom|AOE_Attack
  (Audio|PlaySoundatLocation "/Game/DustDevil/Audio/Feedback/EnemyThree/A_EnemyDigInAndOut_Cue.A_EnemyDigInAndOut_Cue" (Transformation|GetActorLocation) "0, 0, 0" 1.0 1.0 0.0 0 0 0 0)
  (bind _outactors (Collision|SphereOverlapActors (AI|Components|Blackboard|GetValueasVector (AI|GetBlackboard 0) (Utilities|Name|MakeLiteralName "TelegraphLocation")) (* (.x (Transformation|GetActorScale3D)) 2e+02) (Utilities|Array|MakeArray "ObjectTypeQuery8") "/Script/Engine.Actor"))
  (for _array_element _outactors
    (if (== _array_element (Game|Player|GetPlayerPawn 0))
      (GameplayEffects|ApplyGameplayEffectToTarget :self (Ability|GetAbilitySystemComponent 0) :GameplayEffectClass "/Game/DustDevil/Core/GAS/Effects/GE_Damage.GE_Damage_C" :Target (Ability|GetAbilitySystemComponent (Game|Player|GetPlayerPawn 0)) :Level 1.0))))

(event EventOnDeath
  (Utilities|FlowControl|DoOnce false
    (:Completed
      (Default|BossFightEnded (Variables|Default|GetAudioManager))
      (Class|BPICursorCalls|RemoveBossHealthBar(Message) (Game|GetPlayerController 0))
      (Utilities|FlowControl|Sequence
        (:then_0
          (Utilities|FlowControl|Delay 1e+01)
          (Actor|DestroyActor))
        (:then_1
          (CallFunction|SpawnItemDrop)
          (bind _returnvalue (Utilities|Time|SetTimerbyFunctionName 0 "SpawnItemDrop" 0.1 true))
          (Variables|Default|SetItemDropTimer _returnvalue)
          (Utilities|FlowControl|Delay 2.0)
          (Utilities|Time|ClearandInvalidateTimerbyHandle (Variables|Default|GetItemDropTimer)))))))

(event EventOnHealthChanged
  (params (OldValue :type Float%20%28single-precision%29) (NewValue :type Float%20%28single-precision%29))
  (bind _output_get (Variables|Default|SetCumulativeDamage (+ (Variables|Default|GetCumulativeDamage) (- OldValue NewValue))))
  (if (> _output_get 1e+01)
    (Variables|Default|SetCumulativeDamage (- (Variables|Default|GetCumulativeDamage) 1e+01))
    (CallFunction|TakeLargeDamage)))

(event EventOnAttackStart
  (params (TargetActor :type Actor%20Object%20Reference))
  (bind _returnvalue (Ability|GetAbilitySystemComponent 0))
  (bind _returnvalue_2 (Ability|GameplayEffect|AssignTagSetbyCallerMagnitude (GameplayEffects|MakeOutgoingSpec _returnvalue "/Game/DustDevil/Core/GAS/Effects/GE_BasicEnemyCD.GE_BasicEnemyCD_C" 1.0 (GameplayEffects|MakeEffectContext _returnvalue)) "(TagName=\"State.Enemy.Attacking.Cooldown\")" (Variables|Default|GetAttackCooldown)))
  (GameplayEffects|ApplyGameplayEffectSpecToSelf (Ability|GetAbilitySystemComponent 0) _returnvalue_2))

(event EventOnAttackFailed
  (params (TargetActor :type Actor%20Object%20Reference))
  (bind _returnvalue (Transformation|GetActorTransform))
  (Game|SpawnActorfromClass "/Game/DustDevil/Characters/Enemies/BossProjectiles/BP_Glob.BP_Glob_C" (Math|Transform|MakeTransform (Math|Vector|MakeVector (.x (.location _returnvalue)) (.y (.location _returnvalue)) (+ (.z (.location _returnvalue)) (* (.x (.scale _returnvalue)) 4e+02))) (.rotation _returnvalue) (Math|Vector|MakeVector (.x (.scale _returnvalue)) (.y (.scale _returnvalue)) (.z (.scale _returnvalue)))) "AlwaysSpawn" "MultiplyWithRoot" 0 false (Math|Random|RandomFloatinRange 1.5e+03 2.5e+03) self))

(event EventOnAttackSuccess
  (params (TargetActor :type Actor%20Object%20Reference) (HitComponent :type Shape%20Component%20Object%20Reference))
  (bind _returnvalue (Transformation|GetActorTransform))
  (Game|SpawnActorfromClass "/Game/DustDevil/Characters/Enemies/BossProjectiles/BP_Glob.BP_Glob_C" (Math|Transform|MakeTransform (Math|Vector|MakeVector (.x (.location _returnvalue)) (.y (.location _returnvalue)) (+ (.z (.location _returnvalue)) (* (.x (.scale _returnvalue)) 4e+02))) (.rotation _returnvalue) (Math|Vector|MakeVector (.x (.scale _returnvalue)) (.y (.scale _returnvalue)) (.z (.scale _returnvalue)))) "AlwaysSpawn" "MultiplyWithRoot" 0 false (Math|Random|RandomFloatinRange 1.5e+03 2.5e+03) self))

(event EventBeginPlay
  (Utilities|FlowControl|Sequence
    (:then_0
      (Variables|/Script/Engine.CharacterMovementComponent|SetGravityScale (Variables|Character|GetCharacterMovement) 0.0))
    (:then_1
      (Ability|GameplayEffect|AddLooseGameplayTags self (GameplayTags|MakeLiteralGameplayTagContainer "(GameplayTags=((TagName=\"State.Damage.Immune\"),(TagName=\"State.Movement.Burrowing.Ongoing\")))"))
      (Utilities|Time|SetTimerbyFunctionName 0 "LookTowardsTarget" 0.01 true)
      (Ability|Tasks|WaitGameplayTagAddToActor 0 "(TagName=\"State.Movement.Burrowing.Start\")"
        (:then
          (Ability|Tasks|WaitGameplayTagAddToActor 0 "(TagName=\"State.Movement.Emerge.Start\")"
            (:then
              (Ability|Tasks|WaitGameplayTagAddToActor 0 "(TagName=\"State.Movement.Emerge.Finish\")"
                (:then
                  (Ability|Tasks|WaitGameplayTagAddToActor 0 "(TagName=\"State.Movement.Burrowing.Moving\")"
                    (:then
                      (Ability|Tasks|WaitGameplayTagAddToActor 0 "(TagName=\"State.Enemy.Alert\")"
                        (:Added
                          (Utilities|FlowControl|DoOnce false
                            (:Completed
                              (Variables|/Script/Engine.CharacterMovementComponent|SetGravityScale (Variables|Character|GetCharacterMovement) 1.0)
                              (Class|BPICursorCalls|AddBossHealthBar(Message) (Game|GetPlayerController 0) self)
                              (bind _returnvalue (Actor|GetActorOfClass "/Game/DustDevil/Audio/BP_AudioManager.BP_AudioManager_C"))
                              (bind _output_get (Variables|Default|SetAudioManager _returnvalue))
                              (Default|BossFightStarted _output_get))))))
                    (:Added
                      (Utilities|FlowControl|DelayUntilNextTick)
                      (CallFunction|TelegraphToggle true))))
                (:Added
                  (CallFunction|EmergeCollisionFixing))))
            (:Added
              (CallFunction|EmergeShove)
              (CallFunction|TelegraphToggle false))))
        (:Added
          (Collision|SetCollisionEnabled (Variables|Default|GetCylinder) "NoCollision")
          (Utilities|FlowControl|DelayUntilNextTick)
          (CallFunction|TelegraphToggle true))))))

(event Custom|TakeLargeDamage
  (bind _returnvalue (Ability|GetAbilitySystemComponent 0))
  (Utilities|FlowControl|DoOnce false :!label _label
    (:Completed
      (Variables|Default|SetDefaultMaterial (Rendering|Material|GetMaterial (Variables|Character|GetMesh) 0))
      (Rendering|Material|SetMaterial (Variables|Character|GetMesh) 0 (select (< (/ (.ReturnValue (Ability|Attribute|GetFloatAttributefromAbilitySystemComponent _returnvalue "(AttributeName=\"CurrentHealth\",Attribute=/Script/DustDevil.BaseAttributeSet:CurrentHealth,AttributeOwner=\"/Script/CoreUObject.Class'/Script/DustDevil.BaseAttributeSet'\")")) (.ReturnValue (Ability|Attribute|GetFloatAttributefromAbilitySystemComponent _returnvalue "(AttributeName=\"MaxHealth\",Attribute=/Script/DustDevil.BaseAttributeSet:MaxHealth,AttributeOwner=\"/Script/CoreUObject.Class'/Script/DustDevil.BaseAttributeSet'\")"))) 0.3) "/Game/DustDevil/Art/Materials/Enemies/M_EnemyLowHealth.M_EnemyLowHealth" "/Game/DustDevil/UI/Feedback/GlowMaterials/M_FlashEffect.M_FlashEffect"))
      (Audio|PlaySoundatLocation "/Game/DustDevil/Audio/Feedback/BugImpact/A_EnemyDamage_Cue.A_EnemyDamage_Cue" (Transformation|GetActorLocation) "0, 0, 0" 1.0 1.0 0.0 0 0 0 0)
      (Utilities|FlowControl|Delay 0.2)
      (Rendering|Material|SetMaterial (Variables|Character|GetMesh) 0 (Variables|Default|GetDefaultMaterial))
      (goto _label Reset))))

(fn ConstructionScript)

(fn LookTowardsTarget
  (bind _returnvalue (Ability|GetAbilitySystemComponent 0))
  (bind _returnvalue_2 (Transformation|GetActorTransform))
  (if (and (not (GameplayTags|HasMatchingGameplayTag _returnvalue "(TagName=\"State.Movement.Burrowing.Ongoing\")")) (not (GameplayTags|HasMatchingGameplayTag _returnvalue "(TagName=\"State.Enemy.Death\")")))
    (bind _asactor (Utilities|Casting|CastToActor (AI|Components|Blackboard|GetValueasObject (AI|GetBlackboard 0) (Utilities|Name|MakeLiteralName "Target"))))
    (Class|Actor|AddActorWorldRotation (Math|Rotator|MakeRotator 0.0 0.0 (Math|Float|ClampAngle (.yaw (Math|Rotator|FindRelativeLookatRotation (Math|Transform|MakeTransform (Math|Vector|MakeVector (.x (.location _returnvalue_2)) (.y (.location _returnvalue_2)) 0.0) (.rotation _returnvalue_2) (.scale _returnvalue_2)) (Math|Vector|MakeVector (.x (Transformation|GetActorLocation _asactor)) (.y (Transformation|GetActorLocation _asactor)) 0.0))) -0.75 0.75)))))

(fn EmergeCollisionFixing
  (bind _returnvalue (Game|Player|GetPlayerPawn 0))
  (bind _returnvalue_2 (Transformation|GetActorLocation))
  (bind _returnvalue_3 (Transformation|GetActorScale3D))
  (bind _returnvalue_4 (Game|Player|GetPlayerPawn 0))
  (bind _cylinder (Variables|Default|GetCylinder))
  (bind _returnvalue_5 (Transformation|GetActorLocation _returnvalue))
  (bind _returnvalue_6 (+ (.x _returnvalue_3) (.y _returnvalue_3) (.z _returnvalue_3)))
  (bind _returnvalue_7 (- _returnvalue_5 _returnvalue_2))
  (bind _returnvalue_8 (/ _returnvalue_6 3.0))
  (bind _returnvalue_9 (Math|Vector|Normalize _returnvalue_7))
  (bind _returnvalue_10 (* _returnvalue_9 2e+02 _returnvalue_8))
  (bind _returnvalue_11 (+ _returnvalue_5 _returnvalue_10))
  (Collision|SetCollisionEnabled _cylinder "QueryAndPhysics")
  (bind _outactors (Collision|SphereOverlapActors (Transformation|GetActorLocation) (* (.x (Transformation|GetWorldScale _cylinder)) 5e+01) (Utilities|Array|MakeArray "ObjectTypeQuery8") 0))
  (for _array_element _outactors
    (if (== _array_element _returnvalue_4)
      (Transformation|SetActorLocation _returnvalue_4 (Math|Vector|MakeVector (.x _returnvalue_11) (.y _returnvalue_11) (.Z (Math|Vector|BreakVector _returnvalue_5))) false true))))

(fn EmergeShove
  (bind _returnvalue (Game|Player|GetPlayerPawn 0))
  (bind _outactors (Collision|SphereOverlapActors (Transformation|GetActorLocation) (* (.x (Transformation|GetWorldScale (Variables|Default|GetCylinder))) 5e+01) (Utilities|Array|MakeArray "ObjectTypeQuery8") 0))
  (for _array_element _outactors
    (if (== _array_element _returnvalue)
      (GameplayEffects|ApplyGameplayEffectToTarget :self (Ability|GetAbilitySystemComponent 0) :GameplayEffectClass "/Game/DustDevil/Core/GAS/Effects/GE_Damage.GE_Damage_C" :Target (Ability|GetAbilitySystemComponent _returnvalue)))))

(fn TelegraphToggle
  (params (bVisible :type Boolean))
  (bind _returnvalue (AI|GetBlackboard 0))
  (bind _returnvalue_2 (Utilities|Name|MakeLiteralName "TelegraphLocation"))
  (bind _returnvalue_3 (AI|Components|Blackboard|GetValueasVector _returnvalue _returnvalue_2))
  (bind _telegraph (Variables|Default|GetTelegraph)
    (:then
      (Transformation|SetWorldLocation _telegraph (Math|Vector|MakeVector (.x _returnvalue_3) (.y _returnvalue_3) (- (.z _returnvalue_3) 1e+02)) false true)
      (Rendering|SetVisibility _telegraph bVisible false))
    (:else)))

(fn SpawnItemDrop
  (bind _returnvalue (Transformation|GetActorTransform))
  (bind _returnvalue_2 (Transformation|GetActorTransform))
  (bind _returnvalue_3 (Transformation|GetActorTransform))
  (bind _returnvalue_4 (Game|Player|GetPlayerPawn 0))
  (bind _returnvalue_5 (Ability|GetAbilitySystemComponent _returnvalue_4))
  (bind _returnvalue_6 (Class|AbilitySystemComponent|GetGameplayAttributeValue _returnvalue_5 "(AttributeName=\"TankPermaBonus\",Attribute=/Script/DustDevil.VehicleAttributeSet:TankPermaBonus,AttributeOwner=\"/Script/CoreUObject.Class'/Script/DustDevil.VehicleAttributeSet'\")"))
  (if (Math|Random|RandomBoolwithWeight (* (.ReturnValue (Class|AbilitySystemComponent|GetGameplayAttributeValue (Ability|GetAbilitySystemComponent 0) "(AttributeName=\"NuclearMatter\",Attribute=/Script/DustDevil.BaseAttributeSet:NuclearMatter,AttributeOwner=\"/Script/CoreUObject.Class'/Script/DustDevil.BaseAttributeSet'\")")) _returnvalue_6))
    (Game|SpawnActorfromClass "/Game/DustDevil/ItemDrops/BP_NuclearMats.BP_NuclearMats_C" (Math|Transform|MakeTransform (+ (.location _returnvalue_2) "0.000000,0.000000,500.000000") (.rotation _returnvalue_2) "1.000000,1.000000,1.000000") "Undefined" "MultiplyWithRoot" 0 1 0))
  (if (Math|Random|RandomBoolwithWeight (* (Variables|Default|GetChitinDropChance) _returnvalue_6))
    (Game|SpawnActorfromClass "/Game/DustDevil/ItemDrops/BP_MutatedChitin.BP_MutatedChitin_C" (Math|Transform|MakeTransform (+ (.location _returnvalue) "0.000000,0.000000,500.000000") (.rotation _returnvalue) "1.000000,1.000000,1.000000") "Undefined" "MultiplyWithRoot" 0 1 0))
  (Game|SpawnActorfromClass "/Game/DustDevil/ItemDrops/BP_Biomass.BP_Biomass_C" (Math|Transform|MakeTransform (+ (.location _returnvalue_3) "0.000000,0.000000,500.000000") (.rotation _returnvalue_3) "1.000000,1.000000,1.000000") "AlwaysSpawn" "MultiplyWithRoot" 0 (Math|Float|Truncate (* (Variables|Default|GetBiomassDropped) (.ReturnValue (Class|AbilitySystemComponent|GetGameplayAttributeValue _returnvalue_5 "(AttributeName=\"TankBioBonus\",Attribute=/Script/DustDevil.VehicleAttributeSet:TankBioBonus,AttributeOwner=\"/Script/CoreUObject.Class'/Script/DustDevil.VehicleAttributeSet'\")")))) 0))

(fn GetEnemy
  (return 0))