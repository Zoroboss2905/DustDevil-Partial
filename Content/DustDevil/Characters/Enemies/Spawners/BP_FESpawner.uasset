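; Trigger-volume enemy spawner that creates a batch of BP_BugBase enemies when a player actor enters while active.
; Bugs get configured stats, random scale and navigable positions within SpawnLocation, gated by MotherBrain's enemy-cap check when it exists.
; In the tutorial it polls BugBaseArray until empty to clear the second blockage; otherwise it destroys itself after spawning.
; CanRepeatSpawn re-arms and re-fires the DoOnce five seconds after the player exits.
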(event OnComponentBeginOverlap(Trigger)
  (params (OverlappedComponent :type Primitive%20Component%20Object%20Reference) (OtherActor :type Actor%20Object%20Reference) (OtherComp :type Primitive%20Component%20Object%20Reference) (OtherBodyIndex :type Integer) (bFromSweep :type Boolean) (SweepResult :type Hit%20Result%20Structure%20%28by%20ref%29))
  (bind _spawnlocation (Variables|Default|GetSpawnLocation))
  ;[0.02956 0.02956 0.02956] Spawns specified enemy type when player enters trigger
  (if (Utilities|DoesObjectImplementInterface OtherActor "/Game/DustDevil/Core/Interfaces/BPI_PlayerTrigger.BPI_PlayerTrigger_C")
    (if (Variables|Default|GetbIsActive)
      (Utilities|FlowControl|DoOnce false
        (:Completed
          (Variables|Default|SetArrayNumber 0)
          (for _index (range 1 (Variables|EnemyProperties|GetNumberToSpawn))
            (bind _motherbrain (Variables|Default|GetMotherBrain)
              (:then
                (if (Default|CheckifEnemyCapReached _motherbrain)
                  (bind _randomlocation (Class|NavigationSystemV1|GetRandomLocationinNavigableRadius (Transformation|GetWorldLocation _spawnlocation) (Variables|/Script/Engine.SphereComponent|GetSphereRadius _spawnlocation) 0 0 :!label _label))
                  (bind _output_get (Variables|Default|SetRandomSizeValue (Math|Random|RandomFloatinRange 1.5 2.5)))
                  (bind _returnvalue (Game|SpawnActorfromClass "/Game/DustDevil/Characters/EnemyAI/BP_BugBase.BP_BugBase_C" (Math|Transform|MakeTransform _randomlocation "0, 0, 0" (Math|Vector|MakeVector _output_get _output_get _output_get)) "AdjustIfPossibleButAlwaysSpawn" "MultiplyWithRoot" 0 (Variables|EnemyProperties|GetMax%20Attack%20Cooldown) (Variables|EnemyProperties|GetDetection%20Radius) (Variables|EnemyProperties|GetMax%20Health) (Variables|EnemyProperties|GetAttack%20Damage) (Variables|EnemyProperties|GetBiomatter%20Dropped) 0 (Variables|EnemyProperties|GetNuclear%20Mat%20Drop%20Chance) (Variables|EnemyProperties|GetEnemy%20Speed) (Variables|Default|GetChitinDropChance) 0))
                  (bind _returnvalue_2 (Utilities|Array|Add (Variables|Default|GetBug_BaseArray) _returnvalue))
                  (Variables|Default|SetArrayNumber _returnvalue_2)))
              (:else
                (goto _label))))
          ;[1 1 1] tutorial functionality
          (if (Variables|Tutorial|GetbInTutorial)
            (if (== (Utilities|Array|Length (Variables|Default|GetBug_BaseArray)) 0) :!label _label_2
              (Default|DestroyBlockageTwo (Variables|Default|GetTutorialManagerTwo))
              (else
                (Utilities|FlowControl|Delay 0.2)
                (goto _label_2)))
            (else
              (Actor|DestroyActor))))))))

(event OnComponentEndOverlap(Trigger)
  (params (OverlappedComponent :type Primitive%20Component%20Object%20Reference) (OtherActor :type Actor%20Object%20Reference) (OtherComp :type Primitive%20Component%20Object%20Reference) (OtherBodyIndex :type Integer))
  (bind _spawnlocation (Variables|Default|GetSpawnLocation))
  ;[0.02956 0.02956 0.02956] Spawns specified enemy type when player enters trigger
  (if (Utilities|DoesObjectImplementInterface OtherActor "/Game/DustDevil/Core/Interfaces/BPI_PlayerTrigger.BPI_PlayerTrigger_C")
    (if (Variables|Default|GetbCanRepeatSpawn)
      (Utilities|FlowControl|Delay 5.0)
      (Utilities|FlowControl|Sequence
        (:then_0
          (goto _label Reset))
        (:then_1
          (if (Variables|Default|GetbIsActive)
            (Utilities|FlowControl|DoOnce false :!label _label
              (:Completed
                (Variables|Default|SetArrayNumber 0)
                (for _index (range 1 (Variables|EnemyProperties|GetNumberToSpawn))
                  (bind _motherbrain (Variables|Default|GetMotherBrain)
                    (:then
                      (if (Default|CheckifEnemyCapReached _motherbrain)
                        (bind _randomlocation (Class|NavigationSystemV1|GetRandomLocationinNavigableRadius (Transformation|GetWorldLocation _spawnlocation) (Variables|/Script/Engine.SphereComponent|GetSphereRadius _spawnlocation) 0 0 :!label _label_2))
                        (bind _output_get (Variables|Default|SetRandomSizeValue (Math|Random|RandomFloatinRange 1.5 2.5)))
                        (bind _returnvalue (Game|SpawnActorfromClass "/Game/DustDevil/Characters/EnemyAI/BP_BugBase.BP_BugBase_C" (Math|Transform|MakeTransform _randomlocation "0, 0, 0" (Math|Vector|MakeVector _output_get _output_get _output_get)) "AdjustIfPossibleButAlwaysSpawn" "MultiplyWithRoot" 0 (Variables|EnemyProperties|GetMax%20Attack%20Cooldown) (Variables|EnemyProperties|GetDetection%20Radius) (Variables|EnemyProperties|GetMax%20Health) (Variables|EnemyProperties|GetAttack%20Damage) (Variables|EnemyProperties|GetBiomatter%20Dropped) 0 (Variables|EnemyProperties|GetNuclear%20Mat%20Drop%20Chance) (Variables|EnemyProperties|GetEnemy%20Speed) (Variables|Default|GetChitinDropChance) 0))
                        (bind _returnvalue_2 (Utilities|Array|Add (Variables|Default|GetBug_BaseArray) _returnvalue))
                        (Variables|Default|SetArrayNumber _returnvalue_2)))
                    (:else
                      (goto _label_2))))
                ;[1 1 1] tutorial functionality
                (if (Variables|Tutorial|GetbInTutorial)
                  (if (== (Utilities|Array|Length (Variables|Default|GetBug_BaseArray)) 0) :!label _label_3
                    (Default|DestroyBlockageTwo (Variables|Default|GetTutorialManagerTwo))
                    (else
                      (Utilities|FlowControl|Delay 0.2)
                      (goto _label_3)))
                  (else
                    (Actor|DestroyActor)))))))))))

(event Custom|RemoveArray
  ;[1 1 1] tutorial functionality
  (Utilities|Array|RemoveIndex (Variables|Default|GetBug_BaseArray) (Variables|Default|GetArrayNumber))
  (Variables|Default|SetArrayNumber (- (Variables|Default|GetArrayNumber) 1)))

(event EventBeginPlay
  (bind _returnvalue (Actor|GetActorOfClass "/Game/DustDevil/Player/BP_Vehicle.BP_Vehicle_C"))
  (Variables|Default|SetPlayer _returnvalue)
  (bind _returnvalue_2 (Actor|GetActorOfClass "/Game/DustDevil/Characters/EnemyAI/BP_MotherBrain.BP_MotherBrain_C"))
  (Variables|Default|SetMotherBrain _returnvalue_2)
  (bind _returnvalue_3 (Actor|GetActorOfClass "/Game/DustDevil/Tutorials/BP_TutorialManagerTwo.BP_TutorialManagerTwo_C"))
  (Utilities|IsValid _returnvalue_3
    (:Is%20Valid
      (Variables|Default|SetTutorialManagerTwo _returnvalue_3))))

(fn ConstructionScript)