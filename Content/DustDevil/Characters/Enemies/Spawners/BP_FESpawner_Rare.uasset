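; Enemy spawner for a rare, oversized bug variant.
; On BeginPlay it checks MotherBrain's enemy cap, then spawns a scaled-up BP_BugBase at a random navigable point near SpawnArea.
; It passes its combat and drop stats to the bug and applies an alternate material.
; The high-value-target objective marker and its alive-polling cleanup exist, but the marker spawn and polling start are disconnected.
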(event Custom|CheckIfAlive
  (if (Utilities|IsValid (Variables|Default|GetBugBase))
    (Utilities|FlowControl|RetriggerableDelay 0.01)
    (CallFunction|CheckifAlive)
    (else
      (Actor|DestroyActor (Variables|Default|GetObjectiveActor)))))

(event EventBeginPlay
  (bind _returnvalue (Actor|GetActorOfClass "/Game/DustDevil/Characters/EnemyAI/BP_MotherBrain.BP_MotherBrain_C"))
  (bind _output_get (Variables|Default|SetMotherBrain _returnvalue))
  (if (Default|CheckifEnemyCapReached _output_get)
    (bind _randomlocation (Class|NavigationSystemV1|GetRandomLocationinNavigableRadius (Transformation|GetWorldLocation (Variables|Default|GetSpawnArea)) 2e+02 0 0))
    (bind _returnvalue_2 (Game|SpawnActorfromClass "/Game/DustDevil/Characters/EnemyAI/BP_BugBase.BP_BugBase_C" (Math|Transform|MakeTransform _randomlocation "0, 0, 0" "6.000000,6.000000,6.000000") "AlwaysSpawn" "MultiplyWithRoot" 0 (Variables|Default|GetMax%20Attack%20Cooldown) 2e+04 (Variables|Default|GetMax%20Health) (Variables|Default|GetAttack%20Damage) (Variables|Default|GetBiomatter%20Dropped) 1 (Variables|Default|GetNuclear%20Mat%20Drop%20Chance) (Variables|Default|GetEnemy%20Speed) (Variables|Default|GetChitin%20Drop%20Chance) 0))
    (Variables|Default|SetBugBase _returnvalue_2)
    (Variables|/Game/DustDevil/Characters/EnemyAI/BP_BugBase.BP_BugBase_C|SetMaterialValue _returnvalue_2 1)
    (Rendering|Material|SetMaterial (Variables|/Script/Engine.Character|GetMesh _returnvalue_2) 0 "/Game/DustDevil/Art/Materials/Enemies/M_Enemy1_V2.M_Enemy1_V2")))

(fn ConstructionScript
  (|CallParentFunction))