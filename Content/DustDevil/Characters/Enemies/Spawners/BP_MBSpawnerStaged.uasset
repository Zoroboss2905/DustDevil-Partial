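; BP_MBSpawnerStaged is a trigger-based enemy spawner that releases a batch of flying bugs when the player enters its volume.
; While Active, the first overlap by an actor implementing BPI_PlayerTrigger passes a DoOnce and spawns NumberToSpawn BP_BugFlying at random navigable points around the spawner.
; Each bug receives the spawner's stat and drop variables, then gets a dynamic material and fade-in.
; A timeline-driven hover-down entrance remains in the graph but never runs.
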(event OnComponentBeginOverlap(Trigger)
  (params (OverlappedComponent :type Primitive%20Component%20Object%20Reference) (OtherActor :type Actor%20Object%20Reference) (OtherComp :type Primitive%20Component%20Object%20Reference) (OtherBodyIndex :type Integer) (bFromSweep :type Boolean) (SweepResult :type Hit%20Result%20Structure%20%28by%20ref%29))
  ;[0.02956 0.02956 0.02956] Spawns specified enemy type when player enters trigger
  (if (Utilities|DoesObjectImplementInterface OtherActor "/Game/DustDevil/Core/Interfaces/BPI_PlayerTrigger.BPI_PlayerTrigger_C")
    (if (Variables|Default|GetbActive)
      (Utilities|FlowControl|DoOnce false
        (:Completed
          (for _index (range 1 (Variables|EnemyProperties|GetNumberToSpawn))
            (bind _randomlocation (Class|NavigationSystemV1|GetRandomLocationinNavigableRadius (Transformation|GetActorLocation) 5e+02 0 0))
            (bind _returnvalue (Game|SpawnActorfromClass "/Game/DustDevil/Characters/EnemyAI/BP_BugFlying.BP_BugFlying_C" (Math|Transform|MakeTransform _randomlocation "0, 0, 0" "3.000000,3.000000,3.000000") "AdjustIfPossibleButAlwaysSpawn" "MultiplyWithRoot" 0 (Variables|Default|GetMaxAttackCooldown) (Variables|Default|GetDetectionRadius) (Variables|Default|GetMaxHealth) (Variables|Default|GetAttackDamage) (Variables|Default|GetBiomatterDropped) 0 (Variables|Default|GetNuclearMatDropChance) (Variables|Default|GetEnemySpeed) 0.1 0))
            (Default|SetDynamicMaterial _returnvalue)
            (Default|PlayBugFadein _returnvalue)))))))

(fn ConstructionScript)