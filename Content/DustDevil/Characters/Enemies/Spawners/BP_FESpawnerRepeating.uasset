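; Trigger-based enemy spawner that spawns randomly scaled BP_BugBase enemies at random navigable points around its spawn area.
; Player overlap, when active, fires a one-time initial burst gated by MotherBrain's enemy-cap check, plus an optional combat tutorial.
; A looping timer then spawns more, without the cap check, until the total count is reached or the player leaves.
; Exiting can re-arm the trigger after a delay.
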(event OnComponentBeginOverlap(TriggerSphere)
  (params (OverlappedComponent :type Primitive%20Component%20Object%20Reference) (OtherActor :type Actor%20Object%20Reference) (OtherComp :type Primitive%20Component%20Object%20Reference) (OtherBodyIndex :type Integer) (bFromSweep :type Boolean) (SweepResult :type Hit%20Result%20Structure%20%28by%20ref%29))
  ;[0.02956 0.02956 0.02956] Spawns specified enemy type when player enters trigger
  (if (Utilities|DoesObjectImplementInterface OtherActor "/Game/DustDevil/Core/Interfaces/BPI_PlayerTrigger.BPI_PlayerTrigger_C")
    (bind _player (Class|BPIPlayerTrigger|GetPlayerCharacter(Message) OtherActor))
    (Variables|References|SetPlayer _player)
    (if (Variables|Default|GetbIsActive)
      (Utilities|FlowControl|DoOnce false
        (:Completed
          (for _index (range 1 (Variables|EnemyProperties|GetInitialSpawnCount))
            (if (Default|CheckifEnemyCapReached (Variables|References|GetMotherBrain))
              (CallFunction|SpawnEnemy)))
          (CallFunction|CheckforTutorialTrigger)
          (if (Collision|IsOverlappingActor (Variables|Default|GetTriggerSphere) (Variables|References|GetPlayer) :!class /Script/Engine.PrimitiveComponent)
            (bind _returnvalue (Utilities|Time|SetTimerbyFunctionName 0 "SpawnEnemy" 2.0 true))
            (Variables|Default|SetRepeatingSpawnTimer _returnvalue)
            (else
              (Development|PrintString "Player is no longer in range!"))))))))

(event OnComponentEndOverlap(TriggerSphere)
  (params (OverlappedComponent :type Primitive%20Component%20Object%20Reference) (OtherActor :type Actor%20Object%20Reference) (OtherComp :type Primitive%20Component%20Object%20Reference) (OtherBodyIndex :type Integer))
  ;[0.02956 0.02956 0.02956] Spawns specified enemy type when player enters trigger
  (if (Utilities|DoesObjectImplementInterface OtherActor "/Game/DustDevil/Core/Interfaces/BPI_PlayerTrigger.BPI_PlayerTrigger_C")
    (Utilities|Time|ClearandInvalidateTimerbyHandle (Variables|Default|GetRepeatingSpawnTimer))
    (if (Variables|Default|GetbCanReset)
      (Utilities|FlowControl|Delay (Variables|Default|GetResetTimer))
      (Utilities|FlowControl|DoOnce false) ; enters at Reset
    )))

(event EventBeginPlay
  (bind _returnvalue (Actor|GetActorOfClass "/Game/DustDevil/Characters/EnemyAI/BP_MotherBrain.BP_MotherBrain_C"))
  (Variables|References|SetMotherBrain _returnvalue))

(fn ConstructionScript)

(fn CheckforTutorialTrigger
  (if (Variables|Tutorial|GetbInTutorial)
    (bind _tutorialmanager (Variables|Tutorial|GetTutorialManager)
      (:then
        (if (Variables|/Game/DustDevil/Tutorials/BP_TutorialManager.BP_TutorialManager_C|GetbCombatTriggered _tutorialmanager)
          (Development|PrintString "Combat tut already shown")
          (else
            (Default|TutorialAdded (Variables|Tutorial|GetTutorialManager) "NewEnumerator2" false)
            (Variables|/Game/DustDevil/Tutorials/BP_TutorialManager.BP_TutorialManager_C|SetbCombatTriggered (Variables|Tutorial|GetTutorialManager) true))))
      (:else
        (return)))
    (else
      (return))))

(fn SpawnEnemy
  (bind _randomlocation (Class|NavigationSystemV1|GetRandomLocationinNavigableRadius (Transformation|GetWorldLocation (Variables|Default|GetSpawnArea)) 4e+03 0 0))
  (bind _output_get (Variables|Default|SetRandomSizeValue (Math|Random|RandomFloatinRange 1.0 3.0)))
  (Game|SpawnActorfromClass "/Game/DustDevil/Characters/EnemyAI/BP_BugBase.BP_BugBase_C" (Math|Transform|MakeTransform _randomlocation "0, 0, 0" (Math|Vector|MakeVector _output_get _output_get _output_get)) "AdjustIfPossibleButAlwaysSpawn" "MultiplyWithRoot" 0 (Variables|EnemyProperties|GetMaxAttackCooldown) (Variables|EnemyProperties|GetDetectionRadius) (Variables|EnemyProperties|GetMaxHealth) (Variables|EnemyProperties|GetAttackDamage) (Variables|EnemyProperties|GetBiomatterDropped) 0 (Variables|EnemyProperties|GetNuclearMatDropChance) (Variables|EnemyProperties|GetEnemySpeed) 0.1 0)
  (bind _result (Math|Integer|IncrementInt (Variables|EnemyProperties|GetCurrentSpawnCount))
    (:%20%20
      (if (== _result (Variables|EnemyProperties|GetTotalSpawnCount))
        (Utilities|Time|ClearandInvalidateTimerbyHandle (Variables|Default|GetRepeatingSpawnTimer))))))