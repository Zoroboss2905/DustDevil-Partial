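; Enemy spawner that creates irradiated BP_BugBase variants with nuclear material drops at random navigable points.
; In the tutorial it spawns on BeginPlay, then polls its bug array until empty to have the tutorial manager destroy a blockage.
; Otherwise a player overlap fires a DoOnce wave gated by MotherBrain's enemy-cap check, plus one ungated bug, with optional delayed re-arming.
; EndPlay destroys its RadZone; the objective-marker logic is disconnected.
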(event OnComponentBeginOverlap(Trigger)
  (params (OverlappedComponent :type Primitive%20Component%20Object%20Reference) (OtherActor :type Actor%20Object%20Reference) (OtherComp :type Primitive%20Component%20Object%20Reference) (OtherBodyIndex :type Integer) (bFromSweep :type Boolean) (SweepResult :type Hit%20Result%20Structure%20%28by%20ref%29))
  (bind _health (Variables|Default|GetHealth))
  (if (Utilities|DoesObjectImplementInterface OtherActor "/Game/DustDevil/Core/Interfaces/BPI_PlayerTrigger.BPI_PlayerTrigger_C")
    (Utilities|FlowControl|DoOnce false
      (:Completed
        (if (not (Variables|Default|GetbInTutorial))
          (for _index (range 0 (Variables|Default|GetNumberToSpawn))
            (if (Default|CheckifEnemyCapReached (Variables|Default|GetMotherBrain))
              (bind _randomlocation (Class|NavigationSystemV1|GetRandomLocationinNavigableRadius (Transformation|GetWorldLocation (Variables|Default|GetSpawnArea)) (Variables|Default|GetSpawnRadius) 0 0))
              (bind _returnvalue (Game|SpawnActorfromClass "/Game/DustDevil/Characters/EnemyAI/BP_BugBase.BP_BugBase_C" (Math|Transform|MakeTransform _randomlocation (.rotation (Transformation|GetActorTransform)) "2.000000,2.000000,2.000000") "AdjustIfPossibleButAlwaysSpawn" "MultiplyWithRoot" 0 1.0 5e+03 1.0 1e+02 5 0 0.1 6e+02 0.1 0))
              (Variables|Default|SetBugBase _returnvalue)
              (Variables|/Game/DustDevil/Characters/EnemyAI/BP_BugBase.BP_BugBase_C|SetMaterialValue _returnvalue 2)
              (Default|SetDefaultStats _returnvalue _health _health 0.0 (Variables|Default|GetAttack%20Damage) 0.0 1.0 (Variables|Default|GetMovementSpeed))
              (Rendering|Material|SetMaterial (Variables|/Script/Engine.Character|GetMesh _returnvalue) 0 "/Game/DustDevil/Art/Materials/Enemies/M_Enemy1_V3.M_Enemy1_V3")))
          (CallFunction|SetBugBase))))))

(event OnComponentEndOverlap(Trigger)
  (params (OverlappedComponent :type Primitive%20Component%20Object%20Reference) (OtherActor :type Actor%20Object%20Reference) (OtherComp :type Primitive%20Component%20Object%20Reference) (OtherBodyIndex :type Integer))
  (bind _health (Variables|Default|GetHealth))
  (if (Utilities|DoesObjectImplementInterface OtherActor 0)
    (if (Variables|Default|GetbCanRepeatSpawn)
      (Utilities|FlowControl|Delay 5.0)
      (Utilities|FlowControl|Sequence
        (:then_0
          (goto _label Reset))
        (:then_1
          (Utilities|FlowControl|DoOnce false :!label _label
            (:Completed
              (if (not (Variables|Default|GetbInTutorial))
                (for _index (range 0 (Variables|Default|GetNumberToSpawn))
                  (if (Default|CheckifEnemyCapReached (Variables|Default|GetMotherBrain))
                    (bind _randomlocation (Class|NavigationSystemV1|GetRandomLocationinNavigableRadius (Transformation|GetWorldLocation (Variables|Default|GetSpawnArea)) (Variables|Default|GetSpawnRadius) 0 0))
                    (bind _returnvalue (Game|SpawnActorfromClass "/Game/DustDevil/Characters/EnemyAI/BP_BugBase.BP_BugBase_C" (Math|Transform|MakeTransform _randomlocation (.rotation (Transformation|GetActorTransform)) "2.000000,2.000000,2.000000") "AdjustIfPossibleButAlwaysSpawn" "MultiplyWithRoot" 0 1.0 5e+03 1.0 1e+02 5 0 0.1 6e+02 0.1 0))
                    (Variables|Default|SetBugBase _returnvalue)
                    (Variables|/Game/DustDevil/Characters/EnemyAI/BP_BugBase.BP_BugBase_C|SetMaterialValue _returnvalue 2)
                    (Default|SetDefaultStats _returnvalue _health _health 0.0 (Variables|Default|GetAttack%20Damage) 0.0 1.0 (Variables|Default|GetMovementSpeed))
                    (Rendering|Material|SetMaterial (Variables|/Script/Engine.Character|GetMesh _returnvalue) 0 "/Game/DustDevil/Art/Materials/Enemies/M_Enemy1_V3.M_Enemy1_V3")))
                (CallFunction|SetBugBase)))))))))

(event Custom|RemoveArray
  (Utilities|Array|RemoveIndex (Variables|Default|GetBugBaseArray) (Variables|Default|GetArrayNumber))
  (Variables|Default|SetArrayNumber (- (Variables|Default|GetArrayNumber) 1)))

(event Custom|CheckIfAlive
  ;[1 1 1] objective
  (if (Utilities|IsValid (Variables|Default|GetBugBase))
    (Utilities|FlowControl|RetriggerableDelay 0.01)
    (CallFunction|CheckifAlive)
    (else
      (Actor|DestroyActor (Variables|Default|GetObjectiveActor)))))

(event Custom|DestroyBlockage
  (if (== (Utilities|Array|Length (Variables|Default|GetBugBaseArray)) 0) :!label _label
    (Default|DestroyBlockageThree (Variables|Default|GetTutorialManagerTwo))
    (else
      (Utilities|FlowControl|Delay 0.2)
      (goto _label))))

(event Custom|SetBugBase
  (bind _returnvalue (Transformation|GetActorTransform))
  (bind _randomlocation (Class|NavigationSystemV1|GetRandomLocationinNavigableRadius (.location _returnvalue) 2e+02 0 0))
  (bind _returnvalue_2 (Game|SpawnActorfromClass "/Game/DustDevil/Characters/EnemyAI/BP_BugBase.BP_BugBase_C" (Math|Transform|MakeTransform _randomlocation (.rotation _returnvalue) "2.000000,2.000000,2.000000") "AdjustIfPossibleButAlwaysSpawn" "MultiplyWithRoot" 0 1.0 2e+04 25.0 3.0 0 0 1.0 2e+03 0.1 0))
  (Variables|Default|SetBugBase _returnvalue_2)
  (Variables|/Game/DustDevil/Characters/EnemyAI/BP_BugBase.BP_BugBase_C|SetMaterialValue _returnvalue_2 2)
  (Rendering|Material|SetMaterial (Variables|/Script/Engine.Character|GetMesh _returnvalue_2) 0 "/Game/DustDevil/Art/Materials/Enemies/M_Enemy1_V3.M_Enemy1_V3"))

(event EventEndPlay
  (params (EndPlayReason :type EEndPlayReason%20Enum :default "Destroyed"))
  (bind _radzone (Variables|Default|GetRadZone)
    (:then
      (Actor|DestroyActor _radzone))
    (:else)))

(event Collision|EventActorBeginOverlap
  (params (OtherActor :type Actor%20Object%20Reference))
  (|CallParentFunction OtherActor) ; This node is disabled and will not be called.\nDrag off pins to build functionality.
)

(event EventTick
  (params (DeltaSeconds :type Float%20%28single-precision%29))
  (|CallParentFunction DeltaSeconds))

(event EventBeginPlay
  (bind _health (Variables|Default|GetHealth))
  (Utilities|FlowControl|Sequence
    (:then_0
      (if (Variables|Default|GetbInTutorial)
        (for _index (range 1 (Variables|Default|GetNumberToSpawn))
          (bind _randomlocation (Class|NavigationSystemV1|GetRandomLocationinNavigableRadius (Transformation|GetWorldLocation (Variables|Default|GetSpawnArea)) (Variables|Default|GetSpawnRadius) 0 0))
          (if (Variables|Default|GetbInTutorial)
            (bind _returnvalue (Game|SpawnActorfromClass "/Game/DustDevil/Characters/EnemyAI/BP_BugBase.BP_BugBase_C" (Math|Transform|MakeTransform _randomlocation (.rotation (Transformation|GetActorTransform)) "2.000000,2.000000,2.000000") "AdjustIfPossibleButAlwaysSpawn" "MultiplyWithRoot" 0 1.0 2e+04 1.0 3.0 0 0 1.0 2e+03 0.1 0))
            (bind _returnvalue_2 (Utilities|Array|Add (Variables|Default|GetBugBaseArray) _returnvalue))
            (Variables|Default|SetArrayNumber _returnvalue_2)
            (Variables|/Game/DustDevil/Characters/EnemyAI/BP_BugBase.BP_BugBase_C|SetMaterialValue _returnvalue 2)
            (Default|SetDefaultStats _returnvalue _health _health 0.0 (Variables|Default|GetAttack%20Damage) 0.0 1.0 (Variables|Default|GetMovementSpeed))
            (Rendering|Material|SetMaterial (Variables|/Script/Engine.Character|GetMesh _returnvalue) 0 "/Game/DustDevil/Art/Materials/Enemies/M_Enemy1_V3.M_Enemy1_V3")))
        (CallFunction|DestroyBlockage)))
    (:then_1
      (bind _returnvalue_3 (Actor|GetActorOfClass "/Game/DustDevil/Tutorials/BP_TutorialManagerTwo.BP_TutorialManagerTwo_C"))
      (Utilities|IsValid _returnvalue_3
        (:Is%20Valid
          (Variables|Default|SetTutorialManagerTwo _returnvalue_3))))
    (:then_2
      (bind _returnvalue_4 (Actor|GetActorOfClass "/Game/DustDevil/Characters/EnemyAI/BP_MotherBrain.BP_MotherBrain_C"))
      (Variables|Default|SetMotherBrain _returnvalue_4))))

(fn ConstructionScript
  (|CallParentFunction))