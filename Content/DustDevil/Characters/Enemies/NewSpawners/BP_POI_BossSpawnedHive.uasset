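; Boss-spawned hive POI that spawns enemy attack groups through BP_EnemyManager.
; On BeginPlay it applies low-health, zero-damage stats via a GAS set-by-caller effect, takes a random yaw and starts a looping spawn timer.
; Each tick creates a group at the hive while fewer than five are tracked.
; Only one of three random preset options is wired (three Grubs); the Grub/Swarmer mixes are unconnected.
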(event EventBeginPlay
  (|CallParentFunction)
  (CallFunction|SetHiveStats)
  (Transformation|SetActorRotation (Math|Rotator|MakeRotator 0.0 0.0 (Math|Random|RandomFloatinRange -1.8e+02 1.8e+02)) true)
  (bind _returnvalue (Actor|GetActorOfClass "/Game/DustDevil/Characters/Enemies/BP_EnemyManager.BP_EnemyManager_C"))
  (Variables|Default|SetEnemyManager _returnvalue)
  (Utilities|Time|SetTimerbyFunctionName 0 "SpawnEnemySet" 3.0 true true 2.0 1.0))

(fn ConstructionScript
  (|CallParentFunction))

(fn SpawnEnemySet
  (bind _enemymanager (Variables|Default|GetEnemyManager))
  (bind _returnvalue (Class|EnemyManager|GetEnemyPresetbyName _enemymanager "Grub"))
  (if (< (Utilities|Array|Length (Variables|Default|GetSpawnedAttackGroups)) 5)
    (bind _newattackgroup (Class|EnemyManager|CreateAttackGroup (Variables|Default|GetEnemyManager) 0 (Transformation|GetActorLocation) (Utilities|Select :Index (Math|Random|RandomIntegerinRange 0 2) :Option%200 (Utilities|Array|MakeArray _returnvalue _returnvalue _returnvalue) :Option%201 0 :Option%202 0) "/Game/DustDevil/Characters/Enemies/CustomAttackGroups/BP_AttackGroup.BP_AttackGroup_C"))
    (Utilities|Array|Add (Variables|Default|GetSpawnedAttackGroups) _newattackgroup)))

(fn SetHiveStats
  (bind _abilitysystem (Variables|Default|GetAbilitySystem))
  (bind _returnvalue (Ability|GameplayEffect|AssignTagSetbyCallerMagnitude (GameplayEffects|MakeOutgoingSpec _abilitysystem "/Game/DustDevil/Core/GAS/Effects/GE_DefaultEnemyValues.GE_DefaultEnemyValues_C" 0.0 (GameplayEffects|MakeEffectContext _abilitysystem)) "(TagName=\"Stats.Base.Armour\")" 0.0))
  (bind _returnvalue_2 (Ability|GameplayEffect|AssignTagSetbyCallerMagnitude _returnvalue "(TagName=\"Stats.Base.BioMatter\")" 1.0))
  (bind _returnvalue_3 (Ability|GameplayEffect|AssignTagSetbyCallerMagnitude _returnvalue_2 "(TagName=\"Stats.Base.ChitinChance\")" 0.0))
  (bind _returnvalue_4 (Ability|GameplayEffect|AssignTagSetbyCallerMagnitude _returnvalue_3 "(TagName=\"Stats.Base.MaxHealth\")" 4e+01))
  (bind _returnvalue_5 (Ability|GameplayEffect|AssignTagSetbyCallerMagnitude _returnvalue_4 "(TagName=\"Stats.Base.CurrentHealth\")" 4e+01))
  (bind _returnvalue_6 (Ability|GameplayEffect|AssignTagSetbyCallerMagnitude _returnvalue_5 "(TagName=\"Stats.Base.Damage\")" 0.0))
  (bind _returnvalue_7 (Ability|GameplayEffect|AssignTagSetbyCallerMagnitude _returnvalue_6 "(TagName=\"Stats.Base.NuclearMatter\")" 1.0))
  (GameplayEffects|ApplyGameplayEffectSpecToSelf (Variables|Default|GetAbilitySystem) _returnvalue_7))