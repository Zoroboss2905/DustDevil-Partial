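; Point-of-interest spawner that creates a small enemy attack group at its own location.
; On BeginPlay it finds the BP_EnemyManager and asks it to create a BP_AttackGroup from one of three randomly selected compositions.
; The hard-coded compositions mix Swarmer, Grub and BigGrub presets, looked up by name on the manager.
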(event EventBeginPlay
  (bind _returnvalue (Actor|GetActorOfClass "/Game/DustDevil/Characters/Enemies/BP_EnemyManager.BP_EnemyManager_C"))
  (bind _output_get (Variables|Default|SetEnemyManager _returnvalue))
  (Class|EnemyManager|CreateAttackGroup _output_get 0 (Transformation|GetActorLocation) (Utilities|Select :Index (Math|Random|RandomIntegerinRange 0 2) :Option%200 (Utilities|Array|MakeArray (Class|EnemyManager|GetEnemyPresetbyName (Variables|Default|GetEnemyManager) "Swarmer") (Class|EnemyManager|GetEnemyPresetbyName (Variables|Default|GetEnemyManager) "Grub") (Class|EnemyManager|GetEnemyPresetbyName (Variables|Default|GetEnemyManager) "Swarmer") (Class|EnemyManager|GetEnemyPresetbyName (Variables|Default|GetEnemyManager) "Swarmer") (Class|EnemyManager|GetEnemyPresetbyName (Variables|Default|GetEnemyManager) "Swarmer") (Class|EnemyManager|GetEnemyPresetbyName (Variables|Default|GetEnemyManager) "Swarmer")) :Option%201 (Utilities|Array|MakeArray (Class|EnemyManager|GetEnemyPresetbyName (Variables|Default|GetEnemyManager) "Grub") (Class|EnemyManager|GetEnemyPresetbyName (Variables|Default|GetEnemyManager) "Grub") (Class|EnemyManager|GetEnemyPresetbyName (Variables|Default|GetEnemyManager) "Grub") (Class|EnemyManager|GetEnemyPresetbyName (Variables|Default|GetEnemyManager) "Grub")) :Option%202 (Utilities|Array|MakeArray (Class|EnemyManager|GetEnemyPresetbyName (Variables|Default|GetEnemyManager) "Grub") (Class|EnemyManager|GetEnemyPresetbyName (Variables|Default|GetEnemyManager) "Grub") (Class|EnemyManager|GetEnemyPresetbyName (Variables|Default|GetEnemyManager) "BigGrub"))) "/Game/DustDevil/Characters/Enemies/CustomAttackGroups/BP_AttackGroup.BP_AttackGroup_C"))

(fn ConstructionScript
  (|CallParentFunction))