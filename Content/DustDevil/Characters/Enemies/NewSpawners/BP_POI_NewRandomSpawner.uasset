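; BP_POI_NewRandomSpawner is an enemy spawner that registers an attack group at its own location when play begins.
; On BeginPlay it finds and stores the level's BP_EnemyManager, then asks it to create a BP_AttackGroup there.
; Despite the name, the graph contains no randomization: several Grub, BigGrub and Swarmer preset lists are left unconnected.
; The construction script only calls its parent.
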(event EventBeginPlay
  (bind _returnvalue (Actor|GetActorOfClass "/Game/DustDevil/Characters/Enemies/BP_EnemyManager.BP_EnemyManager_C"))
  (bind _output_get (Variables|Default|SetEnemyManager _returnvalue))
  (Class|EnemyManager|CreateAttackGroup _output_get 0 (Transformation|GetActorLocation) 0 "/Game/DustDevil/Characters/Enemies/CustomAttackGroups/BP_AttackGroup.BP_AttackGroup_C"))

(fn ConstructionScript
  (|CallParentFunction))