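; BP_Glob is a boss projectile that leaves acid where it lands.
; On BeginPlay it tilts its mesh, copies StartingVelocity into the projectile movement's initial speed and plays a squish sound.
; On a projectile bounce it spawns a double-scale BP_Acid at its location with random yaw, then destroys itself.
; The SpawnHive check on bounce has empty branches, so no hive is spawned.
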(event OnProjectileBounce(ProjectileMovement)
  (params (ImpactResult :type Hit%20Result%20Structure%20%28by%20ref%29) (ImpactVelocity :type Vector%20%28by%20ref%29 :default "0, 0, 0"))
  (bind _returnvalue (Transformation|GetActorTransform))
  (if (Variables|Default|GetbSpawnHive)
    _
    (else
      _))
  (Game|SpawnActorfromClass "/Game/DustDevil/Characters/Enemies/BossProjectiles/BP_Acid.BP_Acid_C" (Math|Transform|MakeTransform (.location _returnvalue) (Math|Rotator|MakeRotator 0.0 0.0 (Math|Random|RandomFloatinRange -1.8e+02 1.8e+02)) (* (.scale _returnvalue) 2.0)) "AlwaysSpawn" "MultiplyWithRoot" 0 4.0 (Variables|Actor|GetInstigator))
  (Actor|DestroyActor))

(event EventBeginPlay
  (Transformation|AddRelativeRotation (Variables|Default|GetStaticMesh) "40.000000,0.000000,0.000000" false false)
  (Variables|/Script/Engine.ProjectileMovementComponent|SetInitialSpeed (Variables|Default|GetProjectileMovement) (Variables|Default|GetStartingVelocity))
  (Audio|PlaySoundatLocation "/Game/DustDevil/Audio/Feedback/EnemyThree/slime-squish-12-219047.slime-squish-12-219047" (Transformation|GetActorLocation) "0, 0, 0" 1.0 1.0 0.0 0 0 0 0))

(event Collision|EventActorBeginOverlap
  (params (OtherActor :type Actor%20Object%20Reference)))

(event EventTick
  (params (DeltaSeconds :type Float%20%28single-precision%29)))

(fn ConstructionScript)