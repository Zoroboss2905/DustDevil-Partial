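; BP_Acid is a timed acid hazard among the boss projectiles that plays an impact sound on spawn and damages the player while they overlap it.
; A looping timer scans the Sphere's overlapping components for the player pawn's components on a custom collision channel.
; Each hit applies GE_Damage through GAS from the instigator's ability system component to the player's.
; Tick counts Duration down and destroys the actor when it runs out.
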(event Custom|DamageTick
  (bind _returnvalue (Game|Player|GetPlayerPawn 0))
  (for _array_element (Class|PrimitiveComponent|GetOverlappingComponents (Variables|Default|GetSphere))
    (if (and (Utilities|Enum|Equal(Enum) (Collision|GetCollisionObjectType _array_element) "ECC_GameTraceChannel2") (== (Components|GetOwner _array_element) _returnvalue))
      (GameplayEffects|ApplyGameplayEffectToTarget :self (Ability|GetAbilitySystemComponent (Game|GetInstigator)) :GameplayEffectClass "/Game/DustDevil/Core/GAS/Effects/GE_Damage.GE_Damage_C" :Target (Ability|GetAbilitySystemComponent _returnvalue)))))

(event EventBeginPlay
  (Utilities|Time|SetTimerbyEvent (delegate Custom|DamageTick) 0.8 true false 0.5)
  (Audio|PlaySoundatLocation "/Game/DustDevil/Audio/Feedback/EnemyThree/slime-impact-352473.slime-impact-352473" (Transformation|GetActorLocation) "0, 0, 0" 4.0 1.0 0.0 0 0 0 0))

(event EventTick
  (params (DeltaSeconds :type Float%20%28single-precision%29))
  (bind _output_get (Variables|Default|SetDuration (- (Variables|Default|GetDuration) DeltaSeconds)))
  (if (< _output_get 0.0)
    (Actor|DestroyActor)))

(fn ConstructionScript)