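; Vehicle game mode that tracks the player's ability level and spendable ability points.
; On BeginPlay it finds BP_Vehicle and, only in L_WastelandEscape_WP, restores level, points and gained abilities from GI_DDPrototype, re-activating each ability.
; Restored Furious and Grit Incarnate abilities also update the HUD buff bar.
; Level-ups grant a point and notify the HUD, spending decrements a clamped count, and ThresholdCurve supplies level thresholds.
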(event EventBeginPlay
  (bind _returnvalue (Actor|GetActorOfClass "/Game/DustDevil/Player/BP_Vehicle.BP_Vehicle_C"))
  (Variables|References|SetPlayer _returnvalue)
  (bind _returnvalue_2 (Game|GetCurrentLevelName true))
  (if (Utilities|Enum|Equal(Enum) _returnvalue_2 " L_WastelandEscape_WP")
    (bind _asgi_ddprototype (Utilities|Casting|CastToGI_DDPrototype (Game|GetGameInstance)))
    (bind _output_get (Variables|References|SetGameInstance _asgi_ddprototype))
    (bind _keys (Utilities|Map|Keys (Variables|/Game/DustDevil/Core/GI_DDPrototype.GI_DDPrototype_C|GetAbilitiesGained _output_get)))
    (bind _values (Utilities|Map|Values (Variables|/Game/DustDevil/Core/GI_DDPrototype.GI_DDPrototype_C|GetAbilitiesGained _output_get)))
    (for (_array_element _array_index) _keys
      (Default|ActivateGameplayAbility (Variables|References|GetPlayer) _array_element (Utilities|Array|Get(acopy) _values _array_index))
      (CallFunction|AddAbilityBuffs _array_element))
    (Variables|Abilities|SetAbilityLevel (Variables|/Game/DustDevil/Core/GI_DDPrototype.GI_DDPrototype_C|GetAbilityLevel (Variables|References|GetGameInstance)))
    (Variables|Abilities|SetAvailablePoints (Variables|/Game/DustDevil/Core/GI_DDPrototype.GI_DDPrototype_C|GetAbilityPoints (Variables|References|GetGameInstance)))))

(fn ConstructionScript)

(fn IncreaseAbilityLevel
  (Math|Integer|IncrementInt (Variables|Abilities|GetAbilityLevel)
    (:%20%20
      (Math|Integer|IncrementInt (Variables|Abilities|GetAvailablePoints)
        (:%20%20
          (Default|PlayerLevelsUp (Variables|/Game/DustDevil/Player/BP_Vehicle.BP_Vehicle_C|GetHUD (Variables|References|GetPlayer))))))))

(fn GetAbilityData
  (bind _abilitylevel (Variables|Abilities|GetAbilityLevel))
  (return _abilitylevel (Math|Float|Truncate (Math|Curves|GetFloatValue (Variables|Abilities|GetThresholdCurve) (Math|Conversions|ToFloat(Integer) _abilitylevel))) (Math|Float|Truncate (Math|Curves|GetFloatValue (Variables|Abilities|GetThresholdCurve) (Math|Conversions|ToFloat(Integer) (+ _abilitylevel 1)))) (Variables|Abilities|GetAvailablePoints)))

(fn AbilityPointSpent
  (bind _output_get (Variables|Abilities|SetAvailablePoints (Math|Integer|Clamp(Integer) (- (Variables|Abilities|GetAvailablePoints) 1) 0 40)))
  (Development|PrintString (Utilities|String|Append "Player has " (Utilities|String|ToString(Integer) _output_get) " ability points!")))

(fn AddAbilityBuffs
  (params (Ability :type Object%20Class%20Reference))
  (Utilities|FlowControl|Sequence
    (:then_0
      (if (== Ability "/Game/DustDevil/Core/GAS/Abilities/GA_Furious.GA_Furious_C")
        (Class|BPIHUDUpdates|UpdateAbilityBuffsBar(Message) (Variables|/Game/DustDevil/Player/BP_Vehicle.BP_Vehicle_C|GetHUD (Variables|References|GetPlayer)) "NewEnumerator0")))
    (:then_1
      (if (== Ability "/Game/DustDevil/Core/GAS/Abilities/GA_GritIncarnate.GA_GritIncarnate_C")
        (Class|BPIHUDUpdates|UpdateAbilityBuffsBar(Message) (Variables|/Game/DustDevil/Player/BP_Vehicle.BP_Vehicle_C|GetHUD (Variables|References|GetPlayer)) "NewEnumerator2")))))