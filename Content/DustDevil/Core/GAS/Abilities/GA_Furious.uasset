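; GA_Furious is the Gameplay Ability behind the Furious offense upgrade, building Fury on hit events and clearing it on miss events.
; On activation it starts two gameplay event listeners and caches the vehicle controller's HUD.
; A hit applies one GE_Fury stack and fires a gameplay cue, while a miss removes Furious-tagged effects.
; Both refresh the HUD buff bar, and ending the ability ends both listeners.
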(event Ability|EventActivateAbility
  (bind _asynctaskproxy (Ability|Tasks|WaitGameplayEvent "(TagName=\"Upgrades.Offense.Furious.Hit\")" 0)
    (:then
      (Variables|Default|SetFuryHit _asynctaskproxy)
      (bind _asynctaskproxy_2 (Ability|Tasks|WaitGameplayEvent "(TagName=\"Upgrades.Offense.Furious.Miss\")" 0)
        (:then
          (Variables|Default|SetFuryMiss _asynctaskproxy_2)
          (bind _aspc_vehicle_controller (Utilities|Casting|CastToPC_VehicleController (Game|GetPlayerController 0)))
          (Variables|Default|SetHUD (Variables|/Game/DustDevil/Player/PC_VehicleController.PC_VehicleController_C|GetHUD _aspc_vehicle_controller))
          (bind _hud (Variables|Default|GetHUD)
            (:then
              (Class|BPIHUDUpdates|UpdateAbilityBuffsBar(Message) _hud "NewEnumerator0"))
            (:else)))
        (:EventReceived
          (Utilities|FlowControl|Sequence
            (:then_0
              (GameplayEffects|RemoveActiveEffectswithTags (Ability|GetAbilitySystemComponentfromActorInfo) "(GameplayTags=((TagName=\"Upgrades.Offense.Furious\")))"))
            (:then_1
              (bind _hud_2 (Variables|Default|GetHUD :!label _label)
                (:then
                  (Class|BPIHUDUpdates|UpdateAbilityBuffsBar(Message) _hud_2 "NewEnumerator0"))
                (:else
                  (Development|PrintString "GA_Furious - HUD ref not valid!" true true "(R=1.000000,G=0.000000,B=0.031996,A=1.000000)"))))))))
    (:EventReceived
      (Ability|ApplyGameplayEffectToOwner "/Game/DustDevil/Core/GAS/TempUpgrades/GE_Fury.GE_Fury_C" (Ability|GetAbilityLevel))
      (GameplayCue|ExecuteGameplayCue :GameplayCueTag "(TagName=\"GameplayCue.Ability.Furious.Added\")")
      (goto _label))))

(event Ability|EventOnEndAbility
  (params (bWasCancelled :type Boolean))
  (GameplayTasks|EndTask (Variables|Default|GetFuryHit))
  (GameplayTasks|EndTask (Variables|Default|GetFuryMiss)))