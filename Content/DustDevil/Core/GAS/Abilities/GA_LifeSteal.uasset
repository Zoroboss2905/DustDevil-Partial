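; Life steal upgrade ability that heals its owner when an enemy death event reaches the avatar.
; Activation applies GE_LifeSteal at the ability level, then listens for Event.Enemy.Death.
; Each event applies GE_LifeStealInst with a SetByCaller health magnitude, an instigator attribute scaled by an avatar percentage attribute, and triggers BP_Vehicle pickup feedback.
; Ending the ability removes effects tagged Upgrades.Defence.LifeSteal.
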(event Ability|EventActivateAbility
  (GameplayEffects|ApplyGameplayEffectToSelf :self (Ability|GetAbilitySystemComponentfromActorInfo) :GameplayEffectClass "/Game/DustDevil/Core/GAS/TempUpgrades/GE_LifeSteal.GE_LifeSteal_C" :Level (Math|Conversions|ToFloat(Integer) (Ability|GetAbilityLevel)))
  (bind (_asynctaskproxy _payload) (Ability|Async|WaitGameplayEventToActor (Ability|GetAvatarActorfromActorInfo) "(TagName=\"Event.Enemy.Death\")")
    (:then
      (Variables|Default|SetAA_EnemyDeath _asynctaskproxy))
    (:EventReceived
      (bind _returnvalue (Ability|GameplayEffect|AssignTagSetbyCallerMagnitude (GameplayEffects|MakeOutgoingSpec :self (Ability|GetAbilitySystemComponentfromActorInfo) :GameplayEffectClass "/Game/DustDevil/Core/GAS/Effects/GE_LifeStealInst.GE_LifeStealInst_C") "(TagName=\"Stats.Base.CurrentHealth\")" (* (.ReturnValue (Ability|Attribute|GetFloatAttribute (.Instigator (Utilities|Struct|BreakGameplayEventData _payload)) "(AttributeName=\"MaxHealth\",Attribute=/Script/DustDevil.BaseAttributeSet:MaxHealth,AttributeOwner=\"/Script/CoreUObject.Class'/Script/DustDevil.BaseAttributeSet'\")")) (/ (.ReturnValue (Ability|Attribute|GetFloatAttribute (Ability|GetAvatarActorfromActorInfo) "(AttributeName=\"LifeSteal\",Attribute=/Script/DustDevil.VehicleAttributeSet:LifeSteal,AttributeOwner=\"/Script/CoreUObject.Class'/Script/DustDevil.VehicleAttributeSet'\")")) 1e+02))))
      (Ability|ApplyGameplayEffectSpecToOwner _returnvalue)
      (bind _asbp_vehicle (Utilities|Casting|CastToBP_Vehicle (Ability|GetAvatarActorfromActorInfo)))
      (Default|HealthPickUpFeedback _asbp_vehicle))))

(event Ability|EventOnEndAbility
  (params (bWasCancelled :type Boolean))
  (GameplayEffects|RemoveActiveEffectswithTags (Ability|GetAbilitySystemComponentfromActorInfo) "(GameplayTags=((TagName=\"Upgrades.Defence.LifeSteal\")))"))