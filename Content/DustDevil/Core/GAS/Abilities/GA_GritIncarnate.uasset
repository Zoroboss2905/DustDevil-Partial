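; GA_GritIncarnate is a gameplay ability that grants Grit defence stacks as the avatar loses health.
; An attribute-change listener divides the new value by the base value to get a health fraction.
; Each change removes effects tagged GritDefence, then applies GE_GritStack at ability level, one stack per whole percent of missing health.
; The HUD buff bar updates on activation and reapplication, and ending the ability cancels the listener.
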(event Custom|ReApply%20Stacks
  (params (HealthPercent :type Float%20%28double-precision%29))
  (GameplayEffects|RemoveActiveEffectswithTags (Ability|GetAbilitySystemComponentfromActorInfo) "(GameplayTags=((TagName=\"Upgrades.Defence.GritDefence\")))")
  (Ability|ApplyGameplayEffectToOwner "/Game/DustDevil/Core/GAS/TempUpgrades/GE_GritStack.GE_GritStack_C" (Ability|GetAbilityLevel) (Math|Float|Floor (* (- 1.0 HealthPercent) 1e+02)))
  (bind _hud (Variables|Default|GetHUD)
    (:then
      (Class|BPIHUDUpdates|UpdateAbilityBuffsBar(Message) _hud "NewEnumerator2"))
    (:else)))

(event Ability|EventActivateAbility
  (bind _returnvalue (Ability|GetAvatarActorfromActorInfo))
  (bind (_asynctaskproxy _attribute _newvalue) (Ability|Tasks|WaitForAttributeChanged _returnvalue "(AttributeName=\"CurrentHealth\",Attribute=/Script/DustDevil.BaseAttributeSet:CurrentHealth,AttributeOwner=\"/Script/CoreUObject.Class'/Script/DustDevil.BaseAttributeSet'\")")
    (:then
      (Variables|Default|SetAA_Health _asynctaskproxy)
      (bind _aspc_vehicle_controller (Utilities|Casting|CastToPC_VehicleController (Game|GetPlayerController 0)))
      (Variables|Default|SetHUD (Variables|/Game/DustDevil/Player/PC_VehicleController.PC_VehicleController_C|GetHUD _aspc_vehicle_controller))
      (bind _hud (Variables|Default|GetHUD)
        (:then
          (Class|BPIHUDUpdates|UpdateAbilityBuffsBar(Message) _hud "NewEnumerator2"))
        (:else)))
    (:Changed
      (CallFunction|ReApplyStacks (/ _newvalue (Math|Float|Max(Float) (.ReturnValue (Class|AbilitySystemBlueprintLibrary|GetFloatAttributeBasefromAbilitySystemComponent (Ability|GetAbilitySystemComponent _returnvalue) "(AttributeName=\"MaxHealth\",Attribute=/Script/DustDevil.BaseAttributeSet:MaxHealth,AttributeOwner=\"/Script/CoreUObject.Class'/Script/DustDevil.BaseAttributeSet'\")")) 0.01))))))

(event Ability|EventOnEndAbility
  (params (bWasCancelled :type Boolean))
  (AsyncAction|Cancel (Variables|Default|GetAA_Health)))