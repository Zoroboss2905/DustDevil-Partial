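; Engine Nova is an event-triggered gameplay ability that releases a fire shockwave around the instigator, with a ripple effect and impact sound.
; A sphere trace finds shootable actors in range and skips those tagged as damage immune.
; Each hit receives a damage effect plus a fire effect whose duration is set by caller magnitude.
; Ability level scales the wave's visual size, trace radius and burn duration.
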(event Ability|EventActivateAbilityFromEvent
  (params (EventData :type Gameplay%20Event%20Data%20Structure%20%28by%20ref%29))
  (bind _instigator (Utilities|Struct|BreakGameplayEventData EventData))
  (bind _returnvalue (Ability|GetAbilityLevel))
  (bind _returnvalue_2 (Transformation|GetActorLocation _instigator))
  (bind _returnvalue_3 (Ability|GetAbilitySystemComponent _instigator))
  (bind _returnvalue_4 (Utilities|Select :Index _returnvalue :Option%200 1.5e+03 :Option%201 1.5e+03 :Option%202 2e+03 :Option%203 3e+03))
  (Utilities|IsValid _instigator
    (:Is%20Valid
      (bind _returnvalue_5 (Niagara|SpawnSystemAttached "/Game/DustDevil/Effects/Soundwave/NS_FireRipple.NS_FireRipple" (Variables|/Script/Engine.Actor|GetRootComponent _instigator) "None" "0, 0, 0" "0, 0, 0" "KeepRelativeOffset" true))
      (Audio|PlaySound2D "/Game/DustDevil/Audio/Feedback/UpgradesAbilities/fire-spell-impact-393921.fire-spell-impact-393921" 1.0 1.0 0.0 0 0)
      (Effects|Components|ParticleSystem|SetFloatParameter _returnvalue_5 "WaveSize" _returnvalue_4)
      (bind _outhits (Collision|MultiSphereTraceForObjects _returnvalue_2 _returnvalue_2 _returnvalue_4 (Utilities|Array|MakeArray "ObjectTypeQuery8") false (Utilities|Array|MakeArray _instigator) "None" true "(R=1.000000,G=0.000000,B=0.000000,A=1.000000)" "(R=0.000000,G=1.000000,B=0.000000,A=1.000000)" 2.0))
      (for _array_element _outhits
        (if (and (Utilities|DoesObjectImplementInterface (.HitActor (Collision|BreakHitResult _array_element)) "/Game/DustDevil/Core/Interfaces/BPI_Shootable.BPI_Shootable_C") (not (GameplayTags|HasMatchingGameplayTag (Ability|GetAbilitySystemComponent (.HitActor (Collision|BreakHitResult _array_element))) "(TagName=\"State.Damage.Immune\")")))
          (GameplayEffects|ApplyGameplayEffectToTarget :self _returnvalue_3 :GameplayEffectClass "/Game/DustDevil/Core/GAS/Effects/GE_Damage.GE_Damage_C" :Target (Ability|GetAbilitySystemComponent (.HitActor (Collision|BreakHitResult _array_element))) :Level 1.0)
          (bind _returnvalue_6 (Ability|GameplayEffect|AssignTagSetbyCallerMagnitude (GameplayEffects|MakeOutgoingSpec :self _returnvalue_3 :GameplayEffectClass "/Game/DustDevil/Core/GAS/Effects/GE_Fire.GE_Fire_C" :Level 1.0) "(TagName=\"Event.Fire.Duration\")" (Utilities|Select :Index (Ability|GetAbilityLevel) :Option%200 5.0 :Option%201 5.0 :Option%202 7.0 :Option%203 1e+01)))
          (GameplayEffects|ApplyGameplayEffectSpecToTarget (Ability|GetAbilitySystemComponent _instigator) _returnvalue_6 (Ability|GetAbilitySystemComponent (.HitActor (Collision|BreakHitResult _array_element))))))
      (Ability|EndAbility))
    (:Is%20Not%20Valid
      (Ability|EndAbility))))