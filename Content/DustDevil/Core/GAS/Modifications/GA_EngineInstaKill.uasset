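; Event-triggered gameplay ability modification that instantly kills a weakened target when the instigator is boosting.
; It checks the instigator for boost start or ongoing cue tags, then compares a target attribute ratio, presumably health, against a threshold chosen by ability level.
; On success it applies GE_Death from instigator to target and plays a 2D sound.
; Failed checks end the ability, while the success path has no EndAbility call.
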(event Ability|EventActivateAbilityFromEvent
  (params (EventData :type Gameplay%20Event%20Data%20Structure%20%28by%20ref%29))
  (bind (_eventtag _instigator _target) (Utilities|Struct|BreakGameplayEventData EventData))
  (Utilities|IsValid _instigator
    (:Is%20Valid
      (bind _returnvalue (GameplayTags|HasAnyMatchingGameplayTags(Message) (Ability|GetAbilitySystemComponent _instigator) (GameplayTags|MakeGameplayTagContainerfromArray (Utilities|Array|MakeArray "(TagName=\"GameplayCue.Ability.Boost.Ongoing\")" "(TagName=\"GameplayCue.Ability.Boost.Start\")"))))
      (if _returnvalue
        (if (<= (/ (.ReturnValue (Ability|Attribute|GetFloatAttribute _target "(AttributeName=\"CurrentHealth\",Attribute=/Script/DustDevil.BaseAttributeSet:CurrentHealth,AttributeOwner=\"/Script/CoreUObject.Class'/Script/DustDevil.BaseAttributeSet'\")")) (Math|Float|Max(Float) (.ReturnValue (Ability|Attribute|GetFloatAttribute _target "(AttributeName=\"MaxHealth\",Attribute=/Script/DustDevil.BaseAttributeSet:MaxHealth,AttributeOwner=\"/Script/CoreUObject.Class'/Script/DustDevil.BaseAttributeSet'\")")) 1.0)) (Utilities|Select :Index (Ability|GetAbilityLevel) :Option%200 0.05 :Option%201 0.05 :Option%202 0.1 :Option%203 0.15))
          (GameplayEffects|ApplyGameplayEffectToTarget :self (Ability|GetAbilitySystemComponent _instigator) :GameplayEffectClass "/Game/DustDevil/Core/GAS/Effects/GE_Death.GE_Death_C" :Target (Ability|GetAbilitySystemComponent _target))
          (Audio|PlaySound2D "/Game/DustDevil/Audio/Feedback/UpgradesAbilities/ui-designed-hit-modern-interface-impact-sweetener-02-230488.ui-designed-hit-modern-interface-impact-sweetener-02-230488" 1.0 1.0 0.0 0 0)
          (else
            (Ability|EndAbility)))
        (else
          (Ability|EndAbility))))
    (:Is%20Not%20Valid
      (Ability|EndAbility))))