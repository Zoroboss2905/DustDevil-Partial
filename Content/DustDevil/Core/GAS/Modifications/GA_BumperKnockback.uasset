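; Gameplay ability for a bumper knockback that launches the event's target using the instigator's velocity.
; If the target's root is not already simulating physics, it enables physics, plays an impact sound and applies a lifted velocity-change impulse.
; Dot products angle the impulse toward the target's side when it lies ahead of the instigator's motion.
; It then applies GE_Knockback_Cooldown to the target, with SetByCaller duration chosen by ability level.
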(event Ability|EventOnEndAbility
  (params (bWasCancelled :type Boolean)))

(event Ability|EventActivateAbilityFromEvent
  (params (EventData :type Gameplay%20Event%20Data%20Structure%20%28by%20ref%29))
  (bind (_eventtag _instigator _target) (Utilities|Struct|BreakGameplayEventData EventData))
  (bind _returnvalue (Transformation|GetActorLocation _target))
  (bind _returnvalue_2 (Ability|GetAbilitySystemComponent _target))
  (bind _returnvalue_3 (Transformation|GetVelocity _instigator))
  (bind _returnvalue_4 (Transformation|GetActorLocation _instigator))
  (bind _returnvalue_5 (- _returnvalue _returnvalue_4))
  (bind _returnvalue_6 (Math|Vector|Normalize _returnvalue_5))
  (Utilities|IsValid _target
    (:Is%20Valid
      (Utilities|FlowControl|Sequence
        (:then_0
          ;[1 1 1] Knockback
          (Utilities|IsValid _target
            (:Is%20Valid
              (bind _asprimitive_component (Utilities|Casting|CastToPrimitiveComponent (Variables|/Script/Engine.Actor|GetRootComponent _target)))
              (if (not (Physics|IsSimulatingPhysics _asprimitive_component "None"))
                (Collision|SetCollisionEnabled _asprimitive_component "QueryAndPhysics")
                (Physics|SetSimulatePhysics _asprimitive_component true)
                (Class|PrimitiveComponent|SetPhysicsMaxAngularVelocityinDegrees _asprimitive_component 1.8e+02 false "None")
                (Audio|PlaySound2D "/Game/DustDevil/Audio/Feedback/UpgradesAbilities/ui-designed-hit-modern-interface-impact-sweetener-02-230489.ui-designed-hit-modern-interface-impact-sweetener-02-230489" 1.0 1.0 0.0 0 0)
                (Physics|AddImpulse _asprimitive_component (Math|Vector|RotateVectorAroundAxis (* (+ _returnvalue_3 "0.000000,0.000000,100.000000") 1.4) (Math|Float|SelectFloat (Math|Float|SelectFloat -3e+01 3e+01 (< (Math|Vector|DotProduct _returnvalue_6 (Transformation|GetActorRightVector _instigator)) 0.0)) 0.0 (> (Math|Vector|DotProduct (Math|Vector|Normalize _returnvalue_3) _returnvalue_6) 0.0)) "0.000000,0.000000,1.000000") "None" true)
                (bind _returnvalue_7 (Ability|GameplayEffect|AssignTagSetbyCallerMagnitude (GameplayEffects|MakeOutgoingSpec :self _returnvalue_2 :GameplayEffectClass "/Game/DustDevil/Core/GAS/Effects/GE_Knockback_Cooldown.GE_Knockback_Cooldown_C") "(TagName=\"Effect.Mods.Duration\")" (Utilities|Select :Index (Ability|GetAbilityLevel) :Option%200 1.0 :Option%201 1.0 :Option%202 2.0 :Option%203 3.0)))
                (GameplayEffects|ApplyGameplayEffectSpecToTarget _returnvalue_2 _returnvalue_7 _returnvalue_2)))))
        (:then_2
          (Ability|EndAbility :!label _label))))
    (:Is%20Not%20Valid
      (goto _label))))