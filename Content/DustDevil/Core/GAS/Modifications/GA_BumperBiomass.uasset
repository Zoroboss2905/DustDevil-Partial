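; GA_BumperBiomass is an event-triggered gameplay ability that spawns a biomass pickup at the event's target, apparently as a bumper modification.
; With a valid target, it plays a 2D sound and spawns BP_Biomass at that actor's location and rotation, with the amount selected by ability level.
; The new mesh gets an upward velocity impulse with slight random horizontal spread.
; The ability then ends, as it does immediately without a valid target.
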(event Ability|EventActivateAbilityFromEvent
  (params (EventData :type Gameplay%20Event%20Data%20Structure%20%28by%20ref%29))
  (bind _target (Utilities|Struct|BreakGameplayEventData EventData))
  (bind _returnvalue (Transformation|GetActorTransform _target))
  (Utilities|IsValid _target
    (:Is%20Valid
      (Utilities|FlowControl|Sequence
        (:then_0
          (Audio|PlaySound2D "/Game/DustDevil/Audio/Feedback/UpgradesAbilities/ui-alert-menu-modern-interface-confirm-medium-230479.ui-alert-menu-modern-interface-confirm-medium-230479" 1.0 1.0 0.0 0 0)
          (bind _returnvalue_2 (Game|SpawnActorfromClass "/Game/DustDevil/ItemDrops/BP_Biomass.BP_Biomass_C" (Math|Transform|MakeTransform (.location _returnvalue) (.rotation _returnvalue) "1.000000,1.000000,1.000000") "Undefined" "MultiplyWithRoot" 0 (Utilities|Select :Index (Ability|GetAbilityLevel) :Option%200 1 :Option%201 1 :Option%202 2 :Option%203 3) 0))
          (Physics|AddImpulse (Variables|/Game/DustDevil/ItemDrops/BP_Biomass.BP_Biomass_C|GetMesh _returnvalue_2) (Math|Vector|MakeVector (Math|Random|RandomFloatinRange -1e+01 1e+01) (Math|Random|RandomFloatinRange -1e+01 1e+01) 1e+03) "None" true))
        (:then_1
          (Ability|EndAbility :!label _label))))
    (:Is%20Not%20Valid
      (goto _label))))