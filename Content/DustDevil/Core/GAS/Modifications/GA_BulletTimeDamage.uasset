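; Gameplay ability for a wheels damage mod that keeps GE_SlowDmg on its owner while bullet time is active.
; On activation, a looping 0.05-second timer polls global time dilation.
; Below normal speed, it applies the effect at ability level unless one tagged Upgrades.Mods.Wheels.Damage is already active.
; Otherwise it removes every effect with that tag; the ability never clears the timer or ends itself.
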(event Custom|TryApplyEffect
  (if (< (Class|GameplayStatics|GetGlobalTimeDilation) 1.0)
    (bind _returnvalue (GameplayEffects|GetActiveEffectswithAllTags (Ability|GetAbilitySystemComponent (Ability|GetOwningActorfromActorInfo)) "(GameplayTags=((TagName=\"Upgrades.Mods.Wheels.Damage\")))"))
    (if (not (> (Utilities|Array|Length _returnvalue) 0))
      (GameplayEffects|ApplyGameplayEffectToSelf :self (Ability|GetAbilitySystemComponent (Ability|GetOwningActorfromActorInfo)) :GameplayEffectClass "/Game/DustDevil/Core/GAS/Effects/GE_SlowDmg.GE_SlowDmg_C" :Level (Math|Conversions|ToFloat(Integer) (Ability|GetAbilityLevel))))
    (else
      (bind _returnvalue_2 (GameplayEffects|GetActiveEffectswithAllTags (Ability|GetAbilitySystemComponent (Ability|GetOwningActorfromActorInfo)) "(GameplayTags=((TagName=\"Upgrades.Mods.Wheels.Damage\")))"))
      (for _array_element _returnvalue_2
        (Ability|RemoveGameplayEffectFromOwnerWithHandle _array_element)))))

(event Ability|EventActivateAbility
  (Utilities|Time|SetTimerbyEvent (delegate Custom|TryApplyEffect) 0.05 true true))

(event Ability|EventOnEndAbility
  (params (bWasCancelled :type Boolean)))