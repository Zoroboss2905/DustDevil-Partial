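; BP_POI_Objectives is a point-of-interest trigger that shows an objective HUD widget while a BP_Vehicle overlaps it.
; It creates the widget on BeginPlay with configurable text, then adds it to the viewport with an appear animation on overlap.
; When the vehicle leaves, a valid AccessibleActors reference reverses that animation and removes the widget.
; Otherwise it plays the completed animation, removes the widget and destroys itself.
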(event EventBeginPlay
  (bind _returnvalue (UserInterface|CreateWidget "/Game/DustDevil/UI/HUD/WBP_HUDObjectivesInTheMainLevel.WBP_HUDObjectivesInTheMainLevel_C" 0 (Variables|Default|GetText%20Value%20One)))
  (Variables|Default|SetPOI_Widget _returnvalue))

(event Collision|EventActorBeginOverlap
  (params (OtherActor :type Actor%20Object%20Reference))
  (bind _poi_widget (Variables|Default|GetPOI_Widget))
  (bind _asbp_vehicle (Utilities|Casting|CastToBP_Vehicle OtherActor))
  (Variables|Default|SetVehicle _asbp_vehicle)
  (UserInterface|Viewport|AddtoViewport _poi_widget 0)
  (UserInterface|Animation|PlayAnimation _poi_widget (Variables|/Game/DustDevil/UI/HUD/WBP_HUDObjectivesInTheMainLevel.WBP_HUDObjectivesInTheMainLevel_C|GetANIM_ObjAppear _poi_widget) 0.0 1 "Forward" 1.0 false))

(event EventTick
  (params (DeltaSeconds :type Float%20%28single-precision%29)))

(event Collision|EventActorEndOverlap
  (params (OtherActor :type Actor%20Object%20Reference))
  (bind _poi_widget (Variables|Default|GetPOI_Widget))
  (bind _poi_widget_2 (Variables|Default|GetPOI_Widget))
  (Utilities|Casting|CastToBP_Vehicle OtherActor)
  (if (Utilities|IsValid (Variables|Default|GetAccessibleActors))
    (Components|Animation|PlayAnimation _poi_widget (Variables|/Game/DustDevil/UI/HUD/WBP_HUDObjectivesInTheMainLevel.WBP_HUDObjectivesInTheMainLevel_C|GetANIM_ObjAppear _poi_widget) 0.0 1 "Reverse"
      (:Finished
        (Widget|RemovefromParent (Variables|Default|GetPOI_Widget))))
    (else
      (Components|Animation|PlayAnimation _poi_widget_2 (Variables|/Game/DustDevil/UI/HUD/WBP_HUDObjectivesInTheMainLevel.WBP_HUDObjectivesInTheMainLevel_C|GetANIM_ObjCompleted _poi_widget_2) 0.0
        (:Finished
          (Widget|RemovefromParent (Variables|Default|GetPOI_Widget))
          (Actor|DestroyActor))))))

(fn ConstructionScript)