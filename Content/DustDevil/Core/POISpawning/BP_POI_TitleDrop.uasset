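; Point-of-interest trigger that shows a title widget with intro and exit sounds when a BP_Vehicle enters.
; The widget, built on BeginPlay, animates out after a delay or early exit, then re-arms.
; An optional timeline lerps the vehicle's camera boom length on entry and reverses on exit.
; A looping camera trace that outlines the vehicle behind "Blocking" actors exists, but its start and stop calls are disconnected.
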(event Custom|Opacity
  (bind _vehicle (Variables|Default|GetVehicle))
  (bind _camera (Variables|/Script/DustDevil.Vehicle|GetCamera _vehicle))
  (bind _returnvalue (Transformation|GetWorldLocation _camera))
  ;[1 1 1] LerpCheck
  (if (Variables|Default|GetRender)
    (bind _outhit (Collision|LineTraceByChannel _returnvalue (+ (* (Math|Vector|GetForwardVector (Transformation|GetWorldRotation _camera)) (Variables|Default|GetMultiply)) _returnvalue) "TraceTypeQuery1" false 0 "None"))
    (if (.bBlockingHit (Collision|BreakHitResult _outhit))
      (Utilities|IsValid (.HitActor (Collision|BreakHitResult _outhit))
        (:Is%20Valid
          (if (Actor|ActorHasTag (.HitActor (Collision|BreakHitResult _outhit)) "Blocking")
            (Rendering|Material|SetOverlayMaterial (Variables|/Script/DustDevil.Vehicle|GetChassis (Variables|Default|GetVehicle)) "/Game/DustDevil/MaterialLibrary/Materials/M_OutlineEnemy.M_OutlineEnemy" :!class /Script/Engine.MeshComponent)
            (Utilities|FlowControl|RetriggerableDelay 0.05)
            (CallFunction|Opacity)
            (else
              (Rendering|Material|SetOverlayMaterial (Variables|/Script/DustDevil.Vehicle|GetChassis (Variables|Default|GetVehicle)) 0 :!class /Script/Engine.MeshComponent)
              (Utilities|FlowControl|RetriggerableDelay 0.05)
              (CallFunction|Opacity))))
        (:Is%20Not%20Valid
          (Development|PrintString "BP_POI_TitleDrop: Hit Actor not valid!"))))))

(event Custom|ChangeOpacityBack
  ;[1 1 1] LerpCheck
  (Utilities|IsValid (Variables|Default|GetVehicle)
    (:Is%20Valid
      (Rendering|Material|SetOverlayMaterial (Variables|/Script/DustDevil.Vehicle|GetChassis (Variables|Default|GetVehicle)) 0 :!class /Script/Engine.MeshComponent)
      (Utilities|FlowControl|RetriggerableDelay 0.05)
      (CallFunction|Opacity))))

(event EventBeginPlay
  (bind _returnvalue (UserInterface|CreateWidget "/Game/DustDevil/UI/LocationTitles/WBP_EnterPOI_SafeZone.WBP_EnterPOI_SafeZone_C" 0 (Variables|Default|GetText%20Value%20One) (Variables|Default|GetText%20Value%20Two) (Variables|Default|GetChange%20Colour) (Variables|Default|GetText%20Value%20Three)))
  (Variables|Default|SetPOI_Widget _returnvalue))

(event Collision|EventActorBeginOverlap
  (params (OtherActor :type Actor%20Object%20Reference))
  (bind _poi_widget (Variables|Default|GetPOI_Widget))
  (bind _asbp_vehicle (Utilities|Casting|CastToBP_Vehicle OtherActor))
  (Variables|Default|SetVehicle _asbp_vehicle)
  (Utilities|FlowControl|Sequence
    (:then_0
      (if (Variables|Default|GetShowTitle)
        (Variables|Default|SetShowTitle false)
        (UserInterface|Viewport|AddtoViewport _poi_widget 0)
        (Audio|PlaySound2D (Variables|Default|GetIntroAudio) 0.7 1.0 0.0 0 0 false)
        (Variables|Default|SetPlayOutAnimation true)
        (Utilities|FlowControl|Delay 5.0)
        (if (Variables|Default|GetPlayOutAnimation)
          (Default|OutAnimation _poi_widget)
          (Audio|PlaySound2D (Variables|Default|GetOutAnimationSound) 1.0 1.0 0.0 0 0 false)
          (Variables|Default|SetPlayOutAnimation false)
          (Utilities|FlowControl|Delay 1.0)
          (Variables|Default|SetShowTitle true)
          (Widget|RemovefromParent _poi_widget))))
    (:then_1
      (if (Variables|Default|GetCamZoom)
        (bind _targetarmlength (Timeline|Timeline Play)
          (:Update
            (Variables|/Script/Engine.SpringArmComponent|SetTargetArmLength (Variables|/Script/DustDevil.Vehicle|GetCameraBoom (Variables|Default|GetVehicle)) (Math|Float|Lerp (Variables|Default|GetCamZoomValueInitial) (Variables|Default|GetCamZoomValueFinal) _targetarmlength))))))))

(event EventTick
  (params (DeltaSeconds :type Float%20%28single-precision%29)))

(event Collision|EventActorEndOverlap
  (params (OtherActor :type Actor%20Object%20Reference))
  (bind _poi_widget (Variables|Default|GetPOI_Widget))
  (Utilities|Casting|CastToBP_Vehicle OtherActor)
  (Utilities|FlowControl|Sequence
    (:then_0
      (if (Variables|Default|GetPlayOutAnimation)
        (Default|OutOfZone _poi_widget)
        (Audio|PlaySound2D (Variables|Default|GetOutAnimationSound) 1.0 1.0 0.0 0 0 false)
        (Variables|Default|SetPlayOutAnimation false)
        (Utilities|FlowControl|Delay 1.0)
        (Variables|Default|SetShowTitle true)
        (Widget|RemovefromParent _poi_widget)))
    (:then_1
      (if (Variables|Default|GetCamZoom)
        (bind _targetarmlength (Timeline|Timeline Reverse)
          (:Update
            (Variables|/Script/Engine.SpringArmComponent|SetTargetArmLength (Variables|/Script/DustDevil.Vehicle|GetCameraBoom (Variables|Default|GetVehicle)) (Math|Float|Lerp (Variables|Default|GetCamZoomValueInitial) (Variables|Default|GetCamZoomValueFinal) _targetarmlength))))))))

(fn ConstructionScript)