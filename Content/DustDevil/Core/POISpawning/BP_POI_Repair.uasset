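; BP_POI_Repair is a point of interest that spawns repair kit pickups around itself on BeginPlay.
; A loop driven by the RepairKits count spawns BP_Prototype_RepairKit actors, each offset randomly from the root within the SpawnRadius sphere's radius.
; Each kit gets a hardcoded world Z, a fixed roll and a random yaw, and always spawns, adjusting its position around collisions where possible.
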(event EventBeginPlay
  (bind _returnvalue (Math|Random|RandomUnitVector))
  (bind _spawnradius (Variables|Default|GetSpawnRadius))
  (bind _defaultsceneroot (Variables|Default|GetDefaultSceneRoot))
  (bind _returnvalue_2 (Transformation|GetWorldLocation _defaultsceneroot))
  (bind _sphereradius (Variables|/Script/Engine.SphereComponent|GetSphereRadius _spawnradius))
  (bind _returnvalue_3 (Math|Random|RandomFloatinRange 0.0 _sphereradius))
  (bind _returnvalue_4 (* _returnvalue _returnvalue_3))
  (bind _returnvalue_5 (+ _returnvalue_4 _returnvalue_2))
  ;[0.02956 0.02956 0.02956] Spawns the specified number of repair kits in a random location within the spawn radius
  (for _index (range 0 (Variables|Default|GetRepairKits))
    (Game|SpawnActorfromClass "/Game/DustDevil/Prototyping/Blueprints/BP_Prototype_RepairKit.BP_Prototype_RepairKit_C" (Math|Transform|MakeTransform (Math|Vector|MakeVector (.x _returnvalue_5) (.y _returnvalue_5) 4419.448753) (Math|Rotator|MakeRotator 9e+01 0.0 (.yaw (Math|Random|RandomRotator false))) "1.000000,1.000000,1.000000") "AdjustIfPossibleButAlwaysSpawn" "MultiplyWithRoot" 0 0)))

(fn ConstructionScript
  (|CallParentFunction))