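; Manager that spawns points of interest (POIs) as the player's BP_Vehicle approaches their spawner locations.
; Gathers every BP_POISpawner at BeginPlay, with AddSpawner available to append more.
; A looping half-second timer distance-checks the list against the vehicle and tells in-range spawners to spawn a random prefab from the common pool.
; Triggered spawners go into a removal list and are dropped after iteration, preventing repeat activation.
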(event EventBeginPlay
  (CallFunction|CollectSpawners)
  (CallFunction|SpawnifinRange)
  (Utilities|Time|SetTimerbyFunctionName 0 "SpawnIfInRange" 0.5 true true))

(fn ConstructionScript)

(fn AddSpawner
  (params (NewSpawner :type BP%20POI%20Spawner%20Object%20Reference))
  (Utilities|Array|Add (Variables|Default|GetPOI%20Spawners) NewSpawner))

(fn SpawnPOI
  (params (SpawnerToActivate :type BP%20POI%20Spawner%20Object%20Reference))
  ;[1 1 1] Consider Spawn Conditions and Spawn a POI Based on that Information
  (Default|SpawnPOI SpawnerToActivate (.OutItem (Utilities|Array|Random (Variables|POIPrefabs|GetPOI_Prefabs_Common))) false))

(fn SpawnifinRange
  ;[1 1 1] Replace this with the Character Pawn Class
  (bind _asbp_vehicle (Utilities|Casting|CastToBP_Vehicle (Game|Player|GetPlayerPawn 0)))
  (LocalVariables|SetPlayerLoc (Transformation|GetActorLocation _asbp_vehicle))
  (for _array_element (Variables|Default|GetPOI%20Spawners)
    (Utilities|IsValid _array_element
      (:Is%20Valid
        (if (< (Math|Vector|Distance(Vector) (Transformation|GetActorLocation _array_element) (LocalVariables|GetPlayerLoc)) (Variables|Default|GetSpawnerActivationRange)) ; Is Player within range to spawn a POI
          (Utilities|IsValid _array_element
            (:Is%20Valid
              (Utilities|Array|Add (LocalVariables|GetRemovalList) _array_element)
              (CallFunction|SpawnPOI _array_element)))))))
  (for _array_element_2 (LocalVariables|GetRemovalList)
    (Utilities|Array|RemoveItem (Variables|Default|GetPOI%20Spawners) _array_element_2)))

(fn CollectSpawners
  (bind _outactors (Actor|GetAllActorsOfClass "/Game/DustDevil/Core/POISpawning/BP_POISpawner.BP_POISpawner_C"))
  (Variables|Default|SetPOI%20Spawners _outactors))