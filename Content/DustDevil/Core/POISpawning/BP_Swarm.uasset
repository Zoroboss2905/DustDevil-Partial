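; BP_Swarm is a point-of-interest spawner that creates a small swarm of weak, fast bugs around itself on BeginPlay.
; It spawns a random number of half-scale bugs at random navigable points within a radius, favoring BP_BugFlying two to one over BP_BugBase.
; Each spawn is cast to BP_BugBase for shared stat overrides.
; The navigation query's success result has no effect, and spawning ignores collisions.
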(event EventBeginPlay
  (bind _returnvalue (Transformation|GetActorTransform))
  (|CallParentFunction)
  (for _index (range 0 (Math|Random|RandomIntegerinRange 5 15))
    (bind (_randomlocation _returnvalue_2) (Class|NavigationSystemV1|GetRandomLocationinNavigableRadius (.location _returnvalue) 1e+03 0 0))
    (if _returnvalue_2
      _
      (else
        _))
    (bind _returnvalue_3 (Game|SpawnActorfromClass (Utilities|Select :Index (Math|Random|RandomIntegerinRange 0 2) :Option%200 "/Game/DustDevil/Characters/EnemyAI/BP_BugBase.BP_BugBase_C" :Option%201 "/Game/DustDevil/Characters/EnemyAI/BP_BugFlying.BP_BugFlying_C" :Option%202 "/Game/DustDevil/Characters/EnemyAI/BP_BugFlying.BP_BugFlying_C") (Math|Transform|MakeTransform _randomlocation (.rotation _returnvalue) "0.500000,0.500000,0.500000") "AlwaysSpawn" "MultiplyWithRoot" 0 0))
    (bind _asbp_bug_base (Utilities|Casting|CastToBP_BugBase _returnvalue_3))
    (Default|SetDefaultStats _asbp_bug_base 1e+01 1e+01 0.0 5.0 1.0 0.01 1.2e+03)))

(event Collision|EventActorBeginOverlap
  (params (OtherActor :type Actor%20Object%20Reference))
  (|CallParentFunction OtherActor) ; This node is disabled and will not be called.\nDrag off pins to build functionality.
)

(event EventTick
  (params (DeltaSeconds :type Float%20%28single-precision%29))
  (|CallParentFunction DeltaSeconds) ; This node is disabled and will not be called.\nDrag off pins to build functionality.
)

(fn ConstructionScript
  (|CallParentFunction))