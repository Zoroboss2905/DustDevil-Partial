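; Base actor for a shootable hive objective that takes damage through the Gameplay Ability System and explodes at zero health.
; BeginPlay seeds attributes from MaxHealth via a set-by-caller GameplayEffect, then an async attribute listener triggers hit sound and death checks.
; Death hides the mesh, notifies the ObjectiveManager for missile objectives or otherwise updates the InfestationZone, then destroys the actor.
; The hitbox destroys overlapping projectiles; GetWeaponDamage reads the equipped weapon's curve table.
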(event OnComponentBeginOverlap(Hitbox)
  (params (OverlappedComponent :type Primitive%20Component%20Object%20Reference) (OtherActor :type Actor%20Object%20Reference) (OtherComp :type Primitive%20Component%20Object%20Reference) (OtherBodyIndex :type Integer) (bFromSweep :type Boolean) (SweepResult :type Hit%20Result%20Structure%20%28by%20ref%29))
  (if (Utilities|DoesObjectImplementInterface OtherActor "/Game/DustDevil/Core/Interfaces/BPI_Projectile.BPI_Projectile_C")
    (Actor|DestroyActor OtherActor)))

(event Custom|DamageTaken
  (bind _abilitysystem (Variables|Default|GetAbilitySystem))
  (Utilities|FlowControl|Sequence
    (:then_0
      (Audio|PlaySoundatLocation "/Game/DustDevil/Audio/Feedback/BugImpact/A_EnemyDamage_Cue.A_EnemyDamage_Cue" (Transformation|GetActorLocation) "0, 0, 0" 1.0 1.0 0.0 0 "/Game/DustDevil/Audio/Feedback/BugImpact/SC_EnemyDamageCon.SC_EnemyDamageCon" 0 0)
      (Development|PrintString (Utilities|String|Append (Utilities|String|MakeLiteralString "Taken Damage") (Utilities|String|ToString(Float) (.ReturnValue (Ability|Attribute|GetFloatAttributefromAbilitySystemComponent _abilitysystem "(AttributeName=\"CurrentHealth\",Attribute=/Script/DustDevil.BaseAttributeSet:CurrentHealth,AttributeOwner=\"/Script/CoreUObject.Class'/Script/DustDevil.BaseAttributeSet'\")"))) "/" (Utilities|String|ToString(Float) (.ReturnValue (Ability|Attribute|GetFloatAttributefromAbilitySystemComponent _abilitysystem "(AttributeName=\"MaxHealth\",Attribute=/Script/DustDevil.BaseAttributeSet:MaxHealth,AttributeOwner=\"/Script/CoreUObject.Class'/Script/DustDevil.BaseAttributeSet'\")"))))))
    (:then_1
      (if (== (.ReturnValue (Ability|Attribute|GetFloatAttributefromAbilitySystemComponent (Variables|Default|GetAbilitySystem) "(AttributeName=\"CurrentHealth\",Attribute=/Script/DustDevil.BaseAttributeSet:CurrentHealth,AttributeOwner=\"/Script/CoreUObject.Class'/Script/DustDevil.BaseAttributeSet'\")")) 0.0)
        (Utilities|FlowControl|DoOnce false
          (:Completed
            (Niagara|SpawnSystematLocation "/Game/DustDevil/Effects/Explosions/NS_EnemyExplosion.NS_EnemyExplosion" (Transformation|GetWorldLocation (Variables|Default|GetCentrepoint)))
            (Development|SetHiddeninGame (Variables|Default|GetHiveMesh) true false)
            (Utilities|FlowControl|Sequence
              (:then_0
                (if (Variables|Default|GetbMissileObj)
                  (bind _objectivemanager (Variables|Reference|GetObjectiveManager)
                    (:then
                      (Default|HiveDestroyed _objectivemanager (Variables|Default|GetHiveLocation)))
                    (:else))
                  (else
                    (bind _infestationzone (Variables|Reference|GetInfestationZone)
                      (:then
                        (Default|UpdateInfestationLevel _infestationzone (Variables|Attributes|GetInfestationAmount)))
                      (:else)))))
              (:then_1
                (Utilities|FlowControl|Delay 1.0)
                (Actor|DestroyActor)))))))))

(event EventBeginPlay
  (Components|Activation|Activate (Variables|Default|GetAbilitySystem) false)
  (Utilities|FlowControl|DelayUntilNextTick)
  (Utilities|FlowControl|Sequence
    (:then_0
      (CallFunction|SetDefaultStats)
      (bind _asgi_ddprototype (Utilities|Casting|CastToGI_DDPrototype (Game|GetGameInstance)))
      (Variables|Reference|SetGameInstance _asgi_ddprototype))
    (:then_1
      (bind _asynctaskproxy (Ability|Tasks|WaitForAttributeChanged 0 "(AttributeName=\"CurrentHealth\",Attribute=/Script/DustDevil.BaseAttributeSet:CurrentHealth,AttributeOwner=\"/Script/CoreUObject.Class'/Script/DustDevil.BaseAttributeSet'\")")
        (:then
          (Variables|Default|SetAA_Damagetaken _asynctaskproxy))
        (:Changed
          (CallFunction|DamageTaken))))))

(event EventEndPlay
  (params (EndPlayReason :type EEndPlayReason%20Enum :default "Destroyed"))
  (bind _aa_damagetaken (Variables|Default|GetAA_Damagetaken)
    (:then
      (AsyncAction|Cancel _aa_damagetaken))
    (:else)))

(fn ConstructionScript)

(fn GetWeaponDamage
  (switch Utilities|FlowControl|Switch|SwitchonE_WeaponType (Variables|/Game/DustDevil/Core/Saves/SG_DDSaveData.SG_DDSaveData_C|GetEquippedWeapon (Default|GetSaveData (Variables|Reference|GetGameInstance)))
    (:NewEnumerator0
      (bind _outxy (DataTable|EvaluateCurveTableRow "/Game/DustDevil/Data/CT_MachineGun.CT_MachineGun" "Damage")
        (:RowFound
          (return _outxy))))
    (:NewEnumerator1
      (bind _outxy_2 (DataTable|EvaluateCurveTableRow "/Game/DustDevil/Data/CT_MiniGun.CT_MiniGun" "Damage")
        (:RowFound
          (return _outxy_2))))
    (:NewEnumerator2
      (bind _outxy_3 (DataTable|EvaluateCurveTableRow "/Game/DustDevil/Data/CT_Flamethrower.CT_Flamethrower" "Damage")
        (:RowFound
          (return _outxy_3))))
    (:NewEnumerator3
      (bind _outxy_4 (DataTable|EvaluateCurveTableRow "/Game/DustDevil/Data/CT_Autocannon.CT_Autocannon" "Damage")
        (:RowFound
          (return _outxy_4))))
    (:NewEnumerator4
      (bind _outxy_5 (DataTable|EvaluateCurveTableRow "/Game/DustDevil/Data/CT_Soundwave.CT_Soundwave" "Damage")
        (:RowFound
          (return _outxy_5))))))

(fn SetDefaultStats
  (bind _abilitysystem (Variables|Default|GetAbilitySystem))
  (Class|AbilitySystemComponent|InitStats _abilitysystem "/Script/DustDevil.BaseAttributeSet")
  (bind _returnvalue (Ability|GameplayEffect|AssignTagSetbyCallerMagnitude (GameplayEffects|MakeOutgoingSpec _abilitysystem "/Game/DustDevil/Core/GAS/Effects/GE_DefaultEnemyValues.GE_DefaultEnemyValues_C" 1.0 (GameplayEffects|MakeEffectContext _abilitysystem)) "(TagName=\"Stats.Base.MaxHealth\")" (Math|Conversions|ToFloat(Integer) (Variables|Attributes|GetMaxHealth))))
  (bind _returnvalue_2 (Ability|GameplayEffect|AssignTagSetbyCallerMagnitude _returnvalue "(TagName=\"Stats.Base.CurrentHealth\")" (Math|Conversions|ToFloat(Integer) (Variables|Attributes|GetMaxHealth))))
  (bind _returnvalue_3 (Ability|GameplayEffect|AssignTagSetbyCallerMagnitude _returnvalue_2 "(TagName=\"Stats.Base.Armour\")" 0.0))
  (bind _returnvalue_4 (Ability|GameplayEffect|AssignTagSetbyCallerMagnitude _returnvalue_3 "(TagName=\"Stats.Base.BioMatter\")" 0.0))
  (bind _returnvalue_5 (Ability|GameplayEffect|AssignTagSetbyCallerMagnitude _returnvalue_4 "(TagName=\"Stats.Base.Damage\")" 0.0))
  (bind _returnvalue_6 (Ability|GameplayEffect|AssignTagSetbyCallerMagnitude _returnvalue_5 "(TagName=\"Stats.Base.NuclearMatter\")" 0.0))
  (bind _returnvalue_7 (Ability|GameplayEffect|AssignTagSetbyCallerMagnitude _returnvalue_6 "(TagName=\"Stats.Base.ChitinChance\")" 0.0))
  (GameplayEffects|ApplyGameplayEffectSpecToSelf (Variables|Default|GetAbilitySystem) _returnvalue_7))

(fn GetEnemy
  (return 0))

(fn GetInfestationSource
  (return self))