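; BP_InfestationZone is a secondary objective area that tracks how much hive infestation remains and unlocks a missile silo hatch when cleared.
; On BeginPlay it gathers overlapping shootable hives, links them back to itself and sums their infestation as the total.
; Player entry adds the HUD objective widget, re-armed on exit.
; UpdateInfestationLevel subtracts cleared amounts, refreshes the HUD and calls HatchCleared on the silo at zero.
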(event OnComponentBeginOverlap(ZoneRadius)
  (params (OverlappedComponent :type Primitive%20Component%20Object%20Reference) (OtherActor :type Actor%20Object%20Reference) (OtherComp :type Primitive%20Component%20Object%20Reference) (OtherBodyIndex :type Integer) (bFromSweep :type Boolean) (SweepResult :type Hit%20Result%20Structure%20%28by%20ref%29))
  (if (Utilities|DoesObjectImplementInterface OtherActor "/Game/DustDevil/Core/Interfaces/BPI_PlayerTrigger.BPI_PlayerTrigger_C")
    (Utilities|FlowControl|DoOnce false
      (:Completed
        (bind _player (Class|BPIPlayerTrigger|GetPlayerCharacter(Message) OtherActor))
        (Variables|References|SetPlayer _player)
        (CallFunction|AddObjectiveWidget)
        (Class|BPIHUDUpdates|UpdateObjectiveInfestation(Message) (Variables|/Game/DustDevil/Player/BP_Vehicle.BP_Vehicle_C|GetHUD (Variables|References|GetPlayer)) (Variables|Default|GetInfestationLevelCurrent) (Variables|Default|GetInfestationLevelFull))))))

(event OnComponentEndOverlap(ZoneRadius)
  (params (OverlappedComponent :type Primitive%20Component%20Object%20Reference) (OtherActor :type Actor%20Object%20Reference) (OtherComp :type Primitive%20Component%20Object%20Reference) (OtherBodyIndex :type Integer))
  (if (Utilities|DoesObjectImplementInterface OtherActor "/Game/DustDevil/Core/Interfaces/BPI_PlayerTrigger.BPI_PlayerTrigger_C")
    (Utilities|FlowControl|DoOnce false) ; enters at Reset
  ))

(event EventBeginPlay
  (Utilities|FlowControl|Sequence
    (:then_0
      (for _array_element (Collision|GetOverlappingActors (Variables|Default|GetZoneRadius) "/Game/DustDevil/Objectives/BP_ShootableHiveBase.BP_ShootableHiveBase_C" :!class /Script/Engine.PrimitiveComponent)
        (bind _hive (Class|BPIInfestation|GetInfestationSource(Message) _array_element))
        (Utilities|IsValid _hive
          (:Is%20Valid
            (Utilities|Array|Add (Variables|References|GetHives) _hive))
          (:Is%20Not%20Valid
            (Development|PrintString "Shootable hive ref not valid!" true true "(R=1.000000,G=0.000000,B=0.000000,A=1.000000)"))))
      (for _array_element_2 (Variables|References|GetHives)
        (Variables|/Game/DustDevil/Objectives/BP_ShootableHiveBase.BP_ShootableHiveBase_C|SetInfestationZone _array_element_2 self)))
    (:then_2
      (bind _output_get (Variables|Default|SetInfestationLevelFull (CallFunction|CalcInfestationLevel)))
      (Variables|Default|SetInfestationLevelCurrent _output_get))))

(fn ConstructionScript)

(fn CalcInfestationLevel
  (for _array_element (Variables|References|GetHives)
    (LocalVariables|SetLocal_InfestationAmount (+ (Variables|/Game/DustDevil/Objectives/BP_ShootableHiveBase.BP_ShootableHiveBase_C|GetInfestationAmount _array_element) (LocalVariables|GetLocal_InfestationAmount))))
  (return (LocalVariables|GetLocal_InfestationAmount)))

(fn AddObjectiveWidget
  (Class|BPIHUDUpdates|AddSecondaryObjective(Message) (Variables|/Game/DustDevil/Player/BP_Vehicle.BP_Vehicle_C|GetHUD (Variables|References|GetPlayer)) "NewEnumerator0"))

(fn UpdateInfestationLevel
  (params (InfestationCleared :type Float%20%28double-precision%29))
  (Variables|Default|SetInfestationLevelCurrent (- (Variables|Default|GetInfestationLevelCurrent) InfestationCleared))
  (Utilities|FlowControl|Sequence
    (:then_0
      (if (== (Variables|Default|GetInfestationLevelCurrent) 0.0)
        (Default|HatchCleared (Variables|References|GetMissileSilo))))
    (:then_1
      (Class|BPIHUDUpdates|UpdateObjectiveInfestation(Message) (Variables|/Game/DustDevil/Player/BP_Vehicle.BP_Vehicle_C|GetHUD (Variables|References|GetPlayer)) (Variables|Default|GetInfestationLevelCurrent) (Variables|Default|GetInfestationLevelFull)))))