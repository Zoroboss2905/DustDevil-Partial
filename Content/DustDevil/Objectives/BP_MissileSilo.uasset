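; Missile silo objective actor, started by a hold-to-interact prompt when ObjectiveManager allows it.
; On BeginPlay it restores the completed state from save data, or registers its hatch and missile infestation hives with the manager.
; Timelines open the hatch and raise the missile, stalling and reporting to the manager until HatchCleared resumes them.
; MissileCleared fires the missile with thruster flames and sound, completes the objective, then begins the level transition.
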(event OnComponentBeginOverlap(InteractionTrigger)
  (params (OverlappedComponent :type Primitive%20Component%20Object%20Reference) (OtherActor :type Actor%20Object%20Reference) (OtherComp :type Primitive%20Component%20Object%20Reference) (OtherBodyIndex :type Integer) (bFromSweep :type Boolean) (SweepResult :type Hit%20Result%20Structure%20%28by%20ref%29))
  (if (Utilities|DoesObjectImplementInterface OtherActor "/Game/DustDevil/Core/Interfaces/BPI_PlayerTrigger.BPI_PlayerTrigger_C")
    (Utilities|FlowControl|DoOnce false
      (:Completed
        (bind _player (Class|BPIPlayerTrigger|GetPlayerCharacter(Message) OtherActor))
        (Variables|References|SetPlayer _player)
        (if (Math|Boolean|ANDBoolean (Variables|/Game/DustDevil/Objectives/BP_SiloManager_Infestation.BP_SiloManager_Infestation_C|GetbCanStartObj (Variables|References|GetObjectiveManager)) (not (Variables|/Game/DustDevil/Objectives/BP_SiloManager_Infestation.BP_SiloManager_Infestation_C|GetbObjStarted (Variables|References|GetObjectiveManager))) (not (Variables|Default|GetbObjectiveCompleted)))
          (Rendering|SetVisibility (Variables|Default|GetInteractionPrompt) true false)
          (Variables|Default|SetbPromptOpen true)
          (else
            (Class|BPIHUDUpdates|DisplayPopup(Message) (Variables|/Game/DustDevil/Player/BP_Vehicle.BP_Vehicle_C|GetHUD (Variables|References|GetPlayer)) "Missile requires nuclear material to arm!")))))))

(event OnComponentEndOverlap(InteractionTrigger)
  (params (OverlappedComponent :type Primitive%20Component%20Object%20Reference) (OtherActor :type Actor%20Object%20Reference) (OtherComp :type Primitive%20Component%20Object%20Reference) (OtherBodyIndex :type Integer))
  (if (Utilities|DoesObjectImplementInterface OtherActor "/Game/DustDevil/Core/Interfaces/BPI_PlayerTrigger.BPI_PlayerTrigger_C")
    (Utilities|FlowControl|Sequence
      (:then_0
        (Utilities|FlowControl|DoOnce false) ; enters at Reset
      )
      (:then_1
        (Rendering|SetVisibility (Variables|Default|GetInteractionPrompt) false false)
        (Variables|Default|SetbPromptOpen false)))))

(event Custom|BeginMissileLaunch
  (bind _missilemesh (Variables|Default|GetMissileMesh))
  (bind _hatchmesh (Variables|Default|GetHatchMesh))
  (bind _relativerotation (Variables|/Script/Engine.SceneComponent|GetRelativeRotation _hatchmesh))
  (bind _relativelocation (Variables|/Script/Engine.SceneComponent|GetRelativeLocation _missilemesh))
  (Utilities|FlowControl|Sequence
    (:then_0
      (bind _alpha (Timeline|TL_HatchOpening PlayFromStart)
        (:Update
          (Transformation|SetRelativeRotation _hatchmesh (Math|Rotator|MakeRotator (Math|Float|Lerp (Variables|Animations|GetHatchStartRotate) (Variables|Animations|GetHatchEndRotate) _alpha) (.pitch _relativerotation) (.yaw _relativerotation)) false false))))
    (:then_1
      (Utilities|FlowControl|Delay 2.0)
      (bind _alpha_2 (Timeline|TL_MissileRising PlayFromStart)
        (:Update
          (Transformation|SetRelativeLocation _missilemesh (Math|Vector|MakeVector (.x _relativelocation) (.y _relativelocation) (Math|Float|Lerp (Variables|Animations|GetMissileStartLoc) (Variables|Animations|GetMissileFireLoc) _alpha_2)) false false))
        (:Finished
          (Default|MissileStalled (Variables|References|GetObjectiveManager)))))
    (:then_2
      (Utilities|FlowControl|Delay 12.0)
      (CallFunction|HatchStalled)
      (Default|HatchStalled (Variables|References|GetObjectiveManager)))))

(event Custom|HatchStalled
  (bind _missilemesh (Variables|Default|GetMissileMesh))
  (bind _hatchmesh (Variables|Default|GetHatchMesh))
  (bind _relativerotation (Variables|/Script/Engine.SceneComponent|GetRelativeRotation _hatchmesh))
  (bind _relativelocation (Variables|/Script/Engine.SceneComponent|GetRelativeLocation _missilemesh))
  (Utilities|FlowControl|Sequence
    (:then_0
      (bind _alpha (Timeline|TL_HatchOpening Stop)
        (:Update
          (Transformation|SetRelativeRotation _hatchmesh (Math|Rotator|MakeRotator (Math|Float|Lerp (Variables|Animations|GetHatchStartRotate) (Variables|Animations|GetHatchEndRotate) _alpha) (.pitch _relativerotation) (.yaw _relativerotation)) false false))))
    (:then_1
      (bind _alpha_2 (Timeline|TL_MissileRising Stop)
        (:Update
          (Transformation|SetRelativeLocation _missilemesh (Math|Vector|MakeVector (.x _relativelocation) (.y _relativelocation) (Math|Float|Lerp (Variables|Animations|GetMissileStartLoc) (Variables|Animations|GetMissileFireLoc) _alpha_2)) false false))
        (:Finished
          (Default|MissileStalled (Variables|References|GetObjectiveManager)))))))

(event Custom|HatchCleared
  (bind _missilemesh (Variables|Default|GetMissileMesh))
  (bind _hatchmesh (Variables|Default|GetHatchMesh))
  (bind _relativerotation (Variables|/Script/Engine.SceneComponent|GetRelativeRotation _hatchmesh))
  (bind _relativelocation (Variables|/Script/Engine.SceneComponent|GetRelativeLocation _missilemesh))
  (Utilities|FlowControl|Sequence
    (:then_0
      (bind _alpha (Timeline|TL_HatchOpening Play)
        (:Update
          (Transformation|SetRelativeRotation _hatchmesh (Math|Rotator|MakeRotator (Math|Float|Lerp (Variables|Animations|GetHatchStartRotate) (Variables|Animations|GetHatchEndRotate) _alpha) (.pitch _relativerotation) (.yaw _relativerotation)) false false))))
    (:then_1
      (bind _alpha_2 (Timeline|TL_MissileRising Play)
        (:Update
          (Transformation|SetRelativeLocation _missilemesh (Math|Vector|MakeVector (.x _relativelocation) (.y _relativelocation) (Math|Float|Lerp (Variables|Animations|GetMissileStartLoc) (Variables|Animations|GetMissileFireLoc) _alpha_2)) false false))
        (:Finished
          (Default|MissileStalled (Variables|References|GetObjectiveManager)))))))

(event Custom|MissileCleared
  (bind _missilemesh (Variables|Default|GetMissileMesh))
  (bind _relativelocation (Variables|/Script/Engine.SceneComponent|GetRelativeLocation _missilemesh))
  (Variables|Animations|SetMissileEndLoc (.z (Variables|/Script/Engine.SceneComponent|GetRelativeLocation (Variables|Default|GetMissileEndPoint))))
  (for _array_element (Utilities|Array|MakeArray (Variables|Default|GetThrusterPoint00) (Variables|Default|GetThrusterPoint01) (Variables|Default|GetThrusterPoint02) (Variables|Default|GetThrusterPoint03))
    (bind _returnvalue (Niagara|SpawnSystemAttached "/Game/DustDevil/Effects/Flamethrower/NS_FlamesCinematic.NS_FlamesCinematic" (Variables|Default|GetMissileMesh) "None" (Variables|/Script/Engine.SceneComponent|GetRelativeLocation _array_element) (Variables|/Script/Engine.SceneComponent|GetRelativeRotation _array_element) "KeepRelativeOffset" false))
    (Utilities|Array|Add (Variables|Particles|GetFlameThrusters) _returnvalue))
  (Utilities|FlowControl|Sequence
    (:then_0
      (bind _alpha (Timeline|TL_MissileFiring PlayFromStart)
        (:Update
          (Transformation|SetRelativeLocation _missilemesh (Math|Vector|MakeVector (.x _relativelocation) (.y _relativelocation) (Math|Float|Lerp (Variables|Animations|GetMissileFireLoc) (Variables|Animations|GetMissileEndLoc) _alpha)) false false))
        (:Finished
          (Development|SetHiddeninGame (Variables|Default|GetMissileMesh) true false)
          (for _array_element_2 (Variables|Particles|GetFlameThrusters)
            (Components|DestroyComponent _array_element_2))
          (Default|BeginLevelTransition (Variables|References|GetObjectiveManager)))))
    (:then_1
      (Default|ObjectiveCompleted (Variables|References|GetObjectiveManager)))
    (:then_2
      (Audio|PlaySoundatLocation "/Game/DustDevil/Objectives/Audio/A_MissileLaunch.A_MissileLaunch" (Transformation|GetActorLocation) "0, 0, 0" 1.0 1.0 0.0 0 0 0 0))))

(event Custom|LaunchCleared)

(event Input|EnhancedActionEvents|EnhancedInputActionIA_HoldInteract_X
  (params (ActionValue :type Boolean) (ElapsedSeconds :type Float%20%28double-precision%29) (TriggeredSeconds :type Float%20%28double-precision%29) (InputAction :type Input%20Action%20Object%20Reference :default "/Game/DustDevil/Core/Inputs/IA_HoldInteract_X.IA_HoldInteract_X"))
  (:Triggered
    (if (and (Rendering|IsVisible (Variables|Default|GetInteractionPrompt)) (Variables|Default|GetbPromptOpen))
      (bind _promptwidget (Variables|References|GetPromptWidget)
        (:then
          (Default|TriggerPrompt _promptwidget)
          (Rendering|SetVisibility (Variables|Default|GetInteractionPrompt) false false)
          (Variables|Default|SetbPromptOpen false)
          (Default|ObjectiveStarted (Variables|References|GetObjectiveManager))
          (Variables|/Game/DustDevil/Objectives/BP_SiloManager_Infestation.BP_SiloManager_Infestation_C|SetbObjStarted (Variables|References|GetObjectiveManager) true))
        (:else))))
  (:Ongoing
    (if (and (Rendering|IsVisible (Variables|Default|GetInteractionPrompt)) (Variables|Default|GetbPromptOpen))
      (bind _promptwidget_2 (Variables|References|GetPromptWidget)
        (:then
          (Default|HoldPrompt _promptwidget_2 ElapsedSeconds))
        (:else))))
  (:Canceled
    (if (and (Rendering|IsVisible (Variables|Default|GetInteractionPrompt)) (Variables|Default|GetbPromptOpen))
      (bind _promptwidget_3 (Variables|References|GetPromptWidget)
        (:then
          (Default|CancelPrompt _promptwidget_3))
        (:else)))))

(event EventBeginPlay
  (CallFunction|GetReferences)
  (CallFunction|InitialiseSilo)
  (CallFunction|SetupInputPrompt))

(fn ConstructionScript)

(fn InitialiseSilo
  (bind _output_get (Variables|Default|SetbObjectiveCompleted (Variables|/Game/DustDevil/Core/Saves/SG_DDSaveData.SG_DDSaveData_C|GetbSiloComplete (Default|GetSaveData (Variables|References|GetGameInstance)))))
  (if _output_get
    (Development|SetHiddeninGame (Variables|Default|GetMissileMesh) true false)
    (Transformation|SetRelativeRotation (Variables|Default|GetHatchMesh) (Math|Rotator|MakeRotator 1.3e+02 0.0 0.0) false false)
    (for _array_element (Actor|GetAllChildActors true)
      (Actor|DestroyActor _array_element))
    (else
      (Variables|Animations|SetHatchStartRotate 0.0)
      (Variables|Animations|SetHatchEndRotate 1.3e+02)
      (Variables|Animations|SetMissileStartLoc (.z (Variables|/Script/Engine.SceneComponent|GetRelativeLocation (Variables|Default|GetMissileStartPoint))))
      (Variables|Animations|SetMissileFireLoc (.z (Variables|/Script/Engine.SceneComponent|GetRelativeLocation (Variables|Default|GetMissileFirePoint))))
      (Transformation|SetRelativeLocation (Variables|Default|GetMissileMesh) (Variables|/Script/Engine.SceneComponent|GetRelativeLocation (Variables|Default|GetMissileStartPoint)) false false)
      (Transformation|SetRelativeRotation (Variables|Default|GetHatchMesh) "0, 0, 0" false false)
      (Utilities|FlowControl|Sequence
        (:then_0
          (for _array_element_2 (Utilities|Array|MakeArray (Variables|Default|GetHiveHatch00) (Variables|Default|GetHiveHatch01) (Variables|Default|GetHiveHatch02) (Variables|Default|GetHiveHatch03) (Variables|Default|GetHiveHatch04) (Variables|Default|GetHiveHatch05) (Variables|Default|GetHiveHatch06) (Variables|Default|GetHiveHatch07))
            (bind _hive (Class|BPIInfestation|GetInfestationSource(Message) (Variables|/Script/Engine.ChildActorComponent|GetChildActor _array_element_2)))
            (Utilities|IsValid _hive
              (:Is%20Valid
                (Variables|/Game/DustDevil/Objectives/BP_ShootableHiveBase.BP_ShootableHiveBase_C|SetObjectiveManager _hive (Variables|References|GetObjectiveManager))
                (Utilities|Array|Add (Variables|References|GetHatchHives) _hive)
                (Variables|/Game/DustDevil/Objectives/BP_ShootableHiveBase.BP_ShootableHiveBase_C|SetbMissileObj _hive true)
                (Variables|/Game/DustDevil/Objectives/BP_ShootableHiveBase.BP_ShootableHiveBase_C|SetHiveLocation _hive "NewEnumerator0"))
              (:Is%20Not%20Valid
                (Development|PrintString "BP_MissileSilo: GetInfestationSource --> Hive is NOT VALID!" true true "(R=1.000000,G=0.029408,B=0.000000,A=1.000000)"))))
          (Variables|/Game/DustDevil/Objectives/BP_SiloManager_Infestation.BP_SiloManager_Infestation_C|SetHatchHives (Variables|References|GetObjectiveManager) (Variables|References|GetHatchHives)))
        (:then_1
          (for _array_element_3 (Utilities|Array|MakeArray (Variables|Default|GetHiveMissile00) (Variables|Default|GetHiveMissile01) (Variables|Default|GetHiveMissile02) (Variables|Default|GetHiveMissile03) (Variables|Default|GetHiveMissile04) (Variables|Default|GetHiveMissile05) (Variables|Default|GetHiveMissile06) (Variables|Default|GetHiveMissile07) (Variables|Default|GetHiveMissile08))
            (bind _hive_2 (Class|BPIInfestation|GetInfestationSource(Message) (Variables|/Script/Engine.ChildActorComponent|GetChildActor _array_element_3)))
            (Utilities|IsValid _hive_2
              (:Is%20Valid
                (Variables|/Game/DustDevil/Objectives/BP_ShootableHiveBase.BP_ShootableHiveBase_C|SetObjectiveManager _hive_2 (Variables|References|GetObjectiveManager))
                (Utilities|Array|Add (Variables|References|GetMissileHives) _hive_2)
                (Variables|/Game/DustDevil/Objectives/BP_ShootableHiveBase.BP_ShootableHiveBase_C|SetbMissileObj _hive_2 true)
                (Variables|/Game/DustDevil/Objectives/BP_ShootableHiveBase.BP_ShootableHiveBase_C|SetHiveLocation _hive_2 "NewEnumerator1"))
              (:Is%20Not%20Valid
                (Development|PrintString "BP_MissileSilo: GetInfestationSource --> Hive is NOT VALID!" true true "(R=1.000000,G=0.029408,B=0.000000,A=1.000000)"))))
          (Variables|/Game/DustDevil/Objectives/BP_SiloManager_Infestation.BP_SiloManager_Infestation_C|SetMissileHives (Variables|References|GetObjectiveManager) (Variables|References|GetMissileHives)))
        (:then_2
          (for _array_element_4 (Actor|GetAllChildActors true)
            (bind _hive_3 (Class|BPIInfestation|GetInfestationSource(Message) _array_element_4))
            (Utilities|IsValid _hive_3
              (:Is%20Valid
                (Collision|SetCollisionEnabled (Variables|/Game/DustDevil/Objectives/BP_ShootableHiveBase.BP_ShootableHiveBase_C|GetHitbox _hive_3) "NoCollision")))))))))

(fn SetupInputPrompt
  (if (Variables|/Game/DustDevil/Core/GI_DDPrototype.GI_DDPrototype_C|GetbUsingController (Variables|References|GetGameInstance))
    (Default|SetInputType (Variables|References|GetPromptWidget) "NewEnumerator2" "E" "" false "" "Begin missile launch")
    (else
      (Default|SetInputType (Variables|References|GetPromptWidget) "NewEnumerator0" "E" "16px" false "" "Begin missile launch"))))

(fn GetReferences
  (bind _asgi_ddprototype (Utilities|Casting|CastToGI_DDPrototype (Game|GetGameInstance))
    (:then
      (Variables|References|SetGameInstance _asgi_ddprototype))
    (:CastFailed
      _))
  (bind _aswbp_prompt_hold_text (Utilities|Casting|CastToWBP_PromptHoldText (UserInterface|GetUserWidgetObject (Variables|Default|GetInteractionPrompt)))
    (:then
      (Variables|References|SetPromptWidget _aswbp_prompt_hold_text))
    (:CastFailed
      _))
  (bind _aswbp_screen_marker (Utilities|Casting|CastToWBP_ScreenMarker (UserInterface|GetWidget (Variables|Default|GetObjectivePointer)))
    (:then
      (Default|SetMarkerProperties _aswbp_screen_marker "/Game/DustDevil/UI/Textures/HUD/T_UI_Minimap_MissileSilo.T_UI_Minimap_MissileSilo" "(R=0.109462,G=0.130136,B=0.031896,A=1.000000)" 4e+01 4e+01))
    (:CastFailed
      (Development|PrintString "cast failed!"))))