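; Manager for the missile silo infestation objective, coordinating the launch, hive-clearing stages, HUD and save flag.
; Starting it plays music, begins the launch, spawns boundary walls and activates tagged silo spawners.
; Hatch and missile stalls enable hive hitboxes; destroyed hives update the counter, and the last notifies MissileSilo.
; Completion removes walls and saves progress; a separate event fades into the WastelandEscape level, with debug keys for testing.
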(event OnComponentBeginOverlap(ObjectiveTrigger)
  (params (OverlappedComponent :type Primitive%20Component%20Object%20Reference) (OtherActor :type Actor%20Object%20Reference) (OtherComp :type Primitive%20Component%20Object%20Reference) (OtherBodyIndex :type Integer) (bFromSweep :type Boolean) (SweepResult :type Hit%20Result%20Structure%20%28by%20ref%29))
  (if (Utilities|DoesObjectImplementInterface OtherActor "/Game/DustDevil/Core/Interfaces/BPI_PlayerTrigger.BPI_PlayerTrigger_C")
    (bind _player (Class|BPIPlayerTrigger|GetPlayerCharacter(Message) OtherActor))
    (bind _output_get (Variables|References|SetPlayer _player))
    (Utilities|FlowControl|Sequence
      (:then_1
        (if (and (Variables|Bools|GetbObjAdded) (not (Variables|Bools|GetbObjStarted)))
          (Widget|SetVisibility (Variables|/Game/DustDevil/UI/HUD/WBP_HUD.WBP_HUD_C|GetWBP_NucFuelMeter (Variables|/Game/DustDevil/Player/BP_Vehicle.BP_Vehicle_C|GetHUD _output_get)) "SelfHitTestInvisible"))))))

(event OnComponentEndOverlap(ObjectiveTrigger)
  (params (OverlappedComponent :type Primitive%20Component%20Object%20Reference) (OtherActor :type Actor%20Object%20Reference) (OtherComp :type Primitive%20Component%20Object%20Reference) (OtherBodyIndex :type Integer))
  (if (Utilities|DoesObjectImplementInterface OtherActor "/Game/DustDevil/Core/Interfaces/BPI_PlayerTrigger.BPI_PlayerTrigger_C")
    (if (Variables|Bools|GetbObjAdded)
      (Widget|SetVisibility (Variables|/Game/DustDevil/UI/HUD/WBP_HUD.WBP_HUD_C|GetWBP_NucFuelMeter (Variables|/Game/DustDevil/Player/BP_Vehicle.BP_Vehicle_C|GetHUD (Variables|References|GetPlayer))) "SelfHitTestInvisible"))))

(event Custom|ObjectiveStarted
  (Default|ObjectiveStarted (Variables|References|GetAudioManager))
  (bind _returnvalue (Audio|SpawnSound2D (Variables|Audio|GetSiloMusicBase) 1.0 1.0 0.0 0))
  (bind _output_get (Variables|Audio|SetSiloMusic _returnvalue))
  (Audio|Components|Audio|FadeIn _output_get 1.0 1.0 0.0 "Linear" :!class /Script/Engine.AudioComponent)
  (Default|BeginMissileLaunch (Variables|References|GetMissileSilo))
  (CallFunction|SpawnObjBoundaries)
  (Class|BPIHUDUpdates|ClearObjectiveMain(Message) (Variables|/Game/DustDevil/Player/BP_Vehicle.BP_Vehicle_C|GetHUD (Variables|References|GetPlayer)))
  (bind _output_get_2 (Variables|Default|SetHatchHivesNum (Utilities|Array|Length (Variables|References|GetHatchHives))))
  (Variables|Default|SetHatchHivesTotal _output_get_2)
  (bind _output_get_3 (Variables|Default|SetMissileHivesNum (Utilities|Array|Length (Variables|References|GetMissileHives))))
  (Variables|Default|SetMissileHivesTotal _output_get_3)
  (Default|UpdateNucMatsBar (Variables|/Game/DustDevil/Player/BP_Vehicle.BP_Vehicle_C|GetHUD (Variables|References|GetPlayer)) false)
  (Utilities|FlowControl|Sequence
    (:then_0
      (bind _outactors (Actor|GetAllActorsOfClasswithTag "/Game/DustDevil/Characters/Enemies/Spawners/BP_FESpawner.BP_FESpawner_C" "Spawner.Silo"))
      (for _array_element _outactors
        (Variables|/Game/DustDevil/Characters/Enemies/Spawners/BP_FESpawner.BP_FESpawner_C|SetbIsActive _array_element true)))
    (:then_1
      (bind _outactors_2 (Actor|GetAllActorsOfClasswithTag "/Game/DustDevil/Characters/Enemies/Spawners/BP_FESpawnerRepeating.BP_FESpawnerRepeating_C" "Spawner.Silo"))
      (for _array_element_2 _outactors_2
        (Variables|/Game/DustDevil/Characters/Enemies/Spawners/BP_FESpawnerRepeating.BP_FESpawnerRepeating_C|SetbIsActive _array_element_2 true)))
    (:then_2
      (bind _outactors_3 (Actor|GetAllActorsOfClasswithTag "/Game/DustDevil/Characters/Enemies/Spawners/BP_MBSpawner.BP_MBSpawner_C" "Spawner.Silo"))
      (for _array_element_3 _outactors_3
        (Variables|/Game/DustDevil/Characters/Enemies/Spawners/BP_MBSpawner.BP_MBSpawner_C|SetbActive _array_element_3 true)))
    (:then_3
      (bind _outactors_4 (Actor|GetAllActorsOfClasswithTag "/Game/DustDevil/Characters/Enemies/Spawners/BP_MBSpawnerRepeating.BP_MBSpawnerRepeating_C" "Spawner.Silo"))
      (for _array_element_4 _outactors_4
        (Variables|/Game/DustDevil/Characters/Enemies/Spawners/BP_MBSpawnerRepeating.BP_MBSpawnerRepeating_C|SetbIsActive _array_element_4 true)))))

(event Custom|Objective%20Completed
  (Variables|Bools|SetbObjCompleted true)
  (CallFunction|RemoveObjBoundaries)
  (Variables|/Game/DustDevil/Core/Saves/SG_DDSaveData.SG_DDSaveData_C|SetbSiloComplete (Variables|References|GetSaveData) true))

(event Custom|BeginLevelTransition
  (bind _returnvalue (UserInterface|CreateWidget "/Game/DustDevil/UI/CustomisationMenu/WBP_FadeIn.WBP_FadeIn_C" (Game|GetPlayerController 0)))
  (UserInterface|Viewport|AddtoViewport _returnvalue 3)
  (Utilities|FlowControl|Delay 2.0)
  (Game|OpenLevel(byName) "L_WastelandEscape_WP"))

(event EventBeginPlay
  (bind _asgi_ddprototype (Utilities|Casting|CastToGI_DDPrototype (Game|GetGameInstance)))
  (Variables|References|SetSaveData (Default|GetSaveData _asgi_ddprototype)))

(event Input|KeyboardEvents|DebugKeyO
  (params (Key :type Key%20Structure :default "None") (ActionValue :type Input%20Action%20Value%20Structure))
  ;[0.2433 0.07432 1] DEBUGGING
  (:Pressed
    (CallFunction|SpawnObjBoundaries)))

(event Input|KeyboardEvents|DebugKeyL
  (params (Key :type Key%20Structure :default "None") (ActionValue :type Input%20Action%20Value%20Structure))
  ;[0.2433 0.07432 1] DEBUGGING
  (:Pressed
    (CallFunction|ObjectiveStarted)))

(event Input|KeyboardEvents|DebugKeyB
  (params (Key :type Key%20Structure :default "None") (ActionValue :type Input%20Action%20Value%20Structure))
  (:Pressed
    (bind _returnvalue (UserInterface|CreateWidget "/Game/DustDevil/UI/CustomisationMenu/WBP_FadeIn.WBP_FadeIn_C" (Game|GetPlayerController 0)))
    (UserInterface|Viewport|AddtoViewport _returnvalue 3)
    (Utilities|FlowControl|Delay 2.0)
    (Game|OpenLevel(byName) "L_WastelandEscape_WP")))

(event Input|KeyboardEvents|L
  (params (Key :type Key%20Structure :default "None"))
  ;[0.2433 0.07432 1] DEBUGGING
  (:Pressed
    (CallFunction|ObjectiveStarted)))

(fn ConstructionScript)

(fn SpawnObjBoundaries
  (for _array_element (Variables|References|GetBoundarySpawnPoints)
    (bind _returnvalue (Game|SpawnActorfromClass "/Game/DustDevil/Objectives/BP_ObjectivesBoundary.BP_ObjectivesBoundary_C" (Math|Transform|MakeTransform (Transformation|GetActorLocation _array_element) (Transformation|GetActorRotation _array_element) "1.000000,1.000000,1.000000") "Undefined" "MultiplyWithRoot" 0 0))
    (Utilities|Array|Add (Variables|References|GetBoundaryWalls) _returnvalue)))

(fn RemoveObjBoundaries
  (for _array_element (Variables|References|GetBoundaryWalls)
    (Actor|DestroyActor _array_element)))

(fn HiveDestroyed
  (params (HiveLocation :type E_SiloHives%20Enum :default "NewEnumerator0"))
  (switch Utilities|FlowControl|Switch|SwitchonE_SiloHives HiveLocation
    (:NewEnumerator0
      (bind _result (Math|Integer|DecrementInt (Variables|Default|GetHatchHivesNum))
        (:%20%20
          (if (== _result 0)
            (Default|HatchCleared (Variables|References|GetMissileSilo))
            (Class|BPIHUDUpdates|ClearObjectiveMain(Message) (Variables|/Game/DustDevil/Player/BP_Vehicle.BP_Vehicle_C|GetHUD (Variables|References|GetPlayer)))
            (else
              (bind _result_2 (Math|Integer|IncrementInt (Variables|Default|GetHatchHivesDestroyed))
                (:%20%20
                  (Class|BPIHUDUpdates|UpdateObjectiveMain(Message) (Variables|/Game/DustDevil/Player/BP_Vehicle.BP_Vehicle_C|GetHUD (Variables|References|GetPlayer)) (Utilities|String|Append "Destroy the hives " (Utilities|String|ToString(Integer) _result_2) "/" (Utilities|String|ToString(Integer) (Variables|Default|GetHatchHivesTotal)))))))))))
    (:NewEnumerator1
      (bind _result_3 (Math|Integer|DecrementInt (Variables|Default|GetMissileHivesNum))
        (:%20%20
          (if (== _result_3 0)
            (Default|MissileCleared (Variables|References|GetMissileSilo))
            (Class|BPIHUDUpdates|ClearObjectiveMain(Message) (Variables|/Game/DustDevil/Player/BP_Vehicle.BP_Vehicle_C|GetHUD (Variables|References|GetPlayer)))
            (else
              (bind _result_4 (Math|Integer|IncrementInt (Variables|Default|GetMissileHivesDestroyed))
                (:%20%20
                  (Class|BPIHUDUpdates|UpdateObjectiveMain(Message) (Variables|/Game/DustDevil/Player/BP_Vehicle.BP_Vehicle_C|GetHUD (Variables|References|GetPlayer)) (Utilities|String|Append "Destroy the hives " (Utilities|String|ToString(Integer) _result_4) "/" (Utilities|String|ToString(Integer) (Variables|Default|GetMissileHivesTotal)))))))))))))

(fn HatchStalled
  (Class|BPIHUDUpdates|AddNewObjectiveMain(Message) (Variables|/Game/DustDevil/Player/BP_Vehicle.BP_Vehicle_C|GetHUD (Variables|References|GetPlayer)) (Utilities|String|Append "Destroy the hives " "0" "/" (Utilities|String|ToString(Integer) (Variables|Default|GetHatchHivesTotal))))
  (for _array_element (Variables|References|GetHatchHives)
    (Collision|SetCollisionEnabled (Variables|/Game/DustDevil/Objectives/BP_ShootableHiveBase.BP_ShootableHiveBase_C|GetHitbox _array_element) "QueryOnly")))

(fn MissileStalled
  (Class|BPIHUDUpdates|AddNewObjectiveMain(Message) (Variables|/Game/DustDevil/Player/BP_Vehicle.BP_Vehicle_C|GetHUD (Variables|References|GetPlayer)) (Utilities|String|Append "Destroy the hives " "0" "/" (Utilities|String|ToString(Integer) (Variables|Default|GetMissileHivesTotal))))
  (for _array_element (Variables|References|GetMissileHives)
    (Collision|SetCollisionEnabled (Variables|/Game/DustDevil/Objectives/BP_ShootableHiveBase.BP_ShootableHiveBase_C|GetHitbox _array_element) "QueryOnly")))