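; BP_ObjectivesBoundary is a sandstorm boundary that warns players away from the edge of an objective area.
; Two trigger volumes react only to actors implementing BPI_PlayerTrigger.
; VisibilityTrigger shows the Sandstorm component on entry and hides it on exit.
; MessageTrigger shows a dust storm warning on the player's HUD and fades sandstorm audio in, then fades it out on exit.
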(event OnComponentBeginOverlap(MessageTrigger)
  (params (OverlappedComponent :type Primitive%20Component%20Object%20Reference) (OtherActor :type Actor%20Object%20Reference) (OtherComp :type Primitive%20Component%20Object%20Reference) (OtherBodyIndex :type Integer) (bFromSweep :type Boolean) (SweepResult :type Hit%20Result%20Structure%20%28by%20ref%29))
  (if (Utilities|DoesObjectImplementInterface OtherActor "/Game/DustDevil/Core/Interfaces/BPI_PlayerTrigger.BPI_PlayerTrigger_C")
    (bind _player (Class|BPIPlayerTrigger|GetPlayerCharacter(Message) OtherActor))
    (bind _hud (Variables|/Game/DustDevil/Player/BP_Vehicle.BP_Vehicle_C|GetHUD _player)
      (:then
        (Class|BPIHUDUpdates|DisplayWarningMessage(Message) _hud "The dust storm is too intense!")
        (bind _sandstormsfx (Variables|Default|GetSandstormSFX)
          (:then
            (Audio|Components|Audio|FadeIn _sandstormsfx 2.0 1.0 0.0 "Linear" :!class /Script/Engine.AudioComponent))
          (:else)))
      (:else))))

(event OnComponentEndOverlap(MessageTrigger)
  (params (OverlappedComponent :type Primitive%20Component%20Object%20Reference) (OtherActor :type Actor%20Object%20Reference) (OtherComp :type Primitive%20Component%20Object%20Reference) (OtherBodyIndex :type Integer))
  (if (Utilities|DoesObjectImplementInterface OtherActor "/Game/DustDevil/Core/Interfaces/BPI_PlayerTrigger.BPI_PlayerTrigger_C")
    (bind _sandstormsfx (Variables|Default|GetSandstormSFX)
      (:then
        (Audio|Components|Audio|FadeOut _sandstormsfx 2.0 0.0 "Linear" :!class /Script/Engine.AudioComponent))
      (:else))))

(event OnComponentBeginOverlap(VisibilityTrigger)
  (params (OverlappedComponent :type Primitive%20Component%20Object%20Reference) (OtherActor :type Actor%20Object%20Reference) (OtherComp :type Primitive%20Component%20Object%20Reference) (OtherBodyIndex :type Integer) (bFromSweep :type Boolean) (SweepResult :type Hit%20Result%20Structure%20%28by%20ref%29))
  (if (Utilities|DoesObjectImplementInterface OtherActor "/Game/DustDevil/Core/Interfaces/BPI_PlayerTrigger.BPI_PlayerTrigger_C")
    (Development|SetHiddeninGame (Variables|Default|GetSandstorm) false false)))

(event OnComponentEndOverlap(VisibilityTrigger)
  (params (OverlappedComponent :type Primitive%20Component%20Object%20Reference) (OtherActor :type Actor%20Object%20Reference) (OtherComp :type Primitive%20Component%20Object%20Reference) (OtherBodyIndex :type Integer))
  (if (Utilities|DoesObjectImplementInterface OtherActor "/Game/DustDevil/Core/Interfaces/BPI_PlayerTrigger.BPI_PlayerTrigger_C")
    (Development|SetHiddeninGame (Variables|Default|GetSandstorm) true false)))

(fn ConstructionScript)