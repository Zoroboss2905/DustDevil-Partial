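; Cinematic car actor for DustDevil that spins its wheels and can swap its parts for alternate meshes.
; Tick rotates all four wheels on local pitch by WheelSpinning scaled by delta time.
; The ChangeMesh event replaces the engine, bumper, tank, gun and only the left-side wheels with their New mesh variables.
; Nothing in this graph triggers ChangeMesh, as its only call node is disconnected.
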(event Custom|ChangeMesh
  (Utilities|FlowControl|Sequence
    (:then_0
      (Components|StaticMesh|SetStaticMesh (Variables|Default|GetEngine) (Variables|Default|GetNewEngine)))
    (:then_1
      (Components|StaticMesh|SetStaticMesh (Variables|Default|GetBumper) (Variables|Default|GetNewBumper)))
    (:then_2
      (Components|StaticMesh|SetStaticMesh (Variables|Default|GetTank) (Variables|Default|GetNewTank)))
    (:then_3
      (Components|StaticMesh|SetStaticMesh (Variables|Default|GetGun) (Variables|Default|GetNewGun)))
    (:then_4
      (Components|StaticMesh|SetStaticMesh (Variables|Default|GetFrontWheelLeft) (Variables|Default|GetNewWheel)))
    (:then_5
      (Components|StaticMesh|SetStaticMesh (Variables|Default|GetBackWheelLeft) (Variables|Default|GetNewWheel)))))

(event Collision|EventActorBeginOverlap
  (params (OtherActor :type Actor%20Object%20Reference)))

(event EventTick
  (params (DeltaSeconds :type Float%20%28single-precision%29))
  (Transformation|AddLocalRotation (Variables|Default|GetFrontWheelRight) (Math|Rotator|MakeRotator 0.0 (* DeltaSeconds (Variables|Default|GetWheelSpinning)) 0.0) false false))

(event EventBeginPlay)

(fn ConstructionScript)