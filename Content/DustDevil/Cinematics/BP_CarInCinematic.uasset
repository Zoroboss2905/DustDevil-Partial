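; BP_CarInCinematic is a car actor used in cinematics, with animated wheels and flame effects.
; Each tick it pitches the four wheel components by a WheelSpinning rate scaled by delta time.
; The PlayFlames event spawns the NS_FlamesCinematicTwo Niagara system attached at four flame anchor components on the car.
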(event Custom|PlayFlames
  (Niagara|SpawnSystemAttached "/Game/DustDevil/Effects/Flamethrower/NS_FlamesCinematicTwo.NS_FlamesCinematicTwo" (Variables|Default|GetNS_FlamesCinematic) "None" "0, 0, 0" "0, 0, 0" "KeepRelativeOffset" false)
  (Niagara|SpawnSystemAttached "/Game/DustDevil/Effects/Flamethrower/NS_FlamesCinematicTwo.NS_FlamesCinematicTwo" (Variables|Default|GetNS_FlamesCinematic1) "None" "0, 0, 0" "0, 0, 0" "KeepRelativeOffset" false)
  (Niagara|SpawnSystemAttached "/Game/DustDevil/Effects/Flamethrower/NS_FlamesCinematicTwo.NS_FlamesCinematicTwo" (Variables|Default|GetNS_FlamesCinematic3) "None" "0, 0, 0" "0, 0, 0" "KeepRelativeOffset" false)
  (Niagara|SpawnSystemAttached "/Game/DustDevil/Effects/Flamethrower/NS_FlamesCinematicTwo.NS_FlamesCinematicTwo" (Variables|Default|GetNS_FlamesCinematic2) "None" "0, 0, 0" "0, 0, 0" "KeepRelativeOffset" false))

(event EventBeginPlay)

(event Collision|EventActorBeginOverlap
  (params (OtherActor :type Actor%20Object%20Reference)))

(event EventTick
  (params (DeltaSeconds :type Float%20%28single-precision%29))
  (Transformation|AddLocalRotation (Variables|Default|GetFrontWheelRight) (Math|Rotator|MakeRotator 0.0 (* DeltaSeconds (Variables|Default|GetWheelSpinning)) 0.0) false false))

(fn ConstructionScript)