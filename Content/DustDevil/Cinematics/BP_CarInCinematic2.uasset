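; BP_CarInCinematic2 is a car actor for a Dust Devil cinematic, with four wheels that spin continuously.
; Tick adds local pitch rotation to each wheel, scaled by DeltaSeconds and the WheelSpinning rate.
; BeginPlay calls PlayFlames, but that event is empty: the four Niagara flame spawns attached to the NSFlamesCinematic components are disconnected and never run.
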(event Custom|PlayFlames)

(event EventBeginPlay
  (CallFunction|PlayFlames))

(event Collision|EventActorBeginOverlap
  (params (OtherActor :type Actor%20Object%20Reference)))

(event EventTick
  (params (DeltaSeconds :type Float%20%28single-precision%29))
  (Transformation|AddLocalRotation (Variables|Default|GetFrontWheelRight) (Math|Rotator|MakeRotator 0.0 (* DeltaSeconds (Variables|Default|GetWheelSpinning)) 0.0) false false))

(fn ConstructionScript)