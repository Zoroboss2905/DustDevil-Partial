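; Biomass item drop that grants bio fuel to an overlapping actor implementing BPI_Pickups.
; On overlap it scales its amount by a player attribute, applies GE_PickupLoot through GAS set-by-caller magnitudes, plays a sound, messages the player and destroys itself.
; It toggles radial-force response around a short spawn delay for vacuuming and clamps extreme physics velocity on Tick.
; CheckIfVacuumable, which disables pickup at max biomass, is not called here.
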(event OnComponentBeginOverlap(SphereCollision)
  (params (OverlappedComponent :type Primitive%20Component%20Object%20Reference) (OtherActor :type Actor%20Object%20Reference) (OtherComp :type Primitive%20Component%20Object%20Reference) (OtherBodyIndex :type Integer) (bFromSweep :type Boolean) (SweepResult :type Hit%20Result%20Structure%20%28by%20ref%29))
  ;[0.02956 0.02956 0.02956] When picked up, transfers ONLY enough biomass to player and then modifies own value, then destroys self if needed
  (if (Utilities|DoesObjectImplementInterface OtherActor "/Game/DustDevil/Core/Interfaces/BPI_Pickups.BPI_Pickups_C")
    (CallFunction|GivePlayerBiomass OtherActor)))

(event EventBeginPlay
  (bind _player (Class|BPIPlayerTrigger|GetPlayerCharacter(Message) (Game|Player|GetPlayerPawn 0)))
  (Variables|Default|SetPlayer _player)
  (CallFunction|SetVacuumable true)
  (Utilities|FlowControl|Delay 0.5)
  (CallFunction|SetVacuumable (Variables|Default|GetOff)))

(event EventTick
  (params (DeltaSeconds :type Float%20%28single-precision%29))
  (bind _mesh (Variables|Default|GetMesh))
  (bind _returnvalue (Transformation|GetComponentVelocity _mesh))
  (if (> (Math|Vector|VectorLength _returnvalue) 1e+04)
    (Class|PrimitiveComponent|SetAllPhysicsLinearVelocity (Variables|Default|GetMesh) (* (Math|Vector|Normalize _returnvalue) 8e+03) false)))

(fn ConstructionScript)

(fn CheckifVacuumable
  (bind _mesh (Variables|Default|GetMesh))
  (bind _mesh_2 (Variables|Default|GetMesh))
  (bind _spherecollision (Variables|Default|GetSphereCollision))
  (bind _spherecollision_2 (Variables|Default|GetSphereCollision))
  (if (Variables|/Game/DustDevil/Player/BP_Vehicle.BP_Vehicle_C|GetbAtMaxBiomass (Variables|Default|GetPlayer))
    (Variables|/Script/Engine.PrimitiveComponent|SetbIgnoreRadialForce _mesh true)
    (Variables|/Script/Engine.PrimitiveComponent|SetbIgnoreRadialImpulse _mesh true)
    (Variables|/Script/Engine.PrimitiveComponent|SetbIgnoreRadialForce _spherecollision true)
    (Variables|/Script/Engine.PrimitiveComponent|SetbIgnoreRadialImpulse _spherecollision true)
    (Collision|SetCollisionEnabled (Variables|Default|GetSphereCollision) "NoCollision")
    (else
      (Variables|/Script/Engine.PrimitiveComponent|SetbIgnoreRadialForce _mesh_2 false)
      (Variables|/Script/Engine.PrimitiveComponent|SetbIgnoreRadialImpulse _mesh_2 false)
      (Variables|/Script/Engine.PrimitiveComponent|SetbIgnoreRadialForce _spherecollision_2 false)
      (Variables|/Script/Engine.PrimitiveComponent|SetbIgnoreRadialImpulse _spherecollision_2 false)
      (Collision|SetCollisionEnabled (Variables|Default|GetSphereCollision) "QueryOnly"))))

(fn GivePlayerBiomass
  (params (Player :type Actor%20Object%20Reference))
  (bind _returnvalue (Ability|GetAbilitySystemComponent Player))
  (bind _biomassamount (Variables|Default|GetBiomassAmount))
  (bind _returnvalue_2 (Class|AbilitySystemComponent|GetGameplayAttributeValue _returnvalue "(AttributeName=\"TankConvertBonus\",Attribute=/Script/DustDevil.VehicleAttributeSet:TankConvertBonus,AttributeOwner=\"/Script/CoreUObject.Class'/Script/DustDevil.VehicleAttributeSet'\")"))
  (bind _returnvalue_3 (* _biomassamount _returnvalue_2))
  (bind _returnvalue_4 (Math|Float|Truncate _returnvalue_3))
  (bind _returnvalue_5 (Ability|GameplayEffect|AssignTagSetbyCallerMagnitude (GameplayEffects|MakeOutgoingSpec :self _returnvalue :GameplayEffectClass "/Game/DustDevil/Core/GAS/Effects/GE_PickupLoot.GE_PickupLoot_C") "(TagName=\"Stats.Vehicle.BioFuel\")" (Math|Conversions|ToFloat(Integer) _returnvalue_4)))
  (bind _returnvalue_6 (Ability|GameplayEffect|AssignTagSetbyCallerMagnitude _returnvalue_5 "(TagName=\"Stats.Base.NuclearMatter\")" 0.0))
  (bind _returnvalue_7 (Ability|GameplayEffect|AssignTagSetbyCallerMagnitude _returnvalue_6 "(TagName=\"Stats.Vehicle.Chitin\")" 0.0))
  (GameplayEffects|ApplyGameplayEffectSpecToSelf _returnvalue _returnvalue_7)
  (Audio|PlaySound2D "/Game/DustDevil/Audio/Feedback/A_ItemPickup.A_ItemPickup" 1.0 1.0 0.0 0 0)
  (Class|BPIPickups|PickupBiomatter(Message) Player _returnvalue_4 (- _returnvalue_4 (Variables|Default|GetBiomassAmount))) ; Replace with Gameplay Cue Later
  (Actor|DestroyActor))

(fn SetVacuumable
  (params (bOff :type Boolean))
  (bind _mesh (Variables|Default|GetMesh))
  (bind _mesh_2 (Variables|Default|GetMesh))
  (bind _spherecollision (Variables|Default|GetSphereCollision))
  (bind _spherecollision_2 (Variables|Default|GetSphereCollision))
  (if bOff
    (Variables|/Script/Engine.PrimitiveComponent|SetbIgnoreRadialForce _mesh true)
    (Variables|/Script/Engine.PrimitiveComponent|SetbIgnoreRadialImpulse _mesh true)
    (Variables|/Script/Engine.PrimitiveComponent|SetbIgnoreRadialForce _spherecollision true)
    (Variables|/Script/Engine.PrimitiveComponent|SetbIgnoreRadialImpulse _spherecollision true)
    (Collision|SetCollisionEnabled (Variables|Default|GetSphereCollision) "QueryOnly")
    (else
      (Variables|/Script/Engine.PrimitiveComponent|SetbIgnoreRadialForce _mesh_2 false)
      (Variables|/Script/Engine.PrimitiveComponent|SetbIgnoreRadialImpulse _mesh_2 false)
      (Variables|/Script/Engine.PrimitiveComponent|SetbIgnoreRadialForce _spherecollision_2 false)
      (Variables|/Script/Engine.PrimitiveComponent|SetbIgnoreRadialImpulse _spherecollision_2 false)
      (Collision|SetCollisionEnabled (Variables|Default|GetSphereCollision) "QueryOnly"))))