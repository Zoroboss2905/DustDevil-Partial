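; Radiation barrel physics-foliage actor that can randomise its own transform when play begins.
; When RandomiseTransform is set, BeginPlay calls SetRandomTransform, which keeps world X and Y but applies random rotation and per-axis, non-uniform scale.
; Height ignores the placed Z, landing at an absolute world value just below a fixed level.
; The construction script only calls its parent.
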(event EventBeginPlay
  (if (Variables|Default|GetbRandomiseTransform)
    (CallFunction|SetRandomTransform)))

(fn ConstructionScript
  (|CallParentFunction))

(fn SetRandomTransform
  (bind _returnvalue (Math|Random|RandomFloatinRange -9e+01 9e+01))
  (bind _returnvalue_2 (Math|Random|RandomFloatinRange 0.8 1.2))
  (bind _returnvalue_3 (Transformation|GetActorLocation))
  (Transformation|SetActorTransform (Math|Transform|MakeTransform (Math|Vector|MakeVector (.x _returnvalue_3) (.y _returnvalue_3) (- 1e+02 (Math|Random|RandomFloatinRange 1e+01 1.0))) (Math|Rotator|MakeRotator _returnvalue _returnvalue (Math|Random|RandomFloatinRange -1.8e+02 1.8e+02)) (Math|Vector|MakeVector _returnvalue_2 _returnvalue_2 _returnvalue_2))))