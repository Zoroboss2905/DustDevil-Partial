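; Dead tree foliage Blueprint, named as destructible, that randomizes the look of its static mesh when play begins.
; BeginPlay calls SetRandomTransform, which gives the mesh an independent scale per axis, a slight random tilt with any yaw, and a random downward Z offset.
; The construction script only calls the parent, and this file contains no destruction logic.
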(event EventBeginPlay
  (CallFunction|SetRandomTransform))

(fn ConstructionScript
  (|CallParentFunction))

(fn SetRandomTransform
  (bind _returnvalue (Math|Random|RandomFloatinRange 4.0 6.0))
  (bind _staticmesh (Variables|Default|GetStaticMesh))
  (bind _relativelocation (Variables|/Script/Engine.SceneComponent|GetRelativeLocation _staticmesh))
  (Transformation|SetRelativeScale3D (Variables|Default|GetStaticMesh) (Math|Vector|MakeVector _returnvalue _returnvalue _returnvalue))
  (Transformation|SetRelativeRotation (Variables|Default|GetStaticMesh) (Math|Rotator|MakeRotator (Math|Random|RandomFloatinRange -15.0 15.0) (Math|Random|RandomFloatinRange -15.0 15.0) (Math|Random|RandomFloatinRange -1.8e+02 1.8e+02)) false false)
  (Transformation|SetRelativeLocation _staticmesh (Math|Vector|MakeVector (.x _relativelocation) (.y _relativelocation) (Math|Random|RandomFloatinRange -4e+01 0.0)) false false))