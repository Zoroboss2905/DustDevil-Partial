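; Base physics foliage actor that gets knocked loose and destroyed when a player overlaps its sphere trigger.
; Overlappers implementing BPI_PlayerTrigger make the Cube simulate physics, ignore Pawn collision and take an impulse from player velocity plus a strong upward boost.
; An impact particle system and sound play through a DoOnce that resets after a short delay.
; After TimeToDestroy, a destroy effect spawns on the sphere and the actor removes itself shortly afterward.
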(event OnComponentBeginOverlap(Sphere)
  (params (OverlappedComponent :type Primitive%20Component%20Object%20Reference) (OtherActor :type Actor%20Object%20Reference) (OtherComp :type Primitive%20Component%20Object%20Reference) (OtherBodyIndex :type Integer) (bFromSweep :type Boolean) (SweepResult :type Hit%20Result%20Structure%20%28by%20ref%29))
  (if (Utilities|DoesObjectImplementInterface OtherActor "/Game/DustDevil/Core/Interfaces/BPI_PlayerTrigger.BPI_PlayerTrigger_C")
    (bind _player (Class|BPIPlayerTrigger|GetPlayerCharacter(Message) OtherActor))
    (bind _output_get (Variables|Default|SetPlayer _player))
    (Physics|SetSimulatePhysics (Variables|Default|GetCube) true)
    (Physics|AddImpulse (Variables|Default|GetCube) (Math|Vector|MakeVector (.x (Transformation|GetVelocity _output_get)) (.y (Transformation|GetVelocity _output_get)) (+ (.z (Transformation|GetVelocity _output_get)) 1e+04)) "None" false)
    (Collision|SetCollisionResponsetoChannel (Variables|Default|GetCube) "ECC_Pawn" "ECR_Ignore")
    (Utilities|FlowControl|Sequence
      (:then_0
        (Utilities|FlowControl|Delay (Variables|Default|GetTimeToDestroy))
        (Niagara|SpawnSystemAttached (Variables|Default|GetDestroyEffect) (Variables|Default|GetSphere) "None" "0, 0, 0" "0, 0, 0" "KeepRelativeOffset" false)
        (Utilities|FlowControl|Delay 0.175)
        (Actor|DestroyActor))
      (:then_2
        (Utilities|FlowControl|DoOnce false :!label _label
          (:Completed
            (Niagara|SpawnSystematLocation (Variables|Default|GetParticleSystem) (Transformation|GetWorldLocation (Variables|Default|GetCube)) (Transformation|GetActorRotation (Variables|Default|GetPlayer)))
            (Audio|PlaySoundatLocation (Variables|Audio|GetImpactSFX) (Transformation|GetActorLocation) "0, 0, 0" 1.0 1.0 0.0 0 (Variables|Audio|GetImpactConcurrency) 0 0)
            (Utilities|FlowControl|Delay 0.25)
            (goto _label Reset)))))))

(fn ConstructionScript)