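; BP_DestructFoliageBaseTwo is a foliage actor that breaks apart when the player overlaps it.
; On overlap, it filters for actors implementing BPI_PlayerTrigger and retrieves the player character through that interface.
; It plays an impact sound with concurrency settings and spawns a particle system at the mesh location, oriented to the player's rotation.
; The actor then waits one tick and destroys itself.
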(event Collision|EventActorBeginOverlap
  (params (OtherActor :type Actor%20Object%20Reference))
  (if (Utilities|DoesObjectImplementInterface OtherActor "/Game/DustDevil/Core/Interfaces/BPI_PlayerTrigger.BPI_PlayerTrigger_C")
    (bind _player (Class|BPIPlayerTrigger|GetPlayerCharacter(Message) OtherActor))
    (Variables|Default|SetPlayer _player)
    (Utilities|FlowControl|Sequence
      (:then_0
        (Audio|PlaySoundatLocation (Variables|Audio|GetFoliageImpactSFX) (Transformation|GetActorLocation) "0, 0, 0" 1.0 1.0 0.0 0 (Variables|Audio|GetConcurrencySettings) 0 0))
      (:then_1
        (Niagara|SpawnSystematLocation (Variables|Default|GetParticleEffect) (Transformation|GetWorldLocation (Variables|Default|GetStaticMesh)) (Transformation|GetActorRotation (Variables|Default|GetPlayer)))
        (Utilities|FlowControl|DelayUntilNextTick)
        (Actor|DestroyActor)))))

(fn ConstructionScript)