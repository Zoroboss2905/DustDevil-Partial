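; Base physics foliage actor that reacts when an actor implementing BPI_PlayerTrigger overlaps its collision.
; If DestroyOnImpact is set, it spawns a particle effect facing the player's rotation and destroys itself.
; Otherwise the mesh simulates physics, gets launched by player velocity plus an upward boost, ignores Pawns and is destroyed after TimeToDestroy.
; Both paths share a DoOnce-gated impact sound.
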(event OnComponentBeginOverlap(Collision)
  (params (OverlappedComponent :type Primitive%20Component%20Object%20Reference) (OtherActor :type Actor%20Object%20Reference) (OtherComp :type Primitive%20Component%20Object%20Reference) (OtherBodyIndex :type Integer) (bFromSweep :type Boolean) (SweepResult :type Hit%20Result%20Structure%20%28by%20ref%29))
  (if (Utilities|DoesObjectImplementInterface OtherActor "/Game/DustDevil/Core/Interfaces/BPI_PlayerTrigger.BPI_PlayerTrigger_C")
    (bind _player (Class|BPIPlayerTrigger|GetPlayerCharacter(Message) OtherActor))
    (bind _output_get (Variables|References|SetPlayer _player))
    (if (Variables|Default|GetbDestroyOnImpact)
      (Utilities|FlowControl|DoOnce false :!label _label
        (:Completed
          (Audio|PlaySoundatLocation (Variables|Audio|GetImpactSFX) (Transformation|GetActorLocation) "0, 0, 0" 1.0 1.0 0.0 0 (Variables|Audio|GetImpactConcurrency) 0 0)
          (if (Variables|Default|GetbDestroyOnImpact)
            (Niagara|SpawnSystematLocation (Variables|Default|GetParticleEffect) (Transformation|GetWorldLocation (Variables|Default|GetMesh)) (Transformation|GetActorRotation (Variables|References|GetPlayer)))
            (Actor|DestroyActor))))
      (else
        (Physics|SetSimulatePhysics (Variables|Default|GetMesh) true)
        (Physics|AddImpulse (Variables|Default|GetMesh) (Math|Vector|MakeVector (.x (Transformation|GetVelocity _output_get)) (.y (Transformation|GetVelocity _output_get)) (+ (.z (Transformation|GetVelocity _output_get)) 1e+04)) "None" false)
        (Collision|SetCollisionResponsetoChannel (Variables|Default|GetMesh) "ECC_Pawn" "ECR_Ignore")
        (Utilities|FlowControl|Sequence
          (:then_0
            (Utilities|FlowControl|Delay (Variables|Default|GetTimeToDestroy))
            (Actor|DestroyActor))
          (:then_1
            (goto _label)))))))

(fn ConstructionScript)