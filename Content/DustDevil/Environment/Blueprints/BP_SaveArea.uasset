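; BP_SaveArea is a trigger-volume actor, named as a save area, that detects player overlaps but contains no save logic in its graphs.
; On BeginPlay it casts and caches the GI_DDPrototype game instance, which is not used afterward.
; Trigger begin and end overlaps both call GetPlayerCharacterMessage on actors implementing BPI_PlayerTrigger, with nothing done after the call.
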(event OnComponentBeginOverlap(Trigger)
  (params (OverlappedComponent :type Primitive%20Component%20Object%20Reference) (OtherActor :type Actor%20Object%20Reference) (OtherComp :type Primitive%20Component%20Object%20Reference) (OtherBodyIndex :type Integer) (bFromSweep :type Boolean) (SweepResult :type Hit%20Result%20Structure%20%28by%20ref%29))
  (if (Utilities|DoesObjectImplementInterface OtherActor "/Game/DustDevil/Core/Interfaces/BPI_PlayerTrigger.BPI_PlayerTrigger_C")
    (Class|BPIPlayerTrigger|GetPlayerCharacter(Message) OtherActor)))

(event OnComponentEndOverlap(Trigger)
  (params (OverlappedComponent :type Primitive%20Component%20Object%20Reference) (OtherActor :type Actor%20Object%20Reference) (OtherComp :type Primitive%20Component%20Object%20Reference) (OtherBodyIndex :type Integer))
  (if (Utilities|DoesObjectImplementInterface OtherActor "/Game/DustDevil/Core/Interfaces/BPI_PlayerTrigger.BPI_PlayerTrigger_C")
    (Class|BPIPlayerTrigger|GetPlayerCharacter(Message) OtherActor)))

(event EventBeginPlay
  (bind _asgi_ddprototype (Utilities|Casting|CastToGI_DDPrototype (Game|GetGameInstance)))
  (Variables|Default|SetGameInstance _asgi_ddprototype))

(fn ConstructionScript)