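; BP_TurnAround is an overlap trigger actor that tells the player's HUD when they enter or leave an out-of-bounds area.
; Overlapping actors are filtered by the BPI_PlayerTrigger interface, which also supplies the player character reference.
; Begin overlap stores that player and sends OutOfBoundsNotify to its HUD, while end overlap sends OutOfBoundsEnd.
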(event Collision|EventActorBeginOverlap
  (params (OtherActor :type Actor%20Object%20Reference))
  (if (Utilities|DoesObjectImplementInterface OtherActor "/Game/DustDevil/Core/Interfaces/BPI_PlayerTrigger.BPI_PlayerTrigger_C")
    (bind _player (Class|BPIPlayerTrigger|GetPlayerCharacter(Message) OtherActor))
    (bind _output_get (Variables|References|SetPlayer _player))
    (bind _output_get_2 (Variables|References|SetHUD (Variables|/Game/DustDevil/Player/BP_Vehicle.BP_Vehicle_C|GetHUD _output_get)))
    (Class|BPIHUDUpdates|OutOfBoundsNotify(Message) _output_get_2)))

(event Collision|EventActorEndOverlap
  (params (OtherActor :type Actor%20Object%20Reference))
  (if (Utilities|DoesObjectImplementInterface OtherActor "/Game/DustDevil/Core/Interfaces/BPI_PlayerTrigger.BPI_PlayerTrigger_C")
    (bind _player (Class|BPIPlayerTrigger|GetPlayerCharacter(Message) OtherActor))
    (Class|BPIHUDUpdates|OutOfBoundsEnd(Message) (Variables|/Game/DustDevil/Player/BP_Vehicle.BP_Vehicle_C|GetHUD _player))))

(fn ConstructionScript)