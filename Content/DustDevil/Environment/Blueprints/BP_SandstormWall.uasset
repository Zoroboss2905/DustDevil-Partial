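; BP_SandstormWall is an environment actor that shows a Niagara effect, presumably the sandstorm wall, only while a player is nearby.
; The effect is hidden on BeginPlay, then revealed or hidden as actors begin or end overlap with the VisibilityTrigger component.
; Only actors implementing BPI_PlayerTrigger toggle it, through SetHiddenInGame, with no count of how many are inside.
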(event OnComponentBeginOverlap(VisibilityTrigger)
  (params (OverlappedComponent :type Primitive%20Component%20Object%20Reference) (OtherActor :type Actor%20Object%20Reference) (OtherComp :type Primitive%20Component%20Object%20Reference) (OtherBodyIndex :type Integer) (bFromSweep :type Boolean) (SweepResult :type Hit%20Result%20Structure%20%28by%20ref%29))
  (if (Utilities|DoesObjectImplementInterface OtherActor "/Game/DustDevil/Core/Interfaces/BPI_PlayerTrigger.BPI_PlayerTrigger_C")
    (Development|SetHiddeninGame (Variables|Default|GetNiagara) false false)))

(event OnComponentEndOverlap(VisibilityTrigger)
  (params (OverlappedComponent :type Primitive%20Component%20Object%20Reference) (OtherActor :type Actor%20Object%20Reference) (OtherComp :type Primitive%20Component%20Object%20Reference) (OtherBodyIndex :type Integer))
  (if (Utilities|DoesObjectImplementInterface OtherActor "/Game/DustDevil/Core/Interfaces/BPI_PlayerTrigger.BPI_PlayerTrigger_C")
    (Development|SetHiddeninGame (Variables|Default|GetNiagara) true false)))

(event EventBeginPlay
  (Development|SetHiddeninGame (Variables|Default|GetNiagara) true false))

(fn ConstructionScript)