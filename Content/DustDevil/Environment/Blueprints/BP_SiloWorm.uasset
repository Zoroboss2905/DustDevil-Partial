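; BP_SiloWorm is an environment actor with a hatch that swings open when a player trigger enters its sphere.
; BeginPlay resets the hatch mesh rotation and sets the start and end roll angles.
; An overlap by any actor implementing BPI_PlayerTrigger plays a timeline from the start to interpolate the hatch's roll.
; Each qualifying overlap restarts the opening, and no closing logic is present.
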(event OnComponentBeginOverlap(TriggerSphere)
  (params (OverlappedComponent :type Primitive%20Component%20Object%20Reference) (OtherActor :type Actor%20Object%20Reference) (OtherComp :type Primitive%20Component%20Object%20Reference) (OtherBodyIndex :type Integer) (bFromSweep :type Boolean) (SweepResult :type Hit%20Result%20Structure%20%28by%20ref%29))
  (if (Utilities|DoesObjectImplementInterface OtherActor "/Game/DustDevil/Core/Interfaces/BPI_PlayerTrigger.BPI_PlayerTrigger_C")
    (CallFunction|OpenHatch)))

(event Custom|OpenHatch
  (bind _hatchmesh (Variables|Default|GetHatchMesh))
  (bind _relativerotation (Variables|/Script/Engine.SceneComponent|GetRelativeRotation _hatchmesh))
  (bind _alpha (Timeline|TL_HatchOpening PlayFromStart)
    (:Update
      (Transformation|SetRelativeRotation _hatchmesh (Math|Rotator|MakeRotator (Math|Float|Lerp (Variables|Default|GetHatchStartRotate) (Variables|Default|GetHatchEndRotate) _alpha) (.pitch _relativerotation) (.yaw _relativerotation)) false false))))

(event EventBeginPlay
  (CallFunction|Initialise))

(fn ConstructionScript)

(fn Initialise
  (Variables|Default|SetHatchStartRotate 0.0)
  (Variables|Default|SetHatchEndRotate 1.2e+02)
  (Transformation|SetRelativeRotation (Variables|Default|GetHatchMesh) (Math|Rotator|MakeRotator 0.0 0.0 0.0) false false))