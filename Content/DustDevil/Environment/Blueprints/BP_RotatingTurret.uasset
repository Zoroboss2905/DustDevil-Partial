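; Auto-targeting turret that sweeps its gun with a yaw timeline until a shootable enemy enters its detection sphere.
; The enemy reference comes through BPI_Shootable, then looping one-second timers turn the gun toward it and spawn BP_Projectile shots.
; When the target becomes invalid, the timers clear and the sweep resumes.
; The construction script picks the gun mesh from the Weapon setting, while firing is identical for all weapons.
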(event OnComponentBeginOverlap(Sphere)
  (params (OverlappedComponent :type Primitive%20Component%20Object%20Reference) (OtherActor :type Actor%20Object%20Reference) (OtherComp :type Primitive%20Component%20Object%20Reference) (OtherBodyIndex :type Integer) (bFromSweep :type Boolean) (SweepResult :type Hit%20Result%20Structure%20%28by%20ref%29))
  (if (Utilities|DoesObjectImplementInterface OtherActor "/Game/DustDevil/Core/Interfaces/BPI_Shootable.BPI_Shootable_C")
    (bind _enemy (Class|BPIShootable|GetEnemy(Message) OtherActor))
    (bind _output_get (Variables|Default|SetTargetEnemy _enemy))
    (Utilities|IsValid _output_get
      (:Is%20Valid
        (CallFunction|StopNormalRotation)
        (bind _returnvalue (Utilities|Time|SetTimerbyFunctionName 0 "GetEnemyPosition" 1.0 true))
        (Variables|Default|SetFindPositionTimer _returnvalue)
        (bind _returnvalue_2 (Utilities|Time|SetTimerbyEvent (delegate Custom|Targeting) 1.0 true))
        (Variables|Default|SetTargetingTimer _returnvalue_2))
      (:Is%20Not%20Valid
        (Development|PrintString "BP_RotatingTurret: Enemy ref not valid!")))))

(event Custom|RestartRotation
  (bind _gunmesh (Variables|Default|GetGunMesh))
  (bind _relativerotation (Variables|/Script/Engine.SceneComponent|GetRelativeRotation _gunmesh))
  (bind _yaw (Timeline|TL_RotateGun PlayFromStart)
    (:Update
      (Transformation|SetRelativeRotation _gunmesh (Math|Rotator|MakeRotator (.roll _relativerotation) (.pitch _relativerotation) _yaw) false false))
    (:Finished
      (CallFunction|RestartRotation))))

(event Custom|RestartNormalRotation
  (bind _gunmesh (Variables|Default|GetGunMesh))
  (bind _relativerotation (Variables|/Script/Engine.SceneComponent|GetRelativeRotation _gunmesh))
  (bind _yaw (Timeline|TL_RotateGun Play)
    (:Update
      (Transformation|SetRelativeRotation _gunmesh (Math|Rotator|MakeRotator (.roll _relativerotation) (.pitch _relativerotation) _yaw) false false))
    (:Finished
      (CallFunction|RestartRotation))))

(event Custom|StopNormalRotation
  (bind _gunmesh (Variables|Default|GetGunMesh))
  (bind _relativerotation (Variables|/Script/Engine.SceneComponent|GetRelativeRotation _gunmesh))
  (bind _yaw (Timeline|TL_RotateGun Stop)
    (:Update
      (Transformation|SetRelativeRotation _gunmesh (Math|Rotator|MakeRotator (.roll _relativerotation) (.pitch _relativerotation) _yaw) false false))
    (:Finished
      (CallFunction|RestartRotation))))

(event Custom|Targeting
  (bind (_returnvalue _benemyalive) (CallFunction|GetEnemyPosition))
  (Components|MoveComponentTo (Variables|Default|GetGunMesh) (Variables|/Script/Engine.SceneComponent|GetRelativeLocation (Variables|Default|GetGunMesh)) _returnvalue false false 1.0 false)
  (if _benemyalive
    (CallFunction|FireTurret)
    (else
      (Utilities|Time|ClearandInvalidateTimerbyHandle (Variables|Default|GetFindPositionTimer))
      (Utilities|Time|ClearandInvalidateTimerbyHandle (Variables|Default|GetTargetingTimer))
      (CallFunction|RestartNormalRotation))))

(event EventBeginPlay
  (bind _gunmesh (Variables|Default|GetGunMesh))
  (bind _relativerotation (Variables|/Script/Engine.SceneComponent|GetRelativeRotation _gunmesh))
  (Utilities|FlowControl|Sequence
    (:then_0
      (bind _yaw (Timeline|TL_RotateGun SetNewTime)
        (:Update
          (Transformation|SetRelativeRotation _gunmesh (Math|Rotator|MakeRotator (.roll _relativerotation) (.pitch _relativerotation) _yaw) false false))
        (:Finished
          (CallFunction|RestartRotation))))
    (:then_1
      (Timeline|TL_RotateGun Play))))

(fn ConstructionScript
  (switch Utilities|FlowControl|Switch|SwitchonE_WeaponType (Variables|Default|GetWeapon)
    (:NewEnumerator0
      (Components|StaticMesh|SetStaticMesh (Variables|Default|GetGunMesh) "/Game/DustDevil/Art/Meshes/Vehicle/Turrets/SM_BasicTurret.SM_BasicTurret"))
    (:NewEnumerator1
      (Components|StaticMesh|SetStaticMesh (Variables|Default|GetGunMesh) "/Game/DustDevil/Art/Meshes/Vehicle/Turrets/SM_Minigun.SM_Minigun"))
    (:NewEnumerator2
      (Components|StaticMesh|SetStaticMesh (Variables|Default|GetGunMesh) "/Game/DustDevil/Art/Meshes/Vehicle/Turrets/SM_Flamethrower.SM_Flamethrower"))
    (:NewEnumerator3
      (Components|StaticMesh|SetStaticMesh (Variables|Default|GetGunMesh) "/Game/DustDevil/Art/Meshes/Vehicle/Turrets/SM_Autocannon.SM_Autocannon"))
    (:NewEnumerator4
      (Components|StaticMesh|SetStaticMesh (Variables|Default|GetGunMesh) "/Game/DustDevil/Art/Meshes/Vehicle/Turrets/SM_GuitarGun.SM_GuitarGun"))))

(fn FireTurret
  (bind _bulletspawn (Variables|Default|GetBulletSpawn))
  (bind _returnvalue (Transformation|GetRelativeTransform _bulletspawn))
  (Game|SpawnActorfromClass "/Game/DustDevil/Player/Weapons/BP_Projectile.BP_Projectile_C" (Math|Transform|MakeTransform (.location _returnvalue) (.rotation _returnvalue) "1.000000,1.000000,1.000000") "Undefined" "MultiplyWithRoot" 0 5e+04 0))

(fn GetEnemyPosition
  (bind _targetenemy (Variables|Default|GetTargetEnemy)
    (:then
      (return (Math|Rotator|FindLookatRotation (Transformation|GetWorldLocation (Variables|Default|GetGunMesh)) (Transformation|GetActorLocation _targetenemy)) true))
    (:else
      (return "0, 0, 0" false))))