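; Radiation hazard zone that damages the player over time while inside its sphere or box volume, selected by UsesBox on BeginPlay.
; Entry through BPI_PlayerTrigger starts a looping timer applying RadiationDamage, plus player feedback, HUD rad icon and flash, threat-based Geiger audio and AudioManager notification.
; Exit clears the timer, stops the feedback and resets the DoOnce entry gate.
; RadiationLevelFluctuate is defined, but its timer setup never runs.
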(event OnComponentEndOverlap(RadiatianAreaSphere)
  (params (OverlappedComponent :type Primitive%20Component%20Object%20Reference) (OtherActor :type Actor%20Object%20Reference) (OtherComp :type Primitive%20Component%20Object%20Reference) (OtherBodyIndex :type Integer))
  (bind _player (Variables|References|GetPlayer))
  (bind _hud (Variables|/Game/DustDevil/Player/BP_Vehicle.BP_Vehicle_C|GetHUD _player))
  (bind _wbp_healthbar (Variables|/Game/DustDevil/UI/HUD/WBP_HUD.WBP_HUD_C|GetWBP_HealthBar _hud))
  ;[0.02956 0.02956 0.02956] Clears radiation damage timer and calls function subtract max health based on rads taken
  (if (Utilities|DoesObjectImplementInterface OtherActor "/Game/DustDevil/Core/Interfaces/BPI_PlayerTrigger.BPI_PlayerTrigger_C")
    (if (not (Variables|Default|GetbUsesBox))
      (Default|ReverseRadiationFeedback (Variables|References|GetPlayer))
      (Utilities|Time|ClearandInvalidateTimerbyHandle (Variables|Default|GetRadiationTimer))
      (Audio|Components|Audio|FadeOut (Variables|Default|GetGeigerCounter) 1.0 0.0 "Linear" :!class /Script/Engine.AudioComponent)
      (Default|StopRadFlashAnim _wbp_healthbar)
      (Default|StopRadIconPulse _wbp_healthbar (Variables|Default|GetRadiationThreat))
      (CallFunction|ResetRadiation)
      (bind _audiomanager (Variables|References|GetAudioManager)
        (:then
          (Utilities|FlowControl|DoOnce false
            (:Completed
              (Default|RadZoneExited _audiomanager))))
        (:else)))))

(event OnComponentBeginOverlap(RadiatianAreaSphere)
  (params (OverlappedComponent :type Primitive%20Component%20Object%20Reference) (OtherActor :type Actor%20Object%20Reference) (OtherComp :type Primitive%20Component%20Object%20Reference) (OtherBodyIndex :type Integer) (bFromSweep :type Boolean) (SweepResult :type Hit%20Result%20Structure%20%28by%20ref%29))
  ;[0.02956 0.02956 0.02956] When irradiated area is entered retrieve reference to player
  (if (Utilities|DoesObjectImplementInterface OtherActor "/Game/DustDevil/Core/Interfaces/BPI_PlayerTrigger.BPI_PlayerTrigger_C")
    (bind _player (Class|BPIPlayerTrigger|GetPlayerCharacter(Message) OtherActor))
    (Variables|References|SetPlayer _player)
    (Utilities|FlowControl|DoOnce false
      (:Completed
        (Utilities|FlowControl|Sequence
          (:then_0
            (Default|RadiatingFeedback (Variables|References|GetPlayer))
            ;[0.02956 0.02956 0.02956] Starts applying rad damage over time
            (bind _returnvalue (Utilities|Time|SetTimerbyEvent (delegate Custom|Start%20Irradiating%20Player) (Variables|Default|GetRadiationDelay) true))
            (Variables|Default|SetRadiationTimer _returnvalue)
            (CallFunction|PlayGeigerCounterAudio (Variables|Default|GetRadiationThreat))
            (Default|UpdateRadIconPulse (Variables|/Game/DustDevil/UI/HUD/WBP_HUD.WBP_HUD_C|GetWBP_HealthBar (Variables|/Game/DustDevil/Player/BP_Vehicle.BP_Vehicle_C|GetHUD (Variables|References|GetPlayer))) (Variables|Default|GetRadiationThreat))
            (bind _audiomanager (Variables|References|GetAudioManager)
              (:then
                (Default|RadZoneEntered _audiomanager))
              (:else)))
          (:then_1
            ;[0.02956 0.02956 0.02956] Clears radiation damage timer and calls function subtract max health based on rads taken
            (Utilities|FlowControl|DoOnce false) ; enters at Reset
          ))))))

(event OnComponentEndOverlap(RadiationAreaBox)
  (params (OverlappedComponent :type Primitive%20Component%20Object%20Reference) (OtherActor :type Actor%20Object%20Reference) (OtherComp :type Primitive%20Component%20Object%20Reference) (OtherBodyIndex :type Integer))
  (bind _player (Variables|References|GetPlayer))
  (bind _hud (Variables|/Game/DustDevil/Player/BP_Vehicle.BP_Vehicle_C|GetHUD _player))
  (bind _wbp_healthbar (Variables|/Game/DustDevil/UI/HUD/WBP_HUD.WBP_HUD_C|GetWBP_HealthBar _hud))
  ;[0.02956 0.02956 0.02956] Clears radiation damage timer and calls function subtract max health based on rads taken
  (if (Utilities|DoesObjectImplementInterface OtherActor "/Game/DustDevil/Core/Interfaces/BPI_PlayerTrigger.BPI_PlayerTrigger_C")
    (if (Variables|Default|GetbUsesBox)
      (Default|ReverseRadiationFeedback (Variables|References|GetPlayer))
      (Utilities|Time|ClearandInvalidateTimerbyHandle (Variables|Default|GetRadiationTimer))
      (Audio|Components|Audio|FadeOut (Variables|Default|GetGeigerCounter) 1.0 0.0 "Linear" :!class /Script/Engine.AudioComponent)
      (Default|StopRadFlashAnim _wbp_healthbar)
      (Default|StopRadIconPulse _wbp_healthbar (Variables|Default|GetRadiationThreat))
      (CallFunction|ResetRadiation)
      (bind _audiomanager (Variables|References|GetAudioManager)
        (:then
          (Utilities|FlowControl|DoOnce false
            (:Completed
              (Default|RadZoneExited _audiomanager))))
        (:else)))))

(event OnComponentBeginOverlap(RadiationAreaBox)
  (params (OverlappedComponent :type Primitive%20Component%20Object%20Reference) (OtherActor :type Actor%20Object%20Reference) (OtherComp :type Primitive%20Component%20Object%20Reference) (OtherBodyIndex :type Integer) (bFromSweep :type Boolean) (SweepResult :type Hit%20Result%20Structure%20%28by%20ref%29))
  ;[0.02956 0.02956 0.02956] When irradiated area is entered retrieve reference to player
  (if (Utilities|DoesObjectImplementInterface OtherActor "/Game/DustDevil/Core/Interfaces/BPI_PlayerTrigger.BPI_PlayerTrigger_C")
    (bind _player (Class|BPIPlayerTrigger|GetPlayerCharacter(Message) OtherActor))
    (Variables|References|SetPlayer _player)
    (Utilities|FlowControl|Sequence
      (:then_0
        (Utilities|FlowControl|DoOnce false
          (:Completed
            (Utilities|FlowControl|Sequence
              (:then_0
                (Default|RadiatingFeedback (Variables|References|GetPlayer))
                ;[0.02956 0.02956 0.02956] Starts applying rad damage over time
                (bind _returnvalue (Utilities|Time|SetTimerbyEvent (delegate Custom|Start%20Irradiating%20Player) (Variables|Default|GetRadiationDelay) true))
                (Variables|Default|SetRadiationTimer _returnvalue)
                (CallFunction|PlayGeigerCounterAudio (Variables|Default|GetRadiationThreat))
                (Default|UpdateRadIconPulse (Variables|/Game/DustDevil/UI/HUD/WBP_HUD.WBP_HUD_C|GetWBP_HealthBar (Variables|/Game/DustDevil/Player/BP_Vehicle.BP_Vehicle_C|GetHUD (Variables|References|GetPlayer))) (Variables|Default|GetRadiationThreat))
                (bind _audiomanager (Variables|References|GetAudioManager)
                  (:then
                    (Default|RadZoneEntered _audiomanager))
                  (:else)))
              (:then_1
                ;[0.02956 0.02956 0.02956] Clears radiation damage timer and calls function subtract max health based on rads taken
                (Utilities|FlowControl|DoOnce false) ; enters at Reset
              )))))
      (:then_1
        ;[0.02956 0.02956 0.02956] Increases radiation level and updates Rads meter on the HUD
        (Utilities|FlowControl|DoOnce false) ; enters at Reset
      ))))

(event Custom|Start%20Irradiating%20Player
  ;[0.02956 0.02956 0.02956] Increases radiation level and updates Rads meter on the HUD
  (if true
    (Default|RadiationDamage (Variables|References|GetPlayer) (* (Variables|Default|GetRadiationLevelBase) -1.0) (Variables|Default|GetRadiationThreat) self)
    (Utilities|FlowControl|Delay (Math|Random|RandomFloatinRange 0.0 1.0))
    (Utilities|FlowControl|DoOnce false
      (:Completed
        (Default|PlayRadFlashAnim (Variables|/Game/DustDevil/UI/HUD/WBP_HUD.WBP_HUD_C|GetWBP_HealthBar (Variables|/Game/DustDevil/Player/BP_Vehicle.BP_Vehicle_C|GetHUD (Variables|References|GetPlayer))) (Variables|Default|GetRadiationThreat))))))

(event Custom|ResetRadiation
  ;[0.02956 0.02956 0.02956] When irradiated area is entered retrieve reference to player
  (Utilities|FlowControl|DoOnce false) ; enters at Reset
)

(event EventBeginPlay
  (CallFunction|SetCollisionObject))

(fn ConstructionScript)

(fn PlayGeigerCounterAudio
  (params (RadiationThreat :type Integer))
  (Utilities|FlowControl|Sequence
    (:then_0
      (switch string (Utilities|String|ToString(Integer) RadiationThreat)
        (:10
          (Audio|Components|Audio|SetSound (Variables|Default|GetGeigerCounter) (Variables|Audio|GetGeigerCounterLow)))
        (:20
          (Audio|Components|Audio|SetSound (Variables|Default|GetGeigerCounter) (Variables|Audio|GetGeigerCounterMed)))
        (:30
          (Audio|Components|Audio|SetSound (Variables|Default|GetGeigerCounter) (Variables|Audio|GetGeigerCounterHigh) :!label _label)))
      (Audio|Components|Audio|FadeIn (Variables|Default|GetGeigerCounter) 1.0 1.0 0.0 "Linear" :!class /Script/Engine.AudioComponent))
    (:then_1
      (if (> RadiationThreat 30)
        (goto _label)))))

(fn GetRadiationThreatLevel
  (params (NewParam :type Integer)))

(fn GetPlayerRadResist
  (return (.ReturnValue (Ability|Attribute|GetFloatAttributefromAbilitySystemComponent (Ability|GetAbilitySystemComponent (Variables|References|GetPlayer)) "(AttributeName=\"RadShield\",Attribute=/Script/DustDevil.VehicleAttributeSet:RadShield,AttributeOwner=\"/Script/CoreUObject.Class'/Script/DustDevil.VehicleAttributeSet'\")"))))

(fn RadiationLevelFluctuate
  (if (Math|Conversions|ToBoolean(Integer) (Math|Random|RandomIntegerinRange 0 1))
    (Variables|Default|SetNewValue (Math|Float|Clamp(Float) (+ (Variables|Default|GetOldValue) 0.01) (Variables|Default|GetOldValue) (+ (Variables|Default|GetRadiationLevelBase) 0.1)))
    (else
      (Variables|Default|SetNewValue (Math|Float|Clamp(Float) (- (Variables|Default|GetOldValue) 0.01) (- (Variables|Default|GetRadiationLevelBase) 0.1) (Variables|Default|GetOldValue)))))
  (Utilities|FlowControl|Sequence
    (:then_0
      (Variables|Default|SetRadiationLevel (Variables|Default|GetNewValue)))
    (:then_1
      (Variables|Default|SetOldValue (Variables|Default|GetNewValue)))))

(fn SetCollisionObject
  (if (Variables|Default|GetbUsesBox)
    (Collision|SetCollisionResponsetoChannel (Variables|Default|GetRadiatianAreaSphere) "ECC_Pawn" "ECR_Ignore")
    (Collision|SetCollisionResponsetoChannel (Variables|Default|GetRadiationAreaBox) "ECC_Pawn" "ECR_Overlap")
    (Rendering|SetVisibility (Variables|Default|GetRadiatianAreaSphere) false false)
    (Rendering|SetVisibility (Variables|Default|GetRadiationAreaBox) true false)
    (else
      (Collision|SetCollisionResponsetoChannel (Variables|Default|GetRadiatianAreaSphere) "ECC_Pawn" "ECR_Overlap")
      (Collision|SetCollisionResponsetoChannel (Variables|Default|GetRadiationAreaBox) "ECC_Pawn" "ECR_Ignore")
      (Rendering|SetVisibility (Variables|Default|GetRadiatianAreaSphere) true false)
      (Rendering|SetVisibility (Variables|Default|GetRadiationAreaBox) false false))))