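; BP_BunkerDoor is a bunker door that swings open when an actor implementing BPI_PlayerTrigger enters its OpeningTrigger.
; The overlap stores the player character returned by the interface, waits briefly, then plays the TL_RotateDoor timeline.
; The timeline lerps the door mesh's relative roll through a quarter turn, leaving pitch and yaw untouched.
; When it finishes, a delay precedes reversing the timeline to close the door.
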(event OnComponentBeginOverlap(OpeningTrigger)
  (params (OverlappedComponent :type Primitive%20Component%20Object%20Reference) (OtherActor :type Actor%20Object%20Reference) (OtherComp :type Primitive%20Component%20Object%20Reference) (OtherBodyIndex :type Integer) (bFromSweep :type Boolean) (SweepResult :type Hit%20Result%20Structure%20%28by%20ref%29))
  (bind _doormesh (Variables|Default|GetDoorMesh))
  (bind _relativerotation (Variables|/Script/Engine.SceneComponent|GetRelativeRotation _doormesh))
  (if (Utilities|DoesObjectImplementInterface OtherActor "/Game/DustDevil/Core/Interfaces/BPI_PlayerTrigger.BPI_PlayerTrigger_C")
    (bind _player (Class|BPIPlayerTrigger|GetPlayerCharacter(Message) OtherActor))
    (Variables|Default|SetPlayer _player)
    (Utilities|FlowControl|Delay 0.5)
    (bind _alpha (Timeline|TL_RotateDoor Play)
      (:Update
        (Transformation|SetRelativeRotation (Variables|Default|GetDoorMesh) (Math|Rotator|MakeRotator (Math|Float|Lerp (Variables|Default|GetStartRotationX) (Variables|Default|GetEndRotationX) _alpha) (.pitch _relativerotation) (.yaw _relativerotation)) false false))
      (:Finished
        (Utilities|FlowControl|Delay 5.0)
        (Timeline|TL_RotateDoor Reverse)))))

(event EventBeginPlay
  (Variables|Default|SetStartRotationX 0.0)
  (Variables|Default|SetEndRotationX -9e+01))

(fn ConstructionScript)