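; BP_SandstormWall3 is an environment Blueprint that reveals a sandstorm wall while a player trigger is inside its VisibilityTrigger volume.
; Overlapping actors that implement BPI_PlayerTrigger unhide the Sandstorm component on entry and hide it on exit.
; A DoOnce gates the SandstormSFX fade-in and resets on exit, which does not fade the sound out.
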(event OnComponentBeginOverlap(VisibilityTrigger)
  (params (OverlappedComponent :type Primitive%20Component%20Object%20Reference) (OtherActor :type Actor%20Object%20Reference) (OtherComp :type Primitive%20Component%20Object%20Reference) (OtherBodyIndex :type Integer) (bFromSweep :type Boolean) (SweepResult :type Hit%20Result%20Structure%20%28by%20ref%29))
  (if (Utilities|DoesObjectImplementInterface OtherActor "/Game/DustDevil/Core/Interfaces/BPI_PlayerTrigger.BPI_PlayerTrigger_C")
    (Development|SetHiddeninGame (Variables|Default|GetSandstorm) false false)
    (Utilities|FlowControl|DoOnce false
      (:Completed
        (Audio|Components|Audio|FadeIn (Variables|Default|GetSandstormSFX) 0.5 1.0 0.0 "Linear" :!class /Script/Engine.AudioComponent)))))

(event OnComponentEndOverlap(VisibilityTrigger)
  (params (OverlappedComponent :type Primitive%20Component%20Object%20Reference) (OtherActor :type Actor%20Object%20Reference) (OtherComp :type Primitive%20Component%20Object%20Reference) (OtherBodyIndex :type Integer))
  (if (Utilities|DoesObjectImplementInterface OtherActor "/Game/DustDevil/Core/Interfaces/BPI_PlayerTrigger.BPI_PlayerTrigger_C")
    (Development|SetHiddeninGame (Variables|Default|GetSandstorm) true false)
    (Utilities|FlowControl|DoOnce false) ; enters at Reset
  ))

(fn ConstructionScript)