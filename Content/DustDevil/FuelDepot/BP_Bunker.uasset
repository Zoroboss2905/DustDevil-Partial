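; Bunker entrance actor that lets the player travel to the L_Base level.
; An overlap trigger shows a hold-to-interact prompt styled for controller or keyboard, driven by Enhanced Input.
; Completing the hold fades the screen, saves Nuclear Fuel and Mutated Chitin from the player's Ability System attributes via the GameInstance, then loads the base.
; Optionally, a timeline swings the door on BeginPlay with collision disabled, then reverses it after a delay.
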(event OnComponentBeginOverlap(EntryTrigger)
  (params (OverlappedComponent :type Primitive%20Component%20Object%20Reference) (OtherActor :type Actor%20Object%20Reference) (OtherComp :type Primitive%20Component%20Object%20Reference) (OtherBodyIndex :type Integer) (bFromSweep :type Boolean) (SweepResult :type Hit%20Result%20Structure%20%28by%20ref%29))
  ;[0.02956 0.02956 0.02956] Gets reference to player when they enter interaction radius and makes interaction prompt interactable
  (if (Utilities|DoesObjectImplementInterface OtherActor "/Game/DustDevil/Core/Interfaces/BPI_PlayerTrigger.BPI_PlayerTrigger_C")
    (bind _player (Class|BPIPlayerTrigger|GetPlayerCharacter(Message) OtherActor))
    (Variables|References|SetPlayer _player)
    (Rendering|SetVisibility (Variables|Default|GetInteractionPrompt) true false)
    (Variables|Default|SetbPromptOpen true)))

(event OnComponentEndOverlap(EntryTrigger)
  (params (OverlappedComponent :type Primitive%20Component%20Object%20Reference) (OtherActor :type Actor%20Object%20Reference) (OtherComp :type Primitive%20Component%20Object%20Reference) (OtherBodyIndex :type Integer))
  ;[0.02956 0.02956 0.02956] Gets reference to player when they enter interaction radius and makes interaction prompt interactable
  (if (Utilities|DoesObjectImplementInterface OtherActor "/Game/DustDevil/Core/Interfaces/BPI_PlayerTrigger.BPI_PlayerTrigger_C")
    (Rendering|SetVisibility (Variables|Default|GetInteractionPrompt) false false)
    (Variables|Default|SetbPromptOpen false)))

(event Input|EnhancedActionEvents|EnhancedInputActionIA_HoldInteract_X
  (params (ActionValue :type Boolean) (ElapsedSeconds :type Float%20%28double-precision%29) (TriggeredSeconds :type Float%20%28double-precision%29) (InputAction :type Input%20Action%20Object%20Reference :default "/Game/DustDevil/Core/Inputs/IA_HoldInteract_X.IA_HoldInteract_X"))
  ;[0.02956 0.02956 0.02956] Interaction prompt
  (:Triggered
    (if (Rendering|IsVisible (Variables|Default|GetInteractionPrompt))
      (bind _promptwidget (Variables|References|GetPromptWidget)
        (:then
          (Default|TriggerPrompt _promptwidget)
          ;[0.02956 0.02956 0.02956] When interaction prompt is triggered starts level transition
          (Rendering|SetVisibility (Variables|Default|GetInteractionPrompt) false false)
          (Variables|Default|SetbPromptOpen false)
          (bind _returnvalue (UserInterface|CreateWidget "/Game/DustDevil/UI/CustomisationMenu/WBP_FadeIn.WBP_FadeIn_C"))
          (UserInterface|Viewport|AddtoViewport _returnvalue 3)
          (CallFunction|SetSaveData)
          (Default|SaveData (Variables|References|GetGameInstance))
          (Utilities|FlowControl|Delay 2.0)
          (Game|OpenLevel(byName) "L_Base"))
        (:else))))
  (:Ongoing
    (if (Rendering|IsVisible (Variables|Default|GetInteractionPrompt))
      (bind _promptwidget_2 (Variables|References|GetPromptWidget)
        (:then
          (Default|HoldPrompt _promptwidget_2 ElapsedSeconds))
        (:else))))
  (:Canceled
    (if (Rendering|IsVisible (Variables|Default|GetInteractionPrompt))
      (bind _promptwidget_3 (Variables|References|GetPromptWidget)
        (:then
          (Default|CancelPrompt _promptwidget_3))
        (:else)))))

(event EventBeginPlay
  (CallFunction|GetReferences)
  (CallFunction|SetupInputPrompt)
  (CallFunction|SetStartEndPoints)
  (if (Variables|Default|GetbAnimateDoor)
    (Collision|SetCollisionEnabled (Variables|Default|GetBaseDoor) "NoCollision")
    (bind _alpha (Timeline|TL_BaseDoor PlayFromStart)
      (:Update
        (CallFunction|RotateDoor _alpha))
      (:Finished
        (Utilities|FlowControl|Delay 5.0)
        (Collision|SetCollisionEnabled (Variables|Default|GetBaseDoor) "QueryAndPhysics")
        (if (not (Variables|Default|GetbIsOpen))
          (Variables|Default|SetbIsOpen true)
          (Timeline|TL_BaseDoor Reverse))))))

(fn ConstructionScript)

(fn SetupInputPrompt
  (bind _aswbp_prompt_hold_text (Utilities|Casting|CastToWBP_PromptHoldText (UserInterface|GetUserWidgetObject (Variables|Default|GetInteractionPrompt))))
  (Variables|References|SetPromptWidget _aswbp_prompt_hold_text)
  (if (Variables|/Game/DustDevil/Core/GI_DDPrototype.GI_DDPrototype_C|GetbUsingController (Variables|References|GetGameInstance))
    (Default|SetInputType (Variables|References|GetPromptWidget) "NewEnumerator2" "" "" false "" "Enter bunker")
    (else
      (Default|SetInputType (Variables|References|GetPromptWidget) "NewEnumerator0" "E" "16px" false "" "Enter bunker")))
  (Default|SetScale (Variables|References|GetPromptWidget) 1.0))

(fn SetSaveData
  (Utilities|FlowControl|Sequence
    (:then_0
      (Variables|/Game/DustDevil/Core/Saves/SG_DDSaveData.SG_DDSaveData_C|SetNuclearFuel (Default|GetSaveData (Variables|References|GetGameInstance)) (Math|Float|Ceil (.ReturnValue (Ability|Attribute|GetFloatAttributefromAbilitySystemComponent (Ability|GetAbilitySystemComponent (Variables|References|GetPlayer)) "(AttributeName=\"NuclearMatter\",Attribute=/Script/DustDevil.BaseAttributeSet:NuclearMatter,AttributeOwner=\"/Script/CoreUObject.Class'/Script/DustDevil.BaseAttributeSet'\")")))))
    (:then_1
      (Variables|/Game/DustDevil/Core/Saves/SG_DDSaveData.SG_DDSaveData_C|SetMutatedChitin (Default|GetSaveData (Variables|References|GetGameInstance)) (Math|Float|Ceil (.ReturnValue (Ability|Attribute|GetFloatAttributefromAbilitySystemComponent (Ability|GetAbilitySystemComponent (Variables|References|GetPlayer)) "(AttributeName=\"MutatedChitin\",Attribute=/Script/DustDevil.VehicleAttributeSet:MutatedChitin,AttributeOwner=\"/Script/CoreUObject.Class'/Script/DustDevil.VehicleAttributeSet'\")")))))))

(fn GetReferences
  (bind _asgi_ddprototype (Utilities|Casting|CastToGI_DDPrototype (Game|GetGameInstance)))
  (bind _output_get (Variables|References|SetGameInstance _asgi_ddprototype))
  (bind _ddsavedata (Variables|/Game/DustDevil/Core/GI_DDPrototype.GI_DDPrototype_C|GetDDSaveData _output_get)
    (:then
      (Variables|References|SetSaveData _ddsavedata))
    (:else)))

(fn SetStartEndPoints
  (Variables|Default|SetStartRotX 0.0)
  (Variables|Default|SetEndRotX -9e+01))

(fn RotateDoor
  (params (Alpha :type Float%20%28double-precision%29))
  (bind _basedoor (Variables|Default|GetBaseDoor))
  (bind _relativerotation (Variables|/Script/Engine.SceneComponent|GetRelativeRotation _basedoor))
  (Transformation|SetRelativeRotation _basedoor (Math|Rotator|MakeRotator (Math|Float|Lerp (Variables|Default|GetStartRotX) (Variables|Default|GetEndRotX) Alpha) (.pitch _relativerotation) (.yaw _relativerotation)) false false))