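; Fuel depot exit actor that lets the player hold interact to save and return to the bunker level, L_Base.
; Two overlap triggers reveal a pointer and a hold prompt, labelled for controller or keyboard.
; A completed hold fades the screen and HUD, writes fuel and chitin ability-system attributes to save data, then loads the level after a delay.
; The construction script assigns a weapon to its child rotating turret.
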(event OnComponentBeginOverlap(InteractionTrigger)
  (params (OverlappedComponent :type Primitive%20Component%20Object%20Reference) (OtherActor :type Actor%20Object%20Reference) (OtherComp :type Primitive%20Component%20Object%20Reference) (OtherBodyIndex :type Integer) (bFromSweep :type Boolean) (SweepResult :type Hit%20Result%20Structure%20%28by%20ref%29))
  (if (Utilities|DoesObjectImplementInterface OtherActor "/Game/DustDevil/Core/Interfaces/BPI_PlayerTrigger.BPI_PlayerTrigger_C")
    (bind _player (Class|BPIPlayerTrigger|GetPlayerCharacter(Message) OtherActor))
    (bind _output_get (Variables|References|SetPlayer _player))
    (Utilities|IsValid _output_get
      (:Is%20Valid
        (Rendering|SetVisibility (Variables|Default|GetInteractionPrompt) true false)
        (Variables|Default|SetbPromptOpen true)))))

(event OnComponentEndOverlap(InteractionTrigger)
  (params (OverlappedComponent :type Primitive%20Component%20Object%20Reference) (OtherActor :type Actor%20Object%20Reference) (OtherComp :type Primitive%20Component%20Object%20Reference) (OtherBodyIndex :type Integer))
  (if (Utilities|DoesObjectImplementInterface OtherActor "/Game/DustDevil/Core/Interfaces/BPI_PlayerTrigger.BPI_PlayerTrigger_C")
    (Rendering|SetVisibility (Variables|Default|GetInteractionPrompt) false false)
    (Variables|Default|SetbPromptOpen false)))

(event OnComponentBeginOverlap(PointerTrigger)
  (params (OverlappedComponent :type Primitive%20Component%20Object%20Reference) (OtherActor :type Actor%20Object%20Reference) (OtherComp :type Primitive%20Component%20Object%20Reference) (OtherBodyIndex :type Integer) (bFromSweep :type Boolean) (SweepResult :type Hit%20Result%20Structure%20%28by%20ref%29))
  (if (Utilities|DoesObjectImplementInterface OtherActor "/Game/DustDevil/Core/Interfaces/BPI_PlayerTrigger.BPI_PlayerTrigger_C")
    (Rendering|SetVisibility (Variables|Default|GetInteractionPointer) true false)))

(event OnComponentEndOverlap(PointerTrigger)
  (params (OverlappedComponent :type Primitive%20Component%20Object%20Reference) (OtherActor :type Actor%20Object%20Reference) (OtherComp :type Primitive%20Component%20Object%20Reference) (OtherBodyIndex :type Integer))
  (if (Utilities|DoesObjectImplementInterface OtherActor "/Game/DustDevil/Core/Interfaces/BPI_PlayerTrigger.BPI_PlayerTrigger_C")
    (Rendering|SetVisibility (Variables|Default|GetInteractionPointer) false false)))

(event Input|EnhancedActionEvents|EnhancedInputActionIA_HoldInteract_X
  (params (ActionValue :type Boolean) (ElapsedSeconds :type Float%20%28double-precision%29) (TriggeredSeconds :type Float%20%28double-precision%29) (InputAction :type Input%20Action%20Object%20Reference :default "/Game/DustDevil/Core/Inputs/IA_HoldInteract_X.IA_HoldInteract_X"))
  (:Triggered
    (if (Rendering|IsVisible (Variables|Default|GetInteractionPrompt))
      (bind _promptwidget (Variables|References|GetPromptWidget)
        (:then
          (Default|TriggerPrompt _promptwidget)
          (Rendering|SetVisibility (Variables|Default|GetInteractionPrompt) false false)
          (Variables|Default|SetbPromptOpen false)
          (bind _returnvalue (UserInterface|CreateWidget "/Game/DustDevil/UI/CustomisationMenu/WBP_FadeIn.WBP_FadeIn_C"))
          (UserInterface|Viewport|AddtoViewport _returnvalue 0)
          (bind _player (Variables|References|GetPlayer)
            (:then
              (Default|HUDFadeAnimation (Variables|/Game/DustDevil/Player/BP_Vehicle.BP_Vehicle_C|GetHUD _player) false)
              (Default|CrosshairFadeAnim (Variables|/Game/DustDevil/Player/PC_VehicleController.PC_VehicleController_C|GetReticleCursor (.AsPC%20Vehicle%20Controller (Utilities|Casting|CastToPC_VehicleController (Game|GetPlayerController 0)))) false 0.0))
            (:else
              _))
          (CallFunction|SetSaveData)
          (Default|SaveData (Variables|References|GetGameInstance))
          (Utilities|FlowControl|Delay 2.0)
          (Game|OpenLevel(byName) "L_Base"))
        (:else))))
  (:Ongoing
    (if (Rendering|IsVisible (Variables|Default|GetInteractionPrompt))
      (bind _promptwidget_2 (Variables|References|GetPromptWidget)
        (:then
          (Default|HoldPrompt _promptwidget_2 ElapsedSeconds))
        (:else))))
  (:Canceled
    (if (Rendering|IsVisible (Variables|Default|GetInteractionPrompt))
      (bind _promptwidget_3 (Variables|References|GetPromptWidget)
        (:then
          (Default|CancelPrompt _promptwidget_3))
        (:else)))))

(event EventBeginPlay
  (CallFunction|GetReferences)
  (CallFunction|Initialise)
  (CallFunction|SetInputPrompt))

(fn ConstructionScript
  (bind _asbp_rotating_turret (Utilities|Casting|CastToBP_RotatingTurret (Variables|/Script/Engine.ChildActorComponent|GetChildActor (Variables|Default|GetRotatingTurret))))
  (Variables|/Game/DustDevil/Environment/Blueprints/BP_RotatingTurret.BP_RotatingTurret_C|SetWeapon _asbp_rotating_turret (Variables|Default|GetTurret)))

(fn Initialise
  (Rendering|SetVisibility (Variables|Default|GetInteractionPointer) false false))

(fn SetSaveData
  (Utilities|FlowControl|Sequence
    (:then_0
      (Variables|/Game/DustDevil/Core/Saves/SG_DDSaveData.SG_DDSaveData_C|SetNuclearFuel (Variables|References|GetSaveData) (Math|Float|Ceil (.ReturnValue (Ability|Attribute|GetFloatAttributefromAbilitySystemComponent (Ability|GetAbilitySystemComponent (Variables|References|GetPlayer)) "(AttributeName=\"NuclearMatter\",Attribute=/Script/DustDevil.BaseAttributeSet:NuclearMatter,AttributeOwner=\"/Script/CoreUObject.Class'/Script/DustDevil.BaseAttributeSet'\")")))))
    (:then_1
      (Variables|/Game/DustDevil/Core/Saves/SG_DDSaveData.SG_DDSaveData_C|SetMutatedChitin (Variables|References|GetSaveData) (Math|Float|Ceil (.ReturnValue (Ability|Attribute|GetFloatAttributefromAbilitySystemComponent (Ability|GetAbilitySystemComponent (Variables|References|GetPlayer)) "(AttributeName=\"MutatedChitin\",Attribute=/Script/DustDevil.VehicleAttributeSet:MutatedChitin,AttributeOwner=\"/Script/CoreUObject.Class'/Script/DustDevil.VehicleAttributeSet'\")")))))))

(fn SetInputPrompt
  (bind _aswbp_prompt_hold_text (Utilities|Casting|CastToWBP_PromptHoldText (UserInterface|GetUserWidgetObject (Variables|Default|GetInteractionPrompt))))
  (Variables|References|SetPromptWidget _aswbp_prompt_hold_text)
  (if (Variables|/Game/DustDevil/Core/GI_DDPrototype.GI_DDPrototype_C|GetbUsingController (Variables|References|GetGameInstance))
    (Default|SetInputType (Variables|References|GetPromptWidget) "NewEnumerator2" "" "" false "" "Return to bunker")
    (else
      (Default|SetInputType (Variables|References|GetPromptWidget) "NewEnumerator0" "E" "16px" false "" "Return to bunker")))
  (Default|SetScale (Variables|References|GetPromptWidget) 1.0))

(fn GetReferences
  (bind _asgi_ddprototype (Utilities|Casting|CastToGI_DDPrototype (Game|GetGameInstance)))
  (bind _output_get (Variables|References|SetGameInstance _asgi_ddprototype))
  (Variables|References|SetSaveData (Default|GetSaveData _output_get)))