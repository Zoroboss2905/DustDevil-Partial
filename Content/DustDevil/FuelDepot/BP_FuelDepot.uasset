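; Fuel depot actor where the player's vehicle gets a full repair and radiation cure.
; Overlap volumes toggle the map-icon marker, ambient audio, top-mount weapon lockout and a "Repair vehicle" hold prompt, shown if an ability-system attribute differs from base.
; Completing the hold heals immediately, alongside a timed camera move with input disabled, hologram overlay, post-process pulse and popups.
; Depot menu, docking animation and nuclear-fuel deposit code remains largely unwired.
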(event OnComponentBeginOverlap(InteractionRadius)
  (params (OverlappedComponent :type Primitive%20Component%20Object%20Reference) (OtherActor :type Actor%20Object%20Reference) (OtherComp :type Primitive%20Component%20Object%20Reference) (OtherBodyIndex :type Integer) (bFromSweep :type Boolean) (SweepResult :type Hit%20Result%20Structure%20%28by%20ref%29))
  ;[0.02956 0.02956 0.02956] Gets reference to player when they enter interaction radius and makes interaction prompt interactable
  (Utilities|FlowControl|DoOnce false
    (:Completed
      (if (Utilities|DoesObjectImplementInterface OtherActor "/Game/DustDevil/Core/Interfaces/BPI_PlayerTrigger.BPI_PlayerTrigger_C")
        (Class|BPIPlayerTrigger|GetPlayerCharacter(Message) OtherActor)
        (if (CallFunction|CheckifPlayerCanHeal)
          ;[0.02956 0.02956 0.02956] Moves player into depot when interaction prompt is entered and adds depot menu
          (Rendering|SetVisibility (Variables|Default|GetInteractionPrompt) true false)
          (Variables|Default|SetbPromptOpen true)
          (elif (not (Variables|Default|GetbInTutorial))
            (Class|BPIHUDUpdates|DisplayPopup(Message) (Variables|/Game/DustDevil/Player/BP_Vehicle.BP_Vehicle_C|GetHUD (Variables|References|GetPlayer)) "Vehicle is fully repaired!")))))))

(event OnComponentEndOverlap(InteractionRadius)
  (params (OverlappedComponent :type Primitive%20Component%20Object%20Reference) (OtherActor :type Actor%20Object%20Reference) (OtherComp :type Primitive%20Component%20Object%20Reference) (OtherBodyIndex :type Integer))
  ;[0.02956 0.02956 0.02956] Gets reference to player when they enter interaction radius and makes interaction prompt interactable
  (if (Utilities|DoesObjectImplementInterface OtherActor "/Game/DustDevil/Core/Interfaces/BPI_PlayerTrigger.BPI_PlayerTrigger_C")
    (Rendering|SetVisibility (Variables|Default|GetInteractionPrompt) false false)
    (Variables|Default|SetbPromptOpen false)
    (Utilities|FlowControl|DoOnce false) ; enters at Reset
  ))

(event OnComponentBeginOverlap(Barrier)
  (params (OverlappedComponent :type Primitive%20Component%20Object%20Reference) (OtherActor :type Actor%20Object%20Reference) (OtherComp :type Primitive%20Component%20Object%20Reference) (OtherBodyIndex :type Integer) (bFromSweep :type Boolean) (SweepResult :type Hit%20Result%20Structure%20%28by%20ref%29))
  (if (Utilities|DoesObjectImplementInterface OtherActor "/Game/DustDevil/Core/Interfaces/BPI_PlayerTrigger.BPI_PlayerTrigger_C")
    (Collision|SetCollisionResponsetoChannel (Variables|Default|GetBarrier) "ECC_Pawn" "ECR_Block")
    (bind _player (Class|BPIPlayerTrigger|GetPlayerCharacter(Message) OtherActor))
    (bind _output_get (Variables|References|SetPlayer _player))
    (Utilities|IsValid _output_get
      (:Is%20Valid
        (Class|TopMountBase|StopUse (Class|Vehicle|GetTopMount _output_get))
        (Variables|/Script/DustDevil.TopMountBase|SetDisabledReasons (Class|Vehicle|GetTopMount _output_get) (Class|KismetMathLibrary|OrIntInt (Variables|/Script/DustDevil.TopMountBase|GetDisabledReasons (Class|Vehicle|GetTopMount _output_get)) (|BitmaskLiteral 4)))))))

(event OnComponentEndOverlap(Barrier)
  (params (OverlappedComponent :type Primitive%20Component%20Object%20Reference) (OtherActor :type Actor%20Object%20Reference) (OtherComp :type Primitive%20Component%20Object%20Reference) (OtherBodyIndex :type Integer))
  (if (Utilities|DoesObjectImplementInterface OtherActor "/Game/DustDevil/Core/Interfaces/BPI_PlayerTrigger.BPI_PlayerTrigger_C")
    (Collision|SetCollisionResponsetoChannel (Variables|Default|GetBarrier) "ECC_Pawn" "ECR_Overlap")
    (bind _player (Class|BPIPlayerTrigger|GetPlayerCharacter(Message) OtherActor))
    (bind _output_get (Variables|References|SetPlayer _player))
    (Utilities|IsValid _output_get
      (:Is%20Valid
        (Variables|/Script/DustDevil.TopMountBase|SetDisabledReasons (Class|Vehicle|GetTopMount _output_get) (Class|KismetMathLibrary|AndIntInt (Variables|/Script/DustDevil.TopMountBase|GetDisabledReasons (Class|Vehicle|GetTopMount _output_get)) (Class|KismetMathLibrary|NotInt (|BitmaskLiteral 4))))
        (Class|BPIHUDUpdates|RemoveWarningMessage(Message) (Variables|/Game/DustDevil/Player/BP_Vehicle.BP_Vehicle_C|GetHUD _output_get)))
      (:Is%20Not%20Valid
        (Development|PrintString "FuelDepot: Player Not Valid!" true true "(R=0.000000,G=0.660000,B=1.000000,A=1.000000)" 2.0 "FuelDepotPlayer")))))

(event OnComponentBeginOverlap(PointerTrigger)
  (params (OverlappedComponent :type Primitive%20Component%20Object%20Reference) (OtherActor :type Actor%20Object%20Reference) (OtherComp :type Primitive%20Component%20Object%20Reference) (OtherBodyIndex :type Integer) (bFromSweep :type Boolean) (SweepResult :type Hit%20Result%20Structure%20%28by%20ref%29))
  (if (Utilities|DoesObjectImplementInterface OtherActor "/Game/DustDevil/Core/Interfaces/BPI_PlayerTrigger.BPI_PlayerTrigger_C")
    (Rendering|SetVisibility (Variables|Default|GetInteractionPointer) true false)
    (bind _ambientsound (Variables|Default|GetAmbientSound)
      (:then
        (if (not (Audio|Components|Audio|IsPlaying _ambientsound))
          (Audio|Components|Audio|FadeIn (stale _output_get) 1.0 1.0 0.0 "Linear" :!class /Script/Engine.AudioComponent :!label _label)))
      (:else
        (bind _returnvalue (Audio|SpawnSoundatLocation "/Game/DustDevil/Audio/Ambience/A_FuelDepotAmbient.A_FuelDepotAmbient" (Transformation|GetActorLocation) "0, 0, 0" 1.0 1.0 0.0 0 0))
        (bind _output_get (Variables|Default|SetAmbientSound _returnvalue))
        (goto _label)))))

(event OnComponentEndOverlap(PointerTrigger)
  (params (OverlappedComponent :type Primitive%20Component%20Object%20Reference) (OtherActor :type Actor%20Object%20Reference) (OtherComp :type Primitive%20Component%20Object%20Reference) (OtherBodyIndex :type Integer))
  (if (Utilities|DoesObjectImplementInterface OtherActor "/Game/DustDevil/Core/Interfaces/BPI_PlayerTrigger.BPI_PlayerTrigger_C")
    (Rendering|SetVisibility (Variables|Default|GetInteractionPointer) false false)
    (bind _ambientsound (Variables|Default|GetAmbientSound)
      (:then
        (if (Audio|Components|Audio|IsPlaying _ambientsound)
          (Audio|Components|Audio|FadeOut _ambientsound 1.0 0.0 "Linear" :!class /Script/Engine.AudioComponent)))
      (:else))))

(event Custom|Zoom%20Cam%20In
  (bind _player (Variables|References|GetPlayer))
  (bind _springarmdepot (Variables|/Game/DustDevil/Player/BP_Vehicle.BP_Vehicle_C|GetSpringArmDepot _player))
  (Utilities|FlowControl|Sequence
    (:then_0
      (Variables|/Game/DustDevil/Player/BP_Vehicle.BP_Vehicle_C|SetStartZoom _player false)
      (Variables|/Script/DustDevil.Vehicle|SetCameraSweepAggression _player 0.0)
      (Variables|/Script/DustDevil.Vehicle|SetCameraSweepRate _player 0.0)
      (Variables|/Script/DustDevil.TopMountBase|SetbAimable (Class|Vehicle|GetTopMount _player) false)
      (Utilities|FlowControl|Sequence
        (:then_0
          (if (> (Variables|/Game/DustDevil/Player/BP_Vehicle.BP_Vehicle_C|GetZoomValue (Variables|References|GetPlayer)) 0.0)
            (bind _float (Timeline|TimelineOffset Play)
              (:Update
                (Variables|/Script/Engine.SpringArmComponent|SetTargetArmLength (Variables|/Script/DustDevil.Vehicle|GetSweepCameraBoom (Variables|References|GetPlayer)) (Math|Float|Lerp (Variables|/Game/DustDevil/Player/BP_Vehicle.BP_Vehicle_C|GetZoomValue (Variables|References|GetPlayer)) 0.0 _float))))))
        (:then_1
          (Components|MoveComponentTo (Variables|/Script/DustDevil.Vehicle|GetCameraBoom _player) (Math|Vector|MakeVector (.x (Variables|/Script/Engine.SceneComponent|GetRelativeLocation _springarmdepot)) 5e+02 -1e+03) (Math|Rotator|MakeRotator (.roll (Variables|/Script/Engine.SceneComponent|GetRelativeRotation _springarmdepot)) (Variables|Default|GetChangePitchAngle) (Variables|Default|GetChangeYawAngle)) false false 1.75 false))
        (:then_2
          (Audio|PlaySound2D "/Game/DustDevil/Audio/Feedback/UpgradesAbilities/A_DepotHeal.A_DepotHeal" 0.5 2.0 0.0 0 0 false)
          (Audio|PlaySound2D "/Game/DustDevil/Audio/Feedback/UpgradesAbilities/ui-movement-menu-modern-interface-window-open-small-230486.ui-movement-menu-modern-interface-window-open-small-230486" 2.5 0.25 0.0 0 0 false))))
    (:then_1
      (Input|DisableInput (Variables|References|GetPlayer) (Game|GetPlayerController 0)))))

(event Custom|ZoomCamOut
  (bind _player (Variables|References|GetPlayer))
  (bind _cameraboomtwo (Variables|/Game/DustDevil/Player/BP_Vehicle.BP_Vehicle_C|GetCameraBoomTwo _player))
  (Utilities|FlowControl|Sequence
    (:then_0
      (Variables|/Script/DustDevil.TopMountBase|SetbAimable (Class|Vehicle|GetTopMount _player) true)
      (Variables|/Game/DustDevil/Player/BP_Vehicle.BP_Vehicle_C|SetStartZoom _player true)
      (Variables|/Script/DustDevil.Vehicle|SetCameraSweepAggression _player 0.3)
      (Variables|/Script/DustDevil.Vehicle|SetCameraSweepRate _player 1.0)
      (Components|MoveComponentTo (Variables|/Script/DustDevil.Vehicle|GetCameraBoom _player) (Variables|/Script/Engine.SceneComponent|GetRelativeLocation _cameraboomtwo) (Variables|/Script/Engine.SceneComponent|GetRelativeRotation _cameraboomtwo) false false 1.75 false))
    (:then_1
      (bind _float (Timeline|TimelineOffset Reverse)
        (:Update
          (Variables|/Script/Engine.SpringArmComponent|SetTargetArmLength (Variables|/Script/DustDevil.Vehicle|GetSweepCameraBoom (Variables|References|GetPlayer)) (Math|Float|Lerp (Variables|/Game/DustDevil/Player/BP_Vehicle.BP_Vehicle_C|GetZoomValue (Variables|References|GetPlayer)) 0.0 _float)))))
    (:then_2
      (Input|EnableInput (Variables|References|GetPlayer) (Game|GetPlayerController 0))
      (CallFunction|HealFeedbackTwo))))

(event Custom|HealOpacity
  (bind _player (Variables|References|GetPlayer))
  (Rendering|Material|SetOverlayMaterial (Variables|/Script/DustDevil.Vehicle|GetEngineMount _player) "/Game/DustDevil/Effects/Scan/M_Hologram.M_Hologram" :!class /Script/Engine.MeshComponent)
  (Utilities|FlowControl|Delay 2.0)
  (Rendering|Material|SetOverlayMaterial (Variables|/Script/DustDevil.Vehicle|GetWheelFR _player) 0 :!class /Script/Engine.MeshComponent))

(event Custom|HealFeedbackTwo
  (bind _pspfading (Timeline|Timeline_0 PlayFromStart)
    (:Update
      (Variables|/Script/Engine.PostProcessComponent|SetBlendWeight (Variables|/Game/DustDevil/Player/BP_Vehicle.BP_Vehicle_C|GetPostProcessHealthGain (Variables|References|GetPlayer)) _pspfading))))

(event Custom|HealFeedback
  (bind _pspfading (Timeline|Timeline PlayFromStart)
    (:Update
      (Variables|/Script/Engine.PostProcessComponent|SetBlendWeight (Variables|/Game/DustDevil/Player/BP_Vehicle.BP_Vehicle_C|GetPostProcessHealthGain (Variables|References|GetPlayer)) _pspfading))))

(event Input|EnhancedActionEvents|EnhancedInputActionIA_HoldInteract_X
  (params (ActionValue :type Boolean) (ElapsedSeconds :type Float%20%28double-precision%29) (TriggeredSeconds :type Float%20%28double-precision%29) (InputAction :type Input%20Action%20Object%20Reference :default "/Game/DustDevil/Core/Inputs/IA_HoldInteract_X.IA_HoldInteract_X"))
  (bind _player (Variables|References|GetPlayer))
  ;[0.02956 0.02956 0.02956] Interaction prompt
  (:Triggered
    (if (and (Rendering|IsVisible (Variables|Default|GetInteractionPrompt)) (Variables|Default|GetbPromptOpen))
      (bind _promptwidget (Variables|References|GetPromptWidget)
        (:then
          (Default|TriggerPrompt _promptwidget)
          (Utilities|FlowControl|Sequence
            (:then_0
              ;[0.02956 0.02956 0.02956] Moves player into depot when interaction prompt is entered and adds depot menu
              (Rendering|SetVisibility (Variables|Default|GetInteractionPrompt) false false)
              (Variables|Default|SetbPromptOpen false)
              (CallFunction|ZoomCamin)
              (Utilities|FlowControl|Delay 2.0)
              (CallFunction|ZoomCamOut))
            (:then_1
              ;[0.02956 0.02956 0.02956] Repair vehicle and clear radiation
              (Default|CureRads _player)
              (Default|RepairVehicleFull _player)
              (bind _returnvalue (UserInterface|CreateWidget "/Game/DustDevil/UI/HUD/WBP_RepairPopUp.WBP_RepairPopUp_C" (Game|GetPlayerController 0) "REPAIRING..."))
              (UserInterface|Viewport|AddtoViewport _returnvalue 0)
              (Default|PlayFadeinOut _returnvalue)
              (CallFunction|HealOpacity)
              (CallFunction|HealFeedback)
              (Utilities|FlowControl|Delay 2.0)
              (Widget|RemovefromParent _returnvalue)
              (bind _returnvalue_2 (UserInterface|CreateWidget "/Game/DustDevil/UI/HUD/WBP_RepairPopUp.WBP_RepairPopUp_C" (Game|GetPlayerController 0) "Vehicle Fully Repaired!"))
              (UserInterface|Viewport|AddtoViewport _returnvalue_2 0)
              (Utilities|FlowControl|Delay 2.0))))
        (:else))))
  (:Ongoing
    (if (and (Rendering|IsVisible (Variables|Default|GetInteractionPrompt)) (Variables|Default|GetbPromptOpen))
      (bind _promptwidget_2 (Variables|References|GetPromptWidget)
        (:then
          (Default|HoldPrompt _promptwidget_2 ElapsedSeconds))
        (:else))))
  (:Canceled
    (if (and (Rendering|IsVisible (Variables|Default|GetInteractionPrompt)) (Variables|Default|GetbPromptOpen))
      (bind _promptwidget_3 (Variables|References|GetPromptWidget)
        (:then
          (Default|CancelPrompt _promptwidget_3))
        (:else)))))

(event EventBeginPlay
  (CallFunction|GetReferences)
  (CallFunction|SetupInputPrompt)
  (CallFunction|SetupInteractionPointer))

(fn ConstructionScript)

(fn CheckifPlayerHasBiomatter
  (bind _abilitysystem (Variables|Default|GetAbilitySystem))
  (bind (_bsuccessfullyfoundattribute _returnvalue) (Ability|Attribute|GetFloatAttributefromAbilitySystemComponent _abilitysystem "(AttributeName=\"BioMatter\",Attribute=/Script/DustDevil.BaseAttributeSet:BioMatter,AttributeOwner=\"/Script/CoreUObject.Class'/Script/DustDevil.BaseAttributeSet'\")"))
  (if _bsuccessfullyfoundattribute
    (if (== _returnvalue 0.0)
      (return false)
      (else
        (return true)))
    (else
      (Development|PrintString "Attribute not found" true true "(R=1.000000,G=0.000000,B=0.000000,A=1.000000)"))))

(fn SetStartEndPoints
  (bind _player (Variables|References|GetPlayer))
  (bind _southarrow (Variables|Default|GetSouthArrow))
  (bind _northarrow (Variables|Default|GetNorthArrow))
  (bind _southarrow_2 (Variables|Default|GetSouthArrow))
  (bind _southarrow_3 (Variables|Default|GetSouthArrow))
  (bind _returnvalue (Transformation|GetWorldRotation _southarrow))
  (Variables|Default|SetLocationStart (Transformation|GetActorLocation _player))
  (Variables|Default|SetRotationStart (Transformation|GetActorRotation _player))
  (if (Variables|Default|GetbIsRotatedVertical)
    (if (> (.y (Transformation|GetActorForwardVector (Variables|References|GetPlayer))) 0.0)
      (Variables|Default|SetLocationEnd (Transformation|GetWorldLocation _southarrow_2))
      (Variables|Default|SetRotationEnd (Transformation|GetWorldRotation _southarrow_2))
      (else
        (Variables|Default|SetLocationEnd (Transformation|GetWorldLocation _northarrow) :!label _label)
        (Variables|Default|SetRotationEnd (Transformation|GetWorldRotation _northarrow))))
    (elif (> (.x (Transformation|GetActorForwardVector (Variables|References|GetPlayer))) 0.0)
      (goto _label)
      (elif (< (.yaw (Transformation|GetActorRotation (Variables|References|GetPlayer))) 0.0)
        (Variables|Default|SetLocationEnd (Transformation|GetWorldLocation _southarrow))
        (Variables|Default|SetRotationEnd (Math|Rotator|MakeRotator (.roll _returnvalue) (.pitch _returnvalue) (+ (.yaw _returnvalue) -3.6e+02)))
        (else
          (Variables|Default|SetLocationEnd (Transformation|GetWorldLocation _southarrow_3))
          (Variables|Default|SetRotationEnd (Transformation|GetWorldRotation _southarrow_3)))))))

(fn UpdatePlayerLocationRotation
  (params (LocationAlpha :type Float%20%28double-precision%29) (RotationAlpha :type Float%20%28double-precision%29))
  (bind _player (Variables|References|GetPlayer))
  (bind _locationstart (Variables|Default|GetLocationStart))
  (bind _locationend (Variables|Default|GetLocationEnd))
  (bind _returnvalue (Math|Vector|Lerp(Vector) _locationstart _locationend LocationAlpha))
  ;[0.02956 0.02956 0.02956] Updates player location and rotation as part of entry animation
  (Transformation|SetActorLocationAndRotation _player (Math|Vector|MakeVector (.x _returnvalue) (.y _returnvalue) (.z (Transformation|GetActorLocation _player))) (Math|Rotator|Lerp(Rotator) (Variables|Default|GetRotationStart) (Variables|Default|GetRotationEnd) RotationAlpha)))

(fn SetupInputPrompt
  (bind _aswbp_prompt_hold_text (Utilities|Casting|CastToWBP_PromptHoldText (UserInterface|GetUserWidgetObject (Variables|Default|GetInteractionPrompt)))
    (:then
      (Variables|References|SetPromptWidget _aswbp_prompt_hold_text)
      (if (Variables|/Game/DustDevil/Core/GI_DDPrototype.GI_DDPrototype_C|GetbUsingController (Variables|References|GetGameInstance))
        (Default|SetInputType (Variables|References|GetPromptWidget) "NewEnumerator2" "E" "" false "" "Repair vehicle")
        (else
          (Default|SetInputType (Variables|References|GetPromptWidget) "NewEnumerator0" "E" "16px" false "" "Repair vehicle")))
      (return))
    (:CastFailed
      (return))))

(fn MenuClosed
  (Rendering|SetVisibility (Variables|Default|GetInteractionPrompt) true false)
  (Variables|Default|SetbPromptOpen true)
  (Class|BPICursorCalls|SetOpenedMenu(Message) (Game|GetPlayerController 0) "NewEnumerator4")
  (CallFunction|ZoomCamOut)
  (return))

(fn IncreaseDepositedNuclearMats
  (bind _output_get (Variables|Default|SetNuclearStored (Math|Integer|Clamp(Integer) (+ (Variables|Default|GetNuclearStored) 1) 0 (Variables|Default|GetNuclearCapacity))))
  (Utilities|FlowControl|Sequence
    (:then_0
      (Default|UpdateFuelDepotStorage (Variables|References|GetFuelDepotMenu)))
    (:then_1
      (return (>= _output_get (Variables|Default|GetNuclearCapacity))))))

(fn GetReferences
  (bind _returnvalue (Actor|GetActorOfClass "/Game/DustDevil/Player/BP_Vehicle.BP_Vehicle_C"))
  (Variables|References|SetPlayer _returnvalue)
  (Utilities|FlowControl|Sequence
    (:then_0
      (bind _asgi_ddprototype (Utilities|Casting|CastToGI_DDPrototype (Game|GetGameInstance)))
      (bind _output_get (Variables|References|SetGameInstance _asgi_ddprototype))
      (Variables|References|SetSaveData (Variables|/Game/DustDevil/Core/GI_DDPrototype.GI_DDPrototype_C|GetDDSaveData _output_get)))
    (:then_1
      (bind _asgm_vehicle (Utilities|Casting|CastToGM_Vehicle (Game|GetGameMode)))
      (Variables|References|SetGameMode _asgm_vehicle))))

(fn CheckifPlayerCanHeal
  (bind _player (Variables|References|GetPlayer))
  (bind _returnvalue (Ability|GetAbilitySystemComponent _player))
  (return (!= (.ReturnValue (Ability|Attribute|GetFloatAttributefromAbilitySystemComponent _returnvalue "(AttributeName=\"CurrentHealth\",Attribute=/Script/DustDevil.BaseAttributeSet:CurrentHealth,AttributeOwner=\"/Script/CoreUObject.Class'/Script/DustDevil.BaseAttributeSet'\")")) (.ReturnValue (Class|AbilitySystemBlueprintLibrary|GetFloatAttributeBasefromAbilitySystemComponent _returnvalue "(AttributeName=\"MaxHealth\",Attribute=/Script/DustDevil.BaseAttributeSet:MaxHealth,AttributeOwner=\"/Script/CoreUObject.Class'/Script/DustDevil.BaseAttributeSet'\")")))))

(fn CheckifPlayerMissingConsumables
  (bind _player (Variables|References|GetPlayer))
  (return (or (< (Variables|/Game/DustDevil/Player/BP_Vehicle.BP_Vehicle_C|GetRepairKits _player) (Variables|/Game/DustDevil/Player/BP_Vehicle.BP_Vehicle_C|GetMaxRepairKits _player)) (< (Variables|/Game/DustDevil/Player/BP_Vehicle.BP_Vehicle_C|GetDeconKits _player) (Variables|/Game/DustDevil/Player/BP_Vehicle.BP_Vehicle_C|GetMaxDeconKits _player)))))

(fn SetupInteractionPointer
  (bind _aswbp_screen_marker (Utilities|Casting|CastToWBP_ScreenMarker (UserInterface|GetWidget (Variables|Default|GetInteractionPointer))))
  (bind _output_get (Variables|References|SetPointerWidget _aswbp_screen_marker))
  (Default|SetMarkerProperties _output_get "/Game/DustDevil/UI/Textures/HUD/T_UI_Minimap_FuelDepot.T_UI_Minimap_FuelDepot" "(R=0.520996,G=0.208637,B=0.012983,A=1.000000)" 4e+01 4e+01))