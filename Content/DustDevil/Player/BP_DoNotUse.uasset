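; BP_DoNotUse is a player pawn that aims at the mouse cursor; its name and disconnected movement code suggest a retired prototype.
; BeginPlay adds the gameplay Enhanced Input mapping and shows the cursor.
; Each Tick traces under the cursor and yaws ProjectileRef toward the hit point, compensating for actor rotation.
; CamShift switches the view target; physics and input movement experiments are unwired, and SuspensionKart is empty.
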(event Input|EnhancedActionEvents|EnhancedInputActionIA_FixedMovement
  (params (ActionValue :type Vector%202D%20Structure) (ElapsedSeconds :type Float%20%28double-precision%29) (TriggeredSeconds :type Float%20%28double-precision%29) (InputAction :type Input%20Action%20Object%20Reference :default "/Game/DustDevil/Core/Inputs/IA_FixedMovement.IA_FixedMovement")))

(event EventBeginPlay
  (bind _asplayer_controller (Utilities|Casting|CastToPlayerController (Pawn|GetController)))
  (Utilities|IsValid (PlayerController|LocalPlayerSubsystems|GetEnhancedInputLocalPlayerSubsystem _asplayer_controller)
    (:Is%20Valid
      (Input|AddMappingContext (PlayerController|LocalPlayerSubsystems|GetEnhancedInputLocalPlayerSubsystem _asplayer_controller) "/Game/DustDevil/Core/Inputs/IMC_Gameplay.IMC_Gameplay" 0 "(bIgnoreAllPressedKeysUntilRelease=True,bForceImmediately=False,bNotifyUserSettings=False)")
      (Variables|/Script/Engine.PlayerController|SetbShowMouseCursor (Game|GetPlayerController 0) true))))

(event Collision|EventActorBeginOverlap
  (params (OtherActor :type Actor%20Object%20Reference)))

(event EventTick
  (params (DeltaSeconds :type Float%20%28single-precision%29))
  (bind _returnvalue (Transformation|GetActorRotation))
  (bind _projectileref (Variables|Default|GetProjectileRef))
  (bind _returnvalue_2 (Transformation|GetWorldRotation _projectileref))
  (Transformation|SetRelativeRotation _projectileref (Math|Rotator|MakeRotator (- (.roll _returnvalue_2) (.roll _returnvalue)) (- (.pitch _returnvalue_2) (.pitch _returnvalue)) (- (.yaw (Math|Rotator|FindLookatRotation (Transformation|GetWorldLocation _projectileref) (.Location (Collision|BreakHitResult (.HitResult (Game|Player|GetHitResultUnderCursorbyChannel (Game|GetPlayerController 0) "TraceTypeQuery1" true)))))) (.yaw _returnvalue))) false false))

(event Input|KeyboardEvents|S
  (params (Key :type Key%20Structure)))

(event Input|KeyboardEvents|W
  (params (Key :type Key%20Structure)))

(fn ConstructionScript
  (Transformation|AddRelativeRotation (Variables|Default|GetArrow1) (Variables|Default|GetMoveArrowRot) false false))

(fn CamShift
  (params (NewCamRef :type Cam%20One%20Shift%20Object%20Reference))
  (Variables|Default|SetNewCamRef NewCamRef)
  (Game|Player|SetViewTargetwithBlend (Game|GetPlayerController 0) (Variables|Default|GetNewCamRef) 0.0 "VTBlend_Linear" 0.0 false)
  (return))

(fn SuspensionKart)