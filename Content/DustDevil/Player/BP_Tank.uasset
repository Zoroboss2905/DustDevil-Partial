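; BP_Tank is a fuel tank actor that trails behind a followed object and stores fuel up to a maximum capacity.
; Each tick it interpolates toward a point a fixed distance behind FollowObject and turns toward it, applying only the yaw.
; UpdateFuel adds incoming fuel, clamps it at capacity and returns the overflow via modulo, which equals the true excess only while the total stays below twice capacity.
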(event EventTick
  (params (DeltaSeconds :type Float%20%28single-precision%29))
  (bind _returnvalue (Transformation|GetActorLocation))
  (bind _followobject (Variables|Default|GetFollowObject))
  (bind _returnvalue_2 (Transformation|GetActorLocation _followobject))
  (Utilities|IsValid _followobject
    (:Is%20Valid
      (Transformation|SetActorLocationAndRotation (Math|Interpolation|VInterpTo _returnvalue (- _returnvalue_2 (* (Transformation|GetActorForwardVector _followobject) 275.0)) DeltaSeconds 5e+01) (Math|Rotator|MakeRotator 0.0 0.0 (.yaw (Math|Interpolation|RInterpTo (Transformation|GetActorRotation) (Math|Rotator|FindLookatRotation _returnvalue _returnvalue_2) DeltaSeconds 5e+01)))))))

(fn ConstructionScript)

(fn UpdateFuel
  (params (IncomingFuel :type Integer))
  (bind _output_get (LocalVariables|SetInterVal (+ IncomingFuel (Variables|Default|GetFuelCapacity))))
  (if (>= _output_get (Variables|Default|GetFuelCapacityMax))
    (Variables|Default|SetFuelCapacity (Variables|Default|GetFuelCapacityMax))
    (return (Math|Integer|%(Integer) (LocalVariables|GetInterVal) (Variables|Default|GetFuelCapacityMax)))
    (else
      (Variables|Default|SetFuelCapacity (LocalVariables|GetInterVal))
      (return 0))))