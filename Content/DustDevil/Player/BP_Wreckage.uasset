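; BP_Wreckage is a loot pickup that grants Nuclear Matter to the player on contact.
; When the player pawn overlaps its sphere, it builds a GE_PickupLoot spec with NuclearMats as a SetByCaller magnitude under the Stats.Base.NuclearMatter tag.
; It applies that spec through the player's Ability System Component, spawns an effect system at its location and destroys itself.
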(event OnComponentBeginOverlap(Sphere)
  (params (OverlappedComponent :type Primitive%20Component%20Object%20Reference) (OtherActor :type Actor%20Object%20Reference) (OtherComp :type Primitive%20Component%20Object%20Reference) (OtherBodyIndex :type Integer) (bFromSweep :type Boolean) (SweepResult :type Hit%20Result%20Structure%20%28by%20ref%29))
  (bind _returnvalue (Game|Player|GetPlayerPawn 0))
  (bind _returnvalue_2 (Ability|GetAbilitySystemComponent _returnvalue))
  (if (or (== OtherActor _returnvalue) false)
    (bind _returnvalue_3 (Ability|GameplayEffect|AssignTagSetbyCallerMagnitude (GameplayEffects|MakeOutgoingSpec :self _returnvalue_2 :GameplayEffectClass "/Game/DustDevil/Core/GAS/Effects/GE_PickupLoot.GE_PickupLoot_C" :Level 1.0) "(TagName=\"Stats.Base.NuclearMatter\")" (Variables|Default|GetNuclearMats)))
    (GameplayEffects|ApplyGameplayEffectSpecToTarget _returnvalue_2 _returnvalue_3 _returnvalue_2)
    (Niagara|SpawnSystematLocation 0 (Transformation|GetActorLocation))
    (Actor|DestroyActor)))

(fn ConstructionScript)