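; Player controller for the vehicle pawn, managing cursor, input mode, HUD and menus.
; Aim input moves the mouse reticle to a viewport-clamped screen projection along the top mount's forward vector, scaled by input and camera boom length.
; Interface events swap cursors and mapping contexts, relay boss bars, and toggle HUD with minimap icons.
; Pause, ability and fuel silo menus are lazily created and gated by MenuOpened; the first two pause the game.
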(event Input|EnhancedActionEvents|EnhancedInputActionIA_Aim
  (params (ActionValue :type Vector%202D%20Structure) (ElapsedSeconds :type Float%20%28double-precision%29) (TriggeredSeconds :type Float%20%28double-precision%29) (InputAction :type Input%20Action%20Object%20Reference :default "/Game/DustDevil/Core/Inputs/IA_Aim.IA_Aim"))
  (bind _returnvalue (Math|Float|Absolute(Float) (.x ActionValue)))
  (bind _returnvalue_2 (Math|Float|Absolute(Float) (.y ActionValue)))
  (bind _returnvalue_3 (Viewport|GetViewportSize))
  (bind _self self)
  (bind _vehiclepawn (Variables|Default|GetVehiclePawn))
  (bind _returnvalue_4 (Class|Vehicle|GetTopMount _vehiclepawn))
  (bind _returnvalue_5 (Transformation|GetActorLocation _vehiclepawn))
  (bind _returnvalue_6 (Math|Float|Min(Float) _returnvalue_2 0.5))
  (bind _returnvalue_7 (Math|Float|Min(Float) _returnvalue 0.5))
  (bind _cameraboom (Variables|/Script/DustDevil.Vehicle|GetCameraBoom _vehiclepawn))
  (bind _returnvalue_8 (Transformation|GetActorRotation _returnvalue_4))
  (bind _returnvalue_9 (Math|Float|Max(Float) _returnvalue_7 _returnvalue_6))
  (bind _targetarmlength (Variables|/Script/Engine.SpringArmComponent|GetTargetArmLength _cameraboom))
  (bind _returnvalue_10 (Math|Vector|GetForwardVector _returnvalue_8))
  (bind _returnvalue_11 (* _targetarmlength _returnvalue_9 1.5))
  (bind _returnvalue_12 (* _returnvalue_10 _returnvalue_11))
  (bind _returnvalue_13 (+ _returnvalue_5 _returnvalue_12))
  (bind _screenposition (Class|GameplayStatics|ProjectWorldtoScreen _self _returnvalue_13 false))
  ;[0.02956 0.02956 0.02956] Adjusts reticle position in screen
  (if (== (Variables|Default|GetInputMappingContext) "/Game/DustDevil/Core/Inputs/IMC_Gameplay.IMC_Gameplay")
    (Class|PlayerController|SetMouseLocation (Math|Float|Truncate (Math|Float|Clamp(Float) (.x _screenposition) 0.0 (.x _returnvalue_3))) (Math|Float|Truncate (Math|Float|Clamp(Float) (.y _screenposition) 0.0 (.y _returnvalue_3))))))

(event EventBeginPlay
  (bind _returnvalue (UserInterface|CreateWidget "/Game/DustDevil/UI/CustomisationMenu/WBP_FadeOut.WBP_FadeOut_C"))
  (UserInterface|Viewport|AddtoViewport _returnvalue 1))

(event EventToggleGamePaused
  (bind _player (Class|BPIPlayerTrigger|GetPlayerCharacter(Message) (Game|Player|GetPlayerPawn 0)))
  (Utilities|IsValid _player
    (:Is%20Valid
      (Variables|Widgets|GetPauseMenu
        (:then
          (switch Utilities|FlowControl|Switch|SwitchonE_Menus (Variables|Default|GetMenuOpened)
            (:NewEnumerator4
              (UserInterface|Viewport|AddtoViewport (Variables|Widgets|GetPauseMenu) 10 :!label _label)
              (Variables|Default|SetMenuOpened "NewEnumerator0")
              (Game|SetGamePaused true)
              (if (Widget|IsVisible (Variables|Widgets|GetHUD)) :!label _label_2
                (Widget|SetVisibility (Variables|Widgets|GetHUD) "Hidden")
                (CallFunction|UpdateMinimapVisibility false)
                (else
                  (Widget|SetVisibility (Variables|Widgets|GetHUD) "Visible")
                  (CallFunction|UpdateMinimapVisibility true))))
            (:NewEnumerator0
              (if (not (Widget|IsVisible (Variables|/Game/DustDevil/UI/PauseMenu/WBP_PauseMenu.WBP_PauseMenu_C|GetCP_Confirmation (Variables|Widgets|GetPauseMenu))))
                (if (not (== (Class|WidgetSwitcher|GetActiveWidgetIndex (Variables|/Game/DustDevil/UI/PauseMenu/WBP_PauseMenu.WBP_PauseMenu_C|GetWS_PauseMenu (Variables|Widgets|GetPauseMenu))) 1))
                  (Variables|/Game/DustDevil/UI/PauseMenu/WBP_PauseMenu.WBP_PauseMenu_C|GetSettingsMenu (Variables|Widgets|GetPauseMenu)
                    (:then)
                    (:else
                      (Widget|RemovefromParent (Variables|Widgets|GetPauseMenu))
                      (Variables|Default|SetMenuOpened "NewEnumerator4")
                      (Game|SetGamePaused false)
                      (CallFunction|SwitchCursor false)
                      (goto _label_2))))))))
        (:else
          (bind _returnvalue (UserInterface|CreateWidget "/Game/DustDevil/UI/PauseMenu/WBP_PauseMenu.WBP_PauseMenu_C" self 0 0 _player))
          (Variables|Widgets|SetPauseMenu _returnvalue)
          (goto _label))))
    (:Is%20Not%20Valid
      (Development|PrintString "PC - get player ref not valid!"))))

(event EventAddBossHealthBar
  (params (BossEnemy :type Actor%20Object%20Reference))
  (Default|AddBossHealthBar (Variables|Widgets|GetHUD) BossEnemy))

(event EventSwitchCursor
  (params (bInMenu :type Boolean))
  (if bInMenu
    (Class|PlayerController|SetMouseCursorWidget "Default" (Variables|Cursors|GetDefaultCursor))
    (else
      (Class|PlayerController|SetMouseCursorWidget "Default" (Variables|Cursors|GetReticleCursor)))))

(event EventRemoveBossHealthBar
  (Default|RemoveBossHealthBar (Variables|Widgets|GetHUD)))

(event EventToggleCursor
  (params (bEnable :type Boolean) (bInMenu :type Boolean) (FocusedWidget :type Widget%20Object%20Reference))
  (bind _self self)
  (bind _output_get (Variables|Default|SetbShowMouseCursor bEnable))
  (if _output_get
    (Input|SetInputModeGameandUI _self FocusedWidget "DoNotLock" false true)
    (Class|PlayerController|SetMouseCursorWidget "Default" (select bInMenu (Variables|Cursors|GetDefaultCursor) (Variables|Cursors|GetReticleCursor)))
    (else
      (Input|SetInputModeGameOnly _self true))))

(event EventToggleAbilityMenu
  (bind _player (Class|BPIPlayerTrigger|GetPlayerCharacter(Message) (Game|Player|GetPlayerPawn 0)))
  (Utilities|IsValid _player
    (:Is%20Valid
      (Variables|Widgets|GetAbilityMenu
        (:then
          (switch Utilities|FlowControl|Switch|SwitchonE_Menus (Variables|Default|GetMenuOpened)
            (:NewEnumerator4
              (UserInterface|Viewport|AddtoViewport (Variables|Widgets|GetAbilityMenu) 1 :!label _label)
              (Game|SetGamePaused true)
              (Variables|Default|SetMenuOpened "NewEnumerator2"))
            (:NewEnumerator2
              (Widget|RemovefromParent (Variables|Widgets|GetAbilityMenu))
              (Game|SetGamePaused false)
              (Utilities|FlowControl|DelayUntilNextTick)
              (CallFunction|SwitchCursor false))))
        (:else
          (bind _returnvalue (UserInterface|CreateWidget "/Game/DustDevil/UI/AbilityMenu/WBP_AbilitySelection.WBP_AbilitySelection_C" self _player))
          (Variables|Widgets|SetAbilityMenu _returnvalue)
          (goto _label)))
      (if (Widget|IsVisible (Variables|Widgets|GetHUD))
        (Widget|SetVisibility (Variables|Widgets|GetHUD) "Hidden")
        (CallFunction|UpdateMinimapVisibility false)
        (else
          (Widget|SetVisibility (Variables|Widgets|GetHUD) "Visible")
          (CallFunction|UpdateMinimapVisibility true))))
    (:Is%20Not%20Valid
      (Development|PrintString "PC - get player ref not valid!"))))

(event EventSetOpenedMenu
  (params (OpenedMenu :type E_Menus%20Enum :default "NewEnumerator4"))
  (Variables|Default|SetMenuOpened OpenedMenu))

(event EventToggleFuelSiloMenu
  (params (FuelSilo :type BP%20Prototype%20Fuel%20Silo%20Object%20Reference))
  (bind _player (Class|BPIPlayerTrigger|GetPlayerCharacter(Message) (Game|Player|GetPlayerPawn 0)))
  (Utilities|IsValid _player
    (:Is%20Valid
      (Variables|Widgets|GetFuelSiloMenu
        (:then
          (switch Utilities|FlowControl|Switch|SwitchonE_Menus (Variables|Default|GetMenuOpened)
            (:NewEnumerator4
              (UserInterface|Viewport|AddtoViewport (stale _output_get) 0 :!label _label)
              (Utilities|FlowControl|DelayUntilNextTick)
              (Variables|Default|SetMenuOpened "NewEnumerator7"))
            (:NewEnumerator7
              (Widget|RemovefromParent (Variables|Widgets|GetFuelSiloMenu))
              (Utilities|FlowControl|DelayUntilNextTick)
              (Variables|Default|SetMenuOpened "NewEnumerator4"))))
        (:else
          (bind _returnvalue (UserInterface|CreateWidget "/Game/DustDevil/UI/Objectives/WBP_FuelSilo.WBP_FuelSilo_C" self 0 (Variables|Widgets|GetHUD)))
          (bind _output_get (Variables|Widgets|SetFuelSiloMenu _returnvalue))
          (goto _label))))))

(event EventToggleMinimapVisibility
  (params (bIsVisible :type Boolean))
  (CallFunction|UpdateMinimapVisibility bIsVisible))

(event EventToggleHUDVisibility
  (if (Widget|IsVisible (Variables|Widgets|GetHUD))
    (Widget|SetVisibility (Variables|Widgets|GetHUD) "Hidden")
    (CallFunction|UpdateMinimapVisibility false)
    (else
      (Widget|SetVisibility (Variables|Widgets|GetHUD) "Visible")
      (CallFunction|UpdateMinimapVisibility true))))

(event EventSwitchInput
  (params (bInMenu :type Boolean))
  (bind _self self)
  (bind _self_2 self)
  (bind _returnvalue (PlayerController|LocalPlayerSubsystems|GetEnhancedInputLocalPlayerSubsystem _self))
  (bind _returnvalue_2 (PlayerController|LocalPlayerSubsystems|GetEnhancedInputLocalPlayerSubsystem _self_2))
  (bind _returnvalue_3 (PlayerController|LocalPlayerSubsystems|GetEnhancedInputLocalPlayerSubsystem _self_2))
  (bind _returnvalue_4 (PlayerController|LocalPlayerSubsystems|GetEnhancedInputLocalPlayerSubsystem _self))
  (if bInMenu
    (Utilities|FlowControl|Sequence
      (:then_0
        (Utilities|IsValid _returnvalue_4
          (:Is%20Valid
            (Input|RemoveMappingContext _returnvalue_4 "/Game/DustDevil/Core/Inputs/IMC_Gameplay.IMC_Gameplay" "(bIgnoreAllPressedKeysUntilRelease=True,bForceImmediately=False,bNotifyUserSettings=False)"))))
      (:then_1
        (Utilities|IsValid _returnvalue
          (:Is%20Valid
            (Input|AddMappingContext _returnvalue "/Game/DustDevil/Core/Inputs/IMC_Menus.IMC_Menus" 0 "(bIgnoreAllPressedKeysUntilRelease=True,bForceImmediately=False,bNotifyUserSettings=False)")))))
    (else
      (Utilities|FlowControl|Sequence
        (:then_0
          (Utilities|IsValid _returnvalue_2
            (:Is%20Valid
              (Input|RemoveMappingContext _returnvalue_2 "/Game/DustDevil/Core/Inputs/IMC_Menus.IMC_Menus" "(bIgnoreAllPressedKeysUntilRelease=True,bForceImmediately=False,bNotifyUserSettings=False)"))))
        (:then_1
          (Utilities|IsValid _returnvalue_3
            (:Is%20Valid
              (Input|AddMappingContext _returnvalue_3 "/Game/DustDevil/Core/Inputs/IMC_Gameplay.IMC_Gameplay" 0 "(bIgnoreAllPressedKeysUntilRelease=True,bForceImmediately=False,bNotifyUserSettings=False)"))))))))

(fn ConstructionScript)

(fn UpdateMinimapVisibility
  (params (IsVisible :type Boolean))
  (if IsVisible
    (bind _foundwidgets (Widget|GetAllWidgetsOfClass "/Game/DustDevil/UI/HUD/Minimap/TextureBased/WBP_MinimapIcon.WBP_MinimapIcon_C" true))
    (for _array_element _foundwidgets
      (Default|ToggleIconVisibility _array_element true))
    (else
      (bind _foundwidgets_2 (Widget|GetAllWidgetsOfClass "/Game/DustDevil/UI/HUD/Minimap/TextureBased/WBP_MinimapIcon.WBP_MinimapIcon_C" true))
      (for _array_element_2 _foundwidgets_2
        (Default|ToggleIconVisibility _array_element_2 false)))))

(fn GetCursors
  (return (Variables|Cursors|GetReticleCursor) (Variables|Cursors|GetDefaultCursor)))

(fn GetFuelSiloMenu
  (bind _fuelsilomenu (Variables|Widgets|GetFuelSiloMenu)
    (:then
      (return _fuelsilomenu))
    (:else)))

(fn GetOpenedMenu
  (return (Variables|Default|GetMenuOpened)))