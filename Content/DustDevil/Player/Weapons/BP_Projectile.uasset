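; Player weapon bullet in DustDevil that flies forward on Tick until its short lifespan expires.
; Sphere overlaps with shootable, non-immune actors other than the instigator apply GE_Damage through GAS, then stop the bullet and shorten its remaining life.
; It sends the instigator damage and Furious upgrade hit events, flags the GC_Furious cue actor, and reports a miss on EndPlay if nothing was hit.
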(event OnComponentBeginOverlap(CollisionSphere)
  (params (OverlappedComponent :type Primitive%20Component%20Object%20Reference) (OtherActor :type Actor%20Object%20Reference) (OtherComp :type Primitive%20Component%20Object%20Reference) (OtherBodyIndex :type Integer) (bFromSweep :type Boolean) (SweepResult :type Hit%20Result%20Structure%20%28by%20ref%29))
  (bind _returnvalue (Ability|GetAbilitySystemComponent OtherActor))
  (Utilities|FlowControl|Sequence
    (:then_0
      (if (and (Utilities|DoesObjectImplementInterface OtherActor "/Game/DustDevil/Core/Interfaces/BPI_Shootable.BPI_Shootable_C") (!= (Game|GetInstigator) OtherActor))
        (if (not (GameplayTags|HasMatchingGameplayTag _returnvalue "(TagName=\"State.Damage.Immune\")"))
          (GameplayEffects|ApplyGameplayEffectToTarget :self (Ability|GetAbilitySystemComponent (Game|GetInstigator)) :GameplayEffectClass "/Game/DustDevil/Core/GAS/Effects/GE_Damage.GE_Damage_C" :Target _returnvalue :Level 1.0)
          (Utilities|FlowControl|Sequence
            (:then_0
              (Ability|SendGameplayEventtoActor (Game|GetInstigator) "(TagName=\"Upgrades.Offense.Furious.Hit\")")
              (Variables|Default|SetbHitSomething true)
              (bind _returnvalue_2 (Actor|GetActorOfClass "/Game/DustDevil/Core/GAS/Cues/GC_Furious.GC_Furious_C"))
              (Utilities|IsValid _returnvalue_2
                (:Is%20Valid
                  (Variables|/Game/DustDevil/Core/GAS/Cues/GC_Furious.GC_Furious_C|SetHitSomething _returnvalue_2 true))))
            (:then_1
              (Ability|SendGameplayEventtoActor (Game|GetInstigator) "(TagName=\"Event.Damage.Bullet.Instigator\")"))
            (:then_2
              (CallFunction|InvalidateProjectile))))))))

(event EventBeginPlay
  (Actor|SetLifeSpan 5.0))

(event EventEndPlay
  (params (EndPlayReason :type EEndPlayReason%20Enum :default "Destroyed"))
  (bind _returnvalue (Game|GetInstigator))
  (if (not (Variables|Default|GetbHitSomething))
    (if (and (Utilities|IsValid (Ability|GetAbilitySystemComponent _returnvalue)) (Utilities|IsValid _returnvalue))
      (Ability|SendGameplayEventtoActor _returnvalue "(TagName=\"Upgrades.Offense.Furious.Miss\")"))))

(event EventTick
  (params (DeltaSeconds :type Float%20%28single-precision%29))
  (Transformation|AddActorLocalOffset (* DeltaSeconds (Variables|Default|GetSpeed) (Transformation|GetActorForwardVector)) false false))

(fn ConstructionScript)

(fn InvalidateProjectile
  (Variables|Default|SetSpeed 0.0)
  (Collision|SetCollisionEnabled (Variables|Default|GetCollisionSphere) "NoCollision")
  (Actor|SetLifeSpan 1.0))