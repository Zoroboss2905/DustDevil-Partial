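; Player minigun weapon that fires projectiles from the turret barrel and treats its magazine as a heat gauge on the HUD.
; While firing, a looping timer drains ammo as heat, with an ability-system attribute giving a chance to skip the drain.
; Stopping fire triggers cooling through the reload system, while an empty magazine overheats the gun.
; Reload type sets cooling speed, and a second timer maps reload progress back to ammo.
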(event Custom|FadeOutMinigun
  (bind _minigunfiringloop (Variables|Default|GetMinigunFiringLoop)
    (:then
      (Audio|Components|Audio|FadeOut _minigunfiringloop 0.1 0.0 "Linear" :!class /Script/Engine.AudioComponent))
    (:else)))

(event EventOnStopUse
  (bind _overheatuphandle (Variables|Function|GetOverheatUpHandle))
  (if (Class|KismetSystemLibrary|TimerExistsHandle _overheatuphandle)
    (Utilities|Time|ClearandInvalidateTimerbyHandle _overheatuphandle))
  (if (Class|KismetSystemLibrary|TimerExistsHandle (Variables|Function|GetOverheatDownHandle))
    (bind _minigunfiringloop (Variables|Default|GetMinigunFiringLoop :!label _label)
      (:then
        (Audio|Components|Audio|FadeOut _minigunfiringloop 0.1 0.0 "Linear" :!class /Script/Engine.AudioComponent))
      (:else))
    (else
      (Utilities|FlowControl|Sequence
        (:then_0
          (goto _label))
        (:then_1
          (Class|TopMountBase|TryReload "R_MANUAL")
          (Utilities|FlowControl|DelayUntilNextTick)
          (Variables|Default|SetReloadSpeedMulti 0.5))))))

(event EventOnStartUse)

(event EventOnTryReload
  (params (ReloadType :type EReloadType%20Enum :default "R_MANUAL"))
  (Variables|Default|SetReloadSpeedMulti (Utilities|Select :Index ReloadType :R_MANUAL 2.0 :R_EMPTY 1.0 :R_FORCED 1e+01))
  (if (Variables|Default|GetbInputDown)
    (Class|TopMountBase|StopUse)))

(event EventFire
  (bind _returnvalue (|BitmaskLiteral 2))
  (bind _returnvalue_2 (Game|GetInstigator))
  (bind _minigunfiringloop (Variables|Default|GetMinigunFiringLoop))
  (bind _magazinecapacity (Variables|Default|GetMagazineCapacity))
  (if (not (Variables|Function|GetbOverheated))
    (if (<= (Variables|Default|GetMagazineAmmoCount) 0.0)
      (Class|TopMountBase|StopUse)
      (Variables|Function|SetbOverheated true)
      (Default|CallPlayOverheatAnim (Variables|/Game/DustDevil/UI/HUD/WBP_HUD.WBP_HUD_C|GetHeatMeter (Variables|/Game/DustDevil/Player/BP_Vehicle.BP_Vehicle_C|GetHUD (Variables|Default|GetPlayer_0))))
      (if (Variables|Default|GetbAutoReload)
        (Class|TopMountBase|TryReload "R_EMPTY"))
      (else
        (if (== (Class|KismetMathLibrary|AndIntInt (Variables|Default|GetDisabledReasons) _returnvalue) _returnvalue)
          (Class|TopMountBase|CancelReload))
        (if (Audio|Components|Audio|IsPlaying _minigunfiringloop)
          _
          (else
            (Audio|Components|Audio|Play _minigunfiringloop 0.0)))
        (Game|SpawnActorfromClass "/Game/DustDevil/Player/Weapons/BP_Projectile.BP_Projectile_C" (Math|Transform|MakeTransform (Transformation|GetSocketLocation (Variables|Default|GetTurretMesh) "MinigunTurretMesh_Socket") (* (.rotation (Transformation|GetWorldTransform (Variables|Default|GetTurretMesh))) 0.5) "1.000000,1.000000,1.000000") "AlwaysSpawn" "OverrideRootScale" _returnvalue_2 1e+04 _returnvalue_2) ; Fires a projectile Directly from the barrel. Looks better, but much easier to miss the target
        (Default|CamShakeMini (Variables|Default|GetPlayer_0))
        (Niagara|SpawnSystemAttached "/Game/DustDevil/Effects/VehicleBullet/Muzzleflash/NS_Muzzleflash.NS_Muzzleflash" (Variables|Default|GetTurretMesh) "None" "325.000000,0.000000,60.000000" "0.000000,-90.000000,0.000000" "KeepRelativeOffset" false)
        (if (Utilities|Time|IsTimerActivebyHandle (Variables|Function|GetOverheatUpHandle))
          _
          (else
            (bind _returnvalue_3 (Utilities|Time|SetTimerbyFunctionName 0 "IncreaseHeat" 0.01 true))
            (Variables|Function|SetOverheatUpHandle _returnvalue_3)))
        (Default|UpdateHeatMeter (Variables|/Game/DustDevil/Player/BP_Vehicle.BP_Vehicle_C|GetHUD (Variables|Default|GetPlayer_0)) (- _magazinecapacity (Variables|Default|GetMagazineAmmoCount)) _magazinecapacity 0.0)))))

(event EventMisfire
  (params (MisfireReason :type EMisfireType%20Enum :default "M_AMMO"))
  (Utilities|FlowControl|Sequence
    (:then_0
      (switch Utilities|FlowControl|Switch|SwitchonEMisfireType MisfireReason
        (:M_AMMO
          (Development|PrintString "Minigun Out of Ammo!"))
        (:M_COOLDOWN
          (Development|PrintString "Minigun on Cooldown!"))
        (:M_JAMMED
          (Utilities|FlowControl|Sequence
            (:then_0
              (Development|PrintString "Minigun is Jammed!"))
            (:then_1
              (bind _player (Class|BPIPlayerTrigger|GetPlayerCharacter(Message) (Components|GetOwner)))
              (Class|BPIHUDUpdates|DisplayWarningMessage(Message) (Variables|/Game/DustDevil/Player/BP_Vehicle.BP_Vehicle_C|GetHUD _player) (Variables|Default|GetFuelDepotWarningText)))))))
    (:then_1
      (if (Class|KismetSystemLibrary|TimerExistsHandle (Variables|Function|GetOverheatDownHandle))
        (bind _minigunfiringloop (Variables|Default|GetMinigunFiringLoop :!label _label)
          (:then
            (Audio|Components|Audio|FadeOut _minigunfiringloop 0.1 0.0 "Linear" :!class /Script/Engine.AudioComponent))
          (:else))
        (else
          (Utilities|FlowControl|Sequence
            (:then_0
              (goto _label))
            (:then_1
              (Class|TopMountBase|TryReload "R_MANUAL")
              (Utilities|FlowControl|DelayUntilNextTick)
              (Variables|Default|SetReloadSpeedMulti 0.5))))))))

(event EventBeginPlay
  (Variables|Default|SetbAimable true)
  (bind _player (Class|BPIPlayerTrigger|GetPlayerCharacter(Message) (Game|Player|GetPlayerPawn 0)))
  (Variables|Default|SetPlayer_0 _player))

(event EventOnTryReloadFailed
  (params (FailureReason :type EReloadFailureReason%20Enum :default "RF_UNKNOWN"))
  (switch Utilities|FlowControl|Switch|SwitchonEReloadFailureReason FailureReason
    (:RF_CANCELLED
      (Utilities|Time|ClearandInvalidateTimerbyHandle (Variables|Function|GetOverheatDownHandle)) ; Cancel Reloading
      (Utilities|Time|ClearandInvalidateTimerbyHandle (Variables|Function|GetOverheatUpHandle)))
    (:RF_RELOADING
      (Class|TopMountBase|CancelReload)
      (Class|TopMountBase|TryReload "R_MANUAL"))))

(event EventOnReloadStarted
  (Variables|Default|SetReloadTimeCurrent (* (/ (Variables|Default|GetMagazineAmmoCount) (Variables|Default|GetMagazineCapacity)) (Variables|Default|GetReloadTimeMax)))
  (bind _returnvalue (Utilities|Time|SetTimerbyFunctionName 0 "ReduceHeat" 0.1 true))
  (Variables|Function|SetOverheatDownHandle _returnvalue)
  (Utilities|FlowControl|Sequence
    (:then_0
      (bind _minigunfiringloop (Variables|Default|GetMinigunFiringLoop)
        (:then
          (Audio|Components|Audio|FadeOut _minigunfiringloop 0.1 0.0 "Linear" :!class /Script/Engine.AudioComponent))
        (:else)))
    (:then_1
      (bind _minigunoverheat (Variables|Default|GetMinigunOverheat)
        (:then
          (Audio|Components|Audio|FadeIn _minigunoverheat 0.1 1.0 0.0 "Linear" :!class /Script/Engine.AudioComponent))
        (:else)))))

(event EventOnReloadFinished
  (bind _magazinecapacity (Variables|Default|GetMagazineCapacity))
  (Utilities|Time|ClearandInvalidateTimerbyHandle (Variables|Function|GetOverheatDownHandle))
  (Variables|Default|SetMagazineAmmoCount (Variables|Default|GetMagazineCapacity))
  (Default|UpdateHeatMeter (Variables|/Game/DustDevil/Player/BP_Vehicle.BP_Vehicle_C|GetHUD (Variables|Default|GetPlayer_0)) (- _magazinecapacity (Variables|Default|GetMagazineAmmoCount)) _magazinecapacity (Variables|Default|GetMagazineAmmoCount))
  (Variables|Function|SetbOverheated false)
  (Default|ReloadFinished (Variables|/Game/DustDevil/UI/HUD/WBP_HUD.WBP_HUD_C|GetHeatMeter (Variables|/Game/DustDevil/Player/BP_Vehicle.BP_Vehicle_C|GetHUD (Variables|Default|GetPlayer_0))))
  (bind _minigunoverheat (Variables|Default|GetMinigunOverheat)
    (:then
      (Audio|Components|Audio|FadeOut _minigunoverheat 0.0 0.0 "Linear" :!class /Script/Engine.AudioComponent))
    (:else)))

(fn ConstructionScript)

(fn ReduceHeat
  (bind _magazinecapacity (Variables|Default|GetMagazineCapacity))
  (Variables|Default|SetMagazineAmmoCount (* (/ (Variables|Default|GetReloadTimeCurrent) (Variables|Default|GetReloadTimeMax)) (Variables|Default|GetMagazineCapacity)))
  (Default|UpdateHeatMeter (Variables|/Game/DustDevil/Player/BP_Vehicle.BP_Vehicle_C|GetHUD (Variables|Default|GetPlayer_0)) (- _magazinecapacity (Variables|Default|GetMagazineAmmoCount)) _magazinecapacity 0.0))

(fn GetWeaponData
  (return "NewEnumerator1" (Math|Float|Truncate (Variables|Default|GetMagazineCapacity)) (Math|Float|Truncate (Variables|Default|GetMagazineAmmoCount)) (Variables|Default|GetCooldownMax) (Variables|Default|GetCooldownCurrent) (Variables|Default|GetMisfireCDCurrent) 0.0 0.0))

(fn IncreaseHeat
  (if (<= (Math|Random|RandomFloatinRange 1.0 1e+02) (.ReturnValue (Ability|Attribute|GetFloatAttributefromAbilitySystemComponent (Ability|GetAbilitySystemComponent (Components|GetOwner)) "(AttributeName=\"TrickChance\",Attribute=/Script/DustDevil.VehicleAttributeSet:TrickChance,AttributeOwner=\"/Script/CoreUObject.Class'/Script/DustDevil.VehicleAttributeSet'\")")))
    (GameplayCue|ExecuteGameplayCueOnActor(Burst) (Variables|Default|GetInstigator) "(TagName=\"GameplayCue.Ability.BulletFarmer\")" (Ability|GameplayCue|MakeGameplayCueParameters 0.0))
    (else
      (Variables|Default|SetMagazineAmmoCount (- (Variables|Default|GetMagazineAmmoCount) 0.01)))))

(fn UpdateHeatMeter
  (Default|StartReload (Variables|/Game/DustDevil/Player/BP_Vehicle.BP_Vehicle_C|GetHUD (Variables|Default|GetPlayer_0)) (Variables|Default|GetReloadTimeCurrent) (Variables|Default|GetReloadTimeMax)))