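; BP_Autocannon is a player vehicle weapon that fires explosive projectiles from its turret, with blast radius scaled by weapon level.
; Each shot passes the player-to-cursor distance as the explode distance, then adds sound, muzzle flash and camera shake.
; Firing and reload events update the vehicle HUD's ammo meter, with a looping timer driving reload progress.
; Misfires print their reason, and a jam also shows a fuel-storage warning.
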(event EventOnStopUse)

(event EventOnStartUse)

(event EventOnTryReload
  (params (ReloadType :type EReloadType%20Enum :default "R_MANUAL"))
  (switch Utilities|FlowControl|Switch|SwitchonEReloadType ReloadType))

(event EventFire
  (bind _returnvalue (Game|GetInstigator))
  (bind _playerref (Variables|Default|GetPlayerRef))
  (bind _playerref_2 (Variables|Default|GetPlayerRef))
  (bind _hud (Variables|/Game/DustDevil/Player/BP_Vehicle.BP_Vehicle_C|GetHUD _playerref_2))
  (bind _reloadmeter (Variables|/Game/DustDevil/UI/HUD/WBP_HUD.WBP_HUD_C|GetReloadMeter _hud))
  (|CallParentFunction)
  (Audio|PlaySound2D "/Game/DustDevil/Audio/Weapons/A_Autocannon_Cue.A_Autocannon_Cue" 1.0 1.0 0.0 0 0)
  (Game|SpawnActorfromClass "/Game/DustDevil/Player/Weapons/BP_ExplosiveProjectile.BP_ExplosiveProjectile_C" (Math|Transform|MakeTransform (Transformation|GetSocketLocation (Variables|Default|GetTurretMesh) "BasicTurretMeshBarrel_Socket") (* (.rotation (Transformation|GetWorldTransform (Variables|Default|GetTurretMesh))) 0.5) "1.000000,1.000000,1.000000") "AlwaysSpawn" "OverrideRootScale" _returnvalue 5e+04 (Utilities|Select :Index (Math|Float|Floor (Variables|Default|GetWeaponLevel)) :Option%200 4e+02 :Option%201 4e+02 :Option%202 5e+02 :Option%203 6e+02) (Math|Vector|Distance(Vector) (Variables|/Script/DustDevil.Vehicle|GetCursorHitLoc _playerref) (Transformation|GetActorLocation _playerref)) (Variables|Default|GetWeaponLevel) _returnvalue) ; Fires a projectile Directly from the barrel. Looks better, but much easier to miss the target
  (Niagara|SpawnSystemAttached "/Game/DustDevil/Effects/VehicleBullet/Muzzleflash/NS_Muzzleflash.NS_Muzzleflash" (Variables|Default|GetTurretMesh) "AutocannonMeshBarrel_Socket" "350.000000,0.000000,40.000000" "0.000000,-90.000000,0.000000" "KeepRelativeOffset" false)
  (Default|UpdateAmmoCount _reloadmeter (Variables|Default|GetMagazineAmmoCount) 0.0)
  (Default|UpdateAmmoBar _reloadmeter (Variables|Default|GetMagazineAmmoCount) (Variables|Default|GetMagazineCapacity))
  (Default|CamShakeAutoCannon (Variables|Default|GetPlayerRef)))

(event EventMisfire
  (params (MisfireReason :type EMisfireType%20Enum :default "M_AMMO"))
  (Utilities|FlowControl|Sequence
    (:then_0
      (switch Utilities|FlowControl|Switch|SwitchonEMisfireType MisfireReason
        (:M_AMMO
          (Development|PrintString "Machine Gun Out of Ammo!"))
        (:M_COOLDOWN
          (Development|PrintString "Machine Gun on Cooldown!"))
        (:M_JAMMED
          (Utilities|FlowControl|Sequence
            (:then_0
              (Development|PrintString "Machine Gun is Jammed!"))
            (:then_1
              (bind _player (Class|BPIPlayerTrigger|GetPlayerCharacter(Message) (Components|GetOwner)))
              (Class|BPIHUDUpdates|DisplayWarningMessage(Message) (Variables|/Game/DustDevil/Player/BP_Vehicle.BP_Vehicle_C|GetHUD _player) "It would be unwise to fire a gun next to highly flammable fuel storage!"))))))))

(event EventBeginPlay
  (Variables|Default|SetbAimable true)
  (bind _returnvalue (Actor|GetActorOfClass "/Game/DustDevil/Player/BP_Vehicle.BP_Vehicle_C"))
  (Variables|Default|SetPlayerRef _returnvalue)
  (Utilities|FlowControl|Delay 0.2)
  (bind _hud (Variables|/Game/DustDevil/Player/BP_Vehicle.BP_Vehicle_C|GetHUD (Variables|Default|GetPlayerRef))
    (:then
      (Default|UpdateAmmoCount (Variables|/Game/DustDevil/UI/HUD/WBP_HUD.WBP_HUD_C|GetReloadMeter _hud) (Variables|Default|GetMagazineAmmoCount) 0.0))
    (:else)))

(event EventOnTryReloadFailed
  (params (FailureReason :type EReloadFailureReason%20Enum :default "RF_UNKNOWN"))
  (switch Utilities|FlowControl|Switch|SwitchonEReloadFailureReason FailureReason))

(event EventOnReloadStarted
  (Audio|Components|Audio|Play (Variables|Default|GetReload) 0.0)
  (bind _returnvalue (Utilities|Time|SetTimerbyFunctionName 0 "UpdateAmmoMeter" 0.01 true))
  (Variables|Default|SetAmmoMeterTimer _returnvalue)
  (Default|UpdateAmmoCount (Variables|/Game/DustDevil/UI/HUD/WBP_HUD.WBP_HUD_C|GetReloadMeter (Variables|/Game/DustDevil/Player/BP_Vehicle.BP_Vehicle_C|GetHUD (Variables|Default|GetPlayerRef))) 0.0 0.0))

(event EventOnReloadFinished
  (Audio|Components|Audio|FadeOut (Variables|Default|GetReload) 0.25 0.0 "Linear" :!class /Script/Engine.AudioComponent)
  (bind _output_get (Variables|Default|SetMagazineAmmoCount (Variables|Default|GetMagazineCapacity)))
  (Utilities|Time|ClearandInvalidateTimerbyHandle (Variables|Default|GetAmmoMeterTimer))
  (Default|UpdateAmmoCount (Variables|/Game/DustDevil/UI/HUD/WBP_HUD.WBP_HUD_C|GetReloadMeter (Variables|/Game/DustDevil/Player/BP_Vehicle.BP_Vehicle_C|GetHUD (Variables|Default|GetPlayerRef))) _output_get 0.0))

(fn ConstructionScript)

(fn GetWeaponData
  (return "NewEnumerator3" (Math|Float|Truncate (Variables|Default|GetMagazineCapacity)) (Math|Float|Truncate (Variables|Default|GetMagazineAmmoCount)) (Variables|Default|GetCooldownMax) (Variables|Default|GetCooldownCurrent) (Variables|Default|GetMisfireCDCurrent) 0.0 0.0))

(fn UpdateAmmoMeter
  (Default|StartReload (Variables|/Game/DustDevil/Player/BP_Vehicle.BP_Vehicle_C|GetHUD (Variables|Default|GetPlayerRef)) (Variables|Default|GetReloadTimeCurrent) (Variables|Default|GetReloadTimeMax)))