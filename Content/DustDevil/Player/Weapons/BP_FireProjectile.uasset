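; BP_FireProjectile is a short-lived fire projectile that damages and ignites shootable actors through the Gameplay Ability System.
; After a launch delay, Tick moves it and eases its speed toward zero, widening the overlap sphere as it slows.
; Overlapping a non-instigator, non-immune target applies GE_Damage and GE_Fire, with SetByCaller burn duration derived from remaining lifespan.
; A hit or lifespan threshold invalidates it, switching off emitters and overlap collision.
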(event OnComponentBeginOverlap(Sphere)
  (params (OverlappedComponent :type Primitive%20Component%20Object%20Reference) (OtherActor :type Actor%20Object%20Reference) (OtherComp :type Primitive%20Component%20Object%20Reference) (OtherBodyIndex :type Integer) (bFromSweep :type Boolean) (SweepResult :type Hit%20Result%20Structure%20%28by%20ref%29))
  (bind _returnvalue (Game|GetInstigator))
  (bind _returnvalue_2 (Ability|GetAbilitySystemComponent OtherActor))
  (bind _returnvalue_3 (Ability|GetAbilitySystemComponent _returnvalue))
  (if (and (Utilities|DoesObjectImplementInterface OtherActor "/Game/DustDevil/Core/Interfaces/BPI_Shootable.BPI_Shootable_C") (!= (Game|GetInstigator) OtherActor))
    (if (not (GameplayTags|HasMatchingGameplayTag _returnvalue_2 "(TagName=\"State.Damage.Immune\")"))
      (GameplayEffects|ApplyGameplayEffectToTarget :self _returnvalue_3 :GameplayEffectClass "/Game/DustDevil/Core/GAS/Effects/GE_Damage.GE_Damage_C" :Target _returnvalue_2 :Level 1.0)
      (bind _returnvalue_4 (Ability|GameplayEffect|AssignTagSetbyCallerMagnitude (GameplayEffects|MakeOutgoingSpec _returnvalue_3 "/Game/DustDevil/Core/GAS/Effects/GE_Fire.GE_Fire_C" 1.0 (GameplayEffects|MakeEffectContext _returnvalue_3)) "(TagName=\"Event.Fire.Duration\")" (- (Variables|Default|GetFireDurationBase) (Actor|GetLifeSpan))))
      (GameplayEffects|ApplyGameplayEffectSpecToTarget _returnvalue_3 _returnvalue_4 _returnvalue_2)
      (CallFunction|InvalidateProjectile))))

(event EventBeginPlay
  (Actor|SetLifeSpan 4.0)
  (Variables|Default|SetSpeed (Variables|Default|GetInitialSpeed))
  (Variables|Default|SetFireDurationBase 1e+01)
  (CallFunction|SetEmitters false)
  (Utilities|FlowControl|Delay (Variables|Default|GetInitMoveDelay))
  (CallFunction|SetEmitters true))

(event EventTick
  (params (DeltaSeconds :type Float%20%28single-precision%29))
  (bind _output_get (Variables|Default|SetInitMoveDelay (- (Variables|Default|GetInitMoveDelay) DeltaSeconds)))
  (if (< _output_get 0.0)
    (Transformation|AddActorLocalOffset (* (* DeltaSeconds (Variables|Default|GetSpeed)) (Transformation|GetActorForwardVector)) false false)
    (bind _output_get_2 (Variables|Default|SetSpeed (Math|Interpolation|FInterpTo (Variables|Default|GetSpeed) 0.0 DeltaSeconds 2.0)))
    (Components|Sphere|SetSphereRadius (Variables|Default|GetSphere) (* (- 1.0 (/ _output_get_2 (Variables|Default|GetInitialSpeed))) 1e+02) true)
    (if (< (Actor|GetLifeSpan) 3.0)
      (CallFunction|InvalidateProjectile))))

(fn ConstructionScript)

(fn InvalidateProjectile
  (bind _sphere (Variables|Default|GetSphere))
  (Collision|SetCollisionEnabled _sphere "PhysicsOnly")
  (CallFunction|SetEmitters false)
  (Physics|SetSimulatePhysics _sphere false))

(fn SetEmitters
  (params (bEnabled :type Boolean))
  (bind _fireeffect (Variables|Default|GetFireEffect))
  (Effects|Components|ParticleSystem|SetEmitterEnable _fireeffect "Fountain" bEnabled)
  (Effects|Components|ParticleSystem|SetEmitterEnable _fireeffect "Fountain001" bEnabled)
  (Effects|Components|ParticleSystem|SetEmitterEnable _fireeffect "Fountain002" bEnabled)
  (Effects|Components|ParticleSystem|SetEmitterEnable _fireeffect "Fountain003" bEnabled))