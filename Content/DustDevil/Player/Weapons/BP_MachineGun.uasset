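; Aimable machine gun weapon for the player's vehicle, extending a parent weapon class with firing, reload and misfire feedback.
; Each successful shot spawns a fast projectile from the turret barrel socket, adds muzzle flash, reticle kick and camera shake, and updates HUD ammo.
; A DoOnce starts the looping fire sound, which fades and resets on stop or misfire.
; Reloading refills the magazine while a looping timer drives the HUD reload meter.
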(event Custom|ResetSound
  (Utilities|FlowControl|DoOnce false) ; enters at Reset
)

(event Custom|FadeOutAudio
  (Audio|Components|Audio|FadeOut (Variables|Default|GetMachineGunFiringLoop) 0.1 0.0 "Linear" :!class /Script/Engine.AudioComponent))

(event EventOnStopUse
  (bind _reticlecursor (Variables|/Game/DustDevil/Player/BP_Vehicle.BP_Vehicle_C|GetReticleCursor (Variables|Default|GetPlayerRef))
    (:then
      (Default|DetractCentre _reticlecursor))
    (:else
      _))
  (Audio|Components|Audio|FadeOut (Variables|Default|GetMachineGunFiringLoop) 0.1 0.0 "Linear" :!class /Script/Engine.AudioComponent)
  (CallFunction|ResetSound))

(event EventOnStartUse)

(event EventOnTryReload
  (params (ReloadType :type EReloadType%20Enum :default "R_MANUAL"))
  (switch Utilities|FlowControl|Switch|SwitchonEReloadType ReloadType))

(event EventFire
  (bind _returnvalue (Game|GetInstigator))
  (|CallParentFunction)
  (Utilities|FlowControl|Sequence
    (:then_0
      (Utilities|FlowControl|DoOnce false
        (:Completed
          (Audio|Components|Audio|Play (Variables|Default|GetMachineGunFiringLoop) 0.0))))
    (:then_1
      (Game|SpawnActorfromClass "/Game/DustDevil/Player/Weapons/BP_Projectile.BP_Projectile_C" (Math|Transform|MakeTransform (Transformation|GetSocketLocation (Variables|Default|GetTurretMesh) "BasicTurretMeshBarrel_Socket") (* (.rotation (Transformation|GetWorldTransform (Variables|Default|GetTurretMesh))) 0.5) "1.000000,1.000000,1.000000") "AlwaysSpawn" "OverrideRootScale" _returnvalue 5e+04 _returnvalue) ; Fires a projectile Directly from the barrel. Looks better, but much easier to miss the target
      (Niagara|SpawnSystemAttached "/Game/DustDevil/Effects/VehicleBullet/Muzzleflash/NS_Muzzleflash.NS_Muzzleflash" (Variables|Default|GetTurretMesh) "None" "350.000000,0.000000,40.000000" "0.000000,-90.000000,0.000000" "KeepRelativeOffset" false)
      (Default|ExpandCentre (Variables|/Game/DustDevil/Player/BP_Vehicle.BP_Vehicle_C|GetReticleCursor (Variables|Default|GetPlayerRef)))
      (Default|CamShakeMachine (Variables|Default|GetPlayerRef)))
    (:then_2
      (Default|UpdateAmmoCount (Variables|/Game/DustDevil/Player/BP_Vehicle.BP_Vehicle_C|GetHUD (Variables|Default|GetPlayerRef)) (Variables|Default|GetMagazineAmmoCount) (Variables|Default|GetMagazineCapacity)))))

(event EventMisfire
  (params (MisfireReason :type EMisfireType%20Enum :default "M_AMMO"))
  (Utilities|FlowControl|Sequence
    (:then_0
      (switch Utilities|FlowControl|Switch|SwitchonEMisfireType MisfireReason
        (:M_AMMO
          (Development|PrintString "Machine Gun Out of Ammo!"))
        (:M_COOLDOWN
          (Development|PrintString "Machine Gun on Cooldown!"))
        (:M_JAMMED
          (Utilities|FlowControl|Sequence
            (:then_0
              (Development|PrintString "Machine Gun is Jammed!"))
            (:then_1
              (bind _player (Class|BPIPlayerTrigger|GetPlayerCharacter(Message) (Components|GetOwner)))
              (Class|BPIHUDUpdates|DisplayWarningMessage(Message) (Variables|/Game/DustDevil/Player/BP_Vehicle.BP_Vehicle_C|GetHUD _player) (Variables|Default|GetFuelDepotWarningText)))))))
    (:then_1
      (Default|DetractCentre (stale EventOnStopUse _reticlecursor))
      (Audio|Components|Audio|FadeOut (Variables|Default|GetMachineGunFiringLoop) 0.1 0.0 "Linear" :!class /Script/Engine.AudioComponent)
      (CallFunction|ResetSound))))

(event EventBeginPlay
  (Variables|Default|SetbAimable true)
  (bind _returnvalue (Actor|GetActorOfClass "/Game/DustDevil/Player/BP_Vehicle.BP_Vehicle_C"))
  (Variables|Default|SetPlayerRef _returnvalue)
  (Utilities|FlowControl|Delay 0.3)
  (bind _hud (Variables|/Game/DustDevil/Player/BP_Vehicle.BP_Vehicle_C|GetHUD (Variables|Default|GetPlayerRef))
    (:then
      (Default|UpdateAmmoCount (Variables|/Game/DustDevil/UI/HUD/WBP_HUD.WBP_HUD_C|GetReloadMeter _hud) (Variables|Default|GetMagazineAmmoCount) 0.0))
    (:else)))

(event EventOnTryReloadFailed
  (params (FailureReason :type EReloadFailureReason%20Enum :default "RF_UNKNOWN"))
  (switch Utilities|FlowControl|Switch|SwitchonEReloadFailureReason FailureReason))

(event EventOnReloadStarted
  (Audio|Components|Audio|Play (Variables|Default|GetReload) 0.0)
  (Audio|Components|Audio|FadeOut (Variables|Default|GetMachineGunFiringLoop) 0.1 0.0 "Linear" :!class /Script/Engine.AudioComponent)
  (bind _returnvalue (Utilities|Time|SetTimerbyFunctionName 0 "UpdateAmmoMeter" 0.01 true))
  (Variables|Default|SetAmmoMeterTimer _returnvalue)
  (Default|UpdateAmmoCount (Variables|/Game/DustDevil/UI/HUD/WBP_HUD.WBP_HUD_C|GetReloadMeter (Variables|/Game/DustDevil/Player/BP_Vehicle.BP_Vehicle_C|GetHUD (Variables|Default|GetPlayerRef))) 0.0 0.0))

(event EventOnReloadFinished
  (Audio|Components|Audio|FadeOut (Variables|Default|GetReload) 0.25 0.0 "Linear" :!class /Script/Engine.AudioComponent)
  (Variables|Default|SetMagazineAmmoCount (Variables|Default|GetMagazineCapacity))
  (Utilities|Time|ClearandInvalidateTimerbyHandle (Variables|Default|GetAmmoMeterTimer))
  (Default|UpdateAmmoCount (Variables|/Game/DustDevil/UI/HUD/WBP_HUD.WBP_HUD_C|GetReloadMeter (Variables|/Game/DustDevil/Player/BP_Vehicle.BP_Vehicle_C|GetHUD (Variables|Default|GetPlayerRef))) (Variables|Default|GetMagazineCapacity) 0.0)
  (CallFunction|ResetSound))

(fn ConstructionScript)

(fn GetWeaponData
  (return "NewEnumerator0" (Math|Float|Truncate (Variables|Default|GetMagazineCapacity)) (Math|Float|Truncate (Variables|Default|GetMagazineAmmoCount)) (Variables|Default|GetCooldownMax) (Variables|Default|GetCooldownCurrent) (Variables|Default|GetMisfireCDCurrent) 0.0 0.0))

(fn UpdateAmmoMeter
  (Default|StartReload (Variables|/Game/DustDevil/Player/BP_Vehicle.BP_Vehicle_C|GetHUD (Variables|Default|GetPlayerRef)) (Variables|Default|GetReloadTimeCurrent) (Variables|Default|GetReloadTimeMax)))