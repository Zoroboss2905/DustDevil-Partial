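; Explosive player weapon projectile that moves forward each tick and explodes after a set distance or on hitting a non-immune shootable other than its instigator.
; Direct hits apply GAS damage.
; The explosion sphere-traces, applying distance-scaled SetByCaller radial damage (factor capped at 0.2) and weapon-level bleed, spawns Niagara, then disables the projectile.
; It sends the instigator Furious upgrade Hit events on direct hits, otherwise Miss on EndPlay.
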(event OnComponentBeginOverlap(CollisionSphere)
  (params (OverlappedComponent :type Primitive%20Component%20Object%20Reference) (OtherActor :type Actor%20Object%20Reference) (OtherComp :type Primitive%20Component%20Object%20Reference) (OtherBodyIndex :type Integer) (bFromSweep :type Boolean) (SweepResult :type Hit%20Result%20Structure%20%28by%20ref%29))
  (bind _returnvalue (Ability|GetAbilitySystemComponent OtherActor))
  (if (and (Utilities|DoesObjectImplementInterface OtherActor "/Game/DustDevil/Core/Interfaces/BPI_Shootable.BPI_Shootable_C") (!= (Game|GetInstigator) OtherActor))
    (if (not (GameplayTags|HasMatchingGameplayTag _returnvalue "(TagName=\"State.Damage.Immune\")"))
      (GameplayEffects|ApplyGameplayEffectToTarget :self (Ability|GetAbilitySystemComponent (Game|GetInstigator)) :GameplayEffectClass "/Game/DustDevil/Core/GAS/Effects/GE_Damage.GE_Damage_C" :Target _returnvalue :Level 1.0)
      (Utilities|FlowControl|Sequence
        (:then_0
          (Ability|SendGameplayEventtoActor (Game|GetInstigator) "(TagName=\"Upgrades.Offense.Furious.Hit\")")
          (Variables|Default|SetbHitSomething true))
        (:then_1
          (CallFunction|Explode))))))

(event EventBeginPlay
  (Actor|SetLifeSpan 5.0))

(event EventEndPlay
  (params (EndPlayReason :type EEndPlayReason%20Enum :default "Destroyed"))
  (bind _returnvalue (Game|GetInstigator))
  (if (not (Variables|Default|GetbHitSomething))
    (if (and (Utilities|IsValid (Ability|GetAbilitySystemComponent _returnvalue)) (Utilities|IsValid _returnvalue))
      (Ability|SendGameplayEventtoActor _returnvalue "(TagName=\"Upgrades.Offense.Furious.Miss\")"))))

(event EventTick
  (params (DeltaSeconds :type Float%20%28single-precision%29))
  (bind _speed (Variables|Default|GetSpeed))
  (bind _returnvalue (* DeltaSeconds _speed))
  (Transformation|AddActorLocalOffset (* _returnvalue (Transformation|GetActorForwardVector)) false false)
  (bind _output_get (Variables|Default|SetExplodeDistance (- (Variables|Default|GetExplodeDistance) _returnvalue)))
  (if (<= _output_get 0.0)
    (Utilities|FlowControl|DoOnce false
      (:Completed
        (CallFunction|Explode)))))

(fn ConstructionScript)

(fn InvalidateProjectile
  (Variables|Default|SetSpeed 0.0)
  (Collision|SetCollisionEnabled (Variables|Default|GetCollisionSphere) "NoCollision")
  (Actor|SetLifeSpan 1.0))

(fn Explode
  (bind _returnvalue (Transformation|GetActorLocation))
  (bind _instigator (Variables|Actor|GetInstigator))
  (bind _returnvalue_2 (Ability|GetAbilitySystemComponent _instigator))
  (bind _outhits (Collision|MultiSphereTraceForObjects _returnvalue _returnvalue (Variables|Default|GetExplosionRadius) (Utilities|Array|MakeArray "ObjectTypeQuery8") false (Utilities|Array|MakeArray (Variables|Actor|GetInstigator)) "None" true "(R=1.000000,G=0.000000,B=0.000000,A=1.000000)" "(R=0.000000,G=1.000000,B=0.000000,A=1.000000)" 3.0))
  (for _array_element _outhits
    (bind _returnvalue_3 (Ability|GameplayEffect|AssignTagSetbyCallerMagnitude (GameplayEffects|MakeOutgoingSpec :self (Ability|GetAbilitySystemComponent (.HitActor (Collision|BreakHitResult _array_element))) :GameplayEffectClass "/Game/DustDevil/Core/GAS/Effects/GE_RadialDamage.GE_RadialDamage_C") "(TagName=\"Stats.Base.Damage\")" (* (.ReturnValue (Ability|Attribute|GetFloatAttributefromAbilitySystemComponent _returnvalue_2 "(AttributeName=\"Damage\",Attribute=/Script/DustDevil.BaseAttributeSet:Damage,AttributeOwner=\"/Script/CoreUObject.Class'/Script/DustDevil.BaseAttributeSet'\")")) (Math|Float|Min(Float) (/ (Math|Vector|Distance(Vector) (Transformation|GetActorLocation (.HitActor (Collision|BreakHitResult _array_element))) (Transformation|GetActorLocation)) (Variables|Default|GetExplosionRadius)) 0.2))))
    (GameplayEffects|ApplyGameplayEffectSpecToTarget _returnvalue_2 _returnvalue_3 (Ability|GetAbilitySystemComponent (.HitActor (Collision|BreakHitResult _array_element))))
    (GameplayEffects|ApplyGameplayEffectSpecToTarget _returnvalue_2 (GameplayEffects|MakeOutgoingSpec :self (Ability|GetAbilitySystemComponent (.HitActor (Collision|BreakHitResult _array_element))) :GameplayEffectClass "/Game/DustDevil/Core/GAS/Effects/GE_Bleed.GE_Bleed_C" :Level (Variables|Default|GetInstigatorWeaponLevel)) (Ability|GetAbilitySystemComponent (.HitActor (Collision|BreakHitResult _array_element)))))
  (Niagara|SpawnSystematLocation "/Game/DustDevil/Effects/Explosions/NS_EnemyExplosion.NS_EnemyExplosion" (Transformation|GetActorLocation) "0, 0, 0" (Math|Conversions|ToVector(Float) (/ (Variables|Default|GetExplosionRadius) 1e+02)))
  (CallFunction|InvalidateProjectile))