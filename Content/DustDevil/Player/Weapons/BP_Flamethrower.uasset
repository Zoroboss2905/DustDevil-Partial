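; Aimable vehicle flamethrower weapon that sprays fire projectiles, with Niagara flame effects, looping reload-meter updates and sound.
; Each shot calls the parent fire, enables the emitters and spawns five projectiles with random yaw and speed, boosted by instigator velocity and staggered across the cooldown.
; Tick feeds owner velocity to the flame effect, while a DoOnce gates the flame audio.
; Stopping or misfiring cuts flames, and reloading drives the player's HUD meter by timer.
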(event Custom|ResetSound
  (Utilities|FlowControl|DoOnce false) ; enters at Reset
)

(event Custom|FadeOutFlameThrower
  (bind _flames (Variables|Default|GetFlames)
    (:then
      (Audio|Components|Audio|FadeOut _flames 0.1 0.0 "Linear" :!class /Script/Engine.AudioComponent))
    (:else)))

(event EventBeginPlay
  (Variables|Default|SetbAimable true)
  (CallFunction|SetEmitters false)
  (bind _returnvalue (Actor|GetActorOfClass "/Game/DustDevil/Player/BP_Vehicle.BP_Vehicle_C"))
  (Variables|Default|SetPlayerRef _returnvalue))

(event EventFire
  (Utilities|FlowControl|Sequence
    (:then_0
      (Utilities|FlowControl|DoOnce false
        (:Completed
          (Audio|Components|Audio|Play (Variables|Default|GetFlames) 0.0))))
    (:then_1
      (|CallParentFunction)
      (CallFunction|SetEmitters true)
      (for _index (range 0 4)
        (CallFunction|SpawnFireProjectile))
      (bind _hud (Variables|/Game/DustDevil/Player/BP_Vehicle.BP_Vehicle_C|GetHUD (Variables|Default|GetPlayerRef))
        (:then
          (Default|UpdateAmmoCount (Variables|/Game/DustDevil/UI/HUD/WBP_HUD.WBP_HUD_C|GetReloadMeter _hud) (Variables|Default|GetMagazineAmmoCount) (Variables|Default|GetMagazineCapacity))
          (Default|UpdateAmmoBar (Variables|/Game/DustDevil/UI/HUD/WBP_HUD.WBP_HUD_C|GetReloadMeter _hud) (Variables|Default|GetMagazineAmmoCount) (Variables|Default|GetMagazineCapacity))
          (Default|CamShakeMini (Variables|Default|GetPlayerRef)))
        (:else)))))

(event EventTick
  (params (DeltaSeconds :type Float%20%28single-precision%29))
  (Niagara|SetNiagaraVariable(Vector3) (Variables|Default|GetFlameFX) "VehicleVelocity" (Transformation|GetVelocity (Components|GetOwner))))

(event EventOnReloadFinished
  (Variables|Default|SetMagazineAmmoCount (Variables|Default|GetMagazineCapacity))
  (Utilities|Time|ClearandInvalidateTimerbyHandle (Variables|Default|GetAmmoMeterTimer))
  (Default|UpdateAmmoCount (Variables|/Game/DustDevil/UI/HUD/WBP_HUD.WBP_HUD_C|GetReloadMeter (Variables|/Game/DustDevil/Player/BP_Vehicle.BP_Vehicle_C|GetHUD (Variables|Default|GetPlayerRef))) (Variables|Default|GetMagazineCapacity) (Variables|Default|GetMagazineCapacity))
  (bind _reload (Variables|Default|GetReload)
    (:then
      (Audio|Components|Audio|FadeOut _reload 0.0 0.0 "Linear" :!class /Script/Engine.AudioComponent))
    (:else)))

(event EventMisfire
  (params (MisfireReason :type EMisfireType%20Enum :default "M_AMMO"))
  (Utilities|FlowControl|Sequence
    (:then_0
      (CallFunction|SetEmitters false)
      (switch Utilities|FlowControl|Switch|SwitchonEMisfireType MisfireReason
        (:M_AMMO
          (Development|PrintString "Flamethrower Out of Ammo!"))
        (:M_COOLDOWN
          (Development|PrintString "Flamethrower on Cooldown!"))
        (:M_JAMMED
          (Development|PrintString "Flamethrower is Jammed!"))))
    (:then_1
      (CallFunction|SetEmitters false)
      (bind _flames (Variables|Default|GetFlames)
        (:then
          (Audio|Components|Audio|FadeOut _flames 0.1 0.0 "Linear" :!class /Script/Engine.AudioComponent)
          (CallFunction|ResetSound))
        (:else)))))

(event EventOnStopUse
  (CallFunction|SetEmitters false)
  (bind _flames (Variables|Default|GetFlames)
    (:then
      (Audio|Components|Audio|FadeOut _flames 0.1 0.0 "Linear" :!class /Script/Engine.AudioComponent)
      (CallFunction|ResetSound))
    (:else)))

(event EventOnReloadStarted
  (bind _returnvalue (Utilities|Time|SetTimerbyFunctionName 0 "UpdateAmmoMeter" 0.01 true))
  (Variables|Default|SetAmmoMeterTimer _returnvalue)
  (Default|UpdateAmmoCount (Variables|/Game/DustDevil/UI/HUD/WBP_HUD.WBP_HUD_C|GetReloadMeter (Variables|/Game/DustDevil/Player/BP_Vehicle.BP_Vehicle_C|GetHUD (Variables|Default|GetPlayerRef))) 0.0 (Variables|Default|GetMagazineCapacity))
  (CallFunction|ResetSound)
  (Utilities|FlowControl|Sequence
    (:then_0
      (bind _flames (Variables|Default|GetFlames)
        (:then
          (Audio|Components|Audio|FadeOut _flames 0.1 0.0 "Linear" :!class /Script/Engine.AudioComponent))
        (:else)))
    (:then_1
      (bind _reload (Variables|Default|GetReload)
        (:then
          (Audio|Components|Audio|Play _reload 0.0))
        (:else)))))

(fn ConstructionScript)

(fn OverrideFire
  (params (FireDamage :type Float%20%28double-precision%29) (FireDuration :type Float%20%28double-precision%29))
  (Variables|TopMount|Function|Flamethrower|SetFireDamage FireDamage)
  (Variables|TopMount|Function|Flamethrower|SetFireDuration FireDuration))

(fn SetEmitters
  (params (bEnabled :type Boolean))
  (bind _flamefx (Variables|Default|GetFlameFX))
  (Effects|Components|ParticleSystem|SetEmitterEnable _flamefx "Fountain" bEnabled)
  (Effects|Components|ParticleSystem|SetEmitterEnable _flamefx "Fountain001" bEnabled)
  (Effects|Components|ParticleSystem|SetEmitterEnable _flamefx "Fountain002" bEnabled)
  (Effects|Components|ParticleSystem|SetEmitterEnable _flamefx "Fountain003" bEnabled)
  (Effects|Components|ParticleSystem|SetEmitterEnable _flamefx "Grid3D_Gas_Master_Emitter" bEnabled)
  (Effects|Components|ParticleSystem|SetEmitterEnable _flamefx "Source_Flamerthrower" bEnabled))

(fn GetWeaponData
  (return "NewEnumerator2" (Math|Float|Truncate (Variables|Default|GetMagazineCapacity)) (Math|Float|Truncate (Variables|Default|GetMagazineAmmoCount)) (Variables|Default|GetCooldownMax) (Variables|Default|GetCooldownCurrent) (Variables|Default|GetMisfireCDCurrent) 0.0 0.0))

(fn SpawnFireProjectile
  (bind _returnvalue (Game|GetInstigator))
  (bind _barreltip (Variables|Default|GetBarrelTip))
  (bind _returnvalue_2 (Transformation|GetWorldTransform _barreltip))
  (bind _returnvalue_3 (* (.rotation _returnvalue_2) 0.5))
  (Game|SpawnActorfromClass "/Game/DustDevil/Player/Weapons/BP_FireProjectile.BP_FireProjectile_C" (Math|Transform|MakeTransform (.location _returnvalue_2) (Math|Rotator|MakeRotator (.roll _returnvalue_3) (.pitch _returnvalue_3) (+ (.yaw _returnvalue_3) (Math|Random|RandomFloatinRange -5.0 5.0))) "1.000000,1.000000,1.000000") "AlwaysSpawn" "OverrideRootScale" _returnvalue (+ (Math|Vector|VectorLength (Transformation|GetVelocity (Game|GetInstigator))) (Math|Random|RandomFloatinRange 5e+03 1e+04)) (Variables|TopMount|Function|Flamethrower|GetFireDuration) (Math|Random|RandomFloatinRange 0.0 (Variables|Default|GetCooldownMax)) _returnvalue) ; Fires a projectile Directly from the barrel. Looks better, but much easier to miss the target
)

(fn UpdateAmmoMeter
  (Default|StartReload (Variables|/Game/DustDevil/Player/BP_Vehicle.BP_Vehicle_C|GetHUD (Variables|Default|GetPlayerRef)) (Variables|Default|GetReloadTimeCurrent) (Variables|Default|GetReloadTimeMax)))