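; BP_TopMountBase is a base Blueprint for the player's top-mounted weapons, handling ammo consumption when firing.
; BeginPlay caches the BP_Vehicle as Player.
; Fire rolls against an ability-system attribute on the owner: success plays the BulletFarmer gameplay cue and spares the round, otherwise the magazine decrements and auto-reloads when empty if enabled.
; GetWeaponData returns placeholder values, and Tick and the construction script are empty.
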(event EventTick
  (params (DeltaSeconds :type Float%20%28single-precision%29)))

(event EventBeginPlay
  (bind _returnvalue (Actor|GetActorOfClass "/Game/DustDevil/Player/BP_Vehicle.BP_Vehicle_C"))
  (Variables|Default|SetPlayer _returnvalue))

(event EventFire
  (if (<= (Math|Random|RandomFloatinRange 1.0 1e+02) (.ReturnValue (Ability|Attribute|GetFloatAttributefromAbilitySystemComponent (Ability|GetAbilitySystemComponent (Components|GetOwner)) "(AttributeName=\"TrickChance\",Attribute=/Script/DustDevil.VehicleAttributeSet:TrickChance,AttributeOwner=\"/Script/CoreUObject.Class'/Script/DustDevil.VehicleAttributeSet'\")")))
    (GameplayCue|ExecuteGameplayCueOnActor(Burst) 0 "(TagName=\"GameplayCue.Ability.BulletFarmer\")" (Ability|GameplayCue|MakeGameplayCueParameters 0.0))
    (else
      (bind _result (Math|Float|DecrementFloat (Variables|Default|GetMagazineAmmoCount))
        (:%20%20
          (if (<= _result 0.0)
            (Variables|Default|SetMagazineAmmoCount 0.0)
            (if (Variables|Default|GetbAutoReload)
              (Class|TopMountBase|TryReload "R_EMPTY"))))))))

(fn ConstructionScript)

(fn GetWeaponData
  (return "NewEnumerator5" 0 0 0.0 0.0 0.0 0.0 0.0))