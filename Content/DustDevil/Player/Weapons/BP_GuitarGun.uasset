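; BP_GuitarGun is a player weapon that charges while fired, then releases a damaging soundwave around itself.
; Fire starts a looping timer that drains magazine ammo as charge and updates the HUD meter, while stopping use cancels and refills it.
; An empty magazine with AutoReload triggers a reload, whose start event is the actual blast: Niagara wave, sound, camera shake and sphere trace applying GAS damage to non-immune shootables.
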(event EventBeginPlay
  (Utilities|FlowControl|Sequence
    (:then_0
      (Variables|Default|SetbAimable true)
      (bind _returnvalue (Actor|GetActorOfClass "/Game/DustDevil/Player/BP_Vehicle.BP_Vehicle_C"))
      (Variables|Default|SetPlayerRef _returnvalue)
      (bind _player (Class|BPIPlayerTrigger|GetPlayerCharacter(Message) (Game|Player|GetPlayerPawn 0)))
      (Variables|Default|SetPlayer_0 _player))
    (:then_1
      (Effects|Components|ParticleSystem|SetFloatParameter (Variables|Default|GetSoundwave) "WaveSize" (Variables|Default|GetRadius)))))

(event EventOnReloadStarted
  (Utilities|Time|ClearandInvalidateTimerbyHandle (Variables|Default|GetCountDownHandle))
  (Utilities|FlowControl|Sequence
    (:then_0
      (Utilities|FlowControl|DelayUntilNextTick)
      (Default|ClearChargeLevel (Variables|/Game/DustDevil/UI/HUD/WBP_HUD.WBP_HUD_C|GetChargeMeter (Variables|/Game/DustDevil/Player/BP_Vehicle.BP_Vehicle_C|GetHUD (Variables|Default|GetPlayerRef)))))
    (:then_1
      (CallFunction|ResetSoundwave)
      (bind _returnvalue (Audio|SpawnSoundatLocation "/Game/DustDevil/Player/Weapons/Audio/A_SoundwaveFire_MS.A_SoundwaveFire_MS" (Transformation|GetActorLocation) "0, 0, 0" 1.0 1.0 0.0 0 "/Game/DustDevil/Player/Weapons/Audio/SC_SoundwaveGun.SC_SoundwaveGun"))
      (Variables|Default|SetFireSFX _returnvalue)
      (Default|CamShakeGuitar (Variables|Default|GetPlayer_0))
      (bind _outhits (Collision|MultiSphereTraceForObjects (Transformation|GetActorLocation) (+ (Transformation|GetActorLocation) "100.000000,100.000000,100.000000") (Variables|Default|GetRadius) (Utilities|Array|MakeArray "ObjectTypeQuery8") false 0 "None" true "(R=1.000000,G=0.000000,B=0.000000,A=1.000000)" "(R=0.000000,G=1.000000,B=0.000000,A=1.000000)" 2.0))
      (for _array_element _outhits
        (if (and (Utilities|DoesObjectImplementInterface (.HitActor (Collision|BreakHitResult _array_element)) "/Game/DustDevil/Core/Interfaces/BPI_Shootable.BPI_Shootable_C") (!= (Variables|Default|GetPlayerRef) (.HitActor (Collision|BreakHitResult _array_element))))
          (if (not (GameplayTags|HasMatchingGameplayTag (Ability|GetAbilitySystemComponent (.HitActor (Collision|BreakHitResult _array_element))) "(TagName=\"State.Damage.Immune\")"))
            (GameplayEffects|ApplyGameplayEffectToTarget :self (Ability|GetAbilitySystemComponent (Variables|Default|GetPlayerRef)) :GameplayEffectClass "/Game/DustDevil/Core/GAS/Effects/GE_Damage.GE_Damage_C" :Target (Ability|GetAbilitySystemComponent (.HitActor (Collision|BreakHitResult _array_element))) :Level 1.0)))))))

(event EventOnStopUse
  (bind _countdownhandle (Variables|Default|GetCountDownHandle))
  (if (Class|KismetSystemLibrary|TimerExistsHandle _countdownhandle)
    (Utilities|Time|ClearandInvalidateTimerbyHandle _countdownhandle)
    (Variables|Default|SetMagazineAmmoCount (Variables|Default|GetMagazineCapacity))
    (Default|ClearChargeLevel (Variables|/Game/DustDevil/UI/HUD/WBP_HUD.WBP_HUD_C|GetChargeMeter (Variables|/Game/DustDevil/Player/BP_Vehicle.BP_Vehicle_C|GetHUD (Variables|Default|GetPlayerRef))))))

(event EventFire
  (if (not (Class|KismetSystemLibrary|TimerExistsHandle (Variables|Default|GetCountDownHandle)))
    (bind _returnvalue (Utilities|Time|SetTimerbyFunctionName 0 "CountDown" 0.01 true))
    (Variables|Default|SetCountDownHandle _returnvalue)))

(event EventMisfire
  (params (MisfireReason :type EMisfireType%20Enum :default "M_AMMO"))
  (Utilities|FlowControl|Sequence
    (:then_0
      (switch Utilities|FlowControl|Switch|SwitchonEMisfireType MisfireReason
        (:M_AMMO
          (Development|PrintString "Machine Gun Out of Ammo!"))
        (:M_COOLDOWN
          (Development|PrintString "Machine Gun on Cooldown!"))
        (:M_JAMMED
          (Utilities|FlowControl|Sequence
            (:then_0
              (Development|PrintString "Machine Gun is Jammed!"))
            (:then_1
              (bind _player (Class|BPIPlayerTrigger|GetPlayerCharacter(Message) (Components|GetOwner)))
              (Class|BPIHUDUpdates|DisplayWarningMessage(Message) (Variables|/Game/DustDevil/Player/BP_Vehicle.BP_Vehicle_C|GetHUD _player) "It would be unwise to fire a gun next to highly flammable fuel storage!"))))))))

(event EventOnTryReload
  (params (ReloadType :type EReloadType%20Enum :default "R_MANUAL"))
  (switch Utilities|FlowControl|Switch|SwitchonEReloadType ReloadType))

(event EventOnTryReloadFailed
  (params (FailureReason :type EReloadFailureReason%20Enum :default "RF_UNKNOWN"))
  (switch Utilities|FlowControl|Switch|SwitchonEReloadFailureReason FailureReason))

(event EventOnReloadFinished
  (Variables|Default|SetMagazineAmmoCount (Variables|Default|GetMagazineCapacity)))

(fn ConstructionScript)

(fn GetWeaponData
  (return "NewEnumerator4" (Math|Float|Truncate (Variables|Default|GetMagazineCapacity)) (Math|Float|Truncate (Variables|Default|GetMagazineAmmoCount)) (Variables|Default|GetCooldownMax) (Variables|Default|GetCooldownCurrent) (Variables|Default|GetMisfireCDCurrent) 0.0 0.0))

(fn CountDown
  (bind _output_get (Variables|Default|SetMagazineAmmoCount (- (Variables|Default|GetMagazineAmmoCount) (Utilities|Operators|Divide 1.0 (Variables|Default|GetCooldownMax) 1e+02))))
  (Utilities|FlowControl|Sequence
    (:then_0
      (if (and (<= _output_get 0.0) (Variables|Default|GetbAutoReload))
        (Class|TopMountBase|TryReload "R_EMPTY")))
    (:then_1
      (Default|UpdateChargeLevel (Variables|/Game/DustDevil/UI/HUD/WBP_HUD.WBP_HUD_C|GetChargeMeter (Variables|/Game/DustDevil/Player/BP_Vehicle.BP_Vehicle_C|GetHUD (Variables|Default|GetPlayerRef))) (Variables|Default|GetMagazineAmmoCount)))))

(fn ResetSoundwave
  (Niagara|ResetSystem (Variables|Default|GetSoundwave))
  (Effects|Components|ParticleSystem|SetFloatParameter (Variables|Default|GetSoundwave) "WaveSize" (Variables|Default|GetRadius)))