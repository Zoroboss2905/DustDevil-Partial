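; Actor component on BP_Vehicle that applies the player's saved loadout and permanent upgrades at BeginPlay.
; Bumper, engine, tank and wheel choices swap meshes and apply level-scaled GAS effects, abilities, tags or vehicle and save-data values.
; The weapon spawns as the top mount with curve-table stats.
; A tick later, weapon damage and saved upgrade bonuses are applied as SetByCaller GameplayEffects.
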(event EventBeginPlay
  (Utilities|FlowControl|Sequence
    (:then_0
      (CallFunction|SetupReferences))
    (:then_1
      (CallFunction|ApplyModifications))
    (:then_2
      (Utilities|FlowControl|DelayUntilNextTick)
      (CallFunction|ApplyPermaStatChanges))))

(event EventTick
  (params (DeltaSeconds :type Float%20%28single-precision%29)))

(fn SetupReferences
  (bind _asbp_vehicle (Utilities|Casting|CastToBP_Vehicle (Components|GetOwner))
    (:then
      (bind _output_get (Variables|References|SetVehicle _asbp_vehicle))
      (Variables|References|SetABSC (Ability|GetAbilitySystemComponent _output_get)))
    (:CastFailed
      _))
  (bind _asgi_ddprototype (Utilities|Casting|CastToGI_DDPrototype (Game|GetGameInstance)))
  (Variables|References|SetSaveData (Default|GetSaveData _asgi_ddprototype)))

(fn ApplyModifications
  (bind _vehicle (Variables|References|GetVehicle))
  (bind _vehicle_2 (Variables|References|GetVehicle))
  (bind _savedata (Variables|References|GetSaveData))
  (bind _savedata_2 (Variables|References|GetSaveData))
  (bind _savedata_3 (Variables|References|GetSaveData))
  (bind _savedata_4 (Variables|References|GetSaveData))
  (bind _savedata_5 (Variables|References|GetSaveData))
  (Variables|References|GetVehicle
    (:then
      (Variables|References|GetABSC
        (:then
          (Variables|References|GetSaveData
            (:then
              (Utilities|FlowControl|Sequence
                (:then_0
                  ;[1 1 1] Setup Meshes
                  (LocalVariables|SetNewBumperMesh (Variables|/Script/DustDevil.Vehicle|GetFrontMount _vehicle))
                  (LocalVariables|SetNewEngineMesh (Variables|/Script/DustDevil.Vehicle|GetEngineMount _vehicle))
                  (LocalVariables|SetNewTankMesh (Variables|/Game/DustDevil/Player/BP_Vehicle.BP_Vehicle_C|GetRearMount _vehicle))
                  (LocalVariables|SetNewWheelFL (Variables|/Script/DustDevil.Vehicle|GetWheelFL _vehicle))
                  (LocalVariables|SetNewWheelFR (Variables|/Script/DustDevil.Vehicle|GetWheelFR _vehicle))
                  (LocalVariables|SetNewWheelBL (Variables|/Script/DustDevil.Vehicle|GetWheelBL _vehicle))
                  (LocalVariables|SetNewWheelBR (Variables|/Script/DustDevil.Vehicle|GetWheelBR _vehicle)))
                (:then_1
                  ;[1 1 1] Bumper
                  (bind _newbumper (Private|ApplyBumper (Variables|/Game/DustDevil/Core/Saves/SG_DDSaveData.SG_DDSaveData_C|GetEquippedBumper _savedata) (Variables|/Game/DustDevil/Core/Saves/SG_DDSaveData.SG_DDSaveData_C|GetEquippedBumperLevel _savedata) (LocalVariables|GetNewBumperMesh)))
                  (Variables|/Script/DustDevil.Vehicle|SetFrontMount (Variables|References|GetVehicle) _newbumper))
                (:then_2
                  ;[1 1 1] Engine
                  (bind _newengine (Private|ApplyEngine (Variables|/Game/DustDevil/Core/Saves/SG_DDSaveData.SG_DDSaveData_C|GetEquippedEngine _savedata_2) (Variables|/Game/DustDevil/Core/Saves/SG_DDSaveData.SG_DDSaveData_C|GetEquippedEngineLevel _savedata_2) (LocalVariables|GetNewEngineMesh)))
                  (Variables|/Script/DustDevil.Vehicle|SetEngineMount (Variables|References|GetVehicle) _newengine))
                (:then_3
                  ;[1 1 1] Tank
                  (bind _newtank (Private|ApplyTank (Variables|/Game/DustDevil/Core/Saves/SG_DDSaveData.SG_DDSaveData_C|GetEquippedTank _savedata_3) (Variables|/Game/DustDevil/Core/Saves/SG_DDSaveData.SG_DDSaveData_C|GetEquippedTankLevel _savedata_3) (LocalVariables|GetNewTankMesh)))
                  (Variables|/Game/DustDevil/Player/BP_Vehicle.BP_Vehicle_C|SetRearMount (Variables|References|GetVehicle) _newtank))
                (:then_4
                  ;[1 1 1] Wheels
                  (bind (_newwheelfl _newwheelfr _newwheelbl _newwheelbr) (Private|ApplyWheels (Variables|/Game/DustDevil/Core/Saves/SG_DDSaveData.SG_DDSaveData_C|GetEquippedTire _savedata_4) (Variables|/Game/DustDevil/Core/Saves/SG_DDSaveData.SG_DDSaveData_C|GetEquippedTireLevel _savedata_4) (LocalVariables|GetNewWheelFL) (LocalVariables|GetNewWheelFR) (LocalVariables|GetNewWheelBL) (LocalVariables|GetNewWheelBR)))
                  (Variables|/Script/DustDevil.Vehicle|SetWheelFL _vehicle_2 _newwheelfl)
                  (Variables|/Script/DustDevil.Vehicle|SetWheelFR _vehicle_2 _newwheelfr)
                  (Variables|/Script/DustDevil.Vehicle|SetWheelBL _vehicle_2 _newwheelbl)
                  (Variables|/Script/DustDevil.Vehicle|SetWheelBR _vehicle_2 _newwheelbr))
                (:then_5
                  (Private|ApplyWeapon (Variables|/Game/DustDevil/Core/Saves/SG_DDSaveData.SG_DDSaveData_C|GetEquippedWeapon _savedata_5) (Variables|/Game/DustDevil/Core/Saves/SG_DDSaveData.SG_DDSaveData_C|GetEquippedWeaponLevel _savedata_5)))))
            (:else
              (Development|PrintString "UpgradeManager: SaveGame Reference Invalid!" true true "(R=1.000000,G=0.000000,B=0.000000,A=1.000000)" 1e+01))))
        (:else
          (Development|PrintString "UpgradeManager: AbilitySystemComponent Reference Invalid!" true true "(R=1.000000,G=0.000000,B=0.000000,A=1.000000)" 1e+01))))
    (:else
      (Development|PrintString "UpgradeManager: Vehicle Reference Invalid!" true true "(R=1.000000,G=0.000000,B=0.000000,A=1.000000)" 1e+01))))

(fn ApplyPermaStatChanges
  (bind _returnvalue (Components|GetOwner))
  (bind _vehicle (Variables|References|GetVehicle))
  (bind _returnvalue_2 (Ability|GetAbilitySystemComponent _vehicle))
  (bind _returnvalue_3 (Ability|GetAbilitySystemComponent _returnvalue))
  ;[1 1 1] Apply Weapon Damage Number First, must happen here
  (bind _returnvalue_4 (Ability|GameplayEffect|AssignTagSetbyCallerMagnitude (GameplayEffects|MakeOutgoingSpec :self _returnvalue_3 :GameplayEffectClass "/Game/DustDevil/Core/GAS/Effects/GE_ModifyDamage.GE_ModifyDamage_C") "(TagName=\"Stats.Base.Damage\")" (Variables|Default|GetNewWeaponDamageValue)))
  (GameplayEffects|ApplyGameplayEffectSpecToSelf _returnvalue_3 _returnvalue_4)
  (bind _savedata (Variables|References|GetSaveData)
    (:then
      (LocalVariables|SetSpecHandle (GameplayEffects|MakeOutgoingSpec :self _returnvalue_2 :GameplayEffectClass "/Game/DustDevil/Core/GAS/Effects/GE_PermaBonuses.GE_PermaBonuses_C" :Level 1.0))
      (bind _keys (Utilities|Map|Keys (Variables|/Game/DustDevil/Core/Saves/SG_DDSaveData.SG_DDSaveData_C|GetEquippedUpgrades _savedata)))
      (for _array_element _keys
        (Ability|GameplayEffect|AssignTagSetbyCallerMagnitude (LocalVariables|GetSpecHandle) _array_element (.Value (Utilities|Map|Find (Variables|/Game/DustDevil/Core/Saves/SG_DDSaveData.SG_DDSaveData_C|GetEquippedUpgrades _savedata) _array_element))))
      (GameplayEffects|ApplyGameplayEffectSpecToSelf _returnvalue_2 (LocalVariables|GetSpecHandle)))
    (:else
      (Development|PrintString "UpgradeManager: SaveGame Reference Invalid!" true true "(R=1.000000,G=0.000000,B=0.000000,A=1.000000)" 1e+01))))

(fn ApplyBumper
  (params (BumperType :type E_BumperType%20Enum :default "NewEnumerator13") (BumperLevel :type Integer) (BumperMeshComponent :type Static%20Mesh%20Component%20Object%20Reference%20%28by%20ref%29))
  (bind _absc (Variables|References|GetABSC))
  (switch Utilities|FlowControl|Switch|SwitchonE_BumperType BumperType
    (:NewEnumerator0
      (Components|StaticMesh|SetStaticMesh BumperMeshComponent "/Game/DustDevil/Art/Meshes/Vehicle/Bars/SM_BigBasicBar.SM_BigBasicBar")
      (bind _returnvalue (Ability|GameplayEffect|AssignTagSetbyCallerMagnitude (GameplayEffects|MakeOutgoingSpec :self _absc :GameplayEffectClass "/Game/DustDevil/Core/GAS/Effects/GE_ApplyBumperDamage.GE_ApplyBumperDamage_C") "(TagName=\"Stats.Vehicle.RammingDamage\")" (Utilities|Select :Index BumperLevel :Option%200 1.2 :Option%201 1.2 :Option%202 1.5 :Option%203 2.1)))
      (GameplayEffects|ApplyGameplayEffectSpecToSelf _absc _returnvalue))
    (:NewEnumerator1
      (Components|StaticMesh|SetStaticMesh BumperMeshComponent "/Game/DustDevil/Art/Meshes/Vehicle/Bars/SM_BullBar.SM_BullBar")
      (GameplayAbilities|GiveAbility (Variables|References|GetABSC) "/Game/DustDevil/Core/GAS/Modifications/GA_BumperKnockback.GA_BumperKnockback_C" BumperLevel -1))
    (:NewEnumerator2
      (Components|StaticMesh|SetStaticMesh BumperMeshComponent "/Game/DustDevil/Art/Meshes/Vehicle/Bars/SM_SpikedBar.SM_SpikedBar")
      (GameplayAbilities|GiveAbility (Variables|References|GetABSC) "/Game/DustDevil/Core/GAS/Modifications/GA_BumperBleed.GA_BumperBleed_C" BumperLevel -1))
    (:NewEnumerator3
      (Components|StaticMesh|SetStaticMesh BumperMeshComponent "/Game/DustDevil/Art/Meshes/Vehicle/Bars/SM_VacuumBar.SM_VacuumBar")
      (GameplayAbilities|GiveAbility (Variables|References|GetABSC) "/Game/DustDevil/Core/GAS/Modifications/GA_BumperBiomass.GA_BumperBiomass_C" BumperLevel -1)))
  (return BumperMeshComponent))

(fn ApplyEngine
  (params (EngineType :type E_EngineType%20Enum :default "NewEnumerator5") (EngineLevel :type Integer) (EngineMeshComponent :type Static%20Mesh%20Component%20Object%20Reference%20%28by%20ref%29))
  (bind _returnvalue (Utilities|Enum|LiteralenumEDDAbilityInputID "Boost"))
  (bind _absc (Variables|References|GetABSC))
  (bind _returnvalue_2 (Math|Conversions|ToInteger(Byte) _returnvalue))
  (Class|AbilitySystemComponent|ClearAllAbilitieswithInputID _absc _returnvalue_2)
  (GameplayAbilities|GiveAbility _absc "/Game/DustDevil/Core/GAS/Abilities/GA_Boost.GA_Boost_C" EngineLevel _returnvalue_2)
  (switch Utilities|FlowControl|Switch|SwitchonE_EngineType EngineType
    (:NewEnumerator1
      (Components|StaticMesh|SetStaticMesh EngineMeshComponent "/Game/DustDevil/Art/Meshes/Vehicle/Engines/SM_Engine_1.SM_Engine_1")
      (Ability|GameplayEffect|AddLooseGameplayTags (Variables|References|GetVehicle) (GameplayTags|MakeLiteralGameplayTagContainer "(GameplayTags=((TagName=\"Upgrades.Mods.Engine.Efficient\")))")))
    (:NewEnumerator2
      (Components|StaticMesh|SetStaticMesh EngineMeshComponent "/Game/DustDevil/Art/Meshes/Vehicle/Engines/SM_Engine_2.SM_Engine_2")
      (GameplayAbilities|GiveAbility (Variables|References|GetABSC) "/Game/DustDevil/Core/GAS/Modifications/GA_EngineNova.GA_EngineNova_C" EngineLevel -1))
    (:NewEnumerator3
      (Components|StaticMesh|SetStaticMesh EngineMeshComponent "/Game/DustDevil/Art/Meshes/Vehicle/Engines/SM_Engine_3.SM_Engine_3")
      (GameplayAbilities|GiveAbility (Variables|References|GetABSC) "/Game/DustDevil/Core/GAS/Modifications/GA_EngineInstaKill.GA_EngineInstaKill_C" EngineLevel -1)))
  (return EngineMeshComponent))

(fn ApplyTank
  (params (TankType :type E_TankType%20Enum :default "NewEnumerator4") (TankLevel :type Integer) (TankMeshComponent :type Static%20Mesh%20Component%20Object%20Reference%20%28by%20ref%29))
  (bind _vehicle (Variables|References|GetVehicle))
  (bind _absc (Variables|References|GetABSC))
  (switch Utilities|FlowControl|Switch|SwitchonE_TankType TankType
    (:NewEnumerator0
      (Components|StaticMesh|SetStaticMesh TankMeshComponent "/Game/DustDevil/Art/Meshes/Vehicle/Tanks/SM_BulkyTank.SM_BulkyTank")
      (bind _output_get (Variables|/Game/DustDevil/Player/BP_Vehicle.BP_Vehicle_C|SetMaxDeconKits _vehicle (Utilities|Select :Index TankLevel :Option%200 2 :Option%201 4 :Option%202 5 :Option%203 7)))
      (Variables|/Game/DustDevil/Player/BP_Vehicle.BP_Vehicle_C|SetDeconKits _vehicle _output_get)
      (bind _output_get_2 (Variables|/Game/DustDevil/Player/BP_Vehicle.BP_Vehicle_C|SetMaxRepairKits _vehicle (Utilities|Select :Index TankLevel :Option%200 5 :Option%201 7 :Option%202 8 :Option%203 10)))
      (Variables|/Game/DustDevil/Player/BP_Vehicle.BP_Vehicle_C|SetRepairKits _vehicle _output_get_2))
    (:NewEnumerator1
      (Components|StaticMesh|SetStaticMesh TankMeshComponent "/Game/DustDevil/Art/Meshes/Vehicle/Tanks/SM_Bioharvester_Tank.SM_Bioharvester_Tank")
      (LocalVariables|SetBioBonusMulti (Utilities|Select :Index TankLevel :Option%200 1.0 :Option%201 1.02 :Option%202 1.04 :Option%203 1.06)))
    (:NewEnumerator2
      (Components|StaticMesh|SetStaticMesh TankMeshComponent "/Game/DustDevil/Art/Meshes/Vehicle/Tanks/SM_Filtration_Tank.SM_Filtration_Tank")
      (LocalVariables|SetBioPermaBonus (Utilities|Select :Index TankLevel :Option%200 1.0 :Option%201 1.04 :Option%202 1.07 :Option%203 1.12)))
    (:NewEnumerator3
      (Components|StaticMesh|SetStaticMesh TankMeshComponent "/Game/DustDevil/Art/Meshes/Vehicle/Tanks/SM_MatterCompactor.SM_MatterCompactor")
      (LocalVariables|SetBioConvertMulti (Utilities|Select :Index TankLevel :Option%200 1.0 :Option%201 1.3 :Option%202 1.6 :Option%203 2.0))))
  (bind _returnvalue (Ability|GameplayEffect|AssignTagSetbyCallerMagnitude (GameplayEffects|MakeOutgoingSpec :self _absc :GameplayEffectClass "/Game/DustDevil/Core/GAS/Effects/GE_CapacityMulti.GE_CapacityMulti_C") "(TagName=\"Stats.Vehicle.MaxFuelCapacity\")" (LocalVariables|GetFuelCapacityMulti)))
  (bind _returnvalue_2 (Ability|GameplayEffect|AssignTagSetbyCallerMagnitude _returnvalue "(TagName=\"Stats.Vehicle.TankBioBonus\")" (LocalVariables|GetBioBonusMulti)))
  (bind _returnvalue_3 (Ability|GameplayEffect|AssignTagSetbyCallerMagnitude _returnvalue_2 "(TagName=\"Stats.Vehicle.TankPermaBonus\")" (LocalVariables|GetBioPermaBonus)))
  (bind _returnvalue_4 (Ability|GameplayEffect|AssignTagSetbyCallerMagnitude _returnvalue_3 "(TagName=\"Stats.Vehicle.TankConvertBonus\")" (LocalVariables|GetBioConvertMulti)))
  (GameplayEffects|ApplyGameplayEffectSpecToSelf _absc _returnvalue_4)
  (return TankMeshComponent))

(fn ApplyWheels
  (params (TireType :type E_TireType%20Enum :default "NewEnumerator4") (TireLevel :type Integer) (WheelFLComponent :type Static%20Mesh%20Component%20Object%20Reference%20%28by%20ref%29) (WheelFRComponent :type Static%20Mesh%20Component%20Object%20Reference%20%28by%20ref%29) (WheelBLComponent :type Static%20Mesh%20Component%20Object%20Reference%20%28by%20ref%29) (WheelBRComponent :type Static%20Mesh%20Component%20Object%20Reference%20%28by%20ref%29))
  (switch Utilities|FlowControl|Switch|SwitchonE_TireType TireType
    (:NewEnumerator0
      (Components|StaticMesh|SetStaticMesh WheelFLComponent "/Game/DustDevil/Art/Meshes/Vehicle/Wheels/SM_Default_Wheels_FrontL.SM_Default_Wheels_FrontL")
      (Components|StaticMesh|SetStaticMesh WheelFRComponent "/Game/DustDevil/Art/Meshes/Vehicle/Wheels/SM_Default_Wheels_FrontR.SM_Default_Wheels_FrontR")
      (Components|StaticMesh|SetStaticMesh WheelBLComponent "/Game/DustDevil/Art/Meshes/Vehicle/Wheels/SM_Default_Wheels_BackL.SM_Default_Wheels_BackL")
      (Components|StaticMesh|SetStaticMesh WheelBRComponent "/Game/DustDevil/Art/Meshes/Vehicle/Wheels/SM_Default_Wheels_BackR.SM_Default_Wheels_BackR")
      (Variables|/Game/DustDevil/Core/Saves/SG_DDSaveData.SG_DDSaveData_C|SetBTDiminishRate (Variables|References|GetSaveData) (Utilities|Select :Index TireLevel :Option%200 0.02 :Option%201 0.02 :Option%202 0.015 :Option%203 0.01)))
    (:NewEnumerator1
      (Components|StaticMesh|SetStaticMesh WheelFLComponent "/Game/DustDevil/Art/Meshes/Vehicle/Wheels/SM_WheelTier1_FrontL.SM_WheelTier1_FrontL")
      (Components|StaticMesh|SetStaticMesh WheelFRComponent "/Game/DustDevil/Art/Meshes/Vehicle/Wheels/SM_WheelTier1_FrontR.SM_WheelTier1_FrontR")
      (Components|StaticMesh|SetStaticMesh WheelBLComponent "/Game/DustDevil/Art/Meshes/Vehicle/Wheels/SM_WheelTier1_BackL.SM_WheelTier1_BackL")
      (Components|StaticMesh|SetStaticMesh WheelBRComponent "/Game/DustDevil/Art/Meshes/Vehicle/Wheels/SM_WheelTier1_BackR.SM_WheelTier1_BackR")
      (Variables|/Game/DustDevil/Core/Saves/SG_DDSaveData.SG_DDSaveData_C|SetBTRegenRate (Variables|References|GetSaveData) (Utilities|Select :Index TireLevel :Option%200 0.04 :Option%201 0.04 :Option%202 0.08 :Option%203 0.12)))
    (:NewEnumerator2
      (Components|StaticMesh|SetStaticMesh WheelFLComponent "/Game/DustDevil/Art/Meshes/Vehicle/Wheels/Vehicle_FrontWheel_L.Vehicle_FrontWheel_L")
      (Components|StaticMesh|SetStaticMesh WheelFRComponent "/Game/DustDevil/Art/Meshes/Vehicle/Wheels/Vehicle_FrontWheel_R.Vehicle_FrontWheel_R")
      (Components|StaticMesh|SetStaticMesh WheelBLComponent "/Game/DustDevil/Art/Meshes/Vehicle/Wheels/Vehicle_BackWheel_L.Vehicle_BackWheel_L")
      (Components|StaticMesh|SetStaticMesh WheelBRComponent "/Game/DustDevil/Art/Meshes/Vehicle/Wheels/Vehicle_BackWheel_R.Vehicle_BackWheel_R")
      (Class|AbilitySystemComponent|GiveAbilityandActivateOnce (Variables|References|GetABSC) "/Game/DustDevil/Core/GAS/Modifications/GA_BulletTimeDamage.GA_BulletTimeDamage_C" TireLevel -1))
    (:NewEnumerator3
      (Components|StaticMesh|SetStaticMesh WheelFLComponent "/Game/DustDevil/Art/Meshes/Vehicle/Wheels/SM_PaddleWheel_FrontL.SM_PaddleWheel_FrontL")
      (Components|StaticMesh|SetStaticMesh WheelFRComponent "/Game/DustDevil/Art/Meshes/Vehicle/Wheels/SM_PaddleWheel_FrontR.SM_PaddleWheel_FrontR")
      (Components|StaticMesh|SetStaticMesh WheelBLComponent "/Game/DustDevil/Art/Meshes/Vehicle/Wheels/SM_PaddleWheel_BackL.SM_PaddleWheel_BackL")
      (Components|StaticMesh|SetStaticMesh WheelBRComponent "/Game/DustDevil/Art/Meshes/Vehicle/Wheels/SM_PaddleWheel_BackR.SM_PaddleWheel_BackR")
      (Class|AbilitySystemComponent|GiveAbilityandActivateOnce (Variables|References|GetABSC) "/Game/DustDevil/Core/GAS/Modifications/GA_BulletTimeDefence.GA_BulletTimeDefence_C" TireLevel -1)))
  (return WheelFLComponent WheelFRComponent WheelBLComponent WheelBRComponent))

(fn ApplyWeapon
  (params (WeaponType :type E_WeaponType%20Enum :default "NewEnumerator5") (WeaponLevel :type Integer))
  (bind _vehicle (Variables|References|GetVehicle))
  (if (Utilities|Enum|Equal(Enum) WeaponType "NewEnumerator5")
    (Utilities|FlowControl|Sequence
      (:then_0
        (Development|PrintString "Equipped Weapon was set to 'None'" true true "(R=1.000000,G=0.030993,B=0.000000,A=1.000000)" 4.0))
      (:then_1
        (return)))
    (else
      (Utilities|FlowControl|Sequence
        (:then_0
          ;[0.07812 0.07812 0.07812] Spawn Gun Object
          (bind _returnvalue (Game|SpawnActorfromClass (Utilities|Select :Index WeaponType :NewEnumerator5 "/Game/DustDevil/Player/Weapons/BP_TopMountBase.BP_TopMountBase_C" :NewEnumerator0 "/Game/DustDevil/Player/Weapons/BP_MachineGun.BP_MachineGun_C" :NewEnumerator1 "/Game/DustDevil/Player/Weapons/BP_Minigun.BP_Minigun_C" :NewEnumerator2 "/Game/DustDevil/Player/Weapons/BP_Flamethrower.BP_Flamethrower_C" :NewEnumerator3 "/Game/DustDevil/Player/Weapons/BP_Autocannon.BP_Autocannon_C" :NewEnumerator4 "/Game/DustDevil/Player/Weapons/BP_GuitarGun.BP_GuitarGun_C") (Transformation|GetActorTransform _vehicle) "AlwaysSpawn" "OverrideRootScale" _vehicle _vehicle))
          (Class|Vehicle|SetTopMount (Variables|References|GetVehicle) _returnvalue))
        (:then_1
          (Utilities|FlowControl|Sequence
            (:then_0
              (switch Utilities|FlowControl|Switch|SwitchonE_WeaponType WeaponType
                (:NewEnumerator0
                  (bind _outxy (DataTable|EvaluateCurveTableRow "/Game/DustDevil/Data/CT_MachineGun.CT_MachineGun" "FireRate" (Math|Conversions|ToFloat(Integer) WeaponLevel))
                    (:RowFound
                      (LocalVariables|SetNewWeaponFireRate _outxy)
                      (bind _outxy_2 (DataTable|EvaluateCurveTableRow "/Game/DustDevil/Data/CT_MachineGun.CT_MachineGun" "AmmoMagSize" (Math|Conversions|ToFloat(Integer) WeaponLevel))
                        (:RowFound
                          (LocalVariables|SetNewWeaponMagSize _outxy_2)
                          (bind _outxy_3 (DataTable|EvaluateCurveTableRow "/Game/DustDevil/Data/CT_MachineGun.CT_MachineGun" "ReloadTime" (Math|Conversions|ToFloat(Integer) WeaponLevel))
                            (:RowFound
                              (LocalVariables|SetNewWeaponReloadTime _outxy_3)
                              (bind _outxy_4 (DataTable|EvaluateCurveTableRow "/Game/DustDevil/Data/CT_MachineGun.CT_MachineGun" "Damage" (Math|Conversions|ToFloat(Integer) WeaponLevel))
                                (:RowFound
                                  (LocalVariables|SetNewWeaponDamage _outxy_4))))))))))
                (:NewEnumerator1
                  (bind _outxy_5 (DataTable|EvaluateCurveTableRow "/Game/DustDevil/Data/CT_MiniGun.CT_MiniGun" "FireRate" (Math|Conversions|ToFloat(Integer) WeaponLevel))
                    (:RowFound
                      (LocalVariables|SetNewWeaponFireRate _outxy_5)
                      (bind _outxy_6 (DataTable|EvaluateCurveTableRow "/Game/DustDevil/Data/CT_MiniGun.CT_MiniGun" "AmmoMagSize" (Math|Conversions|ToFloat(Integer) WeaponLevel))
                        (:RowFound
                          (LocalVariables|SetNewWeaponMagSize _outxy_6)
                          (bind _outxy_7 (DataTable|EvaluateCurveTableRow "/Game/DustDevil/Data/CT_MiniGun.CT_MiniGun" "ReloadTime" (Math|Conversions|ToFloat(Integer) WeaponLevel))
                            (:RowFound
                              (LocalVariables|SetNewWeaponReloadTime _outxy_7)
                              (bind _outxy_8 (DataTable|EvaluateCurveTableRow "/Game/DustDevil/Data/CT_MiniGun.CT_MiniGun" "Damage" (Math|Conversions|ToFloat(Integer) WeaponLevel))
                                (:RowFound
                                  (LocalVariables|SetNewWeaponDamage _outxy_8))))))))))
                (:NewEnumerator2
                  (bind _outxy_9 (DataTable|EvaluateCurveTableRow "/Game/DustDevil/Data/CT_Flamethrower.CT_Flamethrower" "FireRate" (Math|Conversions|ToFloat(Integer) WeaponLevel))
                    (:RowFound
                      (LocalVariables|SetNewWeaponFireRate _outxy_9)
                      (bind _outxy_10 (DataTable|EvaluateCurveTableRow "/Game/DustDevil/Data/CT_Flamethrower.CT_Flamethrower" "AmmoMagSize" (Math|Conversions|ToFloat(Integer) WeaponLevel))
                        (:RowFound
                          (LocalVariables|SetNewWeaponMagSize _outxy_10)
                          (bind _outxy_11 (DataTable|EvaluateCurveTableRow "/Game/DustDevil/Data/CT_Flamethrower.CT_Flamethrower" "ReloadTime" (Math|Conversions|ToFloat(Integer) WeaponLevel))
                            (:RowFound
                              (LocalVariables|SetNewWeaponReloadTime _outxy_11)
                              (bind _outxy_12 (DataTable|EvaluateCurveTableRow "/Game/DustDevil/Data/CT_Flamethrower.CT_Flamethrower" "Damage" (Math|Conversions|ToFloat(Integer) WeaponLevel))
                                (:RowFound
                                  (LocalVariables|SetNewWeaponDamage _outxy_12)
                                  ;[1 1 1] Set Custom Data for Flamethrower
                                  (bind _asbp_flamethrower (Utilities|Casting|CastToBP_Flamethrower (Class|Vehicle|GetTopMount (Variables|References|GetVehicle))))
                                  (bind _outxy_13 (DataTable|EvaluateCurveTableRow "/Game/DustDevil/Data/CT_Flamethrower.CT_Flamethrower" "FireDuration" (Math|Conversions|ToFloat(Integer) WeaponLevel))
                                    (:RowFound
                                      (Variables|/Game/DustDevil/Player/Weapons/BP_Flamethrower.BP_Flamethrower_C|SetFireDuration _asbp_flamethrower _outxy_13))))))))))))
                (:NewEnumerator3
                  (bind _outxy_14 (DataTable|EvaluateCurveTableRow "/Game/DustDevil/Data/CT_Autocannon.CT_Autocannon" "FireRate" (Math|Conversions|ToFloat(Integer) WeaponLevel))
                    (:RowFound
                      (LocalVariables|SetNewWeaponFireRate _outxy_14)
                      (bind _outxy_15 (DataTable|EvaluateCurveTableRow "/Game/DustDevil/Data/CT_Autocannon.CT_Autocannon" "AmmoMagSize" (Math|Conversions|ToFloat(Integer) WeaponLevel))
                        (:RowFound
                          (LocalVariables|SetNewWeaponMagSize _outxy_15)
                          (bind _outxy_16 (DataTable|EvaluateCurveTableRow "/Game/DustDevil/Data/CT_Autocannon.CT_Autocannon" "ReloadTime" (Math|Conversions|ToFloat(Integer) WeaponLevel))
                            (:RowFound
                              (LocalVariables|SetNewWeaponReloadTime _outxy_16)
                              (bind _outxy_17 (DataTable|EvaluateCurveTableRow "/Game/DustDevil/Data/CT_Autocannon.CT_Autocannon" "Damage" (Math|Conversions|ToFloat(Integer) WeaponLevel))
                                (:RowFound
                                  (LocalVariables|SetNewWeaponDamage _outxy_17)
                                  ;[1 1 1] Set Custom Data for Autocannon
                                  (bind _asbp_autocannon (Utilities|Casting|CastToBP_Autocannon (Class|Vehicle|GetTopMount (Variables|References|GetVehicle))))
                                  (Variables|/Game/DustDevil/Player/Weapons/BP_Autocannon.BP_Autocannon_C|SetWeaponLevel _asbp_autocannon (Math|Conversions|ToFloat(Integer) WeaponLevel)))))))))))
                (:NewEnumerator4
                  (bind _outxy_18 (DataTable|EvaluateCurveTableRow "/Game/DustDevil/Data/CT_Soundwave.CT_Soundwave" "FireRate" (Math|Conversions|ToFloat(Integer) WeaponLevel))
                    (:RowFound
                      (LocalVariables|SetNewWeaponFireRate _outxy_18)
                      (bind _outxy_19 (DataTable|EvaluateCurveTableRow "/Game/DustDevil/Data/CT_Soundwave.CT_Soundwave" "AmmoMagSize" (Math|Conversions|ToFloat(Integer) WeaponLevel))
                        (:RowFound
                          (LocalVariables|SetNewWeaponMagSize _outxy_19)
                          (bind _outxy_20 (DataTable|EvaluateCurveTableRow "/Game/DustDevil/Data/CT_Soundwave.CT_Soundwave" "ReloadTime" (Math|Conversions|ToFloat(Integer) WeaponLevel))
                            (:RowFound
                              (LocalVariables|SetNewWeaponReloadTime _outxy_20)
                              (bind _outxy_21 (DataTable|EvaluateCurveTableRow "/Game/DustDevil/Data/CT_Soundwave.CT_Soundwave" "Damage" (Math|Conversions|ToFloat(Integer) WeaponLevel))
                                (:RowFound
                                  (LocalVariables|SetNewWeaponDamage _outxy_21)
                                  ;[1 1 1] Set Custom Data for Soundwave
                                  (bind _asbp_guitar_gun (Utilities|Casting|CastToBP_GuitarGun (Class|Vehicle|GetTopMount (Variables|References|GetVehicle))))
                                  (bind _outxy_22 (DataTable|EvaluateCurveTableRow "/Game/DustDevil/Data/CT_Soundwave.CT_Soundwave" "Radius" (Math|Conversions|ToFloat(Integer) WeaponLevel))
                                    (:RowFound
                                      (Variables|/Game/DustDevil/Player/Weapons/BP_GuitarGun.BP_GuitarGun_C|SetRadius _asbp_guitar_gun _outxy_22))))))))))))))
            (:then_1
              ;[1 1 1] Actually Applying all the stats
              (Class|TopMountBase|InitWeaponStats (Class|Vehicle|GetTopMount (Variables|References|GetVehicle)) (LocalVariables|GetNewWeaponFireRate) (LocalVariables|GetNewWeaponMagSize) (LocalVariables|GetNewWeaponReloadTime))
              (Variables|Default|SetNewWeaponDamageValue (LocalVariables|GetNewWeaponDamage)))))))))