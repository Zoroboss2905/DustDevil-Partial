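; BP_CamZoom is a prototype trigger that adjusts the camera and vehicle outline while BP_Vehicle overlaps it.
; With CamZoom enabled, a timeline lerps the camera boom length on entry and reverses on exit.
; A camera-forward trace puts an outline overlay on chassis and wheels when it hits a "Blocking"-tagged actor, otherwise clearing it on other hits.
; The check repeats via retriggerable delay only after blocking hits; exit clears the overlay.
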(event Custom|Opacity
  (bind _vehicle (Variables|Default|GetVehicle))
  (bind _camera (Variables|/Script/DustDevil.Vehicle|GetCamera _vehicle))
  (bind _returnvalue (Transformation|GetWorldLocation _camera))
  (if (Variables|Default|GetRender)
    (bind _outhit (Collision|LineTraceByChannel _returnvalue (+ (* (Math|Vector|GetForwardVector (Transformation|GetWorldRotation _camera)) (Variables|Default|GetMultiply)) _returnvalue) "TraceTypeQuery1" false 0 "None"))
    (if (.bBlockingHit (Collision|BreakHitResult _outhit))
      (if (Actor|ActorHasTag (.HitActor (Collision|BreakHitResult _outhit)) "Blocking")
        (Rendering|Material|SetOverlayMaterial (Variables|/Script/DustDevil.Vehicle|GetChassis (Variables|Default|GetVehicle)) "/Game/DustDevil/MaterialLibrary/Materials/M_OutlineEnemy.M_OutlineEnemy" :!class /Script/Engine.MeshComponent)
        (Utilities|FlowControl|RetriggerableDelay 0.05)
        (CallFunction|Opacity)
        (else
          (Rendering|Material|SetOverlayMaterial (Variables|/Script/DustDevil.Vehicle|GetChassis (Variables|Default|GetVehicle)) 0 :!class /Script/Engine.MeshComponent)
          (Utilities|FlowControl|RetriggerableDelay 0.05)
          (CallFunction|Opacity))))))

(event Custom|ChangeOpacityBack
  (Rendering|Material|SetOverlayMaterial (Variables|/Script/DustDevil.Vehicle|GetChassis (Variables|Default|GetVehicle)) 0 :!class /Script/Engine.MeshComponent)
  (Utilities|FlowControl|RetriggerableDelay 0.05)
  (CallFunction|Opacity))

(event EventBeginPlay)

(event Collision|EventActorBeginOverlap
  (params (OtherActor :type Actor%20Object%20Reference))
  (bind _asbp_vehicle (Utilities|Casting|CastToBP_Vehicle OtherActor))
  (bind _output_get (Variables|Default|SetVehicle _asbp_vehicle))
  (Utilities|FlowControl|Sequence
    (:then_0
      (if (Variables|Default|GetCamZoom)
        (bind _targetarmlength (Timeline|PlayAnimation Play)
          (:Update
            (Variables|/Script/Engine.SpringArmComponent|SetTargetArmLength (Variables|/Script/DustDevil.Vehicle|GetCameraBoom _output_get) (Math|Float|Lerp (Variables|Default|GetCamZoomValueInitial) (Variables|Default|GetCamZoomValueFinal) _targetarmlength))))))
    (:then_1
      (Variables|Default|SetRender true)
      (CallFunction|Opacity))))

(event Collision|EventActorEndOverlap
  (params (OtherActor :type Actor%20Object%20Reference))
  (Utilities|Casting|CastToBP_Vehicle OtherActor)
  (Utilities|FlowControl|Sequence
    (:then_0
      (if (Variables|Default|GetCamZoom)
        (bind _targetarmlength (Timeline|PlayAnimation Reverse)
          (:Update
            (Variables|/Script/Engine.SpringArmComponent|SetTargetArmLength (Variables|/Script/DustDevil.Vehicle|GetCameraBoom (stale Collision|EventActorBeginOverlap _output_get)) (Math|Float|Lerp (Variables|Default|GetCamZoomValueInitial) (Variables|Default|GetCamZoomValueFinal) _targetarmlength))))))
    (:then_1
      (Variables|Default|SetRender false)
      (CallFunction|ChangeOpacityBack))))

(fn ConstructionScript)