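; BP_Enemy3Prototype is a prototype burrowing enemy that hides below its placed position until the player approaches, then attacks.
; On BeginPlay it drops underground and stores both burrow heights.
; The first DetectionRadius overlap with a BPI_PlayerTrigger actor caches the player and plays the Emerge timeline to raise it.
; Once emerged, looping timers keep it facing the player and spawn BP_Enemy3SpitPrototype at its Arrow component.
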(event OnComponentBeginOverlap(DetectionRadius)
  (params (OverlappedComponent :type Primitive%20Component%20Object%20Reference) (OtherActor :type Actor%20Object%20Reference) (OtherComp :type Primitive%20Component%20Object%20Reference) (OtherBodyIndex :type Integer) (bFromSweep :type Boolean) (SweepResult :type Hit%20Result%20Structure%20%28by%20ref%29))
  (bind _returnvalue (Transformation|GetActorLocation))
  (if (Utilities|DoesObjectImplementInterface OtherActor "/Game/DustDevil/Core/Interfaces/BPI_PlayerTrigger.BPI_PlayerTrigger_C")
    (bind _player (Class|BPIPlayerTrigger|GetPlayerCharacter(Message) OtherActor))
    (Variables|Default|SetPlayer _player)
    (Utilities|FlowControl|DoOnce false
      (:Completed
        (bind _alpha (Timeline|Emerge PlayFromStart)
          (:Update
            (Transformation|SetActorLocation (Math|Vector|MakeVector (.x _returnvalue) (.y _returnvalue) (Math|Float|Lerp (Variables|Default|GetBurrowStartLoc) (Variables|Default|GetBurrowEndLoc) _alpha)) false false))
          (:Finished
            (bind _returnvalue_2 (Utilities|Time|SetTimerbyFunctionName 0 "RotateToPlayer" 0.01 true))
            (Variables|Default|SetRotateToPlayerTimer _returnvalue_2)
            (bind _returnvalue_3 (Utilities|Time|SetTimerbyEvent (delegate Custom|Start%20Attacking) 1.0 true))
            (Variables|Default|SetAttackTimer _returnvalue_3)))))))

(event Custom|Start%20Attacking
  (bind _arrow (Variables|Default|GetArrow))
  (bind _returnvalue (Transformation|GetWorldTransform _arrow))
  (Game|SpawnActorfromClass "/Game/DustDevil/Prototyping/Blueprints/BP_Enemy3SpitPrototype.BP_Enemy3SpitPrototype_C" (Math|Transform|MakeTransform (.location _returnvalue) (.rotation _returnvalue) "1.000000,1.000000,1.000000") "Undefined" "MultiplyWithRoot" 0 0))

(event EventBeginPlay
  (bind _returnvalue (Transformation|GetActorLocation))
  (Transformation|SetActorLocation (Math|Vector|MakeVector (.x _returnvalue) (.y _returnvalue) (- (.z _returnvalue) 2525.0)) false false)
  (CallFunction|SetBurrowStartEndLocs))

(fn ConstructionScript)

(fn SetBurrowStartEndLocs
  (Variables|Default|SetBurrowStartLoc (.z (Transformation|GetActorLocation)))
  (Variables|Default|SetBurrowEndLoc (+ (.z (Transformation|GetActorLocation)) 2525.0)))

(fn RotatetoPlayer
  (Transformation|SetActorRotation (Math|Rotator|FindLookatRotation (Transformation|GetActorLocation) (Transformation|GetActorLocation (Variables|Default|GetPlayer)))))