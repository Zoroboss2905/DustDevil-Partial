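; Fast travel station that offers to return the player's car to base when it enters the trigger.
; Overlap raises a bug barrier and opens a confirmation popup; accepting plays a timeline easing the car onto the station's arrow, then teleports it behind fade widgets.
; Declining or finishing travel drops the barrier, and leaving the trigger re-arms it.
; Biofuel meter and biomatter deposit helpers are present but never called here.
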(event OnComponentBeginOverlap(Trigger)
  (params (OverlappedComponent :type Primitive%20Component%20Object%20Reference) (OtherActor :type Actor%20Object%20Reference) (OtherComp :type Primitive%20Component%20Object%20Reference) (OtherBodyIndex :type Integer) (bFromSweep :type Boolean) (SweepResult :type Hit%20Result%20Structure%20%28by%20ref%29))
  ;[0.02956 0.02956 0.02956] Gets reference to player when they enter radius
  (if (Utilities|DoesObjectImplementInterface OtherActor "/Game/DustDevil/Core/Interfaces/BPI_PlayerTrigger.BPI_PlayerTrigger_C")
    (Utilities|FlowControl|DoOnce false
      (:Completed
        (Class|BPIPlayerTrigger|GetPlayerCharacter(Message) OtherActor)
        ;[0.02956 0.02956 0.02956] Creates popup window to confirm player wants to enter station and waits for response. If yes, trigger enter animation. If no, release player and adjusts input mode
        (CallFunction|CreatePopupWindow)
        (CallFunction|EnterorExitLocation true)
        (EventDispatchers|BindEventtoClosePopup (delegate Custom|PopupClosed))))))

(event OnComponentEndOverlap(Trigger)
  (params (OverlappedComponent :type Primitive%20Component%20Object%20Reference) (OtherActor :type Actor%20Object%20Reference) (OtherComp :type Primitive%20Component%20Object%20Reference) (OtherBodyIndex :type Integer))
  ;[0.02956 0.02956 0.02956] Gets reference to player when they enter radius
  (if (Utilities|DoesObjectImplementInterface OtherActor "/Game/DustDevil/Core/Interfaces/BPI_PlayerTrigger.BPI_PlayerTrigger_C")
    (bind _popuptext (Variables|References|GetPopupText)
      (:then
        (Widget|RemovefromParent _popuptext)
        (Utilities|FlowControl|DoOnce false) ; enters at Reset
      )
      (:else
        (Utilities|FlowControl|DoOnce false) ; enters at Reset
      ))))

(event Custom|Release%20Player
  (CallFunction|EnterorExitLocation false))

(event Custom|FastTravel
  (bind _fadeout (Variables|Default|GetFadeOut))
  (UserInterface|Viewport|AddtoViewport (Variables|Default|GetFadeIn) 0)
  (Utilities|FlowControl|Delay 1.2)
  (Transformation|SetActorLocationAndRotation (Variables|References|GetPlayer) (Variables|Default|GetWorldLocation) (Variables|Default|GetWorlRotation))
  (Utilities|FlowControl|Delay 0.2)
  (Widget|RemovefromParent (Variables|Default|GetFadeIn))
  (Default|CallFastTravelConcluded)
  (UserInterface|Viewport|AddtoViewport _fadeout 0)
  (Utilities|FlowControl|Delay 1.2)
  (Widget|RemovefromParent _fadeout))

(event Custom|PopupClosed
  (params (EnteringStation :type Boolean))
  ;[0.02956 0.02956 0.02956] Creates popup window to confirm player wants to enter station and waits for response. If yes, trigger enter animation. If no, release player and adjusts input mode
  (if EnteringStation
    (CallFunction|SetStartEndPoints)
    (bind _alpha (Timeline|TL_EnteringStation PlayFromStart)
      (:Update
        (CallFunction|UpdatePlayerLocationRotation _alpha _alpha))
      (:Finished
        (CallFunction|FastTravel)
        (EventDispatchers|BindEventtoFastTravelConcluded (delegate Custom|Release%20Player))))
    (else
      (CallFunction|EnterorExitLocation false))))

(event Custom|FadeInAndOutEffect
  (bind _returnvalue (UserInterface|CreateWidget "/Game/DustDevil/UI/CustomisationMenu/WBP_FadeIn.WBP_FadeIn_C"))
  (Variables|Default|SetFadeIn _returnvalue)
  (bind _returnvalue_2 (UserInterface|CreateWidget "/Game/DustDevil/UI/CustomisationMenu/WBP_FadeOut.WBP_FadeOut_C"))
  (Variables|Default|SetFadeOut _returnvalue_2))

(event EventBeginPlay
  (CallFunction|FadeinandOutEffect)
  (CallFunction|GetReferences))

(fn ConstructionScript)

(fn DisplayFuelAmount
  (bind _player (Variables|References|GetPlayer))
  ;[0.02956 0.02956 0.02956] Rotates biofuel meter towards player camera view so it is always facing the player and can be easily read
  (Utilities|IsValid 0
    (:Is%20Valid
      (Transformation|SetWorldRotation (Variables|/Script/Engine.Actor|GetRootComponent _player) (Math|Rotator|FindLookatRotation (Transformation|GetWorldLocation (Variables|/Script/Engine.Actor|GetRootComponent _player)) (Transformation|GetWorldLocation (Variables|/Game/DustDevil/Player/BP_Car.BP_Car_C|GetCamera (Variables|References|GetPlayer)))) false false))
    (:Is%20Not%20Valid
      (return))))

(fn SetStartEndPoints
  (bind _arrow (Variables|Default|GetArrow))
  (bind _player (Variables|References|GetPlayer))
  ;[0.02956 0.02956 0.02956] Finds the location and rotation of the player relative to the station itself for the enter station animation
  (Variables|Default|SetLocationStart (Transformation|GetActorLocation _player))
  (Variables|Default|SetRotationStart (Transformation|GetActorRotation _player))
  (Variables|Default|SetLocationEnd (Transformation|GetWorldLocation _arrow))
  (Variables|Default|SetRotationEnd (Transformation|GetWorldRotation _arrow)))

(fn CalculateDepositSpeed)

(fn EnterorExitLocation
  (params (EnterStation :type Boolean))
  (bind _bugbarrier (Variables|Default|GetBugBarrier))
  ;[0.02956 0.02956 0.02956] Adjusts input and activates/deactivates bug barrier depending on whether player is entering/exiting
  (if EnterStation
    (Collision|SetCollisionEnabled _bugbarrier "QueryAndPhysics")
    (else
      (Collision|SetCollisionEnabled _bugbarrier "NoCollision"))))

(fn UpdatePlayerLocationRotation
  (params (LocationAlpha :type Float%20%28single-precision%29) (RotationAlpha :type Float%20%28single-precision%29))
  ;[0.02956 0.02956 0.02956] Updates player location and rotation as part of enter base animation
  (Transformation|SetActorLocationAndRotation (Variables|References|GetPlayer) (Math|Vector|Lerp(Vector) (Variables|Default|GetLocationStart) (Variables|Default|GetLocationEnd) LocationAlpha) (Math|Rotator|Lerp(Rotator) (Variables|Default|GetRotationStart) (Variables|Default|GetRotationEnd) RotationAlpha)))

(fn CreatePopupWindow
  ;[0.02956 0.02956 0.02956] Creates popup widget and sets its text. Also passes a reference of this station to the widget to call when the player exits the popup window
  (bind _returnvalue (UserInterface|CreateWidget "/Game/DustDevil/UI/WBP_PopupText.WBP_PopupText_C" (Game|GetPlayerController 0) 0 0 "NewEnumerator2" self 0 (Variables|References|GetPlayer)))
  (bind _output_get (Variables|References|SetPopupText _returnvalue))
  (UserInterface|Viewport|AddtoViewport _output_get 5)
  (Default|SetDescriptionText _output_get "Return to base?"))

(fn CheckifPlayerHasBiomatter
  ;[0.02956 0.02956 0.02956] Check if player has biomatter to deposit
  (if (== (Variables|/Game/DustDevil/Player/BP_Car.BP_Car_C|GetBiomatter (Variables|References|GetPlayer)) 0.0)
    (return false)
    (else
      (return true))))

(fn GetReferences
  ;[0.02956 0.02956 0.02956] Gets relevant blueprint references
  (Utilities|FlowControl|Sequence
    (:then_0
      (bind _asbp_car (Utilities|Casting|CastToBP_Car (Game|Player|GetPlayerPawn 0)))
      (Variables|References|SetPlayer _asbp_car))
    (:then_1
      (bind _asgm_player (Utilities|Casting|CastToGM_Player (Game|GetGameMode)))
      (Variables|References|SetGameMode _asgm_player))))