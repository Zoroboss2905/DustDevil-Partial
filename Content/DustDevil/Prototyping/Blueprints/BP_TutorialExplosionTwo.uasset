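; Tutorial actor that blows up a wall once the player's vehicle has entered its overlap area and a required key is used.
; Overlap starts CheckCanSlowMo, which polls two configured keys on a short Delay loop until either is pressed or held.
; A DoOnce then destroys SMWall, issues several offset Niagara explosion spawns attached to it and plays an explosion sound.
; Despite the event's name, no slow motion happens here.
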(event Custom|CheckCanSlowMo
  (bind _haspressedbutton (CallFunction|KeyHasBeenInteractedwith :!label _label))
  (if _haspressedbutton
    _
    (else
      (bind _haspressedbutton_2 (CallFunction|KeyHasBeenInteractedwith 1))
      (if _haspressedbutton_2
        _
        (else
          (Utilities|FlowControl|Delay 0.05)
          (goto _label)))))
  (Utilities|FlowControl|DoOnce false
    (:Completed
      (Components|DestroyComponent (Variables|Default|GetSM_Wall))
      (Niagara|SpawnSystemAttached "/Game/DustDevil/Effects/Explosions/NS_EnemyExplosion1.NS_EnemyExplosion1" (Variables|Default|GetSM_Wall) "None" "0, 0, 0" "0, 0, 0" "KeepRelativeOffset" false)
      (Niagara|SpawnSystemAttached "/Game/DustDevil/Effects/Explosions/NS_EnemyExplosion1.NS_EnemyExplosion1" (Variables|Default|GetSM_Wall) "None" "0.000000,750.000000,0.000000" "0, 0, 0" "KeepRelativeOffset" false)
      (Niagara|SpawnSystemAttached "/Game/DustDevil/Effects/Explosions/NS_EnemyExplosion1.NS_EnemyExplosion1" (Variables|Default|GetSM_Wall) "None" "250.000000,-750.000000,0.000000" "0, 0, 0" "KeepRelativeOffset" false)
      (Niagara|SpawnSystemAttached "/Game/DustDevil/Effects/Explosions/NS_EnemyExplosion1.NS_EnemyExplosion1" (Variables|Default|GetSM_Wall) "None" "500.000000,-1250.000000,0.000000" "0, 0, 0" "KeepRelativeOffset" false)
      (Audio|PlaySound2D "/Game/DustDevil/Audio/Feedback/Grenade_Explosion_14_-_QuickSounds_com.Grenade_Explosion_14_-_QuickSounds_com" 1.0 1.0 0.0 0 0))))

(event EventBeginPlay
  (bind _returnvalue (Actor|GetActorOfClass "/Game/DustDevil/Player/BP_Vehicle.BP_Vehicle_C"))
  (Variables|Default|SetVehicle _returnvalue))

(event Collision|EventActorBeginOverlap
  (params (OtherActor :type Actor%20Object%20Reference))
  (Utilities|Casting|CastToBP_Vehicle OtherActor)
  (CallFunction|CheckCanSlowMo))

(event EventTick
  (params (DeltaSeconds :type Float%20%28single-precision%29)))

(fn ConstructionScript)

(fn KeyHasBeenInteractedwith
  (params (Int :type Integer))
  (bind _returnvalue (Game|GetPlayerController 0))
  (bind _keyinput (LocalVariables|GetKeyInput))
  (bind _output (Utilities|Array|Get(acopy) _keyinput Int))
  (return (or (Game|Player|WasInputKeyJustPressed _returnvalue _output) (Game|Player|IsInputKeyDown _returnvalue _output))))