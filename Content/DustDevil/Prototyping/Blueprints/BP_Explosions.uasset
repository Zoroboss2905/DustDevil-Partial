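; BP_Explosions is a one-shot exploding oil barrel prop triggered when a BP_Vehicle overlaps it.
; Its Niagara effect starts hidden at BeginPlay.
; On the first vehicle overlap, a DoOnce reveals and resets the effect, plays an attached grenade explosion sound and destroys the barrel component.
; The actor itself remains, since only the barrel component is destroyed.
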(event EventBeginPlay
  (Rendering|SetVisibility (Variables|Default|GetNiagara1) false false))

(event Collision|EventActorBeginOverlap
  (params (OtherActor :type Actor%20Object%20Reference))
  (Utilities|Casting|CastToBP_Vehicle OtherActor)
  (Utilities|FlowControl|DoOnce false
    (:Completed
      (Rendering|SetVisibility (Variables|Default|GetNiagara1) true false)
      (Audio|SpawnSoundAttached "/Game/DustDevil/Audio/Feedback/EnemyThree/Grenade_Explosion_14_-_QuickSounds_com.Grenade_Explosion_14_-_QuickSounds_com" (Variables|Default|GetNiagara1) "None" (Transformation|GetActorLocation) "0, 0, 0" "KeepRelativeOffset" false 1.0 1.0 0.0 0 0)
      (Components|DestroyComponent (Variables|Default|GetBP_PhysicsFoliage_OilBarrell1))
      (Niagara|ResetSystem (Variables|Default|GetNiagara1)))))

(event EventTick
  (params (DeltaSeconds :type Float%20%28single-precision%29)))

(fn ConstructionScript)