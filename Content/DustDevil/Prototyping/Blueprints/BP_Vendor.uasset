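; BP_Vendor is a vendor actor that offers the player a "Browse vendor?" prompt on entering its trigger.
; Overlap by a BPI_PlayerTrigger actor shows a WBP_PopupText widget and enables BugBarrier collision, gated by a DoOnce that resets on exit.
; The popup's close event either opens the WBP_FuelDepot_v1 screen a tick later or, if declined, disables the barrier.
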(event OnComponentBeginOverlap(Trigger)
  (params (OverlappedComponent :type Primitive%20Component%20Object%20Reference) (OtherActor :type Actor%20Object%20Reference) (OtherComp :type Primitive%20Component%20Object%20Reference) (OtherBodyIndex :type Integer) (bFromSweep :type Boolean) (SweepResult :type Hit%20Result%20Structure%20%28by%20ref%29))
  (if (Utilities|DoesObjectImplementInterface OtherActor "/Game/DustDevil/Core/Interfaces/BPI_PlayerTrigger.BPI_PlayerTrigger_C")
    (Utilities|FlowControl|DoOnce false
      (:Completed
        (CallFunction|CreatePopupWindow)
        (CallFunction|PlayerEnterExit true)
        (EventDispatchers|BindEventtoClosePopupVendor (delegate Custom|Vendor%20Popup%20Closed))))))

(event OnComponentEndOverlap(Trigger)
  (params (OverlappedComponent :type Primitive%20Component%20Object%20Reference) (OtherActor :type Actor%20Object%20Reference) (OtherComp :type Primitive%20Component%20Object%20Reference) (OtherBodyIndex :type Integer))
  (if (Utilities|DoesObjectImplementInterface OtherActor "/Game/DustDevil/Core/Interfaces/BPI_PlayerTrigger.BPI_PlayerTrigger_C")
    (bind _popupwidget (Variables|References|GetPopupWidget)
      (:then
        (Widget|RemovefromParent _popupwidget)
        (Utilities|FlowControl|DoOnce false) ; enters at Reset
      )
      (:else
        (Utilities|FlowControl|DoOnce false) ; enters at Reset
      ))))

(event Custom|Vendor%20Popup%20Closed
  (params (EnteringVendor :type Boolean))
  (if EnteringVendor
    (Utilities|FlowControl|DelayUntilNextTick)
    (bind _returnvalue (UserInterface|CreateWidget "/Game/DustDevil/UI/FuelDepotMenu/WBP_FuelDepot_v1.WBP_FuelDepot_v1_C" (Game|GetPlayerController 0) (Variables|References|GetPlayer) 0))
    (UserInterface|Viewport|AddtoViewport _returnvalue 5)
    (else
      (CallFunction|PlayerEnterExit false))))

(fn ConstructionScript)

(fn CreatePopupWindow
  (bind _returnvalue (UserInterface|CreateWidget "/Game/DustDevil/UI/WBP_PopupText.WBP_PopupText_C" (Game|GetPlayerController 0) 0 0 "NewEnumerator3" 0 self (Variables|References|GetPlayer)))
  (bind _output_get (Variables|References|SetPopupWidget _returnvalue))
  (UserInterface|Viewport|AddtoViewport _output_get 5)
  (Default|SetDescriptionText _output_get "Browse vendor?")
  (bind _player (Variables|References|GetPlayer)
    (:then
      (Default|ChangeCursor _player false))
    (:else)))

(fn PlayerEnterExit
  (params (Entering :type Boolean))
  (bind _bugbarrier (Variables|Default|GetBugBarrier))
  (if Entering
    (Collision|SetCollisionEnabled _bugbarrier "QueryAndPhysics")
    (else
      (Collision|SetCollisionEnabled _bugbarrier "NoCollision"))))