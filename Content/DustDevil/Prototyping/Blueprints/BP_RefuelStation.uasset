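; Refuel station actor where the player's car stops to deposit biomatter as base fuel.
; Trigger overlap with a car carrying biomatter opens a confirmation popup and enables the bug barrier's collision.
; Confirming runs a timeline that lerps the car onto the station's arrow, while declining drops the barrier.
; Helpers scale deposit speed by carried biomatter and refresh every station's fuel display, but nothing here calls them.
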(event OnComponentBeginOverlap(Trigger)
  (params (OverlappedComponent :type Primitive%20Component%20Object%20Reference) (OtherActor :type Actor%20Object%20Reference) (OtherComp :type Primitive%20Component%20Object%20Reference) (OtherBodyIndex :type Integer) (bFromSweep :type Boolean) (SweepResult :type Hit%20Result%20Structure%20%28by%20ref%29))
  ;[0.02956 0.02956 0.02956] Gets reference to player when they enter the station radius
  (if (Utilities|DoesObjectImplementInterface OtherActor "/Game/DustDevil/Core/Interfaces/BPI_PlayerTrigger.BPI_PlayerTrigger_C")
    (Utilities|FlowControl|DoOnce false
      (:Completed
        ;[0.02956 0.02956 0.02956] Checks that player has biomatter to deposit and if so allows them to enter station
        (bind _hasbiomatter (CallFunction|CheckifPlayerHasBiomatter))
        (if _hasbiomatter
          ;[0.02956 0.02956 0.02956] Creates popup window to confirm player wants to enter station and waits for response. If yes, trigger enter animation. If no, release player and adjusts input mode
          (CallFunction|CreatePopupWindow)
          (CallFunction|EnterorExitStation true)
          (EventDispatchers|BindEventtoClosePopupFuelDeposit (delegate Custom|Fuel%20Popup%20Closed)))))))

(event OnComponentEndOverlap(Trigger)
  (params (OverlappedComponent :type Primitive%20Component%20Object%20Reference) (OtherActor :type Actor%20Object%20Reference) (OtherComp :type Primitive%20Component%20Object%20Reference) (OtherBodyIndex :type Integer))
  ;[0.02956 0.02956 0.02956] Gets reference to player when they enter the station radius
  (if (Utilities|DoesObjectImplementInterface OtherActor "/Game/DustDevil/Core/Interfaces/BPI_PlayerTrigger.BPI_PlayerTrigger_C")
    (bind _popuptext (Variables|References|GetPopupText)
      (:then
        (Widget|RemovefromParent _popuptext)
        (Utilities|FlowControl|DoOnce false) ; enters at Reset
      )
      (:else
        (Utilities|FlowControl|DoOnce false) ; enters at Reset
      ))))

(event Custom|Fuel%20Popup%20Closed
  (params (EnteringStation :type Boolean))
  ;[0.02956 0.02956 0.02956] Creates popup window to confirm player wants to enter station and waits for response. If yes, trigger enter animation. If no, release player and adjusts input mode
  (if EnteringStation
    (CallFunction|SetStartEndPoints)
    (bind _alpha (Timeline|TL_EnteringStation PlayFromStart)
      (:Update
        (CallFunction|UpdatePlayerLocationRotation _alpha _alpha))
      (:Finished))
    (else
      (CallFunction|EnterorExitStation false))))

(event EventBeginPlay
  ;[0.02956 0.02956 0.02956] Calls function repeatedly to keep biofuel counter facing player
  (CallFunction|GetReferences))

(fn ConstructionScript)

(fn DisplayFuelAmount)

(fn SetStartEndPoints
  (bind _arrow (Variables|Default|GetArrow))
  (bind _player (Variables|References|GetPlayer))
  ;[0.02956 0.02956 0.02956] Finds the location and rotation of the player relative to the station itself for the enter station animation
  (Variables|Default|SetLocationStart (Transformation|GetActorLocation _player))
  (Variables|Default|SetRotationStart (Transformation|GetActorRotation _player))
  (Variables|Default|SetLocationEnd (Transformation|GetWorldLocation _arrow))
  (Variables|Default|SetRotationEnd (Transformation|GetWorldRotation _arrow)))

(fn CalculateDepositSpeed
  (bind _player (Variables|References|GetPlayer))
  (bind _biomatter (Variables|/Game/DustDevil/Player/BP_Car.BP_Car_C|GetBiomatter _player))
  ;[0.02956 0.02956 0.02956] Checks to see how much biomatter the player is carrying and speeds up the deposit rate accordingly
  (if (< _biomatter 5e+01)
    (Variables|Default|SetDepositSpeed 0.05)
    (elif (< _biomatter 1e+02)
      (Variables|Default|SetDepositSpeed 0.04)
      (elif (< _biomatter 1.5e+02)
        (Variables|Default|SetDepositSpeed 0.03)
        (elif (< _biomatter 2e+02)
          (Variables|Default|SetDepositSpeed 0.02)
          (else
            (Variables|Default|SetDepositSpeed 0.005)))))))

(fn EnterorExitStation
  (params (EnterStation :type Boolean))
  (bind _bugbarrier (Variables|Default|GetBugBarrier))
  ;[0.02956 0.02956 0.02956] Adjusts input and activates/deactivates bug barrier depending on whether player is entering/exiting
  (if EnterStation
    (Collision|SetCollisionEnabled _bugbarrier "QueryAndPhysics")
    (else
      (Collision|SetCollisionEnabled _bugbarrier "NoCollision"))))

(fn UpdatePlayerLocationRotation
  (params (LocationAlpha :type Float%20%28single-precision%29) (RotationAlpha :type Float%20%28single-precision%29))
  ;[0.02956 0.02956 0.02956] Updates player location and rotation as part of enter base animation
  (Transformation|SetActorLocationAndRotation (Variables|References|GetPlayer) (Math|Vector|Lerp(Vector) (Variables|Default|GetLocationStart) (Variables|Default|GetLocationEnd) LocationAlpha) (Math|Rotator|Lerp(Rotator) (Variables|Default|GetRotationStart) (Variables|Default|GetRotationEnd) RotationAlpha)))

(fn CreatePopupWindow
  ;[0.02956 0.02956 0.02956] Creates popup widget and sets its text. Also passes a reference of this station to the widget to call when the player exits the popup window
  (bind _returnvalue (UserInterface|CreateWidget "/Game/DustDevil/UI/WBP_PopupText.WBP_PopupText_C" (Game|GetPlayerController 0) self 0 "NewEnumerator0" 0 0 (Variables|References|GetPlayer)))
  (bind _output_get (Variables|References|SetPopupText _returnvalue))
  (UserInterface|Viewport|AddtoViewport _output_get 5)
  (Default|SetDescriptionText _output_get "Deposit biomatter?"))

(fn CheckifPlayerHasBiomatter
  ;[0.02956 0.02956 0.02956] Check if player has biomatter to deposit
  (if (== (Variables|/Game/DustDevil/Player/BP_Car.BP_Car_C|GetBiomatter (Variables|References|GetPlayer)) 0.0)
    (return false)
    (else
      (return true))))

(fn GetReferences
  ;[0.02956 0.02956 0.02956] Gets relevant blueprint references
  (Utilities|FlowControl|Sequence
    (:then_0
      (bind _asbp_car (Utilities|Casting|CastToBP_Car (Game|Player|GetPlayerPawn 0)))
      (Variables|References|SetPlayer _asbp_car))
    (:then_1
      (bind _asgm_player (Utilities|Casting|CastToGM_Player (Game|GetGameMode)))
      (Variables|References|SetGameMode _asgm_player))
    (:then_2
      (bind _aswbp_base_fuel_count (Utilities|Casting|CastToWBP_BaseFuelCount (UserInterface|GetWidget (Variables|Default|GetBaseFuelCount))))
      (Variables|References|SetBaseFuelWidget _aswbp_base_fuel_count))
    (:then_3
      (bind _asgi_ddprototype (Utilities|Casting|CastToGI_DDPrototype (Game|GetGameInstance)))
      (Variables|References|SetGameInstance _asgi_ddprototype))))

(fn UpdateFuelDepositDisplays
  ;[0.02956 0.02956 0.02956] Updates fuel storage display for all other fuel deposit stations as well
  (Utilities|Casting|CastToGI_DDPrototype (Game|GetGameInstance))
  (bind _outactors (Actor|GetAllActorsOfClass "BP_RefuelStation_C"))
  (for _array_element _outactors
    (Default|UpdateBaseFuel (Variables|BP_RefuelStation_C|GetBaseFuelWidget _array_element))))