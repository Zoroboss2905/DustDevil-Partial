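; Prototype nuclear material pickup that grants NuclearMatter to an overlapping actor and then destroys itself.
; On sphere overlap with a BPI_Pickups implementer, it applies GE_PickupLoot to that actor's Ability System Component, passing NuclearMatAmount as a SetByCaller magnitude on Stats.Base.NuclearMatter.
; It also plays a 2D sound, marked for later replacement by a GameplayCue, and sends the actor PickupNuclearMatMessage.
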(event OnComponentBeginOverlap(SphereCollision)
  (params (OverlappedComponent :type Primitive%20Component%20Object%20Reference) (OtherActor :type Actor%20Object%20Reference) (OtherComp :type Primitive%20Component%20Object%20Reference) (OtherBodyIndex :type Integer) (bFromSweep :type Boolean) (SweepResult :type Hit%20Result%20Structure%20%28by%20ref%29))
  (bind _returnvalue (Ability|GetAbilitySystemComponent OtherActor))
  ;[0.02956 0.02956 0.02956] When picked up, transfers NuclearMatter to player and then destroys self
  (if (Utilities|DoesObjectImplementInterface OtherActor "/Game/DustDevil/Core/Interfaces/BPI_Pickups.BPI_Pickups_C")
    (bind _returnvalue_2 (Ability|GameplayEffect|AssignTagSetbyCallerMagnitude (GameplayEffects|MakeOutgoingSpec :self _returnvalue :GameplayEffectClass "/Game/DustDevil/Core/GAS/Effects/GE_PickupLoot.GE_PickupLoot_C") "(TagName=\"Stats.Base.NuclearMatter\")" (Math|Conversions|ToFloat(Integer) (Variables|Default|GetNuclearMatAmount))))
    (GameplayEffects|ApplyGameplayEffectSpecToSelf _returnvalue _returnvalue_2)
    (Audio|PlaySound2D "/Game/DustDevil/Audio/Feedback/viscous-liquid-fall-in-83980.viscous-liquid-fall-in-83980" 1.0 1.0 0.0 0 0)
    (Class|BPIPickups|PickupNuclearMat(Message) OtherActor) ; Replace with a GameplayCue Later
    (Actor|DestroyActor)))

(fn ConstructionScript)