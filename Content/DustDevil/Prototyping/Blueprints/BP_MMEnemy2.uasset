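; Prototype flying enemy actor meant to shuttle along Y between paired start and end points, but its logic is disconnected from the empty BeginPlay.
; The unused chain loops a fly animation, waits randomly, then lerps Y on a timeline, adding random X jitter and a large Z offset each update.
; SetStartEndPoints picks random points by AtStart, which flips as each pass finishes before the timeline reverses.
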(event EventBeginPlay)

(fn ConstructionScript)

(fn SetStartEndPoints
  (bind _startpoints (Variables|Default|GetStartPoints))
  (bind _endpoints (Variables|Default|GetEndPoints))
  (bind (_outitem _outindex) (Utilities|Array|Random _endpoints))
  (bind (_outitem_2 _outindex_2) (Utilities|Array|Random _startpoints))
  (bind _returnvalue (Transformation|GetActorLocation _outitem))
  (bind _returnvalue_2 (Transformation|GetActorLocation _outitem_2))
  (if (Variables|Default|GetbAtStart)
    (Transformation|SetActorLocation _returnvalue_2 false false)
    (Variables|Default|SetStartLoc (.Y (Math|Vector|BreakVector _returnvalue_2)))
    (Variables|Default|SetEndLoc (.y (Transformation|GetActorLocation (Utilities|Array|Get(acopy) (Variables|Default|GetEndPoints) _outindex_2))))
    (else
      (Transformation|SetActorLocation _returnvalue false false)
      (Variables|Default|SetStartLoc (.Y (Math|Vector|BreakVector _returnvalue)))
      (Variables|Default|SetEndLoc (.y (Transformation|GetActorLocation (Utilities|Array|Get(acopy) (Variables|Default|GetStartPoints) _outindex)))))))