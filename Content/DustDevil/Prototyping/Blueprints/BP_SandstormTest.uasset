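; BP_SandstormTest is a prototype sandstorm that travels between two target points and detects players inside it.
; On BeginPlay, a timeline lerps the actor's X location from the first target point to the second.
; Trigger overlaps with BPI_PlayerTrigger implementers store the player and start a looping damage timer, which is cleared on exit.
; The DamagePlayer event is empty, so no damage is applied yet.
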(event OnComponentBeginOverlap(Trigger)
  (params (OverlappedComponent :type Primitive%20Component%20Object%20Reference) (OtherActor :type Actor%20Object%20Reference) (OtherComp :type Primitive%20Component%20Object%20Reference) (OtherBodyIndex :type Integer) (bFromSweep :type Boolean) (SweepResult :type Hit%20Result%20Structure%20%28by%20ref%29))
  (if (Utilities|DoesObjectImplementInterface OtherActor "/Game/DustDevil/Core/Interfaces/BPI_PlayerTrigger.BPI_PlayerTrigger_C")
    (bind _player (Class|BPIPlayerTrigger|GetPlayerCharacter(Message) OtherActor))
    (Variables|Default|SetPlayer _player)
    (bind _returnvalue (Utilities|Time|SetTimerbyEvent (delegate Custom|Damage%20Player) 1.0 true))
    (Variables|Default|SetDamagePlayerTimer _returnvalue)))

(event OnComponentEndOverlap(Trigger)
  (params (OverlappedComponent :type Primitive%20Component%20Object%20Reference) (OtherActor :type Actor%20Object%20Reference) (OtherComp :type Primitive%20Component%20Object%20Reference) (OtherBodyIndex :type Integer))
  (if (Utilities|DoesObjectImplementInterface OtherActor "/Game/DustDevil/Core/Interfaces/BPI_PlayerTrigger.BPI_PlayerTrigger_C")
    (Utilities|Time|ClearandInvalidateTimerbyHandle (Variables|Default|GetDamagePlayerTimer))))

(event Custom|Damage%20Player)

(event EventBeginPlay
  (Variables|Default|SetStartLocation (.x (Transformation|GetActorLocation (Utilities|Array|Get(acopy) (Variables|Default|GetTargetPoints)))))
  (Variables|Default|SetEndLocation (.x (Transformation|GetActorLocation (Utilities|Array|Get(acopy) (Variables|Default|GetTargetPoints) 1))))
  (Transformation|SetActorLocation (Math|Vector|MakeVector (Variables|Default|GetStartLocation) 0.0 0.0) false false)
  (bind _alpha (Timeline|Move PlayFromStart)
    (:Update
      (Transformation|SetActorLocation (Math|Vector|MakeVector (Math|Float|Lerp (Variables|Default|GetStartLocation) (Variables|Default|GetEndLocation) _alpha) 0.0 0.0) false false))))

(fn ConstructionScript)