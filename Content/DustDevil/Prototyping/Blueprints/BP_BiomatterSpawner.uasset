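; BP_BiomatterSpawner is a prototype actor that scatters BP_Biomass pickups around itself when play begins.
; On BeginPlay it spawns NumberToSpawn actors, passing BiomatterAmount to each as its BiomassAmount.
; X and Y come from a random direction and distance within the SpawnRadius sphere around the root, while Z is a hardcoded world height.
; Spawns adjust for collisions where possible but always succeed.
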(event EventBeginPlay
  (bind _returnvalue (Math|Random|RandomUnitVector))
  (bind _spawnradius (Variables|Default|GetSpawnRadius))
  (bind _defaultsceneroot (Variables|Default|GetDefaultSceneRoot))
  (bind _returnvalue_2 (Transformation|GetWorldLocation _defaultsceneroot))
  (bind _sphereradius (Variables|/Script/Engine.SphereComponent|GetSphereRadius _spawnradius))
  (bind _returnvalue_3 (Math|Random|RandomFloatinRange 0.0 _sphereradius))
  (bind _returnvalue_4 (* _returnvalue _returnvalue_3))
  (bind _returnvalue_5 (+ _returnvalue_4 _returnvalue_2))
  ;[0.02956 0.02956 0.02956] Spawns the specified number of biomatter in a random location within the spawn radius
  (for _index (range 0 (Variables|Default|GetNumberToSpawn))
    (Game|SpawnActorfromClass "/Game/DustDevil/ItemDrops/BP_Biomass.BP_Biomass_C" (Math|Transform|MakeTransform (Math|Vector|MakeVector (.x _returnvalue_5) (.y _returnvalue_5) 3.9e+03) "0, 0, 0" "1.000000,1.000000,1.000000") "AdjustIfPossibleButAlwaysSpawn" "MultiplyWithRoot" 0 (Variables|Default|GetBiomatterAmount) 0)))

(fn ConstructionScript)