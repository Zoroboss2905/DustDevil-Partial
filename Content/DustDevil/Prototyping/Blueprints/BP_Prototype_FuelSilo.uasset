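; Prototype fuel silo where the player deposits nuclear material until the missile launch objective can start.
; Overlapping its trigger shows a hold-to-interact prompt and the silo menu.
; A completed hold reads the player's fuel from GAS, clamps the deposit to capacity, records it in save data and starts the menu's deposit display.
; Helper functions scale the gauge, write fuel back through a SetByCaller GameplayEffect and update the HUD objective.
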(event OnComponentBeginOverlap(InteractionTrigger)
  (params (OverlappedComponent :type Primitive%20Component%20Object%20Reference) (OtherActor :type Actor%20Object%20Reference) (OtherComp :type Primitive%20Component%20Object%20Reference) (OtherBodyIndex :type Integer) (bFromSweep :type Boolean) (SweepResult :type Hit%20Result%20Structure%20%28by%20ref%29))
  (bind _returnvalue (Game|GetPlayerController 0))
  (if (Utilities|DoesObjectImplementInterface OtherActor "/Game/DustDevil/Core/Interfaces/BPI_PlayerTrigger.BPI_PlayerTrigger_C")
    (if (not (Variables|Default|GetbFuelCapacityMet))
      (Utilities|FlowControl|DoOnce false
        (:Completed
          (bind _player (Class|BPIPlayerTrigger|GetPlayerCharacter(Message) OtherActor))
          (Variables|References|SetPlayer _player)
          (if (not (Variables|/Game/DustDevil/Core/Saves/SG_DDSaveData.SG_DDSaveData_C|GetbSiloComplete (Default|GetSaveData (Variables|References|GetGameInstance))))
            (if (not (Variables|/Game/DustDevil/Objectives/BP_SiloManager_Infestation.BP_SiloManager_Infestation_C|GetbCanStartObj (Variables|References|GetObjectiveManager)))
              (Rendering|SetVisibility (Variables|Default|GetHoldPrompt) true false)
              (Variables|Default|SetbPromptOpen true)
              (Class|BPICursorCalls|ToggleFuelSiloMenu(Message) _returnvalue self)
              (bind _fuelsilomenu (Class|BPICursorCalls|GetFuelSiloMenu(Message) _returnvalue))
              (bind _output_get (Variables|References|SetFuelSiloMenu _fuelsilomenu))
              (Variables|/Game/DustDevil/UI/Objectives/WBP_FuelSilo.WBP_FuelSilo_C|SetFuelSilo _output_get self)
              (Default|UpdateWidgetsVisibility (Variables|References|GetFuelSiloMenu) true))))))))

(event OnComponentEndOverlap(InteractionTrigger)
  (params (OverlappedComponent :type Primitive%20Component%20Object%20Reference) (OtherActor :type Actor%20Object%20Reference) (OtherComp :type Primitive%20Component%20Object%20Reference) (OtherBodyIndex :type Integer))
  (bind _returnvalue (Game|GetPlayerController 0))
  (if (Utilities|DoesObjectImplementInterface OtherActor "/Game/DustDevil/Core/Interfaces/BPI_PlayerTrigger.BPI_PlayerTrigger_C")
    (if (not (Variables|Default|GetbFuelCapacityMet))
      (Utilities|FlowControl|Sequence
        (:then_0
          (Utilities|FlowControl|DoOnce false) ; enters at Reset
        )
        (:then_1
          (if (not (Variables|/Game/DustDevil/Core/Saves/SG_DDSaveData.SG_DDSaveData_C|GetbSiloComplete (Default|GetSaveData (Variables|References|GetGameInstance))))
            (if (not (Variables|/Game/DustDevil/Objectives/BP_SiloManager_Infestation.BP_SiloManager_Infestation_C|GetbCanStartObj (Variables|References|GetObjectiveManager)))
              (Rendering|SetVisibility (Variables|Default|GetHoldPrompt) false false)
              (Variables|Default|SetbPromptOpen false)
              (bind _menuopened (Class|BPICursorCalls|GetOpenedMenu(Message) (Game|GetPlayerController 0)))
              (switch Utilities|FlowControl|Switch|SwitchonE_Menus _menuopened
                (:NewEnumerator7
                  (Class|BPICursorCalls|ToggleFuelSiloMenu(Message) (Game|GetPlayerController 0) self))))))))))

(event Custom|CloseFuelSiloMenu
  (Class|BPICursorCalls|ToggleFuelSiloMenu(Message) (Game|GetPlayerController 0) self)
  (Rendering|SetVisibility (Variables|/Game/DustDevil/Objectives/BP_MissileSilo.BP_MissileSilo_C|GetObjectivePointer (Variables|/Game/DustDevil/Objectives/BP_SiloManager_Infestation.BP_SiloManager_Infestation_C|GetMissileSilo (Variables|References|GetObjectiveManager))) true false)
  (Rendering|SetVisibility (Variables|Default|GetObjectivePointer) false false))

(event Input|EnhancedActionEvents|EnhancedInputActionIA_HoldInteract_X
  (params (ActionValue :type Boolean) (ElapsedSeconds :type Float%20%28double-precision%29) (TriggeredSeconds :type Float%20%28double-precision%29) (InputAction :type Input%20Action%20Object%20Reference :default "/Game/DustDevil/Core/Inputs/IA_HoldInteract_X.IA_HoldInteract_X"))
  (bind _returnvalue (Game|GetPlayerController 0))
  (:Triggered
    (if (and (Rendering|IsVisible (Variables|Default|GetHoldPrompt)) (Variables|Default|GetbPromptOpen))
      (bind _promptwidget (Variables|References|GetPromptWidget)
        (:then
          (Default|TriggerPrompt _promptwidget)
          (Rendering|SetVisibility (Variables|Default|GetHoldPrompt) false false)
          (Variables|Default|SetbPromptOpen false)
          (CallFunction|GetCurrencies)
          (CallFunction|DepositNuclearFuel)
          (Variables|Default|SetFuelGaugeLevel (.z (Variables|/Script/Engine.SceneComponent|GetRelativeScale3D (Variables|Default|GetSiloFuelGauge))))
          (if (Variables|Default|GetbHasFuelToDeposit)
            (Default|GetFuelValuesfromSilo (Variables|References|GetFuelSiloMenu) (Math|Conversions|ToFloat(Integer) (Variables|Default|GetFuelToDeposit)) (Math|Conversions|ToFloat(Integer) (Variables|Default|GetNuclearFuelTotal)) (Math|Conversions|ToFloat(Integer) (Variables|Default|GetBaseNuclearFuelCurrent)))
            (Default|SetProgressBar (Variables|References|GetFuelSiloMenu))
            (Default|StartFuelDeposit (Variables|References|GetFuelSiloMenu))
            (Default|UpdateWidgetsVisibility (Variables|References|GetFuelSiloMenu) false)
            (Class|BPICursorCalls|ToggleHUDVisibility(Message) _returnvalue)
            (Class|BPICursorCalls|ToggleMinimapVisibility(Message) _returnvalue false)
            (else
              (Class|BPIHUDUpdates|DisplayWarningMessage(Message) (Variables|/Game/DustDevil/Player/BP_Vehicle.BP_Vehicle_C|GetHUD (Variables|References|GetPlayer)) "You don't have any nuclear fuel to deposit!"))))
        (:else))))
  (:Ongoing
    (if (and (Rendering|IsVisible (Variables|Default|GetHoldPrompt)) (Variables|Default|GetbPromptOpen))
      (bind _promptwidget_2 (Variables|References|GetPromptWidget)
        (:then
          (Default|HoldPrompt _promptwidget_2 ElapsedSeconds))
        (:else))))
  (:Canceled
    (if (and (Rendering|IsVisible (Variables|Default|GetHoldPrompt)) (Variables|Default|GetbPromptOpen))
      (bind _promptwidget_3 (Variables|References|GetPromptWidget)
        (:then
          (Default|CancelPrompt _promptwidget_3))
        (:else)))))

(event EventBeginPlay
  (CallFunction|GetReferences)
  (bind _output_get (Variables|Default|SetNuclearFuelCurrent (Variables|/Game/DustDevil/Core/Saves/SG_DDSaveData.SG_DDSaveData_C|GetMissileFuelDeposited (Default|GetSaveData (Variables|References|GetGameInstance)))))
  (Transformation|SetRelativeScale3D (Variables|Default|GetSiloFuelGauge) (Math|Vector|MakeVector 1.0 1.0 (/ (Math|Conversions|ToFloat(Integer) _output_get) (Math|Conversions|ToFloat(Integer) (Variables|Default|GetNuclearFuelTotal)))))
  (CallFunction|SetupInputPrompt)
  (if (Variables|/Game/DustDevil/Core/Saves/SG_DDSaveData.SG_DDSaveData_C|GetbSiloComplete (Default|GetSaveData (Variables|References|GetGameInstance)))
    (Rendering|SetVisibility (Variables|Default|GetObjectivePointer) false false)
    (else
      (Rendering|SetVisibility (Variables|Default|GetObjectivePointer) true false))))

(fn ConstructionScript)

(fn SetupInputPrompt
  (bind _aswbp_prompt_hold_text (Utilities|Casting|CastToWBP_PromptHoldText (UserInterface|GetUserWidgetObject (Variables|Default|GetHoldPrompt))))
  (Variables|References|SetPromptWidget _aswbp_prompt_hold_text)
  (Utilities|FlowControl|Sequence
    (:then_0
      (if (Variables|/Game/DustDevil/Core/GI_DDPrototype.GI_DDPrototype_C|GetbUsingController (Variables|References|GetGameInstance))
        (Default|SetInputType (Variables|References|GetPromptWidget) "NewEnumerator2" "E" "" false "" "Deposit nuclear material")
        (else
          (Default|SetInputType (Variables|References|GetPromptWidget) "NewEnumerator0" "E" "16px" false "" "Deposit nuclear material"))))
    (:then_1
      (bind _aswbp_objective_pointer (Utilities|Casting|CastToWBP_ObjectivePointer (UserInterface|GetUserWidgetObject (Variables|Default|GetObjectivePointer))))
      (Default|SetText _aswbp_objective_pointer "I"))))

(fn GetReferences
  (bind _asgi_ddprototype (Utilities|Casting|CastToGI_DDPrototype (Game|GetGameInstance)))
  (Variables|References|SetGameInstance _asgi_ddprototype))

(fn DepositNuclearFuel
  (bind _output_get (LocalVariables|SetLocal_Difference (- (Variables|Default|GetNuclearFuelTotal) (Variables|Default|GetNuclearFuelCurrent))))
  (if (> _output_get (Variables|Default|GetTempNuclearMats))
    (Variables|Default|SetNuclearFuelCurrent (Math|Integer|Clamp(Integer) (+ (Variables|Default|GetNuclearFuelCurrent) (Variables|Default|GetTempNuclearMats)) 0 (Variables|Default|GetNuclearFuelTotal)))
    (Variables|Default|SetFuelToDeposit (Variables|Default|GetTempNuclearMats))
    (Variables|Default|SetTempNuclearMats 0)
    (else
      (Variables|Default|SetNuclearFuelCurrent (Math|Integer|Clamp(Integer) (+ (LocalVariables|GetLocal_Difference) (Variables|Default|GetNuclearFuelCurrent)) 0 (Variables|Default|GetNuclearFuelTotal)))
      (Variables|Default|SetFuelToDeposit (LocalVariables|GetLocal_Difference))
      (Variables|Default|SetTempNuclearMats (- (Variables|Default|GetTempNuclearMats) (LocalVariables|GetLocal_Difference)))))
  (bind _output_get_2 (Variables|/Game/DustDevil/Objectives/BP_SiloManager_Infestation.BP_SiloManager_Infestation_C|SetbCanStartObj (Variables|References|GetObjectiveManager) (== (Variables|Default|GetNuclearFuelCurrent) (Variables|Default|GetNuclearFuelTotal))))
  (Variables|Default|SetbFuelCapacityMet _output_get_2)
  (bind _output_get_3 (Variables|/Game/DustDevil/Core/Saves/SG_DDSaveData.SG_DDSaveData_C|SetMissileFuelDeposited (Variables|/Game/DustDevil/Core/GI_DDPrototype.GI_DDPrototype_C|GetDDSaveData (Variables|References|GetGameInstance)) (Variables|Default|GetNuclearFuelCurrent)))
  (if (Math|Conversions|ToBoolean(Integer) _output_get_3)
    _))

(fn GetCurrencies
  (bind _player (Variables|References|GetPlayer))
  (bind _returnvalue (Ability|GetAbilitySystemComponent _player))
  (Utilities|IsValid _returnvalue
    (:Is%20Valid
      (Utilities|FlowControl|Sequence
        (:then_0
          (Development|PrintString "BP_FuelSilo: SetCurrencies get ability system component VALID" true true "(R=0.000000,G=1.000000,B=0.012667,A=1.000000)"))
        (:then_1
          (bind _output_get (Variables|Default|SetTempNuclearMats (Math|Float|Truncate (.ReturnValue (Ability|Attribute|GetFloatAttributefromAbilitySystemComponent _returnvalue "(AttributeName=\"NuclearMatter\",Attribute=/Script/DustDevil.BaseAttributeSet:NuclearMatter,AttributeOwner=\"/Script/CoreUObject.Class'/Script/DustDevil.BaseAttributeSet'\")")))))
          (Variables|Default|SetBaseNuclearFuelCurrent (Variables|Default|GetNuclearFuelCurrent))
          (Variables|Default|SetbHasFuelToDeposit (> _output_get 0)))))
    (:Is%20Not%20Valid
      (Development|PrintString "BP_FuelSilo: SetCurrencies get ability system component NOT VALID" true true "(R=1.000000,G=0.000000,B=0.033610,A=1.000000)"))))

(fn SetCurrencies
  (bind _player (Variables|References|GetPlayer))
  (bind _returnvalue (Ability|GetAbilitySystemComponent _player))
  (Utilities|FlowControl|Sequence
    (:then_0
      (Utilities|IsValid _returnvalue
        (:Is%20Valid
          (Utilities|FlowControl|Sequence
            (:then_0
              (Development|PrintString "BP_FuelSilo: SetCurrencies get ability system component VALID" true true "(R=0.000000,G=1.000000,B=0.012667,A=1.000000)"))
            (:then_1
              (LocalVariables|SetLocal_SpecHandle (GameplayEffects|MakeOutgoingSpec :self _returnvalue :GameplayEffectClass "/Game/DustDevil/Core/GAS/Effects/GE_NuclearConversion.GE_NuclearConversion_C"))
              (Utilities|FlowControl|Sequence
                (:then_0
                  (Ability|GameplayEffect|AssignTagSetbyCallerMagnitude (LocalVariables|GetLocal_SpecHandle) "(TagName=\"Stats.Base.NuclearMatter\")" (Math|Conversions|ToFloat(Integer) (Variables|Default|GetTempNuclearMats))))
                (:then_1
                  (GameplayEffects|ApplyGameplayEffectSpecToSelf _returnvalue (LocalVariables|GetLocal_SpecHandle)))))))
        (:Is%20Not%20Valid
          (Development|PrintString "BP_FuelSilo: SetCurrencies get ability system component NOT VALID" true true "(R=1.000000,G=0.000000,B=0.033610,A=1.000000)"))))))

(fn CheckifObjectiveComplete
  (if (Variables|/Game/DustDevil/Objectives/BP_SiloManager_Infestation.BP_SiloManager_Infestation_C|GetbCanStartObj (Variables|References|GetObjectiveManager))
    (Class|BPIHUDUpdates|UpdateObjectiveMain(Message) (Variables|/Game/DustDevil/Player/BP_Vehicle.BP_Vehicle_C|GetHUD (Variables|References|GetPlayer)) "Initiate launch sequence")))

(fn IncreaseFuelGauge
  (params (CurrentDeposited :type Float%20%28double-precision%29))
  (Transformation|SetRelativeScale3D (Variables|Default|GetSiloFuelGauge) (Math|Vector|MakeVector 1.0 1.0 (Math|Float|MapRangeClamped CurrentDeposited (Math|Conversions|ToFloat(Integer) (Variables|Default|GetBaseNuclearFuelCurrent)) (Math|Conversions|ToFloat(Integer) (Variables|Default|GetNuclearFuelTotal)) (Variables|Default|GetFuelGaugeLevel) 1.0))))