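; BP_TutorialExplosion is a tutorial wall actor that blows up when a boosting vehicle hits its overlap.
; On overlap it casts to BP_Vehicle, checks InBoost and fires only once.
; It destroys SMWall, then spawns four offset Niagara explosions attached to that component and plays a 2D blast sound.
; It also clears gameplay effects tagged Event.Vehicle.Tutorial from player 0's ability system, apparently ending a tutorial state.
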(event EventBeginPlay)

(event EventTick
  (params (DeltaSeconds :type Float%20%28single-precision%29)))

(event Collision|EventActorBeginOverlap
  (params (OtherActor :type Actor%20Object%20Reference))
  (bind _asbp_vehicle (Utilities|Casting|CastToBP_Vehicle OtherActor))
  (if (Variables|/Game/DustDevil/Player/BP_Vehicle.BP_Vehicle_C|GetInBoost _asbp_vehicle)
    (Utilities|FlowControl|DoOnce false
      (:Completed
        (Components|DestroyComponent (Variables|Default|GetSM_Wall))
        (Niagara|SpawnSystemAttached "/Game/DustDevil/Effects/Explosions/NS_EnemyExplosion1.NS_EnemyExplosion1" (Variables|Default|GetSM_Wall) "None" "0, 0, 0" "0, 0, 0" "KeepRelativeOffset" false)
        (Niagara|SpawnSystemAttached "/Game/DustDevil/Effects/Explosions/NS_EnemyExplosion1.NS_EnemyExplosion1" (Variables|Default|GetSM_Wall) "None" "0.000000,750.000000,0.000000" "0, 0, 0" "KeepRelativeOffset" false)
        (Niagara|SpawnSystemAttached "/Game/DustDevil/Effects/Explosions/NS_EnemyExplosion1.NS_EnemyExplosion1" (Variables|Default|GetSM_Wall) "None" "250.000000,-750.000000,0.000000" "0, 0, 0" "KeepRelativeOffset" false)
        (Niagara|SpawnSystemAttached "/Game/DustDevil/Effects/Explosions/NS_EnemyExplosion1.NS_EnemyExplosion1" (Variables|Default|GetSM_Wall) "None" "500.000000,-1250.000000,0.000000" "0, 0, 0" "KeepRelativeOffset" false)
        (Audio|PlaySound2D "/Game/DustDevil/Audio/Feedback/Grenade_Explosion_14_-_QuickSounds_com.Grenade_Explosion_14_-_QuickSounds_com" 1.0 1.0 0.0 0 0)
        (GameplayEffects|RemoveActiveEffectswithTags (Ability|GetAbilitySystemComponent (Game|Player|GetPlayerPawn 0)) "(GameplayTags=((TagName=\"Event.Vehicle.Tutorial\")))")))))

(fn ConstructionScript)