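; BP_CamAngleChange is a prototype actor that changes the player's camera angle when overlapped.
; On begin overlap, it gets the player character from the overlapping actor through an interface message and immediately sets the CameraBoom's arm length.
; MoveComponentTo then blends the boom to the configured relative location and rotation over BlendTime.
; Nothing restores the previous camera setup when the overlap ends.
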(event EventBeginPlay)

(event Collision|EventActorBeginOverlap
  (params (OtherActor :type Actor%20Object%20Reference))
  (bind _player (Class|BPIPlayerTrigger|GetPlayerCharacter(Message) OtherActor))
  (Variables|/Script/Engine.SpringArmComponent|SetTargetArmLength (Variables|/Script/DustDevil.Vehicle|GetCameraBoom _player) (Variables|Default|GetTarget%20Arm%20Length))
  (Components|MoveComponentTo (Variables|/Script/DustDevil.Vehicle|GetCameraBoom _player) (Variables|Default|GetLocation) (Math|Rotator|MakeRotator (Variables|Default|GetRoll) (Variables|Default|GetPitch) (Variables|Default|GetYaw)) false false (Variables|Default|GetBlendTime) false))

(event EventTick
  (params (DeltaSeconds :type Float%20%28single-precision%29)))

(fn ConstructionScript)