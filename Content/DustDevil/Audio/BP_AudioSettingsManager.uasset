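; Audio settings manager actor that applies the player's volume levels for Master, SFX, Music and Ambience.
; On BeginPlay it sets the base sound mix and applies the stored Music, SFX and Ambience volumes as instant class overrides, leaving out Master.
; ChangeVolumeLevel maps the chosen setting to its sound class, stores the new level and overrides that class's volume in the mix.
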(event Custom|ChangeVolumeLevel
  (params (AudioSetting :type E_AudioSettings%20Enum :default "NewEnumerator0") (VolumeLevel :type Float%20%28double-precision%29))
  (Variables|Default|SetVolumeLevel VolumeLevel)
  (switch Utilities|FlowControl|Switch|SwitchonE_AudioSettings AudioSetting
    (:NewEnumerator0
      (Variables|Default|SetAffectedSoundClass "/Engine/EngineSounds/Master.Master")
      (Variables|Default|SetMasterVolume (Variables|Default|GetVolumeLevel)))
    (:NewEnumerator1
      (Variables|Default|SetAffectedSoundClass "/Game/DustDevil/Audio/Sound_Classes/SC_Feedback.SC_Feedback")
      (Variables|Default|SetSFXVolume (Variables|Default|GetVolumeLevel)))
    (:NewEnumerator2
      (Variables|Default|SetAffectedSoundClass "/Game/DustDevil/Audio/Sound_Classes/SC_Music.SC_Music")
      (Variables|Default|SetMusicVolume (Variables|Default|GetVolumeLevel)))
    (:NewEnumerator3
      (Variables|Default|SetAffectedSoundClass "/Game/DustDevil/Audio/Sound_Classes/SC_Ambience.SC_Ambience")
      (Variables|Default|SetAmbientVolume (Variables|Default|GetVolumeLevel))))
  (Audio|SetSoundMixClassOverride (Variables|Default|GetBaseSoundMix) (Variables|Default|GetAffectedSoundClass) (Variables|Default|GetVolumeLevel) 1.0 0.0 true))

(event EventBeginPlay
  (Class|GameplayStatics|SetBaseSoundMix (Variables|Default|GetBaseSoundMix))
  (bind _output_get (Variables|Default|SetAffectedSoundClass "/Game/DustDevil/Audio/Sound_Classes/SC_Music.SC_Music"))
  (Audio|SetSoundMixClassOverride (Variables|Default|GetBaseSoundMix) _output_get (Variables|Default|GetMusicVolume) 1.0 0.0 true)
  (bind _output_get_2 (Variables|Default|SetAffectedSoundClass "/Game/DustDevil/Audio/Sound_Classes/SC_Feedback.SC_Feedback"))
  (Audio|SetSoundMixClassOverride (Variables|Default|GetBaseSoundMix) _output_get_2 (Variables|Default|GetSFXVolume) 1.0 0.0 true)
  (bind _output_get_3 (Variables|Default|SetAffectedSoundClass "/Game/DustDevil/Audio/Sound_Classes/SC_Ambience.SC_Ambience"))
  (Audio|SetSoundMixClassOverride (Variables|Default|GetBaseSoundMix) _output_get_3 (Variables|Default|GetAmbientVolume) 1.0 0.0 true))

(fn ConstructionScript)