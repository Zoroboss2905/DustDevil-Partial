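; Audio manager that plays wasteland ambience and switches music between random background tracks, boss fight, radioactive zone and end music.
; BeginPlay, gated by MusicOn, picks the starting track by level name; events for boss fights, rad zones, objectives and player death then fade tracks.
; Start and stop helpers check play state to avoid redundant fades, and boss fight end checks rad-zone overlap to choose what resumes.
; Debug key 8 toggles boss music.
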(event Custom|Boss%20Fight%20Started
  (Utilities|FlowControl|Sequence
    (:then_0
      (CallFunction|StopPlayingTrack (CallFunction|FindBackgroundMusicPlaying))
      (CallFunction|StopPlayingTrack (Variables|Default|GetRadZoneMusic)))
    (:then_1
      (CallFunction|StartPlayingTrack (Variables|Default|GetBossMusic) 0.0))))

(event Custom|Boss%20Fight%20Ended
  (Utilities|FlowControl|Sequence
    (:then_0
      (CallFunction|StopPlayingTrack (Variables|Default|GetBossMusic)))
    (:then_1
      (if (CallFunction|CheckifInsideRadZone)
        (CallFunction|StartPlayingTrack (Variables|Default|GetRadZoneMusic) 0.0)
        (else
          (CallFunction|StartPlayingTrack (CallFunction|PickBackgroundMusicTrack) 0.0))))))

(event Custom|RadZoneExited
  (Utilities|FlowControl|Sequence
    (:then_0
      (CallFunction|StopPlayingTrack (Variables|Default|GetRadZoneMusic)))
    (:then_1
      (CallFunction|StartPlayingTrack (CallFunction|PickBackgroundMusicTrack) 0.0))))

(event Custom|RadZoneEntered
  (Utilities|FlowControl|Sequence
    (:then_0
      (CallFunction|StopPlayingTrack (CallFunction|FindBackgroundMusicPlaying)))
    (:then_1
      (CallFunction|StartPlayingTrack (Variables|Default|GetRadZoneMusic) 0.0))))

(event Custom|PlayerDeath
  (for _array_element (Variables|Default|GetMusicTracks)
    (Utilities|IsValid _array_element
      (:Is%20Valid
        (switch Utilities|FlowControl|Switch|SwitchonEAudioComponentPlayState (Audio|Components|Audio|GetPlayState _array_element)
          (:Playing
            _)
          (:FadingIn
            _))
        (Audio|Components|Audio|FadeOut _array_element 1.0 0.0 "Linear" :!class /Script/Engine.AudioComponent)))))

(event Custom|Fade%20End%20Music
  (bind _endmusic (Variables|Default|GetEndMusic)
    (:then
      (switch Utilities|FlowControl|Switch|SwitchonEAudioComponentPlayState (Audio|Components|Audio|GetPlayState _endmusic)
        (:Playing
          _)
        (:FadingIn
          _))
      (Audio|Components|Audio|FadeOut (Variables|Default|GetEndMusic) 2.0 0.0 "Linear" :!class /Script/Engine.AudioComponent))
    (:else)))

(event Custom|ObjectiveStarted
  (CallFunction|StopPlayingTrack (CallFunction|FindBackgroundMusicPlaying)))

(event EventBeginPlay
  (Variables|Default|SetMusicTracks (Utilities|Array|MakeArray (Variables|Default|GetBossMusic) (Variables|Default|GetRadZoneMusic) (Variables|Default|GetEndMusic) (Variables|Default|GetBackgroundMusic00) (Variables|Default|GetBackgroundMusic01)))
  (Variables|Default|SetBackgroundMusic (Utilities|Array|MakeArray (Variables|Default|GetBackgroundMusic00) (Variables|Default|GetBackgroundMusic01)))
  (if (Variables|Default|GetbMusicOn)
    (Audio|Components|Audio|Play (Variables|Default|GetWastelandAmbience00) 0.0)
    (bind _returnvalue (Game|GetCurrentLevelName true))
    (if (Utilities|Enum|Equal(Enum) _returnvalue "L_WastelandEscape_WP")
      (CallFunction|StartPlayingTrack (Variables|Default|GetEndMusic) 0.0)
      (else
        (CallFunction|StartPlayingTrack (CallFunction|PickBackgroundMusicTrack) 0.0)))))

(event Input|KeyboardEvents|DebugKey8
  (params (Key :type Key%20Structure :default "None") (ActionValue :type Input%20Action%20Value%20Structure))
  (:Pressed
    (Utilities|FlowControl|FlipFlop
      (:A
        (CallFunction|BossFightStarted))
      (:B
        (CallFunction|BossFightEnded)))))

(fn ConstructionScript)

(fn StopPlayingTrack
  (params (MusicTrack :type Audio%20Component%20Object%20Reference))
  (Utilities|IsValid MusicTrack
    (:Is%20Valid
      (switch Utilities|FlowControl|Switch|SwitchonEAudioComponentPlayState (Audio|Components|Audio|GetPlayState MusicTrack)
        (:Playing
          _)
        (:Stopped
          (return))
        (:Paused
          (return))
        (:FadingIn
          _)
        (:FadingOut
          (return)))
      (Audio|Components|Audio|FadeOut MusicTrack 1.0 0.0 "Linear" :!class /Script/Engine.AudioComponent))
    (:Is%20Not%20Valid
      (return))))

(fn StartPlayingTrack
  (params (MusicTrack :type Audio%20Component%20Object%20Reference) (StartTime :type Float%20%28double-precision%29))
  (Utilities|IsValid MusicTrack
    (:Is%20Valid
      (switch Utilities|FlowControl|Switch|SwitchonEAudioComponentPlayState (Audio|Components|Audio|GetPlayState MusicTrack)
        (:Playing
          (return))
        (:Stopped
          _)
        (:Paused
          _)
        (:FadingIn
          (return))
        (:FadingOut
          _))
      (Audio|Components|Audio|FadeIn MusicTrack 1.0 1.0 StartTime "Linear" :!class /Script/Engine.AudioComponent))
    (:Is%20Not%20Valid
      (return))))

(fn CheckifInsideRadZone
  (LocalVariables|SetLocal_ArrayIndex 0)
  (bind _outactors (Actor|GetAllActorsOfClass "/Game/DustDevil/Environment/Blueprints/BP_RadioactiveZone.BP_RadioactiveZone_C"))
  (for _array_element _outactors
    (if (Collision|IsOverlappingActor _array_element (Game|Player|GetPlayerPawn 0) :!class /Script/Engine.Actor)
      (return true)
      (else
        (Math|Integer|IncrementInt (LocalVariables|GetLocal_ArrayIndex)))))
  (if (== (LocalVariables|GetLocal_ArrayIndex) (Utilities|Array|Length _outactors))
    (return false)
    (else
      (return true))))

(fn PickBackgroundMusicTrack
  (return (.OutItem (Utilities|Array|Random (Variables|Default|GetBackgroundMusic)))))

(fn FindBackgroundMusicPlaying
  (bind _array_element (Utilities|Array|ForEachLoopwithBreak (Variables|Default|GetBackgroundMusic) :!label _label)
    (:LoopBody
      (Utilities|IsValid _array_element
        (:Is%20Valid
          (switch Utilities|FlowControl|Switch|SwitchonEAudioComponentPlayState (Audio|Components|Audio|GetPlayState _array_element)
            (:Playing
              _)
            (:FadingIn
              _))
          (Utilities|FlowControl|Sequence
            (:then_0
              (goto _label Break))
            (:then_1
              (return _array_element))))))))